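; Showcase actor that lets the player recolor its mesh through the UMG Color Picker widgets.
; Hovering toggles custom depth and a hand cursor; clicking opens the full picker, while ShowSimpleMenu opens the simple variant.
; Both pickers return the chosen color to ColorSelected, which sets the Color parameter on a dynamic material instance created in the construction script.
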(event `self.ReceiveActorBeginCursorOver`
  ;[1 1 1] Hover effects
  (`PrimitiveComponent.SetRenderCustomDepth` (`self.StaticMesh`) true)
  (set `PlayerController.CurrentMouseCursor` "Hand" (`GameplayStatics.GetPlayerController` 0)))

(event `self.ReceiveActorEndCursorOver`
  ;[1 1 1] Hover effects
  (`PrimitiveComponent.SetRenderCustomDepth` (`self.StaticMesh`) false)
  (set `PlayerController.CurrentMouseCursor` "Default" (`GameplayStatics.GetPlayerController` 0)))

(event `self.ReceiveActorOnClicked`
  ;[1 1 1] Show the UMG Color Picker Widget when clicked.
  (bind _returnvalue (`|CreateWidget` "/Game/UMGColorPicker/UMG/ColorPickerWidget.ColorPickerWidget_C" null (`self.MeshColor`) true true true "Object Color"))
  (`UserWidget.AddToViewport` _returnvalue 0)
  (add `/Game/UMGColorPicker/UMG/ColorPickerWidget.ColorChanged` _returnvalue (delegate `ColorSelected`)))

(event `ShowSimpleMenu`
  ;[1 1 1] Show the UMG Color Picker Widget when clicked.
  (bind _returnvalue (`|CreateWidget` "/Game/UMGColorPicker/UMG/ColorPickerSimple.ColorPickerSimple_C" null true true (`self.MeshColor`) "Color Picker Simple"))
  (`UserWidget.AddToViewport` _returnvalue 0)
  (add `/Game/UMGColorPicker/UMG/ColorPickerSimple.ColorChanged` _returnvalue (delegate `ColorSelected`)))

(event `ColorSelected`
  (params (NewColor :type "LinearColor Structure"))
  ;[1 1 1] Show the UMG Color Picker Widget when clicked.
  (set `self.MeshColor` NewColor)
  (`self.UpdateMeshColor`))

(fn `UpdateMeshColor`
  ;[1 1 1] Update mesh DMI to match our new MeshColor
  (`MaterialInstanceDynamic.SetVectorParameterValue` (`self.MeshDMI`) "Color" (`self.MeshColor`)))

(fn `UserConstructionScript`
  (`StaticMeshComponent.SetStaticMesh` (`self.StaticMesh`) (`self.PreviewMesh`))
  (bind _returnvalue (`PrimitiveComponent.CreateDynamicMaterialInstance` (`self.StaticMesh`) 0 (`self.MeshMaterial`)))
  (bind _output_get (set `self.MeshDMI` _returnvalue))
  (`PrimitiveComponent.SetMaterial` (`self.StaticMesh`) 0 _output_get))