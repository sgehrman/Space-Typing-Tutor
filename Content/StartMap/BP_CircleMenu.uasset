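; BP_CircleMenu is a radial menu actor with Exit, Help, Play and Menu segments, built in construction as BP_QuarterCircleActor child actors around a circle.
; Left click or the gamepad bottom button dismisses it when a segment is selected, performing no item-specific action here.
; When spawned via SetupFromSpawnedActor, it spins and scales in, adding a background disk.
; A per-tick line trace against that disk triggers spin-shrink destruction upon looking away.
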(event Custom|AnimateOutAndDestroy
  (Variables|Default|SetBeing%20Destroyed true)
  (bind _alpha (Timeline|AnimateOutTimer PlayFromStart)
    (:Update
      (Transformation|SetRelativeRotation (Variables|Default|GetSegment%20Container) (Math|Rotator|Lerp(Rotator) (Math|Rotator|MakeRotator 0.0 0.0 0.0) (Math|Rotator|MakeRotator (Math|Float|MapRangeUnclamped _alpha 0.0 1.0 0.0 3.6e+02) 0.0 (Math|Float|MapRangeUnclamped _alpha 0.0 1.0 0.0 3.6e+02)) _alpha) false false)
      (Transformation|SetActorRelativeScale3D (Math|Vector|Lerp(Vector) "1.000000,1.000000,1.000000" "0.100000,0.100000,0.100000" _alpha)))
    (:Finished
      (Actor|DestroyActor))))

(event Custom|RunSpinBounceAnimation
  (params (Location :type Vector))
  (bind _alpha (Timeline|SpinTimeLine PlayFromStart)
    (:Update
      (Transformation|SetRelativeRotation (Variables|Default|GetSegment%20Container) (Math|Rotator|Lerp(Rotator) (Math|Rotator|MakeRotator 0.0 0.0 0.0) (Math|Rotator|MakeRotator (Math|Float|MapRangeUnclamped _alpha 0.0 1.0 0.0 3.6e+02) 0.0 0.0) _alpha) false false)
      (Transformation|SetActorRelativeScale3D (Math|Vector|Lerp(Vector) "0.300000,0.300000,0.300000" "1.000000,1.000000,1.000000" _alpha)))))

(event Custom|PerformSelection
  (CallFunction|AnimateOutandDestroy))

(event EventTick
  (params (DeltaSeconds :type Float%20%28single-precision%29))
  (CallFunction|HandleBackgroundDiskLineTrace))

(event EventBeginPlay
  (Input|EnableInput (Game|GetPlayerController 0)))

(event Input|GamepadEvents|GamepadFaceButtonBottom
  (params (Key :type Key%20Structure :default "AnyKey"))
  (:Pressed
    (bind _index (CallFunction|CurrentSelectedIndex))
    (if (!= _index -1)
      (CallFunction|AnimateOutandDestroy))))

(event Input|MouseEvents|LeftMouseButton
  (params (Key :type Key%20Structure :default "AnyKey"))
  (:Pressed
    (bind _index (CallFunction|CurrentSelectedIndex))
    (if (!= _index -1)
      (CallFunction|AnimateOutandDestroy))))

(fn ConstructionScript
  (CallFunction|BuildCircleSegments)
  (CallFunction|BuildBackgroundDisk))

(fn BuildCircleSegments
  (bind _titles_array (LocalVariables|GetTitles%20Array))
  (Utilities|FlowControl|Sequence
    (:then_0
      (Utilities|Array|Add _titles_array "Exit")
      (Utilities|Array|Add _titles_array "Help")
      (Utilities|Array|Add _titles_array "Play")
      (Utilities|Array|Add _titles_array "Menu"))
    (:then_1
      (for (_array_element _array_index) (LocalVariables|GetTitles%20Array)
        (bind _returnvalue (AddComponent|AddChildActorComponent true (Math|Transform|MakeTransform (.Location (CallFunction|LocationAroundCircle _array_index 4 8.0 "1.000000, 0,0.000000" 0.0)) "0, 0, 0" "1.000000,1.000000,1.000000")))
        (Utilities|FlowControl|Sequence
          (:then_0
            (Class|SceneComponent|Attachto _returnvalue (Variables|Default|GetSegment%20Container) "None" "KeepRelativeOffset" true))
          (:then_1
            ;[1 1 1] Set Rotation around circle
            (if (Math|Float|InRange(Float) (.Degress (CallFunction|LocationAroundCircle _array_index 4 8.0 "1.000000, 0,0.000000" 0.0)) 9e+01 2.7e+02)
              (Transformation|SetRelativeRotation _returnvalue (Math|Rotator|MakeRotator (+ (* (.Degress (CallFunction|LocationAroundCircle _array_index 4 8.0 "1.000000, 0,0.000000" 0.0)) -1.0) 9e+01) 0.0 0.0) false false)
              (else
                (Transformation|SetRelativeRotation _returnvalue (Math|Rotator|MakeRotator (+ (.Degress (CallFunction|LocationAroundCircle _array_index 4 8.0 "1.000000, 0,0.000000" 0.0)) 9e+01) 0.0 0.0) false false))))
          (:then_2
            ;[1 1 1] Set Title
            (bind _asbp_quarter_circle_actor (Utilities|Casting|CastToBP_QuarterCircleActor (Variables|/Script/Engine.ChildActorComponent|GetChildActor _returnvalue)))
            (Default|UpdateTitle _asbp_quarter_circle_actor _array_element))
          (:then_3
            (bind _asbp_quarter_circle_actor_2 (Utilities|Casting|CastToBP_QuarterCircleActor (Variables|/Script/Engine.ChildActorComponent|GetChildActor _returnvalue)))
            (Variables|/Game/StartMap/BP_QuarterCircleActor.BP_QuarterCircleActor_C|SetCicleMenu _asbp_quarter_circle_actor_2 self)))))))

(fn BuildBackgroundDisk
  (if (Variables|Default|GetDestroy%20When%20Looking%20Away)
    (if (== (Variables|Default|GetBackgroundMeshComponent) 0)
      (bind _returnvalue (AddComponent|AddStaticMeshComponent false (Math|Transform|MakeTransform "30.000000, 0,0.000000" "90.000000, 0, 0" "0.700000,0.700000,0.700000")))
      (Components|StaticMesh|SetStaticMesh _returnvalue "/Game/StartMap/SM_CircleMenuBackground.SM_CircleMenuBackground")
      (Rendering|Material|SetMaterial _returnvalue 0 "/Game/StartMap/MT_CircleMenuBackground.MT_CircleMenuBackground")
      (Variables|Default|SetBackgroundMeshComponent _returnvalue))))

(fn HandleBackgroundDiskLineTrace
  (Utilities|FlowControl|Sequence
    (:then_0
      (if (not (Variables|Default|GetBeing%20Destroyed))
        (if (Variables|Default|GetDestroy%20When%20Looking%20Away)
          (if (!= (Variables|Default|GetBackgroundMeshComponent) 0)
            (bind (_start_location _end_location) (CallFunction|StartandEndTraceLocations 5e+03))
            (bind (_outhits _returnvalue) (Class|KismetSystemLibrary|LineTraceMultiforObjects _start_location _end_location (Utilities|Array|MakeArray "ObjectTypeQuery1" "ObjectTypeQuery2") false 0 "None" false))
            (if _returnvalue
              (bind _array_element (Utilities|Array|ForEachLoopwithBreak _outhits)
                (:LoopBody
                  (if (== (.HitComponent (Collision|BreakHitResult _array_element)) (Variables|Default|GetBackgroundMeshComponent))
                    (LocalVariables|SetHit%20Background true)))
                (:Completed
                  (if (not (LocalVariables|GetHit%20Background)) :!label _label
                    (CallFunction|AnimateOutandDestroy))))
              (else
                (goto _label)))))))
    (:then_1
      (return))))

(fn SetupfromSpawnedActor
  ;[1 1 1] Called when spawning actor dynamically
  (Variables|Default|SetDestroy%20When%20Looking%20Away true)
  (CallFunction|BuildBackgroundDisk)
  (CallFunction|RunSpinBounceAnimation "0, 0, 0"))

(fn CurrentSelectedIndex
  (Utilities|FlowControl|Sequence
    (:then_0
      (if (not (Variables|Default|GetBeing%20Destroyed))
        (for (_array_element _array_index) (Components|GetChildrenComponents false)
          (bind _aschild_actor_component (Utilities|Casting|CastToChildActorComponent _array_element))
          (bind _asbp_quarter_circle_actor (Utilities|Casting|CastToBP_QuarterCircleActor (Variables|/Script/Engine.ChildActorComponent|GetChildActor _aschild_actor_component)))
          (if (Variables|/Game/StartMap/BP_QuarterCircleActor.BP_QuarterCircleActor_C|GetIs%20Selected _asbp_quarter_circle_actor)
            (LocalVariables|SetResult%20Index _array_index)))))
    (:then_1
      (return (LocalVariables|GetResult%20Index)))))