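; A quarter-circle menu segment with a settable title that is selected by holding the crosshair over it.
; Construction creates a dynamic material instance, whose GlowStrength changes on hover start and end.
; Crosshair hover handlers forward progress to the CrosshairActor found at BeginPlay.
; At full progress, a DoOnce boosts the glow and calls PerformSelection on the circle menu; other crosshair input handlers return false.
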(event EventBeginPlay
  (bind _ascrosshair_actor (Utilities|Casting|CastToCrosshairActor (.Actor (CallFunction|FindActorwithTag "/Game/ReusableAssets/Crosshair/CrosshairActor.CrosshairActor_C" "None" self))))
  (Variables|Default|SetCrosshair%20Actor _ascrosshair_actor))

(event Collision|EventActorBeginOverlap
  (params (OtherActor :type Actor%20Object%20Reference)))

(event EventTick
  (params (DeltaSeconds :type Float%20%28single-precision%29)))

(fn ConstructionScript
  (bind _returnvalue (Rendering|Material|CreateDynamicMaterialInstance "/Game/StartMap/MT_QuarterCircle1.MT_QuarterCircle1" :!class /Script/Engine.KismetMaterialLibrary))
  (bind _output_get (Variables|Default|SetMID _returnvalue))
  (Rendering|Material|SetMaterial 0 _output_get)
  (Rendering|Material|SetMaterial 1 "/Game/StartMap/MT_QuarterCircle2.MT_QuarterCircle2"))

(fn UpdateTitle
  (params (Title :type String))
  (Rendering|Components|TextRender|SetText (Variables|Default|GetTitleText) (Utilities|Text|ToText(String) Title)))

(fn CrosshairHoverMoved
  (params (Hit%20Location :type Vector :default "0, 0, 0"))
  (return false))

(fn CrosshairHoverProgress
  (params (Progress :type Float%20%28single-precision%29) (Local%20Hit%20Location :type Vector :default "0, 0, 0") (Hit%20Component :type Primitive%20Component%20Object%20Reference))
  (Utilities|FlowControl|Sequence
    (:then_0
      (Default|UpdateProgress (Variables|Default|GetCrosshair%20Actor) Progress))
    (:then_1
      (if (== Progress 1.0)
        (Utilities|FlowControl|DoOnce false
          (:Completed
            (Rendering|Material|SetScalarParameterValue (Variables|Default|GetMID) "GlowStrength" 1e+03 :!class /Script/Engine.MaterialInstanceDynamic)
            (Default|PerformSelection (Variables|Default|GetCicleMenu))))))
    (:then_2
      (return false))))

(fn CrosshairHoverStart
  (params (Finished :type Boolean))
  (Utilities|FlowControl|Sequence
    (:then_0
      (if Finished
        (LocalVariables|SetGlow%20Strength 1.0)
        (Variables|Default|SetIs%20Selected false)
        (else
          (LocalVariables|SetGlow%20Strength 12.0)
          (Variables|Default|SetIs%20Selected true)))
      (Rendering|Material|SetScalarParameterValue (Variables|Default|GetMID) "GlowStrength" (LocalVariables|GetGlow%20Strength) :!class /Script/Engine.MaterialInstanceDynamic))
    (:then_1
      (Default|UpdateProgress (Variables|Default|GetCrosshair%20Actor) 0.0))
    (:then_2
      (return true))))

(fn CrosshairLeftRight
  (params (Left :type Boolean))
  (return false))

(fn CrosshairMouseClick
  (params (Mouse%20Down :type Boolean) (Event%20Type :type E_EventType%20Enum :default "NewEnumerator10") (Hit%20Location :type Vector :default "0, 0, 0") (Hit%20Component :type Primitive%20Component%20Object%20Reference))
  (return false))

(fn CrosshairScrollWheel
  (params (Down :type Boolean) (Hit%20Location :type Vector :default "0, 0, 0") (Hit%20Component :type Primitive%20Component%20Object%20Reference))
  (return false))

(fn CrosshairUpDown
  (params (Up :type Boolean))
  (return false))