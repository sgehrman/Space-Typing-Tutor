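; BP_CyberActor sets up a cyber-themed scene at BeginPlay, showing credits text for code, art and testing.
; A BCPMMAccess component, set up for "credits", returns the PMM through a ready event, which enables the crosshair outside menu mode.
; The startup sequence also adds child actors, including a BP_CheckboxBar, toggles BCLevelCommon's player positioning around a short delay, and spawns a tiled box with Cyber materials.
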(event `CustomEvent_0`
  (params (Result :type "/Game/ReusableAssets/Utilities/BPI_PMM Interface"))
  (bind _output_get (set `self.PLM` Result))
  (`/Game/ReusableAssets/Utilities/BPI_PMM.Enable Crosshair` _output_get true false))

(event `self.ReceiveBeginPlay`
  (`|ExecutionSequence`
    (:`then_0`
      (`TextRenderComponent.K2_SetText` (`self.Credits`) (`KismetTextLibrary.Conv_StringToText` (`VictoryBPFunctionLibrary.AppendMultiple` "Code: 57eve" " \n" "Art: Jazmin" " \n" "Testing: SFKai")))
      (`SceneComponent.K2_SetRelativeLocation` (`self.Credits`) (`/Game/ReusableAssets/Utilities/LIB_Constants.Standard Location` (0.0 0.0 0.0)) false false))
    (:`then_1`
      (bind _returnvalue (`AddComponent|BC_PMMAccess_C_0`))
      (add `/Game/ReusableAssets/Utilities/BC_PMMAccess.PMM Ready` _returnvalue (delegate `CustomEvent_0`))
      (`/Game/ReusableAssets/Utilities/BC_PMMAccess.Setup` _returnvalue "credits"))
    (:`then_2`
      (`AddComponent|ChildActorComponent_105` :`RelativeTransform` (`KismetMathLibrary.MakeTransform` (4444.0 0.0 4444.0) (struct :`Roll` 18.0) (1.0 1.0 1.0))))
    (:`then_4`
      (`/Game/ReusableAssets/Utilities/BC_LevelCommon.Move Player into Position` (`self.BC_LevelCommon`) true)
      (`KismetSystemLibrary.Delay` 0.5)
      (`/Game/ReusableAssets/Utilities/BC_LevelCommon.Move Player into Position` (`self.BC_LevelCommon`) false))
    (:`then_5`
      (`|SpawnActorFromClass` "/Game/Typewriter/CreditsMap/BP_CreateTiledBoxActor.BP_CreateTiledBoxActor_C" (`KismetMathLibrary.MakeTransform` (55.0 0.0 0.0) (struct) (1.0 1.0 1.0)) "Undefined" "OverrideRootScale" null (`KismetMathLibrary.MakeVector` 99.0 165.0 66.0) (`|MakeArray` "/Game/Materials/Cyber/CyberAmber_MAT_UV_Inst.CyberAmber_MAT_UV_Inst" "/Game/Materials/Cyber/CyberBorg_MAT_UV_Inst.CyberBorg_MAT_UV_Inst" "/Game/Materials/Cyber/CyberBorgNeon_MAT_UV_Inst.CyberBorgNeon_MAT_UV_Inst" "/Game/Materials/Cyber/CyberCircuitBoard_MAT_UV_Inst.CyberCircuitBoard_MAT_UV_Inst" "/Game/Materials/Cyber/CyberCircuitry_MAT_UV_Inst.CyberCircuitry_MAT_UV_Inst" "/Game/Materials/Cyber/CyberShapeless_MAT_UV_Inst.CyberShapeless_MAT_UV_Inst" :!type "MaterialInstance Object Reference")) ; Spawn Tiled Box :)
    )
    (:`then_6`
      (bind _returnvalue_2 (`AddComponent|ChildActorComponent_2288` :`RelativeTransform` (`KismetMathLibrary.MakeTransform` (-5.0 -36.0 0.0))))
      (cast `/Game/ReusableAssets/Buttons/BP_CheckboxBar` (`ChildActorComponent.ChildActor` _returnvalue_2)))))

(fn `UserConstructionScript`)