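; BP_MagnetComponent pulls its owner's physics body back toward the world location where it started, like a magnet.
; On initialization it stores that location and makes the owner's first primitive component a damped, gravity-free simulated body.
; Each tick, straying past a threshold latches a mass-scaled return force, stronger when farther away.
; The force releases once the component moves fast enough and heads almost straight back to the start.
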(event EventTick
  (params (DeltaSeconds :type Float%20%28single-precision%29))
  (CallFunction|MoveonTick))

(event EventInitializeComponent
  (Utilities|FlowControl|Sequence
    (:then_0
      (Variables|Default|SetStart%20Location (Transformation|GetWorldLocation)))
    (:then_1
      (Variables|Default|SetPrimativeComponent (Utilities|Array|Get(acopy) (Actor|GetComponentsByClass (Components|GetOwner) "/Script/Engine.PrimitiveComponent")))
      (Physics|SetSimulatePhysics (Variables|Default|GetPrimativeComponent) true)
      (Physics|SetEnableGravity (Variables|Default|GetPrimativeComponent) false)
      (Class|PrimitiveComponent|SetLinearDamping (Variables|Default|GetPrimativeComponent) (Variables|Default|GetLinear%20Damping))
      (Class|PrimitiveComponent|SetAngularDamping (Variables|Default|GetPrimativeComponent) (Variables|Default|GetAngular%20Damping)))))

(fn MoveonTick
  (bind _returnvalue (Physics|GetMass))
  (Utilities|FlowControl|Sequence
    (:then_0
      (Variables|Default|SetVector%20Back%20to%20Start (- (Variables|Default|GetStart%20Location) (Transformation|GetWorldLocation))))
    (:then_1
      ;[1 1 1] Are we too far away?
      (if (> (Math|Vector|VectorLength (Variables|Default|GetVector%20Back%20to%20Start)) 44.0)
        (LocalVariables|SetAdd%20Force true)))
    (:then_2
      (if (LocalVariables|GetAdd%20Force)
        (if (not (< (Math|Vector|VectorLength (Transformation|GetComponentVelocity)) 5.0))
          (if (< (Class|KismetMathLibrary|DegAcos (Math|Vector|DotProduct (Math|Vector|Normalize (Transformation|GetComponentVelocity)) (Math|Vector|Normalize (Variables|Default|GetVector%20Back%20to%20Start)))) 1e+01)
            (LocalVariables|SetAdd%20Force false)))))
    (:then_3
      (if (LocalVariables|GetAdd%20Force)
        (if (< (Math|Vector|VectorLength (Variables|Default|GetVector%20Back%20to%20Start)) 88.0)
          (Physics|AddForce (Variables|Default|GetPrimativeComponent) (* (Math|Vector|Normalize (Variables|Default|GetVector%20Back%20to%20Start)) (* _returnvalue 22.0)) "None")
          (else
            (Physics|AddForce (Variables|Default|GetPrimativeComponent) (* (Math|Vector|Normalize (Variables|Default|GetVector%20Back%20to%20Start)) (* _returnvalue 44.0)) "None")))))
    (:then_4
      (return))))