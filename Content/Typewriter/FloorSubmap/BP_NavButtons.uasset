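; BP_NavButtons is a navigation button actor in the floor submap that provides a circular "Back" button for returning to the Menu level.
; Setup stores the PLM reference, spawns a BP_ToggleButton child actor in push mode and adds a procedural box mesh behind it using a dynamic steel material.
; Button clicks route by ID: Menu loads the level through PLM, Quit exits the game, and other IDs send a MainButtonClick event.
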(event Custom|Listen%20to%20Main%20Menu%20Button%20Events
  (EventDispatchers|BindEventtoButtonClickedbyUser (Variables|Default|GetMain%20Menu%20Button) (delegate Custom|Main%20Menu%20Clicked)))

(event Custom|Main%20Menu%20Clicked
  (params (Button%20ID :type String) (Hit%20Location :type Vector))
  (switch string Button%20ID
    (:Default
      (Utilities|SendEvent "MainButtonClick" Button%20ID))
    (:menu
      (Default|LoadLevel (Variables|Default|GetPLM) "Menu"))
    (:quit
      (Game|QuitGame (Game|GetPlayerController 0) "Quit"))))

(fn ConstructionScript
  (bind _returnvalue (Rendering|Material|CreateDynamicMaterialInstance "/Game/StarterContent/Materials/M_Metal_Burnished_Steel.M_Metal_Burnished_Steel" :!class /Script/Engine.KismetMaterialLibrary))
  (Variables|Default|SetMID%20Background%20Normal _returnvalue))

(fn SetMainButton
  (params (Title :type String) (Button%20ID :type String))
  (Default|Setup (Variables|Default|GetMain%20Menu%20Button) (CallFunction|StandardButtonSize) false Title Button%20ID true))

(fn Setup
  (params (PMM :type BPI%20PMM%20Interface))
  (Utilities|FlowControl|Sequence
    (:then_0
      (Variables|Default|SetPLM PMM))
    (:then_1
      (bind _returnvalue (AddComponent|AddChildActorComponent false (Math|Transform|MakeTransform "0.000000,0.000000,0.000000" "-45.000000, 0, 0" "1.000000,1.000000,1.000000")))
      (bind _asbp_toggle_button (Utilities|Casting|CastToBP_ToggleButton (Variables|/Script/Engine.ChildActorComponent|GetChildActor _returnvalue)))
      (bind _output_get (Variables|Default|SetMain%20Menu%20Button _asbp_toggle_button))
      (Variables|/Game/ReusableAssets/Buttons/BP_ToggleButton.BP_ToggleButton_C|SetPush%20Button%20Mode _output_get true)
      (CallFunction|SetMainButton "Back" "menu"))
    (:then_2
      (CallFunction|ListentoMainMenuButtonEvents))
    (:then_3
      (bind _returnvalue_2 (AddComponent|AddProceduralMeshComponent false (Math|Transform|MakeTransform "0.000000,0.000000,-12.000000" "-45.000000, 0,0.000000" "1.000000,1,1")))
      (bind _output_get_2 (Variables|Default|SetButton%20Backgound _returnvalue_2))
      (CallFunction|SetupBoxMesh _output_get_2 (LocalVariables|GetBackground%20Size) (Variables|Default|GetMID%20Background%20Normal) true))))