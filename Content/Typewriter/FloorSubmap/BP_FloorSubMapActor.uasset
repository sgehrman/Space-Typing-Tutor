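; BP_FloorSubMapActor sets up a floor submap with a circular "Back" push button and three particle system actors in a row.
; BeginPlay spawns these as child actor components and requests PMM access, storing the result as PLM before binding the button click.
; Clicks route by button ID, either loading the Menu level through PLM or quitting the game.
; SetMenuButtonToQuit relabels the same button as "Quit".
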(event `self.ReceiveBeginPlay`
  (`|ExecutionSequence`
    (:`then_0`
      (bind _returnvalue (`AddComponent|ChildActorComponent_11226` :`RelativeTransform` (`KismetMathLibrary.MakeTransform` (111.0 0.0 -144.0) (struct :`Pitch` -45.0) (1.0 1.0 1.0))))
      (bind _asbp_toggle_button (cast `/Game/ReusableAssets/Buttons/BP_ToggleButton` (`ChildActorComponent.ChildActor` _returnvalue)))
      (bind _output_get (set `self.Main Menu Button` _asbp_toggle_button))
      (`/Game/ReusableAssets/Buttons/BP_ToggleButton.Setup` _output_get (`/Game/ReusableAssets/Utilities/LIB_Constants.Standard Button Size`) false "Back" "menu" true)
      (set `/Game/ReusableAssets/Buttons/BP_ToggleButton.Push Button Mode` true _output_get))
    (:`then_1`
      (bind _returnvalue_2 (`AddComponent|BC_PMMAccess_C_0`))
      (add `/Game/ReusableAssets/Utilities/BC_PMMAccess.PMM Ready` _returnvalue_2 (delegate `CustomEvent_0`))
      (`/Game/ReusableAssets/Utilities/BC_PMMAccess.Setup` _returnvalue_2 "None"))
    (:`then_2`
      (bind _returnvalue_3 (`AddComponent|Child Actor Component_33` :`RelativeTransform` (`KismetMathLibrary.MakeTransform` (2222.0 -1200.0 -200.0))))
      (bind _asbp_particle_system_actor (cast `/Game/Typewriter/BP_ParticleSystemActor` (`ChildActorComponent.ChildActor` _returnvalue_3)))
      (set `/Game/Typewriter/BP_ParticleSystemActor.Particle System Index` 31 _asbp_particle_system_actor)
      (`/Game/Typewriter/BP_ParticleSystemActor.Update Particle System` _asbp_particle_system_actor))
    (:`then_3`
      (bind _returnvalue_4 (`AddComponent|ChildActorComponent_34` :`RelativeTransform` (`KismetMathLibrary.MakeTransform` (2222.0 0.0 -200.0))))
      (bind _asbp_particle_system_actor_2 (cast `/Game/Typewriter/BP_ParticleSystemActor` (`ChildActorComponent.ChildActor` _returnvalue_4)))
      (set `/Game/Typewriter/BP_ParticleSystemActor.Particle System Index` 31 _asbp_particle_system_actor_2)
      (`/Game/Typewriter/BP_ParticleSystemActor.Update Particle System` _asbp_particle_system_actor_2))
    (:`then_4`
      (bind _returnvalue_5 (`AddComponent|ChildActorComponent_35` :`RelativeTransform` (`KismetMathLibrary.MakeTransform` (2222.0 1200.0 -200.0))))
      (bind _asbp_particle_system_actor_3 (cast `/Game/Typewriter/BP_ParticleSystemActor` (`ChildActorComponent.ChildActor` _returnvalue_5)))
      (set `/Game/Typewriter/BP_ParticleSystemActor.Particle System Index` 31 _asbp_particle_system_actor_3)
      (`/Game/Typewriter/BP_ParticleSystemActor.Update Particle System` _asbp_particle_system_actor_3))))

(event `Listen to Main Menu Button Events`
  (add `/Game/ReusableAssets/Buttons/BP_ToggleButton.ButtonClickedByUser` (`self.Main Menu Button`) (delegate `Main Menu Clicked`)))

(event `CustomEvent_0`
  (params (Result :type "/Game/ReusableAssets/Utilities/BPI_PMM Interface"))
  (set `self.PLM` Result)
  (`self.Listen to Main Menu Button Events`))

(event `Main Menu Clicked`
  (params (`Button ID` :type String) (`Hit Location` :type "Vector Structure"))
  (switch `string` `Button ID`
    (:`menu`
      (`/Game/ReusableAssets/Utilities/BPI_PMM.Load Level` (`self.PLM`) "Menu" ""))
    (:`quit`
      (`KismetSystemLibrary.QuitGame` (`GameplayStatics.GetPlayerController` 0) "Quit"))))

(fn `Set Menu Button to Quit`
  (`/Game/ReusableAssets/Buttons/BP_ToggleButton.Setup` (`self.Main Menu Button`) (`/Game/ReusableAssets/Utilities/LIB_Constants.Standard Button Size`) false "Quit" "quit" true))

(fn `UserConstructionScript`)