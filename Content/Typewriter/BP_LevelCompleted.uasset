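; BP_LevelCompleted is an actor that announces a finished level in the Typewriter game and waits for the player to continue.
; On BeginPlay it finds the message box manager and key event listener actors and binds to key sequence events.
; LevelCompleted shows a numbered completion message, listens for Enter and plays a delayed sound.
; Enter hides the message, fires the continue-after-level event and destroys the actor.
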(event `self.ReceiveBeginPlay`
  (`|ExecutionSequence`
    (:`then_0`
      (bind _asbp_message_box_manager (cast `/Game/ReusableAssets/MessageBox/BP_MessageBoxManager` (`.Actor` (`/Game/ReusableAssets/Utilities/LIB_Utilities.FindActorWithTag` "/Game/ReusableAssets/MessageBox/BP_MessageBoxManager.BP_MessageBoxManager_C" "None" self))))
      (set `self.Message Manager` _asbp_message_box_manager))
    (:`then_1`
      (bind _asbp_key_event_listener (cast `/Game/ReusableAssets/Keyboard/BP_KeyEventListener` (`.Actor` (`/Game/ReusableAssets/Utilities/LIB_Utilities.FindActorWithTag` "/Game/ReusableAssets/Keyboard/BP_KeyEventListener.BP_KeyEventListener_C" "None" self))))
      (bind _output_get (set `self.Key Event Listener` _asbp_key_event_listener))
      (add `/Game/ReusableAssets/Keyboard/BP_KeyEventListener.Key Sequence Event` _output_get (delegate `Key Sequence Event`)))))

(event `Key Sequence Event`
  (params (`Event Name` :type String))
  (switch `string` `Event Name`
    (:`Enter Key`
      (`/Game/ReusableAssets/MessageBox/BP_MessageBoxManager.Hide Message` (`self.Message Manager`))
      (`self.Continue After Level Complete`)
      (`self.K2_DestroyActor`))))

(event `Level Completed`
  (params (Level :type Integer))
  (`/Game/ReusableAssets/MessageBox/BP_MessageBoxManager.Show Message` (`self.Message Manager`) (222.0 0.0 88.0) (`|MakeArray` (`VictoryBPFunctionLibrary.AppendMultiple` "Level " (`KismetStringLibrary.Conv_IntToString` (+ Level 1)) " Completed!") "Press Enter to continue"))
  (`/Game/ReusableAssets/Keyboard/BP_KeyEventListener.Listen For Key Sequence` (`self.Key Event Listener`) "Enter Key" (`|MakeArray` (make `/Game/ReusableAssets/Keyboard/KeyboardKeySpec` "" "NewEnumerator2")))
  (`KismetSystemLibrary.Delay` 1.0)
  (`GameplayStatics.PlaySoundAtLocation` "/Game/UserInterfaceSFX/Starts/Wavs/start10.start10"))

(fn `UserConstructionScript`)