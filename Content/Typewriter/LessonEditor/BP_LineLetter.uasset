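; BP_LineLetter is a single clickable letter in the Typewriter lesson editor, tracked by its index.
; Setup spawns a BP_ToggleButton child actor, titles and sizes it to the letter, and gives it dynamic materials for on, off and hover.
; Button click and crosshair-move events are re-broadcast with the letter's index and hit location.
; Helper functions pass width, state and character through to the button.
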(event `Listen for Button Events`
  (add `/Game/ReusableAssets/Buttons/BP_ToggleButton.ButtonClickedByUser` (`self.Button`) (delegate `Click Event`))
  (add `/Game/ReusableAssets/Buttons/BP_ToggleButton.Crosshair Moved` (`self.Button`) (delegate `Crosshair Moved Event`)))

(event `Crosshair Moved Event`
  (params (`Hit Location` :type "Vector Structure"))
  (`self.Crosshair Moved` `Hit Location` (`self.Index`)))

(event `Click Event`
  (params (`Button ID` :type String) (`Hit Location` :type "Vector Structure"))
  (`self.State Changed` true (`self.Index`) `Hit Location`))

(fn `Get Character`
  (returns (Character :type String))
  (return (`/Game/ReusableAssets/Buttons/BP_ToggleButton.Get Title` (`self.Button`))))

(fn `Get State`
  (returns (State :type Boolean))
  (bind _state (`/Game/ReusableAssets/Buttons/BP_ToggleButton.Get State` (`self.Button`)))
  (return _state))

(fn `Get Width`
  (returns (Width :type "Float (double-precision)"))
  (return (`/Game/ReusableAssets/Buttons/BP_ToggleButton.Get Width` (`self.Button`))))

(fn `Set State`
  (params (State :type Boolean))
  (`/Game/ReusableAssets/Buttons/BP_ToggleButton.Set State` (`self.Button`) State))

(fn `Setup`
  (params (Letter :type String))
  (bind _letter_width (`self.Letter Width`))
  (`|ExecutionSequence`
    (:`then_2`
      (bind _returnvalue (`AddComponent|ChildActorComponent_806` :`RelativeTransform` (`/Game/ReusableAssets/Utilities/LIB_Utilities.Trans`)))
      (bind _asbp_toggle_button (cast `/Game/ReusableAssets/Buttons/BP_ToggleButton` (`ChildActorComponent.ChildActor` _returnvalue)))
      (bind _output_get (set `self.Button` _asbp_toggle_button))
      (`/Game/ReusableAssets/Buttons/BP_ToggleButton.Set Font Size` _output_get (`self.Font Size`))
      (`/Game/ReusableAssets/Buttons/BP_ToggleButton.Set Title and Size` _output_get (`KismetMathLibrary.MakeVector` _letter_width _letter_width (* _letter_width 1.6)) true Letter "")
      (`/Game/ReusableAssets/Buttons/BP_ToggleButton.Set State` _output_get false))
    (:`then_3`
      (`self.Listen for Button Events`))
    (:`then_4`
      (bind _returnvalue_2 (`KismetMaterialLibrary.CreateDynamicMaterialInstance` "/Game/ReusableAssets/Materials/MT_Opaque.MT_Opaque"))
      (bind _output_get_2 (set `self.MID On` _returnvalue_2))
      (`MaterialInstanceDynamic.SetVectorParameterValue` _output_get_2 "Color" (struct :`R` 0.053081 :`G` 0.366474 :`B` 0.64 :`A` 1.0)))
    (:`then_5`
      (bind _returnvalue_3 (`KismetMaterialLibrary.CreateDynamicMaterialInstance` "/Game/ReusableAssets/Materials/MT_Opaque.MT_Opaque"))
      (bind _output_get_3 (set `self.MID hover` _returnvalue_3))
      (`MaterialInstanceDynamic.SetVectorParameterValue` _output_get_3 "Color" (struct :`R` 0.053081 :`G` 0.366474 :`B` 0.64 :`A` 1.0)))
    (:`then_6`
      (bind _returnvalue_4 (`KismetMaterialLibrary.CreateDynamicMaterialInstance` "/Game/ReusableAssets/Materials/MT_Opaque.MT_Opaque"))
      (bind _output_get_4 (set `self.MID Off` _returnvalue_4))
      (`MaterialInstanceDynamic.SetVectorParameterValue` _output_get_4 "Color" (struct :`R` 0.053081 :`G` 0.366474 :`B` 0.64 :`A` 1.0)))
    (:`then_7`
      (`/Game/ReusableAssets/Buttons/BP_ToggleButton.Update Materials` (`self.Button`) (`self.MID On`) (`self.MID Off`) (`self.MID hover`)))))

(fn `Update Index`
  (params (Index :type Integer))
  (set `self.Index` Index))

(fn `UserConstructionScript`)