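; One page of a selectable lesson grid in the typewriter lesson editor.
; BuildGrid spawns BP_GridItem child actors at grid positions, turning end cells into Back/Next buttons when needed and disabling cells past TotalItems.
; Hover or arrow/WASD keys move the selection, wrapping at edges.
; Clicks broadcast the selected item rather than the clicked one; Back/Next then rebuild the grid without changing StartIndex, which Setup supplies.
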(event Custom|Listen%20for%20Button%20Events
  (for _array_element (Variables|Default|GetGrid%20Items)
    (EventDispatchers|BindEventtoItemClicked _array_element (delegate Custom|Clicked%20Event))
    (EventDispatchers|BindEventtoItemHovered _array_element (delegate Custom|Hovered%20Event))))

(event Custom|Clicked%20Event
  (params (Index :type Integer))
  (bind _index (CallFunction|GetSelectedIndex))
  (bind _grid_items (Variables|Default|GetGrid%20Items))
  (bind _item (Utilities|Array|Get(acopy) _grid_items _index))
  (bind (_item_data _type) (Default|GetData _item))
  (Default|CallClickedItem _item_data _type)
  (switch Utilities|FlowControl|Switch|SwitchonE_GridItemType _type
    (:NewEnumerator2
      (CallFunction|BuildGrid))
    (:NewEnumerator3
      (CallFunction|BuildGrid))))

(event Custom|Hovered%20Event
  (params (Grid%20Index :type Integer) (Finished :type Boolean))
  (if (not Finished)
    (CallFunction|SetSelectedIndex Grid%20Index)))

(event EventBeginPlay
  (Input|EnableInput (Game|GetPlayerController 0)))

(event Input|KeyboardEvents|A
  (:Pressed
    (bind (_index _is_valid) (CallFunction|GetNextSelectedIndex 0 -1))
    (if _is_valid
      (CallFunction|SetSelectedIndex _index))))

(event Input|KeyboardEvents|D
  (:Pressed
    (bind (_index _is_valid) (CallFunction|GetNextSelectedIndex 0 1))
    (if _is_valid
      (CallFunction|SetSelectedIndex _index))))

(event Input|KeyboardEvents|W
  (:Pressed
    (bind (_index _is_valid) (CallFunction|GetNextSelectedIndex -1))
    (if _is_valid
      (CallFunction|SetSelectedIndex _index))))

(event Input|KeyboardEvents|S
  (:Pressed
    (bind (_index _is_valid) (CallFunction|GetNextSelectedIndex 1))
    (if _is_valid
      (CallFunction|SetSelectedIndex _index))))

(event Input|KeyboardEvents|Up
  (:Pressed
    (bind (_index _is_valid) (CallFunction|GetNextSelectedIndex -1))
    (if _is_valid
      (CallFunction|SetSelectedIndex _index))))

(event Input|KeyboardEvents|Down
  (:Pressed
    (bind (_index _is_valid) (CallFunction|GetNextSelectedIndex 1))
    (if _is_valid
      (CallFunction|SetSelectedIndex _index))))

(event Input|KeyboardEvents|Left
  (:Pressed
    (bind (_index _is_valid) (CallFunction|GetNextSelectedIndex 0 -1))
    (if _is_valid
      (CallFunction|SetSelectedIndex _index))))

(event Input|KeyboardEvents|Right
  (:Pressed
    (bind (_index _is_valid) (CallFunction|GetNextSelectedIndex 0 1))
    (if _is_valid
      (CallFunction|SetSelectedIndex _index))))

(fn ConstructionScript
  (Utilities|FlowControl|Sequence
    (:then_0
      (Variables|Default|SetNum%20Grid%20Items (* (Variables|Default|GetNum%20Rows) (Variables|Default|GetNum%20Cols))))
    (:then_1
      (CallFunction|BuildGrid))))

(fn BuildGrid
  (Utilities|FlowControl|Sequence
    (:then_0
      (for _array_element (Variables|Default|GetGrid%20Items)
        (Actor|DestroyActor _array_element))
      (Utilities|Array|Clear (Variables|Default|GetGrid%20Items)))
    (:then_1
      (bind (_needs_previous_button _needs_next_button) (CallFunction|CalcParameters (Variables|Default|GetStart%20Index) (Variables|Default|GetTotal%20Items)))
      (LocalVariables|SetMake%20Prev%20Button _needs_previous_button)
      (LocalVariables|SetMake%20Next%20Button _needs_next_button)
      (Variables|Default|SetItem%20Locations (CallFunction|PositionsinGrid (Variables|Default|GetNum%20Grid%20Items) (Variables|Default|GetNum%20Cols) 4.0 (Math|Conversions|ToVector(Float) (Variables|Default|GetMesh%20Size))))
      (LocalVariables|SetLast%20Index (- (Variables|Default|GetNum%20Grid%20Items) 1)))
    (:then_6
      (for (_array_element_2 _array_index) (Variables|Default|GetItem%20Locations)
        (LocalVariables|SetLoop%20Index _array_index)
        (LocalVariables|SetNeeds%20Setup true)
        (Utilities|FlowControl|Sequence
          (:then_0
            (bind _returnvalue (AddComponent|AddChildActorComponent false (Math|Transform|MakeTransform _array_element_2)))
            (bind _asbp_grid_item (Utilities|Casting|CastToBP_GridItem (Variables|/Script/Engine.ChildActorComponent|GetChildActor _returnvalue)))
            (bind _output_get (LocalVariables|SetNew%20Item _asbp_grid_item))
            (Utilities|Array|Add (Variables|Default|GetGrid%20Items) _output_get))
          (:then_1
            (Utilities|FlowControl|Sequence
              (:then_0
                (if (== (LocalVariables|GetLoop%20Index) 0)
                  (if (LocalVariables|GetMake%20Prev%20Button)
                    (Default|Setup (LocalVariables|GetNew%20Item) "" 0 "NewEnumerator2" (LocalVariables|GetLoop%20Index))
                    (LocalVariables|SetNeeds%20Setup false))
                  (elif (== (LocalVariables|GetLoop%20Index) (LocalVariables|GetLast%20Index))
                    (if (LocalVariables|GetMake%20Next%20Button)
                      (Default|Setup (LocalVariables|GetNew%20Item) "" 0 "NewEnumerator3" (LocalVariables|GetLoop%20Index))
                      (LocalVariables|SetNeeds%20Setup false)))))
              (:then_1
                (if (LocalVariables|GetNeeds%20Setup)
                  (Utilities|FlowControl|Sequence
                    (:then_0
                      (LocalVariables|SetCurrent%20Index (+ (LocalVariables|GetLoop%20Index) (Variables|Default|GetStart%20Index)))
                      (if (LocalVariables|GetMake%20Prev%20Button)
                        (Math|Integer|DecrementInt (LocalVariables|GetCurrent%20Index))))
                    (:then_1
                      (if (< (LocalVariables|GetCurrent%20Index) (Variables|Default|GetTotal%20Items))
                        (Default|Setup (LocalVariables|GetNew%20Item) (Class|VictoryBPFunctionLibrary|AppendMultiple "Lesson: " (Utilities|String|ToString(Integer) (+ (LocalVariables|GetCurrent%20Index) 1))) (LocalVariables|GetCurrent%20Index) "NewEnumerator0" (LocalVariables|GetLoop%20Index))
                        (else
                          (Default|Setup (LocalVariables|GetNew%20Item) "" 0 "NewEnumerator1" (LocalVariables|GetLoop%20Index)))))))))))))
    (:then_8
      (CallFunction|ListenforButtonEvents))))

(fn CalcParameters
  (params (Start%20index :type Integer) (Total%20Items :type Integer))
  (Utilities|FlowControl|Sequence
    (:then_0
      (LocalVariables|SetNum%20Items%20to%20Display (Variables|Default|GetNum%20Grid%20Items)))
    (:then_1
      (LocalVariables|SetPrev%20Button%20Result (!= Start%20index 0)))
    (:then_2
      (if (LocalVariables|GetPrev%20Button%20Result)
        (Math|Integer|DecrementInt (LocalVariables|GetNum%20Items%20to%20Display))))
    (:then_3
      (LocalVariables|SetNext%20Button%20Result (< (+ Start%20index (LocalVariables|GetNum%20Items%20to%20Display)) Total%20Items)))
    (:then_6
      (return (LocalVariables|GetPrev%20Button%20Result) (LocalVariables|GetNext%20Button%20Result)))))

(fn FadeOut
  (params (Fade%20In :type Boolean))
  (for _array_element (Variables|Default|GetGrid%20Items)
    (Default|FadeOut _array_element Fade%20In)))

(fn GetSelectedIndex
  (Utilities|FlowControl|Sequence
    (:then_0
      (for (_array_element _array_index) (Variables|Default|GetGrid%20Items)
        (if (not (LocalVariables|GetResult%20Valid))
          (LocalVariables|SetResult%20Valid (Default|IsSelected _array_element))
          (LocalVariables|SetResult%20Index _array_index))))
    (:then_3
      (return (LocalVariables|GetResult%20Index) (LocalVariables|GetResult%20Valid)))))

(fn GetNextSelectedIndex
  (params (Vertical%20Axis :type Integer) (Horizontal%20Axis :type Integer))
  (bind (_index _is_valid) (CallFunction|GetSelectedIndex))
  (Utilities|FlowControl|Sequence
    (:then_0
      (LocalVariables|SetResult%20Valid _is_valid)
      (LocalVariables|SetResult%20Index _index))
    (:then_1
      (if (LocalVariables|GetResult%20Valid)
        (Utilities|FlowControl|Sequence
          (:then_0
            (LocalVariables|SetNew%20Row (.Row (CallFunction|RowColforIndex (LocalVariables|GetResult%20Index))))
            (LocalVariables|SetNew%20Column (.Column (CallFunction|RowColforIndex (LocalVariables|GetResult%20Index))))
            (if (!= Vertical%20Axis 0)
              (LocalVariables|SetNew%20Row (+ (LocalVariables|GetNew%20Row) Vertical%20Axis))
              (elif (!= Horizontal%20Axis 0)
                (LocalVariables|SetNew%20Column (+ (LocalVariables|GetNew%20Column) Horizontal%20Axis)))))
          (:then_1
            (if (< (LocalVariables|GetNew%20Row) 0)
              (LocalVariables|SetNew%20Row (- (Variables|Default|GetNum%20Rows) 1))
              (elif (>= (LocalVariables|GetNew%20Row) (Variables|Default|GetNum%20Rows))
                (LocalVariables|SetNew%20Row 0))))
          (:then_2
            (if (< (LocalVariables|GetNew%20Column) 0)
              (LocalVariables|SetNew%20Column (- (Variables|Default|GetNum%20Cols) 1))
              (elif (>= (LocalVariables|GetNew%20Column) (Variables|Default|GetNum%20Cols))
                (LocalVariables|SetNew%20Column 0))))
          (:then_3
            (LocalVariables|SetResult%20Index (CallFunction|IndexforRowCol (LocalVariables|GetNew%20Row) (LocalVariables|GetNew%20Column)))))
        (else
          (LocalVariables|SetResult%20Valid true)
          (LocalVariables|SetResult%20Index 0))))
    (:then_3
      (return (LocalVariables|GetResult%20Index) (LocalVariables|GetResult%20Valid)))))

(fn RowColforIndex
  (params (Index :type Integer))
  (bind _num_cols (Variables|Default|GetNum%20Cols))
  (return (/ Index _num_cols) (Math|Integer|%(Integer) Index _num_cols)))

(fn IndexforRowCol
  (params (Row :type Integer) (Column :type Integer))
  (return (+ (* Row (Variables|Default|GetNum%20Cols)) Column)))

(fn SetSelectedIndex
  (params (Index :type Integer))
  (for (_array_element _array_index) (Variables|Default|GetGrid%20Items)
    (Default|Select _array_element (== Index _array_index))))

(fn Setup
  (params (Start%20Index :type Integer) (Total%20Items :type Integer))
  (Variables|Default|SetStart%20Index Start%20Index)
  (Variables|Default|SetTotal%20Items Total%20Items)
  (CallFunction|BuildGrid))