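; Grid tile for the Typewriter lesson editor, acting as a numbered, named item, disabled slot or Back/Next button.
; Construction builds a procedural physics box without gravity, reattaches both text labels to it and creates normal and emissive selected materials.
; Setup sets type and labels, Select swaps material and text color, and timelines animate opacity and quarter-turn rotation.
; Crosshair hover, click and scroll handlers report the tile's grid index through ItemHovered and ItemClicked calls.
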(event `Fade Out`
  (params (`Fade In` :type Boolean))
  (`TimelineComponent.SetPlayRate` (`self.Fade Out Timeline`) 0.5)
  (if `Fade In`
    (bind (_direction _c_genericcurve) (`Timeline|Fade Out Timeline` :!via `PlayFromStart` :!label _label)
      (:`Update`
        (`MaterialInstanceDynamic.SetScalarParameterValue` (`self.MID`) "Opacity" _c_genericcurve)
        (`MaterialInstanceDynamic.SetScalarParameterValue` (`self.MID Button`) "Opacity" _c_genericcurve)))
    (else
      (goto _label :!via `ReverseFromEnd`))))

(event `Rotate Right`
  (params (Left :type Boolean) (Index :type Integer))
  (`KismetSystemLibrary.Delay` (* 0 0.01))
  (switch `/Game/Typewriter/LessonEditor/E_GridItemType` (`self.Type`)
    (:`NewEnumerator0`
      (`TimelineComponent.SetPlayRate` (`self.Rotate Timeline`) 3.0)
      (bind (_direction _c_genericcurve) (`Timeline|Rotate Timeline` :!via `PlayFromStart`)
        (:`Update`
          (if Left
            (`SceneComponent.K2_SetRelativeRotation` (`self.Mesh`) (`KismetMathLibrary.RLerp` (struct :`Yaw` 90.0) (struct) _c_genericcurve) false)
            (else
              (`SceneComponent.K2_SetRelativeRotation` (`self.Mesh`) (`KismetMathLibrary.RLerp` (struct :`Yaw` -90.0) (struct) _c_genericcurve) false))))))))

(fn `Crosshair Hover Progress`
  (params (Progress :type "Float (double-precision)") (`Local Hit Location` :type "Vector Structure") (`Hit Component` :type "PrimitiveComponent Object Reference"))
  (returns (Success :type Boolean))
  (return false))

(fn `Crosshair Hover Start`
  (params (Finished :type Boolean))
  (returns (Success :type Boolean))
  (`self.Item Hovered` (`self.Grid Index`) Finished)
  (return true))

(fn `Crosshair LeftRight`
  (params (Left :type Boolean))
  (returns (Success :type Boolean))
  (return false))

(fn `Crosshair Mouse Click`
  (params (`Mouse Down` :type Boolean) (`Event Type` :type "/Game/ReusableAssets/Utilities/E_EventType Enum" :default "NewEnumerator10") (`Hit Location` :type "Vector Structure") (`Hit Component` :type "PrimitiveComponent Object Reference"))
  (returns (Success :type Boolean))
  (`|ExecutionSequence`
    (:`then_0`
      (switch `/Game/ReusableAssets/Utilities/E_EventType` `Event Type`
        (:`NewEnumerator0`
          _)
        (:`NewEnumerator3`
          _))
      (if `Mouse Down`
        (`self.Item Clicked` (`self.Grid Index`) (`|EnumEquality` `Event Type` "NewEnumerator3"))))
    (:`then_2`
      (return true))))

(fn `Crosshair Scroll Wheel`
  (params (Down :type Boolean) (`Hit Location` :type "Vector Structure") (`Hit Component` :type "PrimitiveComponent Object Reference"))
  (returns (Success :type Boolean))
  (`|ExecutionSequence`
    (:`then_0`
      (switch `/Game/Typewriter/LessonEditor/E_GridItemType` (`self.Type`)
        (:`NewEnumerator2`
          _)
        (:`NewEnumerator3`
          _))
      (`self.Item Clicked` (`self.Grid Index`)))
    (:`then_2`
      (return true))))

(fn `Crosshair UpDown`
  (params (Up :type Boolean))
  (returns (Success :type Boolean))
  (return true))

(fn `Get Data`
  (returns (`Item Data` :type Integer) (Type :type "/Game/Typewriter/LessonEditor/E_GridItemType Enum"))
  (return (`self.Item Data`) (`self.Type`)))

(fn `Is Selected`
  (returns (Result :type Boolean))
  (return (`self.Selected`)))

(fn `Select`
  (params (Select :type Boolean))
  (`|ExecutionSequence`
    (:`then_0`
      (if (`|EnumInequality` (`self.Type`) "NewEnumerator1")
        (set `self.Selected` Select)
        (else
          (set `self.Selected` false))))
    (:`then_1`
      (if (`self.Selected`)
        (switch `/Game/Typewriter/LessonEditor/E_GridItemType` (`self.Type`)
          (:`NewEnumerator0`
            (`PrimitiveComponent.SetMaterial` (`self.Mesh`) 0 (`self.MID Selected`)))
          (:`NewEnumerator2`
            (`PrimitiveComponent.SetMaterial` (`self.Mesh`) 0 (`self.MID Button Selected`) :!label _label))
          (:`NewEnumerator3`
            (goto _label)))
        (`TextRenderComponent.SetTextRenderColor` (`self.Name`) (make `Color` 0 0 0 255))
        (`TextRenderComponent.SetTextRenderColor` (`self.Number`) (make `Color` 0 0 0 255))
        (else
          (switch `/Game/Typewriter/LessonEditor/E_GridItemType` (`self.Type`)
            (:`NewEnumerator0`
              (`PrimitiveComponent.SetMaterial` (`self.Mesh`) 0 (`self.MID`)))
            (:`NewEnumerator2`
              (`PrimitiveComponent.SetMaterial` (`self.Mesh`) 0 (`self.MID Button`) :!label _label_2))
            (:`NewEnumerator3`
              (goto _label_2)))
          (`TextRenderComponent.SetTextRenderColor` (`self.Name`) (make `Color` 255 255 255 255))
          (`TextRenderComponent.SetTextRenderColor` (`self.Number`) (make `Color` 255 255 255 255)))))))

(fn `Setup`
  (params (`Item Name` :type String) (`Item Data` :type Integer) (`Item Type` :type "/Game/Typewriter/LessonEditor/E_GridItemType Enum") (`Grid Index` :type Integer))
  (bind _output_get (set `self.Type` `Item Type`))
  (set `self.Grid Index` `Grid Index`)
  (switch `/Game/Typewriter/LessonEditor/E_GridItemType` _output_get
    (:`NewEnumerator0`
      (set `self.Item Name` `Item Name`)
      (set `self.Item Data` `Item Data`)
      (`self.Update Number and Name` (`KismetTextLibrary.Conv_IntToText` (+ (`self.Item Data`) 1) true 2) (`KismetTextLibrary.Conv_StringToText` (`self.Item Name`))))
    (:`NewEnumerator1`
      (`self.Update Number and Name` ""))
    (:`NewEnumerator2`
      (`self.Update Number and Name` "<-" "Back")
      (`PrimitiveComponent.SetMaterial` (`self.Mesh`) 0 (`self.MID Button`) :!label _label))
    (:`NewEnumerator3`
      (`self.Update Number and Name` "->" "Next")
      (goto _label))))

(fn `Update Number and Name`
  (params (`Number Text` :type Text) (`Name Text` :type Text))
  (`TextRenderComponent.K2_SetText` (`self.Number`) `Number Text`)
  (`TextRenderComponent.K2_SetText` (`self.Name`) `Name Text`))

(fn `UserConstructionScript`
  (bind _mesh (`self.Mesh`))
  (bind _number (`self.Number`))
  (bind _name (`self.Name`))
  (`|ExecutionSequence`
    (:`then_0`
      (bind _returnvalue (`KismetMaterialLibrary.CreateDynamicMaterialInstance` "/Game/ReusableAssets/Materials/MT_Opaque.MT_Opaque"))
      (bind _output_get (set `self.MID Button` _returnvalue))
      (`MaterialInstanceDynamic.SetVectorParameterValue` _output_get "Color" (struct :`R` 0.54 :`B` 0.028099 :`A` 1.0))
      (`MaterialInstanceDynamic.SetScalarParameterValue` _output_get "Roughness" 0.0))
    (:`then_1`
      (bind _returnvalue_2 (`KismetMaterialLibrary.CreateDynamicMaterialInstance` "/Game/ReusableAssets/Materials/MT_Opaque.MT_Opaque" :!label _label))
      (bind _output_get_2 (set `self.MID` _returnvalue_2))
      (`MaterialInstanceDynamic.SetVectorParameterValue` _output_get_2 "Color" (struct :`R` 0.053081 :`G` 0.366474 :`B` 0.64 :`A` 1.0))
      (`MaterialInstanceDynamic.SetScalarParameterValue` _output_get_2 "Roughness" 0.0))
    (:`then_2`
      (bind _returnvalue_3 (`KismetMaterialLibrary.CreateDynamicMaterialInstance` "/Game/ReusableAssets/Materials/MT_Opaque.MT_Opaque"))
      (bind _output_get_3 (set `self.MID Button Selected` _returnvalue_3))
      (`MaterialInstanceDynamic.SetVectorParameterValue` _output_get_3 "EmissiveColor" (struct :`R` 0.541176 :`B` 0.027451 :`A` 1.0))
      (`MaterialInstanceDynamic.SetScalarParameterValue` _output_get_3 "Emission" 4.0))
    (:`then_3`
      (goto _label))
    (:`then_4`
      (bind _returnvalue_4 (`KismetMaterialLibrary.CreateDynamicMaterialInstance` "/Game/ReusableAssets/Materials/MT_Opaque.MT_Opaque"))
      (bind _output_get_4 (set `self.MID Selected` _returnvalue_4))
      (`MaterialInstanceDynamic.SetVectorParameterValue` _output_get_4 "EmissiveColor" (struct :`R` 0.053081 :`G` 0.366474 :`B` 0.64 :`A` 1.0))
      (`MaterialInstanceDynamic.SetScalarParameterValue` _output_get_4 "Emission" 4.0))
    (:`then_5`
      (bind _returnvalue_5 (`AddComponent|ProceduralMeshComponent_1` :`RelativeTransform` (`/Game/ReusableAssets/Utilities/LIB_Utilities.Trans`)))
      (bind _output_get_5 (set `self.Mesh` _returnvalue_5))
      (`PrimitiveComponent.SetMaterial` _output_get_5 0 (`self.MID`))
      (`PrimitiveComponent.SetSimulatePhysics` _mesh true)
      (`PrimitiveComponent.SetEnableGravity` _mesh false)
      (bind (_vertices _triangles _normals _uvs _tangents) (`KismetProceduralMeshLibrary.GenerateBoxMesh` (/ (`KismetMathLibrary.Conv_DoubleToVector` (`self.Mesh Size`)) 2.0)))
      (`ProceduralMeshComponent.CreateMeshSection` :`self` (`self.Mesh`) :`Vertices` _vertices :`Triangles` _triangles :`Normals` _normals :`UV0` _uvs :`Tangents` _tangents :`bCreateCollision` true)
      (`PrimitiveComponent.SetCollisionEnabled` (`self.Mesh`) "QueryAndPhysics"))
    (:`then_6`
      ;[1 1 1] Reattach to procedural mesh so it will follow with phyics
      (`SceneComponent.DetachFromParent` _number false true)
      (`SceneComponent.K2_AttachTo` _number (`self.Mesh`) "None" "KeepRelativeOffset" true)
      (`SceneComponent.DetachFromParent` _name false true)
      (`SceneComponent.K2_AttachTo` _name (`self.Mesh`) "None" "KeepRelativeOffset" true))))