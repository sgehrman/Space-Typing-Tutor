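; Lesson browser actor for the typewriter lesson editor that pages between a grid of lessons and each lesson's sentences.
; It builds grid node arrays from PLM lesson data and rebuilds the current page on "Lessons Modified" messages.
; Clicking a lesson opens its sentences in editor mode, otherwise lessons and sentences raise ClickedItem.
; Pages are spawned child actors swapped with staggered hide/show animations, and an X button returns to lessons or signals editor closed.
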(event Custom|Bind%20Page%20Events
  (EventDispatchers|BindEventtoClickedItem (Variables|Default|GetMain%20Page) (delegate Custom|Clicked%20Event)))

(event Custom|CustomEvent_0
  (params (Result :type BPI%20PMM%20Interface))
  (bind _output_get (Variables|Default|SetPLM Result))
  (Utilities|FlowControl|Sequence
    (:then_0
      (Actor|DestroyActor (Variables|Default|GetMain%20Page))
      (CallFunction|LoadLessonPage))
    (:then_1
      (bind _depot (Default|MessageDepot _output_get))
      (EventDispatchers|BindEventtoMessageEvent _depot (delegate Custom|CustomEvent_1)))))

(event Custom|Clicked%20Event
  (params (Item%20Location :type Vector) (Item%20Index :type Integer) (Data%20Node :type S%20Grid%20Data%20Node%20Structure))
  (bind (_listid _listindex _name _datatoken) (Utilities|Struct|BreakS_GridDataNode Data%20Node))
  (if (not (Variables|Default|GetDisabled))
    (switch string _listid
      (:s
        (Default|CallClickedItem _name _datatoken))
      (:l
        (if (Variables|Default|GetEditor%20Mode)
          (bind _returnvalue (AddComponent|AddChildActorComponent false))
          (bind _asbp_grid_item_page (Utilities|Casting|CastToBP_GridItemPage (Variables|/Script/Engine.ChildActorComponent|GetChildActor _returnvalue)))
          (CallFunction|RefreshPageData _listindex "Sentences" _asbp_grid_item_page)
          (CallFunction|SwitchPage _asbp_grid_item_page (Class|VictoryBPFunctionLibrary|AppendMultiple "Lesson #" (Utilities|String|ToString(Integer) (+ _listindex 1))) Item%20Index "sub")
          (else
            (Default|CallClickedItem _name _datatoken)))))))

(event Custom|CustomEvent_1
  (params (Message%20ID :type String) (Parameter :type String))
  (bind _main_page (Variables|Default|GetMain%20Page))
  (bind _main_page_2 (Variables|Default|GetMain%20Page))
  (bind _parent_token (Default|GetParentToken _main_page))
  (switch string Message%20ID
    (:Lessons%20Modified
      (if (== (Utilities|String|Len _parent_token) 0)
        (CallFunction|RefreshPageData 0 "Lessons" _main_page_2)
        (else
          (Default|UpdateDataArray _main_page_2 (CallFunction|DataArrayforToken _parent_token) _parent_token (Variables|Default|GetEditor%20Mode)))))))

(event Custom|Listen%20For%20Editor%20Events
  (EventDispatchers|BindEventtoFinishedEditing (Variables|Default|GetEditor%20Line) (delegate Custom|Finished%20Editing%20Event)))

(event Custom|Finished%20Editing%20Event
  (params (String :type String) (Data%20Token :type String))
  (Actor|DestroyActor (Variables|Default|GetEditor%20Line)))

(event Custom|BackButtonClicked
  (params (Button%20ID :type String) (Hit%20Location :type Vector))
  (if (not (Variables|Default|GetDisabled))
    (switch string Button%20ID
      (:back
        (switch string (Variables|Default|GetDisplayed%20Page%20ID)
          (:Default
            (CallFunction|LoadLessonPage))
          (:main
            (Default|CallEditorClosed)))))))

(event Custom|Load%20Lesson%20Page
  (bind _returnvalue (AddComponent|AddChildActorComponent false))
  (bind _asbp_grid_item_page (Utilities|Casting|CastToBP_GridItemPage (Variables|/Script/Engine.ChildActorComponent|GetChildActor _returnvalue)))
  (CallFunction|RefreshPageData 0 "Lessons" _asbp_grid_item_page)
  (CallFunction|SwitchPage _asbp_grid_item_page "Lessons" 0 "main"))

(event Custom|Refresh%20Page%20Data
  (params (Index :type Integer) (List%20ID :type String) (Page :type BP%20Grid%20Item%20Page%20Object%20Reference))
  (bind (_data_array _parent_token) (CallFunction|MakeDataArray List%20ID Index))
  (Default|UpdateDataArray Page _data_array _parent_token (Variables|Default|GetEditor%20Mode)))

(event EventBeginPlay
  (Utilities|FlowControl|Sequence
    (:then_0
      (bind _returnvalue (AddComponent|AddBCPMMAccess))
      (EventDispatchers|BindEventtoPMMReady _returnvalue (delegate Custom|CustomEvent_0))
      (Default|Setup _returnvalue "None"))
    (:then_1
      (EventDispatchers|BindEventtoButtonClickedbyUser (Variables|Default|GetBack%20Toolbar%20Button) (delegate Custom|BackButtonClicked)))))

(fn ConstructionScript
  (Utilities|FlowControl|Sequence
    (:then_0
      (bind _returnvalue (Rendering|Material|CreateDynamicMaterialInstance "/Game/ReusableAssets/Materials/MT_Opaque.MT_Opaque" :!class /Script/Engine.KismetMaterialLibrary))
      (bind _output_get (Variables|Default|SetMID%20Back%20Button _returnvalue))
      (Rendering|Material|SetVectorParameterValue _output_get "EmissiveColor" "(R=0.615000,G=0.000000,B=0.101352,A=1.000000)" :!class /Script/Engine.MaterialInstanceDynamic)
      (Rendering|Material|SetScalarParameterValue _output_get "Emission" 12.0 :!class /Script/Engine.MaterialInstanceDynamic))
    (:then_1
      (bind _returnvalue_2 (Rendering|Material|CreateDynamicMaterialInstance "/Game/ReusableAssets/Materials/MT_Opaque.MT_Opaque" :!class /Script/Engine.KismetMaterialLibrary))
      (bind _output_get_2 (Variables|Default|SetMID%20Back%20Button%20Selected _returnvalue_2))
      (Rendering|Material|SetVectorParameterValue _output_get_2 "EmissiveColor" "(R=0.615000,G=0.000000,B=0.101352,A=1.000000)" :!class /Script/Engine.MaterialInstanceDynamic)
      (Rendering|Material|SetScalarParameterValue _output_get_2 "Emission" 12.0 :!class /Script/Engine.MaterialInstanceDynamic))
    (:then_2
      (bind _returnvalue_3 (AddComponent|AddChildActorComponent false))
      (bind _asbp_grid_item_page (Utilities|Casting|CastToBP_GridItemPage (Variables|/Script/Engine.ChildActorComponent|GetChildActor _returnvalue_3)))
      (Variables|Default|SetMain%20Page _asbp_grid_item_page))
    (:then_3
      (bind _returnvalue_4 (AddComponent|AddChildActorComponent false (Math|Transform|MakeTransform "-1.000000,-40.000000,50.000000")))
      (bind _asbp_toggle_button (Utilities|Casting|CastToBP_ToggleButton (Variables|/Script/Engine.ChildActorComponent|GetChildActor _returnvalue_4)))
      (bind _output_get_3 (Variables|Default|SetBack%20Toolbar%20Button _asbp_toggle_button))
      (Default|SetFontSize _output_get_3 5.0)
      (Default|SetTitleandSize _output_get_3 "6.000000,8.000000,6.000000" false "X" "back")
      (Default|SetState _output_get_3 false)
      (Rendering|SetVisibility (Variables|/Game/ReusableAssets/Buttons/BP_ToggleButton.BP_ToggleButton_C|GetRoot _output_get_3) false true))))

(fn MakeDataArray
  (params (List%20ID :type String) (Index :type Integer))
  (Utilities|FlowControl|Sequence
    (:then_0
      (switch string List%20ID
        (:Sentences
          (bind _lesson_data (Default|LessonData (Variables|Default|GetPLM)))
          (bind _lesson (Default|ILessonatIndex _lesson_data Index))
          (LocalVariables|SetResult%20Parent%20Token (.DataToken (Utilities|Struct|BreakS_KeyboardLesson _lesson))))))
    (:then_3
      (return (CallFunction|DataArrayforToken (LocalVariables|GetResult%20Parent%20Token)) (LocalVariables|GetResult%20Parent%20Token)))))

(fn UpdateTitle
  (params (Title :type Text) (Number%20Of%20Items :type Integer))
  (Utilities|FlowControl|Sequence
    (:then_0
      (Rendering|Components|TextRender|SetText (Variables|Default|GetTitle) Title))
    (:then_1
      (Rendering|Components|TextRender|SetText (Variables|Default|GetSubtitle) (Utilities|Text|ToText(String) (Class|VictoryBPFunctionLibrary|AppendMultiple (Utilities|String|ToString(Text) (Utilities|Text|ToText(Integer) Number%20Of%20Items true 2)) " Items"))))))

(fn SwitchPage
  (params (Page :type BP%20Grid%20Item%20Page%20Object%20Reference) (Title :type String) (Click%20Index :type Integer) (Page%20ID :type String))
  (Utilities|FlowControl|Sequence
    (:then_0
      (if (!= (Variables|Default|GetMain%20Page) 0)
        ;[1 1 1] This auto destroys after hide
        (Default|RunShowAnimation (Variables|Default|GetMain%20Page) Click%20Index 0.0 true)))
    (:then_1
      (Variables|Default|SetMain%20Page Page)
      (CallFunction|BindPageEvents))
    (:then_2
      (Default|RunShowAnimation Page Click%20Index 0.6 false))
    (:then_3
      (CallFunction|UpdateTitle (Utilities|Text|ToText(String) Title) (Default|NumberOfItems (Variables|Default|GetMain%20Page))))
    (:then_4
      (Variables|Default|SetDisplayed%20Page%20ID Page%20ID))))

(fn Disable
  (params (Disable :type Boolean))
  (Variables|Default|SetDisabled Disable))

(fn DataArrayforToken
  (params (Token :type String))
  (Utilities|FlowControl|Sequence
    (:then_0
      (if (== (Utilities|String|Len Token) 0)
        (bind _lesson_data (Default|LessonData (Variables|Default|GetPLM)))
        (bind _count (Default|ILessonCount _lesson_data))
        (for _index (range 0 (- _count 1))
          (bind _lesson_data_2 (Default|LessonData (Variables|Default|GetPLM)))
          (bind _lesson (Default|ILessonatIndex _lesson_data_2 _index))
          (Utilities|Array|Add (LocalVariables|GetResult%20Data) (Utilities|Struct|MakeS_GridDataNode "l" _index (.Name (Utilities|Struct|BreakS_KeyboardLesson _lesson)) (.DataToken (Utilities|Struct|BreakS_KeyboardLesson _lesson)))))
        (else
          (bind _lesson_data_3 (Default|LessonData (Variables|Default|GetPLM)))
          (bind _lesson_2 (Default|LessonforToken _lesson_data_3 Token))
          (for (_array_element _array_index) (.Strings (Utilities|Struct|BreakS_KeyboardLesson _lesson_2))
            (Utilities|Array|Add (LocalVariables|GetResult%20Data) (Utilities|Struct|MakeS_GridDataNode "s" _array_index (.String (Utilities|Struct|BreakS_StringAndToken _array_element)) (.DataToken (Utilities|Struct|BreakS_StringAndToken _array_element))))))))
    (:then_3
      (return (LocalVariables|GetResult%20Data)))))

(fn EnableEditorMode
  (Variables|Default|SetEditor%20Mode true)
  (CallFunction|ShowCloseButton))

(fn ShowCloseButton
  (Rendering|SetVisibility (Variables|/Game/ReusableAssets/Buttons/BP_ToggleButton.BP_ToggleButton_C|GetRoot (Variables|Default|GetBack%20Toolbar%20Button)) true true))