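; BP_DisplayBox is a lesson editor display panel: a procedurally built box with a raised frame, title, subtitle and optional close button.
; Setup optionally overrides size and margins, then BuildDisplayBox generates body and four margin bars as collidable procedural meshes with two tinted dynamic materials.
; BuildCloseButton spawns a hidden BP_ToggleButton child actor, whose clicks fire the CloseButtonClicked dispatcher.
; The color picker code in the event graph never runs.
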(event Custom|ColorChanged_Event_0
  (params (NewColor :type Linear%20Color%20Structure))
  (Rendering|Material|SetVectorParameterValue (Variables|Default|GetMID) "Color" NewColor :!class /Script/Engine.MaterialInstanceDynamic))

(event Custom|Listen%20To%20Close%20Button
  (EventDispatchers|BindEventtoButtonClickedbyUser (Variables|Default|GetBack%20Toolbar%20Button) (delegate Custom|Button%20Clicked)))

(event Custom|Button%20Clicked
  (params (Button%20ID :type String) (Hit%20Location :type Vector))
  (Default|CallCloseButtonClicked))

(event EventBeginPlay)

(fn ConstructionScript)

(fn BuildDisplayBox
  (bind _box_size (Variables|Default|GetBox%20Size))
  (bind _box_size_2 (Variables|Default|GetBox%20Size))
  (bind _box_size_3 (Variables|Default|GetBox%20Size))
  (bind _margin_depth (Variables|Default|GetMargin%20Depth))
  (bind _box_size_4 (Variables|Default|GetBox%20Size))
  (bind _margin_top (Variables|Default|GetMargin%20Top))
  (bind _box_size_5 (Variables|Default|GetBox%20Size))
  (bind _returnvalue (/ _margin_top 2.0))
  (bind _returnvalue_2 (/ (.z _box_size_4) 2.0))
  (bind _returnvalue_3 (+ _margin_depth 4.0))
  (bind _returnvalue_4 (Class|TKMathFunctionLibrary|NegateFloat _returnvalue_3))
  (bind _returnvalue_5 (- _returnvalue_2 _returnvalue))
  (Utilities|FlowControl|Sequence
    (:then_0
      (bind _returnvalue_6 (Rendering|Material|CreateDynamicMaterialInstance "/Game/ReusableAssets/Materials/MT_Opaque.MT_Opaque" :!class /Script/Engine.KismetMaterialLibrary))
      (bind _output_get (Variables|Default|SetMID%20Frame _returnvalue_6))
      (Rendering|Material|SetVectorParameterValue _output_get "Color" "(R=0.310000,G=0.039188,B=0.024379,A=1.000000)" :!class /Script/Engine.MaterialInstanceDynamic))
    (:then_1
      (bind _returnvalue_7 (Rendering|Material|CreateDynamicMaterialInstance "/Game/ReusableAssets/Materials/MT_Opaque.MT_Opaque" :!class /Script/Engine.KismetMaterialLibrary))
      (bind _output_get_2 (Variables|Default|SetMID _returnvalue_7))
      (Rendering|Material|SetVectorParameterValue _output_get_2 "Color" "(R=0.350000,G=0.247370,B=0.192695,A=1.000000)" :!class /Script/Engine.MaterialInstanceDynamic))
    (:then_2
      (LocalVariables|SetSidebar%20Height (/ (- (.z (Variables|Default|GetBox%20Size)) (+ (Variables|Default|GetMargin%20Top) (Variables|Default|GetMargin%20Bottom))) 2.0))
      (LocalVariables|SetHalf%20Height (/ (.z (Variables|Default|GetBox%20Size)) 2.0)))
    (:then_3
      (bind _returnvalue_8 (AddComponent|AddProceduralMeshComponent true))
      (CallFunction|SetupBoxMesh _returnvalue_8 (Variables|Default|GetBox%20Size) (Variables|Default|GetMID) true)
      (Class|SceneComponent|Attachto _returnvalue_8 (Variables|Default|GetBox%20Container) "None" "KeepRelativeOffset" true))
    (:then_4
      ;[1 1 1] Top
      (bind _returnvalue_9 (AddComponent|AddProceduralMeshComponent true (Math|Transform|MakeTransform (Math|Vector|MakeVector (Class|TKMathFunctionLibrary|NegateFloat (/ (+ (.x _box_size_3) (Variables|Default|GetMargin%20Depth)) 2.0)) 0.0 (/ (- (.z _box_size_3) (Variables|Default|GetMargin%20Top)) 2.0)))))
      (CallFunction|SetupBoxMesh _returnvalue_9 (Math|Vector|MakeVector (Variables|Default|GetMargin%20Depth) (.y (Variables|Default|GetBox%20Size)) (Variables|Default|GetMargin%20Top)) (Variables|Default|GetMID%20Frame) true)
      (Class|SceneComponent|Attachto _returnvalue_9 (Variables|Default|GetBox%20Container) "None" "KeepRelativeOffset" true))
    (:then_5
      (bind _returnvalue_10 (AddComponent|AddProceduralMeshComponent true (Math|Transform|MakeTransform (Math|Vector|MakeVector (Class|TKMathFunctionLibrary|NegateFloat (/ (+ (.x _box_size_5) (Variables|Default|GetMargin%20Depth)) 2.0)) (/ (- (.y _box_size_5) (Variables|Default|GetMargin%20Width)) 2.0) (- (- (LocalVariables|GetHalf%20Height) (Variables|Default|GetMargin%20Top)) (LocalVariables|GetSidebar%20Height))))))
      (CallFunction|SetupBoxMesh _returnvalue_10 (Math|Vector|MakeVector (Variables|Default|GetMargin%20Depth) (Variables|Default|GetMargin%20Width) (- (.z (Variables|Default|GetBox%20Size)) (+ (Variables|Default|GetMargin%20Bottom) (Variables|Default|GetMargin%20Top)))) (Variables|Default|GetMID%20Frame) true)
      (Class|SceneComponent|Attachto _returnvalue_10 (Variables|Default|GetBox%20Container) "None" "KeepRelativeOffset" true))
    (:then_6
      (bind _returnvalue_11 (AddComponent|AddProceduralMeshComponent true (Math|Transform|MakeTransform (Math|Vector|MakeVector (Class|TKMathFunctionLibrary|NegateFloat (/ (+ (.x _box_size) (Variables|Default|GetMargin%20Depth)) 2.0)) (Class|TKMathFunctionLibrary|NegateFloat (/ (- (.y _box_size) (Variables|Default|GetMargin%20Width)) 2.0)) (- (- (LocalVariables|GetHalf%20Height) (Variables|Default|GetMargin%20Top)) (LocalVariables|GetSidebar%20Height))))))
      (CallFunction|SetupBoxMesh _returnvalue_11 (Math|Vector|MakeVector (Variables|Default|GetMargin%20Depth) (Variables|Default|GetMargin%20Width) (- (.z (Variables|Default|GetBox%20Size)) (+ (Variables|Default|GetMargin%20Bottom) (Variables|Default|GetMargin%20Top)))) (Variables|Default|GetMID%20Frame) true)
      (Class|SceneComponent|Attachto _returnvalue_11 (Variables|Default|GetBox%20Container) "None" "KeepRelativeOffset" true))
    (:then_7
      ;[1 1 1] Bottom
      (bind _returnvalue_12 (AddComponent|AddProceduralMeshComponent true (Math|Transform|MakeTransform (Math|Vector|MakeVector (Class|TKMathFunctionLibrary|NegateFloat (/ (+ (.x _box_size_2) (Variables|Default|GetMargin%20Depth)) 2.0)) 0.0 (Class|TKMathFunctionLibrary|NegateFloat (/ (- (.z _box_size_2) (Variables|Default|GetMargin%20Bottom)) 2.0))))))
      (CallFunction|SetupBoxMesh _returnvalue_12 (Math|Vector|MakeVector (Variables|Default|GetMargin%20Depth) (.y (Variables|Default|GetBox%20Size)) (Variables|Default|GetMargin%20Bottom)) (Variables|Default|GetMID%20Frame) true)
      (Class|SceneComponent|Attachto _returnvalue_12 (Variables|Default|GetBox%20Container) "None" "KeepRelativeOffset" true))
    (:then_9
      (Transformation|SetRelativeLocation (Variables|Default|GetBox%20Container) (Math|Vector|MakeVector (/ (.x (Variables|Default|GetBox%20Size)) 2.0) 0.0 0.0) false false))
    (:then_10
      (Transformation|SetRelativeLocation (Variables|Default|GetTitle) (Math|Vector|MakeVector _returnvalue_4 0.0 _returnvalue_5) false false))
    (:then_11
      (Transformation|SetRelativeLocation (Variables|Default|GetSubtitle) (Math|Vector|MakeVector _returnvalue_4 0.0 (- _returnvalue_5 6.0)) false false))))

(fn Setup
  (params (Use%20Defaults :type Boolean) (Box%20Size :type Vector) (Margin%20Depth :type Float%20%28single-precision%29) (Margin%20Top :type Float%20%28single-precision%29) (Margin%20Width :type Float%20%28single-precision%29) (Margin%20Bottom :type Float%20%28single-precision%29))
  (Utilities|FlowControl|Sequence
    (:then_0
      (if (not Use%20Defaults)
        (Variables|Default|SetBox%20Size Box%20Size)
        (Variables|Default|SetMargin%20Depth Margin%20Depth)
        (Variables|Default|SetMargin%20Top Margin%20Top)
        (Variables|Default|SetMargin%20Width Margin%20Width)
        (Variables|Default|SetMargin%20Bottom Margin%20Bottom)))
    (:then_3
      (CallFunction|BuildDisplayBox)
      (CallFunction|BuildCloseButton))))

(fn SetTitle
  (params (Title :type String) (Subtitle :type String))
  (Rendering|Components|TextRender|SetText (Variables|Default|GetTitle) (Utilities|Text|ToText(String) Title))
  (Rendering|Components|TextRender|SetText (Variables|Default|GetSubtitle) (Utilities|Text|ToText(String) Subtitle)))

(fn BuildCloseButton
  (bind _box_size (Variables|Default|GetBox%20Size))
  (bind _close_button_size (Variables|Default|GetClose%20Button%20Size))
  (bind (_x _y _z) (Math|Vector|BreakVector _close_button_size))
  (bind _returnvalue (AddComponent|AddChildActorComponent false (Math|Transform|MakeTransform (Math|Vector|MakeVector (Class|TKMathFunctionLibrary|NegateFloat (Variables|Default|GetMargin%20Depth)) (+ (Class|TKMathFunctionLibrary|NegateFloat (/ (.y _box_size) 2.0)) _y) (+ (- (/ (.z _box_size) 2.0) (Variables|Default|GetMargin%20Top)) _z)))))
  (bind _asbp_toggle_button (Utilities|Casting|CastToBP_ToggleButton (Variables|/Script/Engine.ChildActorComponent|GetChildActor _returnvalue)))
  (bind _output_get (Variables|Default|SetBack%20Toolbar%20Button _asbp_toggle_button))
  (Default|SetFontSize _output_get 5.0)
  (CallFunction|UpdateCloseButton "X")
  (Default|SetState _output_get false)
  (Rendering|SetVisibility (Variables|/Game/ReusableAssets/Buttons/BP_ToggleButton.BP_ToggleButton_C|GetRoot _output_get) false true)
  (CallFunction|ListentoCloseButton))

(fn ShowCloseButton
  (params (Show :type Boolean) (Button%20Text :type String))
  (Utilities|FlowControl|Sequence
    (:then_0
      (Rendering|SetVisibility (Variables|/Game/ReusableAssets/Buttons/BP_ToggleButton.BP_ToggleButton_C|GetRoot (Variables|Default|GetBack%20Toolbar%20Button)) Show true))
    (:then_2
      (if (not (== (Utilities|String|Len Button%20Text) 0))
        (CallFunction|UpdateCloseButton Button%20Text)))))

(fn UpdateCloseButton
  (params (Title :type String))
  (Default|SetTitleandSize (Variables|Default|GetBack%20Toolbar%20Button) (Variables|Default|GetClose%20Button%20Size) false Title "back"))