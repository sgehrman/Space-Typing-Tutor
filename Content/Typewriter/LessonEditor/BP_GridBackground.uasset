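; Grid background actor for the typewriter lesson editor: a procedurally built backing board with a raised rectangular frame.
; The construction script creates two dynamic instances of MT_Opaque, a board color and a darker frame color, both with zero roughness.
; It adds five procedural mesh components built by SetupBoxMesh with collision: the board plus four border bars on its -X face, sized from BoxSize, MarginWidth and MarginDepth.
; The event graph is unused.
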(event `self.ReceiveBeginPlay`)

(event `self.ReceiveActorBeginOverlap`
  (params (OtherActor :type "Actor Object Reference")))

(event `self.ReceiveTick`
  (params (DeltaSeconds :type "Float (single-precision)")))

(fn `UserConstructionScript`
  (bind (_box_size_x _box_size_y) (`KismetMathLibrary.BreakVector` (`self.Box Size`)))
  (bind (_box_size_x_2 _box_size_y_2 _box_size_z) (`KismetMathLibrary.BreakVector` (`self.Box Size`)))
  (bind (_box_size_x_3 _box_size_y_3 _box_size_z_2) (`KismetMathLibrary.BreakVector` (`self.Box Size`)))
  (bind (_box_size_x_4 _box_size_y_4) (`KismetMathLibrary.BreakVector` (`self.Box Size`)))
  (bind (_box_size_x_5 _box_size_y_5) (`KismetMathLibrary.BreakVector` (`self.Box Size`)))
  (bind (_box_size_x_6 _box_size_y_6 _box_size_z_3) (`KismetMathLibrary.BreakVector` (`self.Box Size`)))
  (bind (_box_size_x_7 _box_size_y_7 _box_size_z_4) (`KismetMathLibrary.BreakVector` (`self.Box Size`)))
  (bind (_box_size_x_8 _box_size_y_8) (`KismetMathLibrary.BreakVector` (`self.Box Size`)))
  (`|ExecutionSequence`
    (:`then_0`
      (bind _returnvalue (`KismetMaterialLibrary.CreateDynamicMaterialInstance` "/Game/ReusableAssets/Materials/MT_Opaque.MT_Opaque"))
      (bind _output_get (set `self.MID Frame` _returnvalue))
      (`MaterialInstanceDynamic.SetVectorParameterValue` _output_get "Color" (struct :`R` 0.31 :`G` 0.039188 :`B` 0.024379 :`A` 1.0))
      (`MaterialInstanceDynamic.SetScalarParameterValue` _output_get "Roughness" 0.0))
    (:`then_1`
      (bind _returnvalue_2 (`KismetMaterialLibrary.CreateDynamicMaterialInstance` "/Game/ReusableAssets/Materials/MT_Opaque.MT_Opaque"))
      (bind _output_get_2 (set `self.MID` _returnvalue_2))
      (`MaterialInstanceDynamic.SetVectorParameterValue` _output_get_2 "Color" (struct :`R` 0.35 :`G` 0.24737 :`B` 0.192695 :`A` 1.0))
      (`MaterialInstanceDynamic.SetScalarParameterValue` _output_get_2 "Roughness" 0.0))
    (:`then_3`
      (bind _returnvalue_3 (`AddComponent|ProceduralMeshComponent_0` :`RelativeTransform` (`/Game/ReusableAssets/Utilities/LIB_Utilities.Trans`)))
      (`/Game/ReusableAssets/Utilities/LIB_Utilities.Setup Box Mesh` _returnvalue_3 (`self.Box Size`) (`self.MID`) true))
    (:`then_4`
      ;[1 1 1] Top
      (bind _returnvalue_4 (`AddComponent|ProceduralMeshComponent_1` :`RelativeTransform` (`KismetMathLibrary.MakeTransform` (`KismetMathLibrary.MakeVector` (- (/ (+ _box_size_x_7 (`self.Margin Depth`)) 2.0)) 0.0 (/ (- _box_size_z_4 (`self.Margin Width`)) 2.0)))))
      (`/Game/ReusableAssets/Utilities/LIB_Utilities.Setup Box Mesh` _returnvalue_4 (`KismetMathLibrary.MakeVector` (`self.Margin Depth`) _box_size_y_8 (`self.Margin Width`)) (`self.MID Frame`) true))
    (:`then_5`
      (bind _returnvalue_5 (`AddComponent|ProceduralMeshComponent_2` :`RelativeTransform` (`KismetMathLibrary.MakeTransform` (`KismetMathLibrary.MakeVector` (- (/ (+ _box_size_x_5 (`self.Margin Depth`)) 2.0)) (/ (- _box_size_y_5 (`self.Margin Width`)) 2.0)))))
      (`/Game/ReusableAssets/Utilities/LIB_Utilities.Setup Box Mesh` _returnvalue_5 (`KismetMathLibrary.MakeVector` (`self.Margin Depth`) (`self.Margin Width`) (- _box_size_z_3 (* (`self.Margin Width`) 2.0))) (`self.MID Frame`) true))
    (:`then_6`
      (bind _returnvalue_6 (`AddComponent|ProceduralMeshComponent_3` :`RelativeTransform` (`KismetMathLibrary.MakeTransform` (`KismetMathLibrary.MakeVector` (- (/ (+ _box_size_x (`self.Margin Depth`)) 2.0)) (- (/ (- _box_size_y (`self.Margin Width`)) 2.0))))))
      (`/Game/ReusableAssets/Utilities/LIB_Utilities.Setup Box Mesh` _returnvalue_6 (`KismetMathLibrary.MakeVector` (`self.Margin Depth`) (`self.Margin Width`) (- _box_size_z (* (`self.Margin Width`) 2.0))) (`self.MID Frame`) true))
    (:`then_7`
      ;[1 1 1] Bottom
      (bind _returnvalue_7 (`AddComponent|ProceduralMeshComponent_4` :`RelativeTransform` (`KismetMathLibrary.MakeTransform` (`KismetMathLibrary.MakeVector` (- (/ (+ _box_size_x_3 (`self.Margin Depth`)) 2.0)) 0.0 (- (/ (- _box_size_z_2 (`self.Margin Width`)) 2.0))))))
      (`/Game/ReusableAssets/Utilities/LIB_Utilities.Setup Box Mesh` _returnvalue_7 (`KismetMathLibrary.MakeVector` (`self.Margin Depth`) _box_size_y_4 (`self.Margin Width`)) (`self.MID Frame`) true))))