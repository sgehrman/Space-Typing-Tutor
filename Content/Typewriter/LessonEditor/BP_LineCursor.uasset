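; BP_LineCursor is a cursor actor for the typewriter lesson editor, built as a procedural box mesh.
; Construction creates flickering, dimmed and hidden dynamic materials, which UpdateMaterial swaps between.
; Setup picks either a tall flickering bar or a small dimmed cube with auto-hide and tick enabled.
; MoveToLocation repositions it, lowering the dimmed variant and restarting the one-second timer after which Tick hides it.
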(event EventTick
  (params (DeltaSeconds :type Float%20%28single-precision%29))
  (if (Variables|Default|GetAuto%20Hide%20Enabled)
    (if (Variables|Default|GetCheck%20Auto%20Hide%20On%20Tick)
      (if (> (Math|Timespan|GetTotalSeconds (- (Math|DateTime|Now) (Variables|Default|GetHide%20Start%20Time))) 1.0)
        (Utilities|FlowControl|Sequence
          (:then_0
            (Variables|Default|SetCheck%20Auto%20Hide%20On%20Tick false))
          (:then_1
            (CallFunction|UpdateMaterial true)))))
    (else
      (CallFunction|Logg "Something's wrong"))))

(event EventBeginPlay
  ;[1 1 1] Enabled if needed in setup
  (Actor|Tick|SetActorTickEnabled false))

(fn ConstructionScript
  (Utilities|FlowControl|Sequence
    (:then_0
      (bind _returnvalue (Rendering|Material|CreateDynamicMaterialInstance "/Game/ReusableAssets/Materials/MT_Opaque.MT_Opaque" :!class /Script/Engine.KismetMaterialLibrary))
      (Variables|Default|SetMID%20Cursor _returnvalue)
      (Rendering|Material|SetScalarParameterValue _returnvalue "Emission" 1.0 :!class /Script/Engine.MaterialInstanceDynamic)
      (Rendering|Material|SetScalarParameterValue _returnvalue "Flicker Mode" 1.0 :!class /Script/Engine.MaterialInstanceDynamic)
      (Rendering|Material|SetScalarParameterValue _returnvalue "Flicker Speed" 1.0 :!class /Script/Engine.MaterialInstanceDynamic)
      (Rendering|Material|SetScalarParameterValue _returnvalue "Flicker Boost" 111.0 :!class /Script/Engine.MaterialInstanceDynamic))
    (:then_1
      (bind _returnvalue_2 (Rendering|Material|CreateDynamicMaterialInstance "/Game/ReusableAssets/Materials/MT_Transparent.MT_Transparent" :!class /Script/Engine.KismetMaterialLibrary))
      (Variables|Default|SetMID%20Dimmed%20Cursor _returnvalue_2)
      (Rendering|Material|SetScalarParameterValue _returnvalue_2 "Emission" 1.0 :!class /Script/Engine.MaterialInstanceDynamic)
      (Rendering|Material|SetVectorParameterValue _returnvalue_2 "EmissiveColor" "(R=1.000000,G=1.000000,B=1.000000,A=1.000000)" :!class /Script/Engine.MaterialInstanceDynamic)
      (Rendering|Material|SetScalarParameterValue _returnvalue_2 "Opacity" 0.1 :!class /Script/Engine.MaterialInstanceDynamic))
    (:then_2
      (bind _returnvalue_3 (Rendering|Material|CreateDynamicMaterialInstance "/Game/ReusableAssets/Materials/MT_Transparent.MT_Transparent" :!class /Script/Engine.KismetMaterialLibrary))
      (Variables|Default|SetMID%20Hidden%20Cursor _returnvalue_3)
      (Rendering|Material|SetScalarParameterValue _returnvalue_3 "Opacity" 0.0 :!class /Script/Engine.MaterialInstanceDynamic))))

(fn Setup
  (params (Dimmed :type Boolean))
  (Utilities|FlowControl|Sequence
    (:then_0
      (Variables|Default|SetDimmed Dimmed))
    (:then_2
      (bind _returnvalue (AddComponent|AddProceduralMeshComponent false))
      (bind _output_get (Variables|Default|SetCursor _returnvalue))
      (if (Variables|Default|GetDimmed)
        (CallFunction|SetupBoxMesh _output_get "4.000000,4.000000,4.000000" (Variables|Default|GetMID%20Cursor) false)
        (else
          (CallFunction|SetupBoxMesh _output_get "1.000000,1.000000,24.000000" (Variables|Default|GetMID%20Cursor) false))))
    (:then_3
      (bind _output_get_2 (Variables|Default|SetAuto%20Hide%20Enabled (Variables|Default|GetDimmed)))
      (if _output_get_2
        (Actor|Tick|SetActorTickEnabled true)
        (CallFunction|UpdateMaterial false)))))

(fn MovetoLocation
  (params (Location :type Vector))
  (Utilities|FlowControl|Sequence
    (:then_0
      (bind _output_get (LocalVariables|SetNew%20Location Location))
      (if (Variables|Default|GetDimmed)
        (LocalVariables|SetNew%20Location (+ _output_get "0, 0,-12.000000"))))
    (:then_1
      (Transformation|SetActorRelativeLocation (LocalVariables|GetNew%20Location))
      (if (Variables|Default|GetAuto%20Hide%20Enabled)
        (Variables|Default|SetHide%20Start%20Time (Math|DateTime|Now))
        (Variables|Default|SetCheck%20Auto%20Hide%20On%20Tick true)
        (CallFunction|UpdateMaterial false)))))

(fn UpdateMaterial
  (params (Hide :type Boolean))
  (Utilities|FlowControl|Sequence
    (:then_0
      (LocalVariables|SetMaterial (Variables|Default|GetMID%20Cursor)))
    (:then_1
      (if (Variables|Default|GetDimmed)
        (LocalVariables|SetMaterial (Variables|Default|GetMID%20Dimmed%20Cursor))))
    (:then_2
      (if Hide
        (LocalVariables|SetMaterial (Variables|Default|GetMID%20Hidden%20Cursor))))
    (:then_3
      (Rendering|Material|SetMaterial (Variables|Default|GetCursor) 0 (LocalVariables|GetMaterial)))))