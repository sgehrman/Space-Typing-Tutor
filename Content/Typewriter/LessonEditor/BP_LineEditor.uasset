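; BP_LineEditor is an in-world single-line text editor for the Typewriter lesson editor, built from BP_LineLetter child actors laid out by width.
; Key events insert or delete letters and move the insertion index, with Delete acting as Backspace and Enter signalling FinishedEditing.
; Two procedural box cursors mark positions: a dimmed one follows crosshair hovers, a bright one the insertion point.
; Letter state changes set that point before or after the hit letter.
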(event Custom|Listen%20to%20Letter
  (params (Letter :type BP%20Line%20Letter%20Object%20Reference))
  (EventDispatchers|BindEventtoStateChanged Letter (delegate Custom|State%20Change%20Event))
  (EventDispatchers|BindEventtoCrosshairMoved Letter (delegate Custom|CustomEvent_0)))

(event Custom|State%20Change%20Event
  (params (On%20State :type Boolean) (Index :type Integer) (Hit%20Location :type Vector))
  (if On%20State
    (bind _result_index (CallFunction|IndexforHitPosition Index Hit%20Location))
    (CallFunction|SetCursorIndex _result_index)))

(event Custom|CustomEvent_0
  (params (Hit%20Location :type Vector) (Index :type Integer))
  (bind _result_index (CallFunction|IndexforHitPosition Index Hit%20Location))
  (CallFunction|PositionCursor _result_index true))

(fn ConstructionScript
  (Utilities|FlowControl|Sequence
    (:then_0
      (bind _returnvalue (Rendering|Material|CreateDynamicMaterialInstance "/Game/ReusableAssets/Materials/MT_Opaque.MT_Opaque" :!class /Script/Engine.KismetMaterialLibrary))
      (Variables|Default|SetMID%20Cursor _returnvalue)
      (Rendering|Material|SetScalarParameterValue _returnvalue "Emission" 122.0 :!class /Script/Engine.MaterialInstanceDynamic))
    (:then_1
      (bind _returnvalue_2 (Rendering|Material|CreateDynamicMaterialInstance "/Game/ReusableAssets/Materials/MT_Transparent.MT_Transparent" :!class /Script/Engine.KismetMaterialLibrary))
      (Variables|Default|SetMID%20Dimmed%20Cursor _returnvalue_2)
      (Rendering|Material|SetScalarParameterValue _returnvalue_2 "Emission" 1.0 :!class /Script/Engine.MaterialInstanceDynamic)
      (Rendering|Material|SetVectorParameterValue _returnvalue_2 "EmissiveColor" "(R=1.000000,G=1.000000,B=1.000000,A=1.000000)" :!class /Script/Engine.MaterialInstanceDynamic)
      (Rendering|Material|SetScalarParameterValue _returnvalue_2 "Opacity" 0.1 :!class /Script/Engine.MaterialInstanceDynamic))
    (:then_2
      (bind _returnvalue_3 (AddComponent|AddProceduralMeshComponent false (CallFunction|Trans)))
      (bind _output_get (Variables|Default|SetCursor _returnvalue_3))
      (CallFunction|SetupBoxMesh _output_get (Variables|Default|GetCursor%20Size) (Variables|Default|GetMID%20Cursor) false))
    (:then_3
      (bind _returnvalue_4 (AddComponent|AddProceduralMeshComponent false (CallFunction|Trans)))
      (bind _output_get_2 (Variables|Default|SetDimmed%20Cursor _returnvalue_4))
      (CallFunction|SetupBoxMesh _output_get_2 (Variables|Default|GetCursor%20Size) (Variables|Default|GetMID%20Dimmed%20Cursor) false))))

(fn BuildSentence
  (params (Sentence :type String))
  (Utilities|FlowControl|Sequence
    (:then_0
      (for _array_element (Utilities|String|GetCharacterArrayfromString Sentence)
        (bind _letter (CallFunction|CreateLetter _array_element))
        (Utilities|Array|Add (Variables|Default|GetLetters) _letter)))
    (:then_1
      (CallFunction|LayoutLetters))))

(fn SetCursorIndex
  (params (Index :type Integer))
  (bind _output_get (Variables|Default|SetCursor%20Insert%20Index Index))
  (CallFunction|PositionCursor _output_get false))

(fn HandleKeyboardEvent
  (params (Character :type String) (Key%20Type :type E_KeyType%20Enum))
  (Utilities|FlowControl|Sequence
    (:then_3
      (switch Utilities|FlowControl|Switch|SwitchonE_KeyType Key%20Type
        (:NewEnumerator0
          (bind _letter (CallFunction|CreateLetter Character))
          (Utilities|Array|Insert (Variables|Default|GetLetters) _letter (Variables|Default|GetCursor%20Insert%20Index))
          (CallFunction|LayoutLetters)
          (CallFunction|SetCursorIndex (+ (Variables|Default|GetCursor%20Insert%20Index) 1)))
        (:NewEnumerator1
          (CallFunction|HandleDeleteKey :!label _label))
        (:NewEnumerator2
          (Default|CallFinishedEditing))
        (:NewEnumerator7
          (LocalVariables|SetArrow%20Increment -1)
          (bind _next_index (CallFunction|NextIndex (Variables|Default|GetCursor%20Insert%20Index) (+ (Utilities|Array|Length (Variables|Default|GetLetters)) 1) (LocalVariables|GetArrow%20Increment) true :!label _label_2))
          (CallFunction|SetCursorIndex _next_index))
        (:NewEnumerator8
          (LocalVariables|SetArrow%20Increment 1)
          (goto _label_2))
        (:NewEnumerator11
          (goto _label))))))

(fn LayoutLetters
  (Utilities|FlowControl|Sequence
    (:then_0
      (for (_array_element _array_index) (Variables|Default|GetLetters)
        (Default|UpdateIndex _array_element _array_index)
        (LocalVariables|SetY%20Offset (+ (LocalVariables|GetY%20Offset) (/ (Default|GetWidth _array_element) 2.0)))
        (Transformation|SetRelativeLocation (Variables|/Game/Typewriter/LessonEditor/BP_LineLetter.BP_LineLetter_C|GetScene _array_element) (Math|Vector|MakeVector 0.0 (LocalVariables|GetY%20Offset) 0.0) false)
        (LocalVariables|SetY%20Offset (+ (LocalVariables|GetY%20Offset) (/ (Default|GetWidth _array_element) 2.0)))))
    (:then_2
      (CallFunction|PositionCursor (Variables|Default|GetCursor%20Insert%20Index) false))))

(fn CreateLetter
  (params (Character :type String))
  (Utilities|FlowControl|Sequence
    (:then_0
      (bind _returnvalue (AddComponent|AddChildActorComponent true (CallFunction|Trans)))
      (Class|SceneComponent|Attachto _returnvalue (Variables|Default|GetLetters%20Container) "None" "KeepRelativeOffset" true)
      (bind _asbp_line_letter (Utilities|Casting|CastToBP_LineLetter (Variables|/Script/Engine.ChildActorComponent|GetChildActor _returnvalue)))
      (Default|Setup _asbp_line_letter Character)
      (LocalVariables|SetLetter%20Result _asbp_line_letter))
    (:then_1
      (CallFunction|ListentoLetter (LocalVariables|GetLetter%20Result)))
    (:then_2
      (return (LocalVariables|GetLetter%20Result)))))

(fn PositionCursor
  (params (Insert%20Index :type Integer) (Dimmed :type Boolean))
  (bind _location (CallFunction|CalcCursorPosition Insert%20Index))
  (if Dimmed
    (Transformation|SetRelativeLocation (Variables|Default|GetDimmed%20Cursor) (Math|Transform|InverseTransformLocation (Transformation|GetActorTransform) _location) false)
    (else
      (Transformation|SetRelativeLocation (Variables|Default|GetCursor) (Math|Transform|InverseTransformLocation (Transformation|GetActorTransform) _location) false))))

(fn HandleDeleteKey
  (if (> (Variables|Default|GetCursor%20Insert%20Index) 0)
    (Utilities|FlowControl|Sequence
      (:then_0
        (LocalVariables|SetDelete%20Index (- (Variables|Default|GetCursor%20Insert%20Index) 1)))
      (:then_1
        (Actor|DestroyActor (Utilities|Array|Get(acopy) (Variables|Default|GetLetters) (LocalVariables|GetDelete%20Index))))
      (:then_2
        (Utilities|Array|RemoveIndex (Variables|Default|GetLetters) (LocalVariables|GetDelete%20Index))
        (CallFunction|LayoutLetters))
      (:then_3
        (CallFunction|SetCursorIndex (Math|Integer|Max(Integer) (LocalVariables|GetDelete%20Index)))))))

(fn CalcCursorPosition
  (params (Insert%20Index :type Integer))
  (Utilities|FlowControl|Sequence
    (:then_0
      (LocalVariables|SetLocal%20Letter%20Index Insert%20Index)
      (LocalVariables|SetLocal%20Multiplier -1.0))
    (:then_1
      (if (== (LocalVariables|GetLocal%20Letter%20Index) (Utilities|Array|Length (Variables|Default|GetLetters)))
        (LocalVariables|SetLocal%20Letter%20Index (Utilities|Array|LastIndex (Variables|Default|GetLetters)))
        (LocalVariables|SetLocal%20Multiplier 1.0)))
    (:then_2
      (return (Math|Vector|MakeVector (- (.X (Math|Vector|BreakVector (Transformation|GetActorLocation (Utilities|Array|Get(acopy) (Variables|Default|GetLetters) (LocalVariables|GetLocal%20Letter%20Index))))) 12.0) (+ (.Y (Math|Vector|BreakVector (Transformation|GetActorLocation (Utilities|Array|Get(acopy) (Variables|Default|GetLetters) (LocalVariables|GetLocal%20Letter%20Index))))) (* (/ (Default|GetWidth (Utilities|Array|Get(acopy) (Variables|Default|GetLetters) (LocalVariables|GetLocal%20Letter%20Index))) 2.0) (LocalVariables|GetLocal%20Multiplier))) (.Z (Math|Vector|BreakVector (Transformation|GetActorLocation (Utilities|Array|Get(acopy) (Variables|Default|GetLetters) (LocalVariables|GetLocal%20Letter%20Index))))))))))

(fn IndexforHitPosition
  (params (Index :type Integer) (Hit%20Position :type Vector))
  (Utilities|FlowControl|Sequence
    (:then_0
      (LocalVariables|SetIndex%20Out Index))
    (:then_3
      (if (not (< (.Y (Math|Vector|BreakVector Hit%20Position)) 0.0))
        (LocalVariables|SetIndex%20Out (+ Index 1))))
    (:then_5
      (return (LocalVariables|GetIndex%20Out)))))