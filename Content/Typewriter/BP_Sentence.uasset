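; BP_Sentence is a typing-game actor that shows a sentence as a row of physical letters and checks typed characters against it.
; BuildSentence spawns one BP_SentenceLetter child actor per character, evenly spaced inside LetterContainer.
; IncrementCharacterOffset slides the container to the current letter and flags the end; ProcessTypedCharacter enables gravity on a matched letter.
; FadeoutSentence blasts the letters apart with physics, radial impulses and explosion effects, then destroys the actor after a delay.
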(event Custom|Destroy%20After%20Delay
  (Utilities|FlowControl|Delay 4.0)
  (Actor|DestroyActor))

(fn ConstructionScript)

(fn BuildSentence
  (params (Sentence :type String))
  (Utilities|FlowControl|Sequence
    (:then_0
      (CallFunction|DestroyChildComponents (Variables|Default|GetLetterContainer))
      (Utilities|Array|Clear (Variables|Default|GetLetter%20Array))
      (Utilities|Array|Clear (Variables|Default|GetLetter%20Component%20Array)))
    (:then_1
      (Variables|Default|SetSentence Sentence))
    (:then_2
      (CallFunction|IncrementCharacterOffset 0 true))
    (:then_3
      (for (_array_element _array_index) (Utilities|String|GetCharacterArrayfromString (Variables|Default|GetSentence))
        (bind _returnvalue (AddComponent|AddChildActorComponent true (Math|Transform|MakeTransform (Math|Vector|MakeVector 0.0 (* _array_index (Variables|Default|GetParam%20Item%20Width)) 0.0) "0, 0, 0" "2.000000,2.000000,2.000000")))
        (Utilities|FlowControl|Sequence
          (:then_0
            (Class|SceneComponent|Attachto _returnvalue (Variables|Default|GetLetterContainer) "None" "KeepRelativeOffset" true))
          (:then_1
            (bind _asbp_sentence_letter (Utilities|Casting|CastToBP_SentenceLetter (Variables|/Script/Engine.ChildActorComponent|GetChildActor _returnvalue)))
            (Utilities|Array|Add (Variables|Default|GetLetter%20Array) _asbp_sentence_letter)
            (Default|UpdateCharacter _asbp_sentence_letter _array_element))
          (:then_2
            (Utilities|Array|Add (Variables|Default|GetLetter%20Component%20Array) _returnvalue)))))))

(fn IncrementCharacterOffset
  (params (Offset :type Integer :default 0) (Reset :type Boolean :default false))
  (if Reset
    (Variables|Default|SetCharacter%20Offset 0)
    (else
      (Utilities|FlowControl|Sequence
        (:then_0
          (bind (_next_index _valid) (CallFunction|NextIndex (Variables|Default|GetCharacter%20Offset) (Utilities|Array|Length (Variables|Default|GetLetter%20Component%20Array)) Offset false))
          (bind _output_get (Variables|Default|SetCharacter%20Offset _next_index))
          (Variables|Default|SetReached%20End (and (> _output_get 0) (not _valid))))
        (:then_1
          (if (not (Variables|Default|GetReached%20End))
            (Transformation|SetRelativeLocation (Variables|Default|GetLetterContainer) (Math|Vector|MakeVector 0.0 (* (.y (Variables|/Script/Engine.SceneComponent|GetRelativeLocation (Utilities|Array|Get(acopy) (Variables|Default|GetLetter%20Component%20Array) (Variables|Default|GetCharacter%20Offset)))) -1.0) 0.0) false)))))))

(fn ProcessTypedCharacter
  (params (Character :type String))
  (bind _character_offset (Variables|Default|GetCharacter%20Offset))
  (bind _letter_array (Variables|Default|GetLetter%20Array))
  (bind _item (Utilities|Array|Get(acopy) _letter_array _character_offset))
  (Utilities|FlowControl|Sequence
    (:then_0
      (bind _matches (Default|DoesKeyMatch _item Character))
      (if _matches
        (Physics|SetEnableGravity _item true)
        (LocalVariables|SetResult true)))
    (:then_1
      (return (LocalVariables|GetResult)))))

(fn IsatEnd
  (return (Variables|Default|GetReached%20End)))

(fn FadeoutSentence
  (bind _root (Variables|Default|GetRoot))
  (Utilities|FlowControl|Sequence
    (:then_0
      (for _array_element (Variables|Default|GetLetter%20Array)
        (Physics|SetSimulatePhysics _array_element true))
      (for _array_element_2 (Variables|Default|GetLetter%20Array)
        (Class|RadialForceComponent|FireImpulse (Variables|Default|GetRadialForce))
        (Class|GameplayStatics|PlaySoundAttached "/Game/StarterContent/Audio/Explosion01.Explosion01" _root "None" "0, 0, 0" "KeepRelativeOffset" false 0.1 0.3)
        (Effects|SpawnEmitteratLocation "/Game/StarterContent/Particles/P_Explosion.P_Explosion" (Transformation|GetWorldLocation _root))))
    (:then_1
      (CallFunction|DestroyAfterDelay))))

(fn GetNextCharacter
  (Utilities|FlowControl|Sequence
    (:then_0
      (if (Utilities|Array|IsValidIndex (Variables|Default|GetLetter%20Array) (Variables|Default|GetCharacter%20Offset))
        (LocalVariables|SetResult%20Character (Variables|/Game/Typewriter/BP_SentenceLetter.BP_SentenceLetter_C|GetCharacter (Utilities|Array|Get(acopy) (Variables|Default|GetLetter%20Array) (Variables|Default|GetCharacter%20Offset))))
        (LocalVariables|SetResult%20Valid true)))
    (:then_1
      (return (LocalVariables|GetResult%20Valid) (LocalVariables|GetResult%20Character)))))

(fn GetWidth
  (return (* (Variables|Default|GetParam%20Item%20Width) (Math|Conversions|ToFloat(Integer) (Utilities|Array|Length (Variables|Default|GetLetter%20Array))))))