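; BP_SentenceLetter is a typewriter actor that displays a single character of a sentence and can be tested against a typed key.
; UpdateCharacter stores the character and writes it to a TextRender, while DoesKeyMatch compares a supplied character to the stored one.
; The construction script gives the static mesh a dynamic MT_Opaque material instance with zero roughness.
; The event graph is empty, so other code drives the letter through these functions.
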(event `self.ReceiveBeginPlay`)

(event `self.ReceiveActorBeginOverlap`
  (params (OtherActor :type "Actor Object Reference")))

(event `self.ReceiveTick`
  (params (DeltaSeconds :type "Float (single-precision)")))

(fn `DoesKeyMatch`
  (params (`Test Character` :type String))
  (returns (Matches :type Boolean))
  (return (`KismetStringLibrary.EqualEqual_StrStr` `Test Character` (`self.Character`))))

(fn `UpdateCharacter`
  (params (Character :type String))
  (bind _output_get (set `self.Character` Character))
  (`TextRenderComponent.K2_SetText` (`self.TextRender`) (`KismetTextLibrary.Conv_StringToText` _output_get)))

(fn `UserConstructionScript`
  (`|ExecutionSequence`
    (:`then_0`
      (bind _returnvalue (`KismetMaterialLibrary.CreateDynamicMaterialInstance` "/Game/ReusableAssets/Materials/MT_Opaque.MT_Opaque"))
      (bind _output_get (set `self.MID` _returnvalue))
      (`MaterialInstanceDynamic.SetScalarParameterValue` _output_get "Roughness" 0.0))
    (:`then_2`
      (`PrimitiveComponent.SetMaterial` (`self.StaticMesh`) 0 (`self.MID`)))))