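; Typewriter display actor that shows either a typing speed in words per minute or a running event count.
; In WPM mode, a looping two-second timer converts accumulated key-down events, at five characters per word, into a per-minute rate and resets the count.
; Otherwise, IncrementEventCount updates the same text.
; Setup sets title and mode; construction defaults to counter mode.
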(event `self.ReceiveBeginPlay`
  (if (`self.WPM Mode`)
    (`KismetSystemLibrary.K2_SetTimer` null "TimerFired" 2.0 true)))

(event `KeyDownEvent`
  (set `self.Character Count` (+ (`self.Character Count`) 1)))

(event `TimerFired`
  (`TextRenderComponent.K2_SetText` (`self.WPM`) (`KismetTextLibrary.Conv_StringToText` (`KismetStringLibrary.Conv_DoubleToString` (* (/ (`KismetMathLibrary.Conv_IntToDouble` (`self.Character Count`)) 5.0) 30.0))))
  (set `self.Character Count` 0))

(event `self.ReceiveActorBeginOverlap`
  (params (OtherActor :type "Actor Object Reference")))

(event `self.ReceiveTick`
  (params (DeltaSeconds :type "Float (single-precision)")))

(fn `Increment Event Count`
  (if (`self.WPM Mode`)
    (`/Game/ReusableAssets/Utilities/LIB_Utilities.Logg` "Wrong mode.  WPM mode")
    (else
      (bind _output_get (set `self.Event Count` (+ (`self.Event Count`) 1)))
      (`TextRenderComponent.K2_SetText` (`self.WPM`) (`KismetTextLibrary.Conv_IntToText` _output_get)))))

(fn `Setup`
  (params (Title :type String) (`WPM Mode` :type Boolean))
  (`TextRenderComponent.K2_SetText` (`self.Title`) (`KismetTextLibrary.Conv_StringToText` Title))
  (set `self.WPM Mode` `WPM Mode`))

(fn `UserConstructionScript`
  (`self.Setup` "Default"))