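; Leaderboard actor that displays online scores fetched through a DreamLo component it adds at BeginPlay.
; When the component signals a refresh, it spawns a BP_LeaderboardRow child actor per score, offset vertically by row height, without clearing earlier rows.
; In debug mode it logs the scores and spawns a button bar to refetch, clear or add dummy data.
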(event Custom|Button%20Clicked
  (params (Button%20ID :type String))
  (bind _dreamlo (Variables|Default|GetDreamLo))
  (switch string Button%20ID
    (:dump
      (Default|FetchJSON _dreamlo))
    (:clear
      (Default|ClearScores _dreamlo))
    (:build
      (Default|AddDummyData _dreamlo))))

(event Custom|Scores%20Refreshed
  (CallFunction|BuildLeaderboard)
  (if (Variables|Default|GetDebugging)
    (CallFunction|LogScores (CallFunction|GetScores))))

(event EventBeginPlay
  (Utilities|FlowControl|Sequence
    (:then_0
      (bind _returnvalue (AddComponent|AddBCDreamLoLeaderboard))
      (bind _output_get (Variables|Default|SetDreamLo _returnvalue))
      (EventDispatchers|BindEventtoScoresRefreshed _output_get (delegate Custom|Scores%20Refreshed)))
    (:then_1
      (Default|FetchJSON (Variables|Default|GetDreamLo)))
    (:then_3
      (if (Variables|Default|GetDebugging)
        (CallFunction|BuildDebugButtons)
        (EventDispatchers|BindEventtoButtonClicked (Variables|Default|GetButton%20Bar) (delegate Custom|Button%20Clicked))))))

(fn ConstructionScript)

(fn BuildDebugButtons
  (bind _returnvalue (AddComponent|AddChildActorComponent false (Math|Transform|MakeTransform (CallFunction|StandardLocation "0,100.000000, 0"))))
  (bind _asbp_button_bar (Utilities|Casting|CastToBP_ButtonBar (Variables|/Script/Engine.ChildActorComponent|GetChildActor _returnvalue)))
  (Variables|Default|SetButton%20Bar _asbp_button_bar)
  (Default|ReplaceButtons _asbp_button_bar (Utilities|Array|MakeArray (Utilities|Struct|MakeS_StringAndToken "Dump" "dump") (Utilities|Struct|MakeS_StringAndToken "Clear" "clear") (Utilities|Struct|MakeS_StringAndToken "Build" "build"))))

(fn LogScores
  (params (Scores :type Array%20of%20S%20Leader%20Score%20Structures))
  (CallFunction|ClearLogg)
  (for _array_element Scores
    (CallFunction|Logg (Utilities|String|Append "entry: " (.Name (Utilities|Struct|BreakS_LeaderScore _array_element)) ", s: " (Utilities|String|ToString(Float) (.Score (Utilities|Struct|BreakS_LeaderScore _array_element))) ", date: " (.Date (Utilities|Struct|BreakS_LeaderScore _array_element)) ", text: " (.Text (Utilities|Struct|BreakS_LeaderScore _array_element)) ", seconds: " (Utilities|String|ToString(Float) (.Seconds (Utilities|Struct|BreakS_LeaderScore _array_element)))))))

(fn BuildLeaderboard
  (for (_array_element _array_index) (CallFunction|GetScores)
    (bind _returnvalue (AddComponent|AddChildActorComponent false (Math|Transform|MakeTransform (Math|Vector|MakeVector 0.0 0.0 (* (Variables|Default|GetRow%20Height) (Math|Conversions|ToFloat(Integer) _array_index))))))
    (bind _asbp_leaderboard_row (Utilities|Casting|CastToBP_LeaderboardRow (Variables|/Script/Engine.ChildActorComponent|GetChildActor _returnvalue)))
    (Default|Setup _asbp_leaderboard_row _array_index (.Name (Utilities|Struct|BreakS_LeaderScore _array_element)) (.Score (Utilities|Struct|BreakS_LeaderScore _array_element)) (.Seconds (Utilities|Struct|BreakS_LeaderScore _array_element)))))

(fn GetScores
  (Utilities|FlowControl|Sequence
    (:then_0
      (Utilities|IsValid (Variables|Default|GetDreamLo)
        (:Is%20Valid
          (LocalVariables|SetResult (Default|GetScores (Variables|Default|GetDreamLo))))))
    (:then_1
      (return (LocalVariables|GetResult)))))