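; BP_KeyboardLessonsMap runs the typewriter lesson-selection menu map, streaming in a floor submap on BeginPlay.
; Once the PMM access component reports ready, it fades the screen, plays music, enables the crosshair, and spawns a grid pager and push-button child actors.
; A picked lesson loads the Typewriter level with its token.
; The buttons open the editor, credits or drills maps, or quit the game.
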(event `self.ReceiveBeginPlay`
  (`|ExecutionSequence`
    (:`then_0`
      (`GameplayStatics.LoadStreamLevel` "FloorSubmap" true))
    (:`then_1`
      (bind _returnvalue (`AddComponent|BC PMMAccess_0`))
      (add `/Game/ReusableAssets/Utilities/BC_PMMAccess.PMM Ready` _returnvalue (delegate `CustomEvent_0`))
      (`/Game/ReusableAssets/Utilities/BC_PMMAccess.Setup` _returnvalue))))

(event `CustomEvent_0`
  (params (Result :type "/Game/ReusableAssets/Utilities/BPI_PMM Interface"))
  (set `self.PLM` Result)
  (`|ExecutionSequence`
    (:`then_0`
      (`/Game/ReusableAssets/Utilities/LIB_Utilities.FadeOutScreen` true))
    (:`then_1`
      (`/Game/ReusableAssets/Utilities/BPI_PMM.Play Ambient Sound` (`self.PLM`) "/Game/Typewriter/LessonMap/SC_KeyboardLessonMusic.SC_KeyboardLessonMusic"))
    (:`then_2`
      (bind _returnvalue (`|SpawnActorFromClass` "/Game/Typewriter/LessonEditor/BP_GridItemPager.BP_GridItemPager_C" (`KismetMathLibrary.MakeTransform` (188.0 -75.0 0.0)) false self))
      (bind _output_get (set `self.Lesson Chooser` _returnvalue))
      (add `/Game/Typewriter/LessonEditor/BP_GridItemPager.Clicked Item` _output_get (delegate `Clicked Item`)))
    (:`then_3`
      (`/Game/ReusableAssets/Utilities/BPI_PMM.Enable Crosshair` (`self.PLM`) true false))
    (:`then_4`
      (`|ExecutionSequence`
        (:`then_0`
          (bind _returnvalue_2 (`AddComponent|Child Actor Component_8` :`RelativeTransform` (`KismetMathLibrary.MakeTransform` (200.0 75.0 44.0))))
          (bind _asbp_toggle_button (cast `/Game/ReusableAssets/Buttons/BP_ToggleButton` (`ChildActorComponent.ChildActor` _returnvalue_2)))
          (`/Game/ReusableAssets/Buttons/BP_ToggleButton.Set Title and Size` _asbp_toggle_button (`/Game/ReusableAssets/Utilities/LIB_Constants.Standard Button Size`) false "Edit" "edit")
          (`KismetArrayLibrary.Array_Add` (`self.Buttons`) _asbp_toggle_button))
        (:`then_1`
          (bind _returnvalue_3 (`AddComponent|ChildActorComponent_282` :`RelativeTransform` (`KismetMathLibrary.MakeTransform` (200.0 75.0 -22.0))))
          (bind _asbp_toggle_button_2 (cast `/Game/ReusableAssets/Buttons/BP_ToggleButton` (`ChildActorComponent.ChildActor` _returnvalue_3)))
          (`/Game/ReusableAssets/Buttons/BP_ToggleButton.Set Title and Size` _asbp_toggle_button_2 (`/Game/ReusableAssets/Utilities/LIB_Constants.Standard Button Size`) false "Quit" "quit")
          (`KismetArrayLibrary.Array_Add` (`self.Buttons`) _asbp_toggle_button_2))
        (:`then_2`
          (bind _returnvalue_4 (`AddComponent|ChildActorComponent_382` :`RelativeTransform` (`KismetMathLibrary.MakeTransform` (200.0 75.0 22.0))))
          (bind _asbp_toggle_button_3 (cast `/Game/ReusableAssets/Buttons/BP_ToggleButton` (`ChildActorComponent.ChildActor` _returnvalue_4)))
          (`/Game/ReusableAssets/Buttons/BP_ToggleButton.Set Title and Size` _asbp_toggle_button_3 (`/Game/ReusableAssets/Utilities/LIB_Constants.Standard Button Size`) false "Credits" "Credits")
          (`KismetArrayLibrary.Array_Add` (`self.Buttons`) _asbp_toggle_button_3))
        (:`then_4`
          (bind _returnvalue_5 (`AddComponent|ChildActorComponent_261` :`RelativeTransform` (`KismetMathLibrary.MakeTransform` (200.0 75.0 0.0))))
          (bind _asbp_toggle_button_4 (cast `/Game/ReusableAssets/Buttons/BP_ToggleButton` (`ChildActorComponent.ChildActor` _returnvalue_5)))
          (`/Game/ReusableAssets/Buttons/BP_ToggleButton.Set Title and Size` _asbp_toggle_button_4 (`/Game/ReusableAssets/Utilities/LIB_Constants.Standard Button Size`) false "Drills" "Drills")
          (`KismetArrayLibrary.Array_Add` (`self.Buttons`) _asbp_toggle_button_4))
        (:`then_5`
          (for _array_element (`self.Buttons`)
            (set `/Game/ReusableAssets/Buttons/BP_ToggleButton.Push Button Mode` true _array_element)
            (add `/Game/ReusableAssets/Buttons/BP_ToggleButton.ButtonClickedByUser` _array_element (delegate `click`))))))))

(event `Clicked Item`
  (params (String :type String) (`Data Token` :type String))
  (`/Game/ReusableAssets/Utilities/BPI_PMM.Load Level` (`self.PLM`) "Typewriter" `Data Token`))

(event `click`
  (params (`Button ID` :type String) (`Hit Location` :type "Vector Structure"))
  (switch `string` `Button ID`
    (:`quit`
      (`KismetSystemLibrary.QuitGame` (`GameplayStatics.GetPlayerController` 0) "Quit"))
    (:`edit`
      (`/Game/ReusableAssets/Utilities/BPI_PMM.Load Level` (`self.PLM`) "LessonEditorMap" ""))
    (:`credits`
      (`/Game/ReusableAssets/Utilities/BPI_PMM.Load Level` (`self.PLM`) "CreditsMap" ""))
    (:`Drills`
      (`/Game/ReusableAssets/Utilities/BPI_PMM.Load Level` (`self.PLM`) "SpeedTyperMap" ""))))

(fn `UserConstructionScript`)