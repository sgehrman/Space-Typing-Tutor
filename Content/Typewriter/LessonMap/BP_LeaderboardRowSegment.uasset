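; Leaderboard row segment for the lesson map: one cell with a background box and a text label.
; Setup stores the width, then BuildRow creates a procedural box mesh with the given material and adds a text render component.
; CreateTextRender places the label just off the box face, offset by alignment and margin.
; It builds an ellipsis-truncated string for long text but displays the original untruncated Text.
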(fn ConstructionScript)

(fn Setup
  (params (Name :type String) (Width :type Float%20%28single-precision%29) (Alignment :type EHorizontalAlignment%20Enum) (Material :type Material%20Interface%20Object%20Reference))
  (Utilities|FlowControl|Sequence
    (:then_2
      (Variables|Default|SetBackground%20Width Width))
    (:then_9
      (CallFunction|BuildRow Alignment Name Material))))

(fn BuildRow
  (params (Alignment :type EHorizontalAlignment%20Enum) (Name :type String) (Material :type Material%20Interface%20Object%20Reference))
  (Utilities|FlowControl|Sequence
    (:then_1
      (bind _returnvalue (AddComponent|AddProceduralMeshComponent false (Math|Transform|MakeTransform "0, 0, 0")))
      (bind _output_get (Variables|Default|SetBackgroundMesh _returnvalue))
      (CallFunction|SetupBoxMesh _output_get (Math|Vector|MakeVector (Variables|Default|GetBackground%20Depth) (Variables|Default|GetBackground%20Width) (Variables|Default|GetBackground%20Height)) Material false))
    (:then_2
      (CallFunction|CreateTextRender Name 12.0 Alignment))))

(fn CreateTextRender
  (params (Text :type String) (Text%20Size :type Float%20%28single-precision%29) (Alignment :type EHorizontalAlignment%20Enum))
  (Utilities|FlowControl|Sequence
    (:then_0
      (switch Utilities|FlowControl|Switch|SwitchonEHorizontalAlignment Alignment
        (:HAlign_Left
          (LocalVariables|SetAlign "EHTA_Left")
          (LocalVariables|SetYOffset (+ (Class|TKMathFunctionLibrary|NegateFloat (/ (Variables|Default|GetBackground%20Width) 2.0)) (LocalVariables|GetText%20Margin))))
        (:HAlign_Center
          (LocalVariables|SetAlign "EHTA_Center"))
        (:HAlign_Right
          (LocalVariables|SetAlign "EHTA_Right")
          (LocalVariables|SetYOffset (- (/ (Variables|Default|GetBackground%20Width) 2.0) (LocalVariables|GetText%20Margin))))))
    (:then_1
      (LocalVariables|SetLocation (Math|Vector|MakeVector (Class|TKMathFunctionLibrary|NegateFloat (+ (/ (Variables|Default|GetBackground%20Depth) 2.0) 1.0)) (LocalVariables|GetYOffset) 0.0)))
    (:then_2
      (LocalVariables|SetText%20String Text))
    (:then_4
      (if (> (Utilities|String|Len (LocalVariables|GetText%20String)) (Variables|Default|GetMax%20Character%20Count))
        (LocalVariables|SetText%20String (Class|VictoryBPFunctionLibrary|AppendMultiple (Utilities|String|GetSubstring (LocalVariables|GetText%20String) 0 (Variables|Default|GetMax%20Character%20Count)) "..."))))
    (:then_5
      (bind _returnvalue (AddComponent|AddTextRenderComponent false (Math|Transform|MakeTransform (LocalVariables|GetLocation))))
      (Rendering|Components|TextRender|SetText _returnvalue (Utilities|Text|ToText(String) Text))
      (Rendering|SetVisibility _returnvalue true false)
      (Rendering|Components|TextRender|SetWorldSize _returnvalue Text%20Size)
      (Rendering|Components|TextRender|SetHorizontalAlignment _returnvalue (LocalVariables|GetAlign))
      (Transformation|SetRelativeRotation _returnvalue "0.000000,180.000000,0.000000" false false)
      (Class|SystemUtils|SetTextRendersVerticalAlign _returnvalue))
    (:then_6
      (return _returnvalue))))