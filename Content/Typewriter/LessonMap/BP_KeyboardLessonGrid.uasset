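; Actor that lays out the typewriter lesson map as a three-column grid of BP_KeyboardLesson child actors, one per lesson.
; Setup stores the persistent map manager and triggers the layout, which reads the lesson count from the manager's lesson data.
; Each grid position gets a runtime-added child actor component, whose actor is stored in Lessons and initialized with the lesson's name, index and manager.
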(fn `Layout Lessons`
  (bind _lesson_data (`/Game/ReusableAssets/Utilities/BPI_PMM.Lesson Data` (`self.PLM`)))
  (bind _count (`/Game/Typewriter/BPI_LessonData.iLesson Count` _lesson_data))
  (for (_array_element _array_index) (`/Game/ReusableAssets/Utilities/LIB_Utilities.Positions In Grid` _count 3 1.0 (10.0 224.0 238.0))
    (bind _returnvalue (`AddComponent|Child Actor Component_746` :`RelativeTransform` (`KismetMathLibrary.MakeTransform` _array_element (struct :`Pitch` 90.0))))
    (bind _asbp_keyboard_lesson (cast `/Game/Typewriter/LessonMap/BP_KeyboardLesson` (`ChildActorComponent.ChildActor` _returnvalue)))
    (`KismetArrayLibrary.Array_Add` (`self.Lessons`) _asbp_keyboard_lesson)
    (bind _lesson_data_2 (`/Game/ReusableAssets/Utilities/BPI_PMM.Lesson Data` (`self.PLM`)))
    (bind _lesson (`/Game/Typewriter/BPI_LessonData.iLesson At Index` _lesson_data_2 _array_index))
    (`/Game/Typewriter/LessonMap/BP_KeyboardLesson.Setup` _asbp_keyboard_lesson (break `/Game/Typewriter/S_KeyboardLesson` _lesson) _array_index (`self.PLM`))))

(fn `Setup`
  (params (`Persistent Map Manager` :type "/Game/ReusableAssets/Utilities/BPI_PMM Interface"))
  (set `self.PLM` `Persistent Map Manager`)
  (`self.Layout Lessons`))

(fn `UserConstructionScript`)