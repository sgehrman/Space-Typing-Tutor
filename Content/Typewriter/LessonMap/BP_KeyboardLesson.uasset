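; BP_KeyboardLesson is a selectable lesson panel that loads the Typewriter level at its lesson index when clicked with the crosshair.
; Construction builds a procedural box behind the widget, sized to its draw size, with dynamic translucent normal and emissive-highlight materials.
; Setup receives the lesson name, index and persistent map manager, passing the name to the WBP_KeyboardLesson widget.
; Crosshair hover swaps the box material to show selection.
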(event `self.ReceiveBeginPlay`
  (`|ExecutionSequence`
    (:`then_1`
      (bind _aswbp_keyboard_lesson (cast `/Game/Typewriter/LessonMap/WBP_KeyboardLesson` (`WidgetComponent.GetUserWidgetObject` (`self.Widget`))))
      (set `self.Lesson Widget` _aswbp_keyboard_lesson))))

(fn `Crosshair Hover Moved`
  (params (`Hit Location` :type "Vector Structure"))
  (returns (Success :type Boolean))
  (return false))

(fn `Crosshair Hover Progress`
  (params (Progress :type "Float (double-precision)") (`Local Hit Location` :type "Vector Structure") (`Hit Component` :type "PrimitiveComponent Object Reference"))
  (returns (Success :type Boolean))
  (return true))

(fn `Crosshair Hover Start`
  (params (Finished :type Boolean))
  (returns (Success :type Boolean))
  (`|ExecutionSequence`
    (:`then_0`
      (if Finished
        (`PrimitiveComponent.SetMaterial` (`self.Background Mesh`) 0 (`self.Background MID`))
        (else
          (`PrimitiveComponent.SetMaterial` (`self.Background Mesh`) 0 (`self.Background MID Selected`)))))
    (:`then_1`
      (return true))))

(fn `Crosshair LeftRight`
  (params (Left :type Boolean))
  (returns (Success :type Boolean))
  (return false))

(fn `Crosshair Mouse Click`
  (params (`Mouse Down` :type Boolean) (`Event Type` :type "/Game/ReusableAssets/Utilities/E_EventType Enum" :default "NewEnumerator10") (`Hit Location` :type "Vector Structure") (`Hit Component` :type "PrimitiveComponent Object Reference"))
  (returns (Success :type Boolean))
  (`|ExecutionSequence`
    (:`then_0`
      (if `Mouse Down`
        (`/Game/ReusableAssets/Utilities/BPI_PMM.Load Level` (`self.PLM`) "Typewriter" (`self.Lesson Index`))))
    (:`then_1`
      (return true))))

(fn `Crosshair Scroll Wheel`
  (params (Down :type Boolean) (`Hit Location` :type "Vector Structure") (`Hit Component` :type "PrimitiveComponent Object Reference"))
  (returns (Success :type Boolean))
  (return false))

(fn `Crosshair UpDown`
  (params (Up :type Boolean))
  (returns (Success :type Boolean))
  (return false))

(fn `Setup`
  (params (`Level Name` :type String) (`Lesson Index` :type Integer) (`Persistent Map Manager` :type "/Game/ReusableAssets/Utilities/BPI_PMM Interface"))
  (bind _output_get (set `self.Lesson Name` `Level Name`))
  (set `self.Lesson Index` `Lesson Index`)
  (set `/Game/Typewriter/LessonMap/WBP_KeyboardLesson.Lesson Name` _output_get (`self.Lesson Widget`))
  (set `self.PLM` `Persistent Map Manager`))

(fn `UserConstructionScript`
  (bind (_returnvalue_x _returnvalue_y) (`KismetMathLibrary.BreakVector2D` (`WidgetComponent.GetDrawSize` (`self.Widget`))))
  (`|ExecutionSequence`
    (:`then_0`
      (bind _returnvalue (`KismetMaterialLibrary.CreateDynamicMaterialInstance` "/Game/ReusableAssets/Materials/MT_Transparent.MT_Transparent"))
      (bind _output_get (set `self.Background MID` _returnvalue))
      (`MaterialInstanceDynamic.SetVectorParameterValue` _output_get "Color" (struct :`A` 1.0))
      (`MaterialInstanceDynamic.SetScalarParameterValue` _output_get "Opacity" 0.4))
    (:`then_1`
      (bind _returnvalue_2 (`KismetMaterialLibrary.CreateDynamicMaterialInstance` "/Game/ReusableAssets/Materials/MT_Transparent.MT_Transparent"))
      (bind _output_get_2 (set `self.Background MID Selected` _returnvalue_2))
      (`MaterialInstanceDynamic.SetScalarParameterValue` _output_get_2 "Emission" 4.0)
      (`MaterialInstanceDynamic.SetVectorParameterValue` _output_get_2 "EmissiveColor" (struct :`B` 0.32 :`A` 1.0))
      (`MaterialInstanceDynamic.SetScalarParameterValue` _output_get_2 "Opacity" 0.3))
    (:`then_3`
      (bind _returnvalue_3 (`AddComponent|ProceduralMeshComponent_1` :`RelativeTransform` (`KismetMathLibrary.MakeTransform` (0.0 0.0 -11.0) (struct :`Pitch` 90.0) (1.0 1.0 1.0))))
      (set `self.Background Mesh` _returnvalue_3)
      (bind (_vertices _triangles _normals _uvs _tangents) (`KismetProceduralMeshLibrary.GenerateBoxMesh` (/ (`KismetMathLibrary.MakeVector` 1.0 _returnvalue_x _returnvalue_y) 2.0)))
      (`ProceduralMeshComponent.CreateMeshSection` :`self` _returnvalue_3 :`Vertices` _vertices :`Triangles` _triangles :`Normals` _normals :`UV0` _uvs :`Tangents` _tangents))
    (:`then_5`
      (`PrimitiveComponent.SetMaterial` (`self.Background Mesh`) 0 (`self.Background MID`)))))