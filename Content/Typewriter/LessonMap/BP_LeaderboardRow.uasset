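; Leaderboard row actor for the typewriter lesson map, built from four side-by-side segment child actors.
; Construction defines fixed column widths and spacing and totals them for GetWidth.
; Setup creates two colored dynamic materials, picks one by index parity for alternating stripes, then builds the row from the passed fields.
; Each segment is spawned along Y with its text, width, material and left or right alignment.
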(fn ConstructionScript
  (bind _segment_widths (Variables|Default|GetSegment%20Widths))
  (Utilities|FlowControl|Sequence
    (:then_0
      (Variables|Default|SetSegment%20Space 4.0))
    (:then_1
      (Utilities|Array|Add _segment_widths 2e+01))
    (:then_2
      (Utilities|Array|Add _segment_widths 8e+01))
    (:then_3
      (Utilities|Array|Add _segment_widths 4e+01))
    (:then_4
      (Utilities|Array|Add _segment_widths 4e+01))
    (:then_6
      (for _array_element (Variables|Default|GetSegment%20Widths)
        (Variables|Default|SetTotal%20Width (+ (Variables|Default|GetTotal%20Width) _array_element))))
    (:then_7
      (Variables|Default|SetTotal%20Width (+ (Variables|Default|GetTotal%20Width) (* (- (Utilities|Array|Length (Variables|Default|GetSegment%20Widths)) 1) (Variables|Default|GetSegment%20Space)))))))

(fn Setup
  (params (Index :type Integer) (Fields :type Array%20of%20Strings))
  (Utilities|FlowControl|Sequence
    (:then_1
      (bind _returnvalue (Rendering|Material|CreateDynamicMaterialInstance "/Game/ReusableAssets/Materials/MT_Opaque.MT_Opaque" :!class /Script/Engine.KismetMaterialLibrary))
      (bind _output_get (Variables|Default|SetMID%20Background _returnvalue))
      (Rendering|Material|SetScalarParameterValue _output_get "Opacity" 1.0 :!class /Script/Engine.MaterialInstanceDynamic)
      (Rendering|Material|SetVectorParameterValue _output_get "Color" "(R=0.063676,G=0.212754,B=0.555000,A=1.000000)" :!class /Script/Engine.MaterialInstanceDynamic))
    (:then_2
      (bind _returnvalue_2 (Rendering|Material|CreateDynamicMaterialInstance "/Game/ReusableAssets/Materials/MT_Opaque.MT_Opaque" :!class /Script/Engine.KismetMaterialLibrary))
      (bind _output_get_2 (Variables|Default|SetMID%20Alt%20Background _returnvalue_2))
      (Rendering|Material|SetScalarParameterValue _output_get_2 "Opacity" 1.0 :!class /Script/Engine.MaterialInstanceDynamic)
      (Rendering|Material|SetVectorParameterValue _output_get_2 "Color" "(R=0.082369,G=0.480464,B=0.555000,A=1.000000)" :!class /Script/Engine.MaterialInstanceDynamic))
    (:then_3
      (if (== (Math|Integer|%(Integer) Index 2) 0)
        (Variables|Default|SetMaterial (Variables|Default|GetMID%20Background))
        (else
          (Variables|Default|SetMaterial (Variables|Default|GetMID%20Alt%20Background)))))
    (:then_4
      (CallFunction|BuildRow Fields))))

(fn BuildRow
  (params (Fields :type Array%20of%20Strings))
  (bind _segment_widths (Variables|Default|GetSegment%20Widths))
  (Utilities|FlowControl|Sequence
    (:then_0
      (LocalVariables|SetWidth (Utilities|Array|Get(acopy) _segment_widths))
      (bind _out__yoffset (CallFunction|BuildSegment (LocalVariables|GetYOffset) (LocalVariables|GetWidth) (Utilities|Array|Get(acopy) Fields) "HAlign_Left"))
      (LocalVariables|SetYOffset _out__yoffset))
    (:then_1
      (LocalVariables|SetWidth (Utilities|Array|Get(acopy) _segment_widths 1))
      (bind _out__yoffset_2 (CallFunction|BuildSegment (LocalVariables|GetYOffset) (LocalVariables|GetWidth) (Utilities|Array|Get(acopy) Fields 1) "HAlign_Left"))
      (LocalVariables|SetYOffset _out__yoffset_2))
    (:then_2
      (LocalVariables|SetWidth (Utilities|Array|Get(acopy) _segment_widths 2))
      (bind _out__yoffset_3 (CallFunction|BuildSegment (LocalVariables|GetYOffset) (LocalVariables|GetWidth) (Utilities|Array|Get(acopy) Fields 2) "HAlign_Right"))
      (LocalVariables|SetYOffset _out__yoffset_3))
    (:then_3
      (LocalVariables|SetWidth (Utilities|Array|Get(acopy) _segment_widths 3))
      (bind _out__yoffset_4 (CallFunction|BuildSegment (LocalVariables|GetYOffset) (LocalVariables|GetWidth) (Utilities|Array|Get(acopy) Fields 3) "HAlign_Right"))
      (LocalVariables|SetYOffset _out__yoffset_4))))

(fn BuildSegment
  (params (YOffset :type Float%20%28single-precision%29) (Width :type Float%20%28single-precision%29) (Name :type String) (Alignment :type EHorizontalAlignment%20Enum))
  (Utilities|FlowControl|Sequence
    (:then_0
      (LocalVariables|SetResult YOffset))
    (:then_1
      (bind _returnvalue (AddComponent|AddChildActorComponent false (Math|Transform|MakeTransform (Math|Vector|MakeVector 0.0 (+ YOffset (/ Width 2.0)) 0.0))))
      (bind _asbp_leaderboard_row_segment (Utilities|Casting|CastToBP_LeaderboardRowSegment (Variables|/Script/Engine.ChildActorComponent|GetChildActor _returnvalue)))
      (Default|Setup _asbp_leaderboard_row_segment Name Width Alignment (Variables|Default|GetMaterial))
      (LocalVariables|SetResult (+ YOffset Width (Variables|Default|GetSegment%20Space))))
    (:then_2
      (return (LocalVariables|GetResult)))))

(fn GetWidth
  (return (Variables|Default|GetTotal%20Width)))