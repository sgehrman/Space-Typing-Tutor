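; Typing-lesson game actor that spawns each level's sentences as stacked child actors and checks typed characters against the front sentence.
; Levels come from PLM's current lesson, while the construction script uses built-in test sentences to avoid file reads.
; Correct and wrong keys flash the pyramid pointer; finished sentences fade out and the remaining rows animate into place.
; Countdown, LED stopwatch and level-completed actors drive level progression until the lesson finishes.
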(event Custom|ThreeTwoOne%20Animation%20Done
  (Variables|Default|SetGame%20Playing true)
  (Audio|PlaySoundatLocation "/Game/Typewriter/StartBeep.StartBeep" "0, 0, 0")
  (Default|StartStopwatch (Variables|Default|GetLED%20Timer%20Sign)))

(event Custom|Load%20Next%20Level
  (Default|PauseStopwatch (Variables|Default|GetLED%20Timer%20Sign))
  (Rendering|SetVisibility false true)
  (bind _returnvalue (Game|SpawnActorfromClass "/Game/Typewriter/BP_LevelCompleted.BP_LevelCompleted_C" (Math|Transform|MakeTransform "0, 0, 0") true self 0))
  (Default|LevelCompleted _returnvalue (Variables|Default|GetCurrent%20Level))
  (EventDispatchers|BindEventtoContinueAfterLevelComplete _returnvalue (delegate Custom|Continue%20After%20Complete)))

(event Custom|CountDownGo
  (bind _returnvalue (Game|SpawnActorfromClass "/Game/ReusableAssets/MessageBox/BP_ThreeTwoOne.BP_ThreeTwoOne_C" (Math|Transform|MakeTransform (Transformation|GetActorLocation (Game|Player|GetPlayerPawn 0)) "0, 0,0.000000") false self 0))
  (EventDispatchers|BindEventtoAnimationDone _returnvalue (delegate Custom|ThreeTwoOne%20Animation%20Done))
  (Default|Start _returnvalue (Utilities|Text|ToText(String) (Class|VictoryBPFunctionLibrary|AppendMultiple "Lesson: " (Variables|Default|GetLesson%20Name))) (Utilities|Text|ToText(String) (Class|VictoryBPFunctionLibrary|AppendMultiple "Level" " " (Utilities|String|ToString(Integer) (+ (Variables|Default|GetCurrent%20Level) 1)) "/" (Utilities|String|ToString(Integer) (Utilities|Array|Length (Variables|Default|GetLevels))))))
  (Default|AnimateandDestroy _returnvalue))

(event Custom|CustomEvent_0
  (params (Result :type BPI%20PMM%20Interface))
  (Variables|Default|SetPLM Result))

(event Custom|Continue%20After%20Complete
  (CallFunction|LoadUpLevel (+ (Variables|Default|GetCurrent%20Level) 1) true))

(event Custom|Load%20Up%20Level
  (params (Level%20Index :type Integer) (Start%20Count%20Down :type Boolean))
  (bind _returnvalue (Transformation|GetActorLocation))
  (if (!= Level%20Index (Variables|Default|GetCurrent%20Level))
    (Variables|Default|SetCurrent%20Level Level%20Index)
    (Utilities|FlowControl|Delay 0.5)
    (bind _success (CallFunction|BuildSentences false))
    (if _success
      (Utilities|FlowControl|Sequence
        (:then_0
          (Rendering|SetVisibility true true))
        (:then_1
          (CallFunction|AnimatetoLocation self (+ _returnvalue "0, 0,1111.000000") _returnvalue 0 1.0 false false false))
        (:then_2
          (Variables|Default|SetGame%20Playing false)
          (Default|CallStateChangeEvent))
        (:then_3
          (if Start%20Count%20Down
            (CallFunction|CountDownGo))))
      (else
        (Default|CallLessonFinished)))))

(event EventBeginPlay
  (Utilities|FlowControl|Sequence
    (:then_0
      (Utilities|Array|Clear (Variables|Default|GetLevels))
      (CallFunction|DestroyExistingSentences))
    (:then_1
      (bind _asbp_ledsign (Utilities|Casting|CastToBP_LEDSign (.Actor (CallFunction|FindActorwithTag "/Game/ReusableAssets/LEDBoard/BP_LEDSign.BP_LEDSign_C" "None" self))))
      (Variables|Default|SetLED%20Timer%20Sign _asbp_ledsign))
    (:then_2
      (bind _returnvalue (AddComponent|AddBCPMMAccess))
      (EventDispatchers|BindEventtoPMMReady _returnvalue (delegate Custom|CustomEvent_0))
      (Default|Setup _returnvalue))))

(fn ConstructionScript
  (Utilities|FlowControl|Sequence
    (:then_0
      (bind _asbp_pyramid_pointer (Utilities|Casting|CastToBP_PyramidPointer (Variables|/Script/Engine.ChildActorComponent|GetChildActor (Variables|Default|GetPyramid%20Component))))
      (Variables|Default|SetPyramid _asbp_pyramid_pointer))
    (:then_1
      (CallFunction|BuildSentences true))))

(fn ProcessTypedCharacter
  (params (Character :type String) (Key%20Type :type E_KeyType%20Enum))
  (bind _bp_sentences (Variables|Default|GetBP%20Sentences))
  (bind _bp_sentences_2 (Variables|Default|GetBP%20Sentences))
  (bind _pyramid (Variables|Default|GetPyramid))
  (bind _item (Utilities|Array|Get(acopy) _bp_sentences))
  (bind _item_2 (Utilities|Array|Get(acopy) _bp_sentences_2))
  (Utilities|FlowControl|Sequence
    (:then_0
      (if (Variables|Default|GetGame%20Playing)
        (Utilities|FlowControl|Sequence
          (:then_0
            (switch Utilities|FlowControl|Switch|SwitchonE_KeyType Key%20Type
              (:NewEnumerator0
                (bind _success (Default|ProcessTypedCharacter _item Character))
                (bind _output_get (LocalVariables|SetResult%20Success _success))
                (if _output_get
                  (Default|IncrementCharacterOffset _item 1 false)
                  (Default|FlashCorrect _pyramid)
                  (else
                    (Audio|PlaySoundatLocation "/Game/UserInterfaceSFX/Cancel/cancel_error02_Cue.cancel_error02_Cue" "0, 0, 0")
                    (Default|FlashError _pyramid))))
              (:NewEnumerator1
                (Default|IncrementCharacterOffset _item -1 false))
              (:NewEnumerator3
                ;[1 1 1] Debug only
                (CallFunction|LoadNextLevel))))
          (:then_1
            ;[1 1 1] If done with sentence, kill it
            (bind _result (Default|IsatEnd _item_2))
            (if _result
              (Default|FadeoutSentence _item_2)
              (LocalVariables|SetLine%20was%20deleted true)
              (Utilities|Array|RemoveIndex (Variables|Default|GetBP%20Sentences))
              (Utilities|Array|RemoveIndex (Variables|Default|GetSentenceActors))))
          (:then_2
            (if (LocalVariables|GetLine%20was%20deleted)
              (if (== (Utilities|Array|Length (Variables|Default|GetSentenceActors)) 0)
                (CallFunction|LoadNextLevel)
                (else
                  (CallFunction|LayoutSentences true)))))
          (:then_3
            (Default|CallStateChangeEvent)))))
    (:then_1
      (return (LocalVariables|GetResult%20Success)))))

(fn BuildSentences
  (params (Construction :type Boolean))
  (Utilities|FlowControl|Sequence
    (:then_0
      (bind (_is_valid _strings) (CallFunction|NextLevelStrings Construction))
      (if _is_valid
        (LocalVariables|SetSuccess%20Result true)
        (Variables|Default|SetSentences _strings)
        (CallFunction|BuildSentenceRows)
        (CallFunction|LayoutSentences false)))
    (:then_3
      (return (LocalVariables|GetSuccess%20Result)))))

(fn BuildSentenceRows
  (CallFunction|DestroyExistingSentences)
  (for _array_element (Variables|Default|GetSentences)
    (bind _returnvalue (AddComponent|AddChildActorComponent false (Math|Transform|MakeTransform (Math|Vector|MakeVector 0.0 0.0 0.0))))
    (Utilities|Array|Add (Variables|Default|GetSentenceActors) _returnvalue)
    (bind _asbp_sentence (Utilities|Casting|CastToBP_Sentence (Variables|/Script/Engine.ChildActorComponent|GetChildActor _returnvalue)))
    (Utilities|Array|Add (Variables|Default|GetBP%20Sentences) _asbp_sentence)
    (Default|BuildSentence _asbp_sentence _array_element))
  (return))

(fn NextLevelStrings
  (params (Construction :type Boolean))
  (CallFunction|LoadLevels Construction)
  (Utilities|FlowControl|Sequence
    (:then_0
      (if (Utilities|Array|IsValidIndex (Variables|Default|GetLevels) (Variables|Default|GetCurrent%20Level))
        (LocalVariables|SetStrings%20Result (.Sentences (Utilities|Struct|BreakS_KeyboardLessonLevel (Utilities|Array|Get(acopy) (Variables|Default|GetLevels) (Variables|Default|GetCurrent%20Level)))))
        (LocalVariables|SetValid%20Result true)))
    (:then_1
      (return (LocalVariables|GetValid%20Result) (LocalVariables|GetStrings%20Result)))))

(fn GetNextCharacter
  (Utilities|FlowControl|Sequence
    (:then_0
      (if (Utilities|Array|IsValidIndex (Variables|Default|GetBP%20Sentences))
        (bind (_valid _character) (Default|GetNextCharacter (Utilities|Array|Get(acopy) (Variables|Default|GetBP%20Sentences))))
        (LocalVariables|SetResult%20Character _character)
        (LocalVariables|SetResult%20Valid _valid)))
    (:then_2
      (return (LocalVariables|GetResult%20Valid) (LocalVariables|GetResult%20Character)))))

(fn LayoutSentences
  (params (Animate :type Boolean))
  (for (_array_element _array_index) (Variables|Default|GetSentenceActors)
    (Utilities|FlowControl|Sequence
      (:then_0
        (bind _asbp_sentence (Utilities|Casting|CastToBP_Sentence (Variables|/Script/Engine.ChildActorComponent|GetChildActor _array_element)))
        (bind _width (Default|GetWidth _asbp_sentence))
        (LocalVariables|SetMax%20Width (Math|Float|Max(Float) (LocalVariables|GetMax%20Width) _width)))
      (:then_1
        (LocalVariables|SetZOffset (* _array_index (Variables|Default|GetParam%20Sentence%20Height)))
        (if (> _array_index 0)
          (LocalVariables|SetZOffset (+ (LocalVariables|GetZOffset) (Variables|Default|GetParam%20Sentence%20Height))))
        (if Animate
          (CallFunction|AnimatetoLocation (Variables|/Script/Engine.ChildActorComponent|GetChildActor _array_element) (Variables|/Script/Engine.SceneComponent|GetRelativeLocation (VehicleSound|GetRootComponent (Variables|/Script/Engine.ChildActorComponent|GetChildActor _array_element))) (Math|Vector|MakeVector 0.0 0.0 (LocalVariables|GetZOffset)) 0 5.0 false false true)
          (else
            (Transformation|SetActorRelativeLocation (Variables|/Script/Engine.ChildActorComponent|GetChildActor _array_element) (Math|Vector|MakeVector 0.0 0.0 (LocalVariables|GetZOffset))))))))
  (bind _asbp_spotlightbar (Utilities|Casting|CastToBP_Spotlightbar (Variables|/Script/Engine.ChildActorComponent|GetChildActor (Variables|Default|GetLightbar))))
  (Default|LayoutLights _asbp_spotlightbar "0,-222.000000, 0" "0,222.000000, 0" (Math|Float|Ceil (/ (+ (LocalVariables|GetMax%20Width) 222.0) 222.0))))

(fn LoadLevels
  (params (Construction :type Boolean))
  (if (== (Utilities|Array|Length (Variables|Default|GetLevels)) 0)
    (if Construction
      ;[1 1 1] Data for the contruction script.  Faster than reading a file
      (Utilities|Array|Add (Variables|Default|GetLevels) (Utilities|Struct|MakeS_KeyboardLessonLevel (Utilities|Array|MakeArray "This is test data for the constructor." "It's faster than reading a file!" "No big deal.")))
      (else
        (bind _lesson (Default|CurrentLesson (Variables|Default|GetPLM)))
        (Utilities|Array|AppendArray (Variables|Default|GetLevels) (.levels _lesson))
        (Variables|Default|SetLesson%20Name (.name _lesson))))))

(fn DestroyExistingSentences
  (for _array_element (Variables|Default|GetSentenceActors)
    (Components|DestroyComponent _array_element))
  (Utilities|Array|Clear (Variables|Default|GetSentenceActors))
  (Utilities|Array|Clear (Variables|Default|GetBP%20Sentences)))