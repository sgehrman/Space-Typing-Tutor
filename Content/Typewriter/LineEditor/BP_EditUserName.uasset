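; BP_EditUserName is an actor that opens a typewriter-style line editor for editing a user name, currently prefilled with a hardcoded test name.
; After a short delay on BeginPlay, ShowEditor spawns BP_Typewriter and BP_LineEditor as child actor components and seeds the editor with the text and a data token.
; The editor's finished-editing event returns the result, which is only logged.
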(event `self.ReceiveBeginPlay`
  (`KismetSystemLibrary.Delay` 2.0)
  (`self.Show Editor` "Steve")
  (add `/Game/Typewriter/LineEditor/BP_LineEditor.Finished Editing` (`self.Editor Line`) (delegate `Finished Editing`)))

(event `Finished Editing`
  (params (String :type String) (`Data Token` :type String))
  (`/Game/ReusableAssets/Utilities/LIB_Utilities.Logg` String))

(fn `Show Editor`
  (params (String :type String) (Token :type String))
  (`|ExecutionSequence`
    (:`then_0`
      (bind _returnvalue (`AddComponent|ChildActorComponent_1647` :`RelativeTransform` (`/Game/ReusableAssets/Utilities/LIB_Constants.Keyboard Transform`)))
      (bind _asbp_typewriter (cast `/Game/ReusableAssets/Keyboard/BP_Typewriter` (`ChildActorComponent.ChildActor` _returnvalue)))
      (set `self.Keyboard` _asbp_typewriter))
    (:`then_1`
      (bind _returnvalue_2 (`AddComponent|ChildActorComponent_1648`))
      (bind _asbp_line_editor (cast `/Game/Typewriter/LineEditor/BP_LineEditor` (`ChildActorComponent.ChildActor` _returnvalue_2)))
      (bind _output_get (set `self.Editor Line` _asbp_line_editor))
      (`/Game/Typewriter/LineEditor/BP_LineEditor.Setup Editor` _output_get String Token))))

(fn `UserConstructionScript`)