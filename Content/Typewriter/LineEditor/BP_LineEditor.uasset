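; In-world single-line text editor for the typewriter, built from per-character BP_LineLetter child actors.
; Keyboard events insert, delete and step the cursor; Enter sends the joined string and data token to the finished-editing callback.
; Each letter reports crosshair hover and state changes, moving a preview cursor or setting the insert cursor on the nearer side.
; Tick interpolates the letters container to keep the line centered on the cursor.
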(event Custom|Listen%20to%20Letter
  (params (Letter :type BP%20Line%20Letter%20Object%20Reference))
  (EventDispatchers|BindEventtoStateChanged Letter (delegate Custom|State%20Change%20Event))
  (EventDispatchers|BindEventtoCrosshairMoved Letter (delegate Custom|CustomEvent_0)))

(event Custom|State%20Change%20Event
  (params (On%20State :type Boolean) (Index :type Integer) (Hit%20Location :type Vector))
  (if On%20State
    (bind _result_index (CallFunction|IndexforHitPosition Index Hit%20Location))
    (CallFunction|SetCursorIndex _result_index)))

(event Custom|CustomEvent_0
  (params (Hit%20Location :type Vector) (Index :type Integer))
  (bind _result_index (CallFunction|IndexforHitPosition Index Hit%20Location))
  (CallFunction|PositionCursor _result_index true))

(event EventTick
  (params (DeltaSeconds :type Float%20%28single-precision%29))
  (bind _letters_container (Variables|Default|GetLetters%20Container))
  (bind _relativelocation (Variables|/Script/Engine.SceneComponent|GetRelativeLocation _letters_container))
  (bind (_x _y _z) (Math|Vector|BreakVector _relativelocation))
  ;[1 1 1] Center line on cursor location
  (Transformation|SetRelativeLocation (Variables|Default|GetLetters%20Container) (Math|Interpolation|VInterpTo (Variables|/Script/Engine.SceneComponent|GetRelativeLocation (Variables|Default|GetLetters%20Container)) (Math|Vector|MakeVector _x (Class|TKMathFunctionLibrary|NegateFloat (.Y (Math|Vector|BreakVector (.location (Transformation|GetRelativeTransform (Variables|/Game/Typewriter/LineEditor/BP_LineCursor.BP_LineCursor_C|GetDefaultSceneRoot (Variables|Default|GetNormal%20Cursor))))))) _z) DeltaSeconds 5.0) false false))

(fn ConstructionScript
  (Utilities|FlowControl|Sequence
    (:then_4
      (bind _returnvalue (AddComponent|AddChildActorComponent true))
      (bind _asbp_line_cursor (Utilities|Casting|CastToBP_LineCursor (Variables|/Script/Engine.ChildActorComponent|GetChildActor _returnvalue)))
      (bind _output_get (Variables|Default|SetNormal%20Cursor _asbp_line_cursor))
      (Default|Setup _output_get false)
      (Class|SceneComponent|Attachto _returnvalue (Variables|Default|GetLetters%20Container) "None" "KeepRelativeOffset" true))
    (:then_5
      (bind _returnvalue_2 (AddComponent|AddChildActorComponent true))
      (bind _asbp_line_cursor_2 (Utilities|Casting|CastToBP_LineCursor (Variables|/Script/Engine.ChildActorComponent|GetChildActor _returnvalue_2)))
      (bind _output_get_2 (Variables|Default|SetPointer%20Cursor _asbp_line_cursor_2))
      (Default|Setup _output_get_2 true)
      (Class|SceneComponent|Attachto _returnvalue_2 (Variables|Default|GetLetters%20Container) "None" "KeepRelativeOffset" true))))

(fn SetupEditor
  (params (Sentence :type String) (DataToken :type String))
  (Utilities|FlowControl|Sequence
    (:then_0
      (for _array_element (Utilities|String|GetCharacterArrayfromString Sentence)
        (bind _letter (CallFunction|CreateLetter _array_element))
        (Utilities|Array|Add (Variables|Default|GetLetters) _letter)))
    (:then_1
      (CallFunction|LayoutLetters))
    (:then_2
      (Variables|Default|SetData%20Token DataToken))
    (:then_3
      (bind _returnvalue (AddComponent|AddChildActorComponent false (Math|Transform|MakeTransform "12.000000, 0,-180.000000" "0,180.000000, 0")))
      (bind _astext_render_actor (Utilities|Casting|CastToTextRenderActor (Variables|/Script/Engine.ChildActorComponent|GetChildActor _returnvalue)))
      (Rendering|Components|TextRender|SetText (Variables|/Script/Engine.TextRenderActor|GetTextRender _astext_render_actor) (Utilities|Text|MakeLiteralText "Press Enter to close Editor"))
      (Rendering|Components|TextRender|SetHorizontalAlignment (Variables|/Script/Engine.TextRenderActor|GetTextRender _astext_render_actor) "EHTA_Center"))))

(fn SetCursorIndex
  (params (Index :type Integer))
  (bind _output_get (Variables|Default|SetCursor%20Insert%20Index Index))
  (CallFunction|PositionCursor _output_get false))

(fn HandleKeyboardEvent
  (params (Character :type String) (Key%20Type :type E_KeyType%20Enum))
  (switch Utilities|FlowControl|Switch|SwitchonE_KeyType Key%20Type
    (:NewEnumerator0
      (bind _letter (CallFunction|CreateLetter Character))
      (Utilities|Array|Insert (Variables|Default|GetLetters) _letter (Variables|Default|GetCursor%20Insert%20Index))
      (CallFunction|LayoutLetters)
      (CallFunction|SetCursorIndex (+ (Variables|Default|GetCursor%20Insert%20Index) 1)))
    (:NewEnumerator1
      (CallFunction|HandleDeleteKey :!label _label))
    (:NewEnumerator2
      (for _array_element (Variables|Default|GetLetters)
        (bind _character (Default|GetCharacter _array_element))
        (LocalVariables|SetResult%20String (Utilities|String|Append (LocalVariables|GetResult%20String) _character)))
      (Default|CallFinishedEditing (LocalVariables|GetResult%20String) (Variables|Default|GetData%20Token)))
    (:NewEnumerator7
      (LocalVariables|SetArrow%20Increment -1)
      (bind _next_index (CallFunction|NextIndex (Variables|Default|GetCursor%20Insert%20Index) (+ (Utilities|Array|Length (Variables|Default|GetLetters)) 1) (LocalVariables|GetArrow%20Increment) true :!label _label_2))
      (CallFunction|SetCursorIndex _next_index))
    (:NewEnumerator8
      (LocalVariables|SetArrow%20Increment 1)
      (goto _label_2))
    (:NewEnumerator11
      (goto _label))))

(fn LayoutLetters
  (Utilities|FlowControl|Sequence
    (:then_0
      (for (_array_element _array_index) (Variables|Default|GetLetters)
        (Default|UpdateIndex _array_element _array_index)
        (LocalVariables|SetY%20Offset (+ (LocalVariables|GetY%20Offset) (/ (Default|GetWidth _array_element) 2.0)))
        (Transformation|SetRelativeLocation (Variables|/Game/Typewriter/LineEditor/BP_LineLetter.BP_LineLetter_C|GetScene _array_element) (Math|Vector|MakeVector 0.0 (LocalVariables|GetY%20Offset) 0.0) false false)
        (LocalVariables|SetY%20Offset (+ (LocalVariables|GetY%20Offset) (/ (Default|GetWidth _array_element) 2.0)))))
    (:then_2
      (CallFunction|PositionCursor (Variables|Default|GetCursor%20Insert%20Index) false))))

(fn CreateLetter
  (params (Character :type String))
  (Utilities|FlowControl|Sequence
    (:then_0
      (bind _returnvalue (AddComponent|AddChildActorComponent true))
      (Class|SceneComponent|Attachto _returnvalue (Variables|Default|GetLetters%20Container) "None" "KeepRelativeOffset" true)
      (bind _asbp_line_letter (Utilities|Casting|CastToBP_LineLetter (Variables|/Script/Engine.ChildActorComponent|GetChildActor _returnvalue)))
      (Default|Setup _asbp_line_letter Character)
      (LocalVariables|SetLetter%20Result _asbp_line_letter))
    (:then_1
      (CallFunction|ListentoLetter (LocalVariables|GetLetter%20Result)))
    (:then_2
      (return (LocalVariables|GetLetter%20Result)))))

(fn PositionCursor
  (params (Insert%20Index :type Integer) (Dimmed :type Boolean))
  (bind _location (CallFunction|CalcCursorPosition Insert%20Index))
  (if Dimmed
    (Default|MovetoLocation (Variables|Default|GetPointer%20Cursor) (Math|Transform|InverseTransformLocation (Transformation|GetWorldTransform (Variables|Default|GetLetters%20Container)) _location))
    (else
      (Default|MovetoLocation (Variables|Default|GetNormal%20Cursor) (Math|Transform|InverseTransformLocation (Transformation|GetWorldTransform (Variables|Default|GetLetters%20Container)) _location)))))

(fn HandleDeleteKey
  (if (> (Variables|Default|GetCursor%20Insert%20Index) 0)
    (Utilities|FlowControl|Sequence
      (:then_0
        (LocalVariables|SetDelete%20Index (- (Variables|Default|GetCursor%20Insert%20Index) 1)))
      (:then_1
        (Actor|DestroyActor (Utilities|Array|Get(acopy) (Variables|Default|GetLetters) (LocalVariables|GetDelete%20Index))))
      (:then_2
        (Utilities|Array|RemoveIndex (Variables|Default|GetLetters) (LocalVariables|GetDelete%20Index))
        (CallFunction|LayoutLetters))
      (:then_3
        (CallFunction|SetCursorIndex (Math|Integer|Max(Integer) (LocalVariables|GetDelete%20Index)))))))

(fn CalcCursorPosition
  (params (Insert%20Index :type Integer))
  (Utilities|FlowControl|Sequence
    (:then_0
      (LocalVariables|SetLocal%20Letter%20Index Insert%20Index)
      (LocalVariables|SetLocal%20Multiplier -1.0))
    (:then_1
      (if (== (LocalVariables|GetLocal%20Letter%20Index) (Utilities|Array|Length (Variables|Default|GetLetters)))
        (LocalVariables|SetLocal%20Letter%20Index (Utilities|Array|LastIndex (Variables|Default|GetLetters)))
        (LocalVariables|SetLocal%20Multiplier 1.0)))
    (:then_2
      (return (Math|Vector|MakeVector (- (.X (Math|Vector|BreakVector (Transformation|GetActorLocation (Utilities|Array|Get(acopy) (Variables|Default|GetLetters) (LocalVariables|GetLocal%20Letter%20Index))))) 12.0) (+ (.Y (Math|Vector|BreakVector (Transformation|GetActorLocation (Utilities|Array|Get(acopy) (Variables|Default|GetLetters) (LocalVariables|GetLocal%20Letter%20Index))))) (* (/ (Default|GetWidth (Utilities|Array|Get(acopy) (Variables|Default|GetLetters) (LocalVariables|GetLocal%20Letter%20Index))) 2.0) (LocalVariables|GetLocal%20Multiplier))) (.Z (Math|Vector|BreakVector (Transformation|GetActorLocation (Utilities|Array|Get(acopy) (Variables|Default|GetLetters) (LocalVariables|GetLocal%20Letter%20Index))))))))))

(fn IndexforHitPosition
  (params (Index :type Integer) (Hit%20Position :type Vector))
  (Utilities|FlowControl|Sequence
    (:then_0
      (LocalVariables|SetIndex%20Out Index))
    (:then_3
      (if (not (< (.Y (Math|Vector|BreakVector Hit%20Position)) 0.0))
        (LocalVariables|SetIndex%20Out (+ Index 1))))
    (:then_5
      (return (LocalVariables|GetIndex%20Out)))))

(fn StringValue
  (for _array_element (Variables|Default|GetLetters)
    (bind _character (Default|GetCharacter _array_element))
    (LocalVariables|SetResult%20String (Utilities|String|Append (LocalVariables|GetResult%20String) _character)))
  (return (LocalVariables|GetResult%20String) (Variables|Default|GetData%20Token)))