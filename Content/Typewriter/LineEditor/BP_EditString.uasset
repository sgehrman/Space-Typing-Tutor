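; BP_EditString is an actor that runs an on-screen string editing session with a typewriter keyboard and an animated editor line.
; ShowEditor spawns BP_Typewriter and BP_LineEditor as child actors, seeds the line with the string and a data token, then slides both in.
; Key presses are forwarded to the line editor.
; When editing finishes, it reports the string and token through CallEditorClosed and animates both parts back out asynchronously.
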(event Custom|Key%20Pressed
  (params (Character :type String) (Key%20Type :type E_KeyType%20Enum))
  (Default|HandleKeyboardEvent (Variables|Default|GetEditor%20Line) Character Key%20Type))

(event Custom|Bind%20Line%20Editor
  (EventDispatchers|BindEventtoFinishedEditing (Variables|Default|GetEditor%20Line) (delegate Custom|Finished%20Editing))
  (CallFunction|AnimateLinein true))

(event Custom|Finished%20Editing
  (params (String :type String) (Data%20Token :type String))
  (Default|CallEditorClosed false String Data%20Token)
  (CallFunction|AnimateLinein false)
  (CallFunction|AnimateKeyboardin false))

(event Custom|Bind%20Keyboard
  (EventDispatchers|BindEventtoKeyPressedEvent (Variables|Default|GetKeyboard) (delegate Custom|Key%20Pressed))
  (CallFunction|AnimateKeyboardin true))

(event EventBeginPlay)

(fn ConstructionScript)

(fn ShowEditor
  (params (String :type String) (Event%20Parameter :type String))
  (Utilities|FlowControl|Sequence
    (:then_0
      (bind _returnvalue (AddComponent|AddChildActorComponent false (CallFunction|KeyboardTransform)))
      (bind _asbp_typewriter (Utilities|Casting|CastToBP_Typewriter (Variables|/Script/Engine.ChildActorComponent|GetChildActor _returnvalue)))
      (Variables|Default|SetKeyboard _asbp_typewriter)
      (CallFunction|BindKeyboard))
    (:then_1
      (bind _returnvalue_2 (AddComponent|AddChildActorComponent false))
      (bind _asbp_line_editor (Utilities|Casting|CastToBP_LineEditor (Variables|/Script/Engine.ChildActorComponent|GetChildActor _returnvalue_2)))
      (bind _output_get (Variables|Default|SetEditor%20Line _asbp_line_editor))
      (Default|SetupEditor _output_get String Event%20Parameter)
      (CallFunction|BindLineEditor))))

(fn AnimateKeyboardin
  (params (Animate%20In :type Boolean))
  (Utilities|FlowControl|Sequence
    (:then_1
      (if Animate%20In
        (LocalVariables|SetStart "0, 0,1200.000000")
        (LocalVariables|SetEnd "0, 0, 0")
        (else
          (LocalVariables|SetStart "0, 0, 0")
          (LocalVariables|SetEnd "0, 0,1200.000000"))))
    (:then_3
      (CallFunction|AnimatewithParams (Utilities|Array|MakeArray (Utilities|Struct|MakeS_AnimationParams (Variables|Default|GetKeyboard) true (LocalVariables|GetStart) (LocalVariables|GetEnd) true)) true))))

(fn AnimateLinein
  (params (Animate%20In :type Boolean))
  (Utilities|FlowControl|Sequence
    (:then_1
      (if Animate%20In
        (LocalVariables|SetStart (LocalVariables|GetDefault%20Out%20Position))
        (LocalVariables|SetEnd (LocalVariables|GetDefault%20Position))
        (else
          (LocalVariables|SetStart (LocalVariables|GetDefault%20Position))
          (LocalVariables|SetEnd (LocalVariables|GetDefault%20Out%20Position)))))
    (:then_3
      (CallFunction|AnimatewithParams (Utilities|Array|MakeArray (Utilities|Struct|MakeS_AnimationParams (Variables|Default|GetEditor%20Line) true (LocalVariables|GetStart) (LocalVariables|GetEnd))) true))))