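; Modal string editor actor that lets the user edit a line of text with an in-world typewriter keyboard and Save or Cancel buttons.
; ShowEditor spawns keyboard, line editor and buttons as child actors, then animates keyboard and line into place.
; Key presses, except one filtered key type, feed the line editor.
; Save or Cancel reports the result, string and token through EditorClosed and animates keyboard and line out.
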(event Custom|Key%20Pressed
  (params (Character :type String) (Key%20Type :type E_KeyType%20Enum))
  (if (not (Utilities|Enum|Equal(Enum) Key%20Type "NewEnumerator2"))
    (Default|HandleKeyboardEvent (Variables|Default|GetEditor%20Line) Character Key%20Type)))

(event Custom|Bind%20Buttons
  (EventDispatchers|BindEventtoButtonClickedbyUser (Variables|Default|GetCancel%20Button) (delegate Custom|Canceled))
  (EventDispatchers|BindEventtoButtonClickedbyUser (Variables|Default|GetSave%20Button) (delegate Custom|Saved)))

(event Custom|Bind%20Line%20Editor
  (CallFunction|AnimateLinein true))

(event Custom|Canceled
  (params (Button%20ID :type String) (Hit%20Location :type Vector))
  (CallFunction|Finished true))

(event Custom|Saved
  (params (Button%20ID :type String) (Hit%20Location :type Vector))
  (bind _editor_line (Variables|Default|GetEditor%20Line))
  (bind (_string _token) (Default|StringValue _editor_line))
  (CallFunction|Finished false _string _token))

(event Custom|Finished
  (params (Canceled :type Boolean) (String :type String) (Token :type String))
  (Default|CallEditorClosed Canceled String Token)
  (CallFunction|AnimateLinein false)
  (CallFunction|AnimateKeyboardin false))

(event Custom|Bind%20Keyboard
  (EventDispatchers|BindEventtoKeyPressedEvent (Variables|Default|GetKeyboard) (delegate Custom|Key%20Pressed))
  (CallFunction|AnimateKeyboardin true))

(fn ConstructionScript)

(fn ShowEditor
  (params (String :type String) (Event%20Parameter :type String))
  (bind _size (CallFunction|StandardButtonSize))
  (bind _size_2 (CallFunction|StandardButtonSize))
  (bind _returnvalue (/ (.y _size) 1.95))
  (Utilities|FlowControl|Sequence
    (:then_0
      (bind _returnvalue_2 (AddComponent|AddChildActorComponent false (CallFunction|KeyboardTransform)))
      (bind _asbp_typewriter (Utilities|Casting|CastToBP_Typewriter (Variables|/Script/Engine.ChildActorComponent|GetChildActor _returnvalue_2)))
      (Variables|Default|SetKeyboard _asbp_typewriter)
      (CallFunction|BindKeyboard))
    (:then_1
      (bind _returnvalue_3 (AddComponent|AddChildActorComponent false))
      (bind _asbp_line_editor (Utilities|Casting|CastToBP_LineEditor (Variables|/Script/Engine.ChildActorComponent|GetChildActor _returnvalue_3)))
      (bind _output_get (Variables|Default|SetEditor%20Line _asbp_line_editor))
      (Default|SetupEditor _output_get String Event%20Parameter)
      (CallFunction|BindLineEditor))
    (:then_4
      (bind _returnvalue_4 (AddComponent|AddChildActorComponent false (Math|Transform|MakeTransform (CallFunction|StandardLocation (Math|Vector|MakeVector 0.0 (Class|TKMathFunctionLibrary|NegateFloat _returnvalue) 0.0)))))
      (bind _asbp_toggle_button (Utilities|Casting|CastToBP_ToggleButton (Variables|/Script/Engine.ChildActorComponent|GetChildActor _returnvalue_4)))
      (Default|Setup _asbp_toggle_button _size_2 false "Cancel" "cancel" false)
      (Variables|Default|SetCancel%20Button _asbp_toggle_button))
    (:then_5
      (bind _returnvalue_5 (AddComponent|AddChildActorComponent false (Math|Transform|MakeTransform (CallFunction|StandardLocation (Math|Vector|MakeVector 0.0 _returnvalue 0.0)))))
      (bind _asbp_toggle_button_2 (Utilities|Casting|CastToBP_ToggleButton (Variables|/Script/Engine.ChildActorComponent|GetChildActor _returnvalue_5)))
      (Default|Setup _asbp_toggle_button_2 _size_2 false "Save" "" false)
      (Variables|Default|SetSave%20Button _asbp_toggle_button_2))
    (:then_6
      (CallFunction|BindButtons))))

(fn AnimateKeyboardin
  (params (Animate%20In :type Boolean))
  (Utilities|FlowControl|Sequence
    (:then_1
      (if Animate%20In
        (LocalVariables|SetStart "0, 0,1200.000000")
        (LocalVariables|SetEnd "0, 0, 0")
        (else
          (LocalVariables|SetStart "0, 0, 0")
          (LocalVariables|SetEnd "0, 0,1200.000000"))))
    (:then_3
      (CallFunction|AnimatewithParams (Utilities|Array|MakeArray (Utilities|Struct|MakeS_AnimationParams (Variables|Default|GetKeyboard) true (LocalVariables|GetStart) (LocalVariables|GetEnd) true)) true))))

(fn AnimateLinein
  (params (Animate%20In :type Boolean))
  (Utilities|FlowControl|Sequence
    (:then_1
      (if Animate%20In
        (LocalVariables|SetStart (LocalVariables|GetDefault%20Out%20Position))
        (LocalVariables|SetEnd (LocalVariables|GetDefault%20Position))
        (else
          (LocalVariables|SetStart (LocalVariables|GetDefault%20Position))
          (LocalVariables|SetEnd (LocalVariables|GetDefault%20Out%20Position)))))
    (:then_3
      (CallFunction|AnimatewithParams (Utilities|Array|MakeArray (Utilities|Struct|MakeS_AnimationParams (Variables|Default|GetEditor%20Line) true (LocalVariables|GetStart) (LocalVariables|GetEnd))) true))))