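; BP_FingerIndicator is a typewriter display that shows a row of small meshes for eight fingers, thumbs excluded, highlighting and naming the current one.
; The construction script creates plain and emissive dynamic materials, then builds the meshes from the finger enum, split left and right around a central gap.
; UpdateCurrentFinger swaps materials and sets the name text.
; RunFlashingAnimation blinks all meshes through a delayed, counted event loop, then restores the displayed finger.
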(event Custom|Refresh%20After%20Delay
  (params (Delay :type Float%20%28single-precision%29) (Flash%20Count :type Integer) (On%20State :type Boolean))
  (Utilities|FlowControl|Delay Delay)
  (if (== Flash%20Count 0)
    (CallFunction|UpdateCurrentFinger (Variables|Default|GetDisplayed%20Finger))
    (else
      (CallFunction|RunFlashingAnimation Flash%20Count On%20State))))

(fn ConstructionScript
  (Utilities|FlowControl|Sequence
    (:then_0
      (bind _returnvalue (Rendering|Material|CreateDynamicMaterialInstance "/Game/ReusableAssets/Materials/MT_Opaque.MT_Opaque" :!class /Script/Engine.KismetMaterialLibrary))
      (bind _output_get (Variables|Default|SetMID _returnvalue))
      (Rendering|Material|SetVectorParameterValue _output_get "Color" "(R=0.077259,G=0.091372,B=0.105000,A=1.000000)" :!class /Script/Engine.MaterialInstanceDynamic))
    (:then_1
      (bind _returnvalue_2 (Rendering|Material|CreateDynamicMaterialInstance "/Game/ReusableAssets/Materials/MT_Opaque.MT_Opaque" :!class /Script/Engine.KismetMaterialLibrary))
      (bind _output_get_2 (Variables|Default|SetSelected%20MID _returnvalue_2))
      (Rendering|Material|SetVectorParameterValue _output_get_2 "EmissiveColor" "(R=0.014125,G=0.125000,B=0.013057,A=1.000000)" :!class /Script/Engine.MaterialInstanceDynamic)
      (Rendering|Material|SetScalarParameterValue _output_get_2 "Emission" 1e+02 :!class /Script/Engine.MaterialInstanceDynamic))
    (:then_2
      (CallFunction|BuildUI))))

(fn BuildUI
  (bind _item_width (LocalVariables|GetItem%20Width))
  (bind _enumvalue (|ForEachFingerEnum)
    (:LoopBody
      (Utilities|FlowControl|Sequence
        (:then_0
          (LocalVariables|SetYOffset -5e+04))
        (:then_1
          (switch Utilities|FlowControl|Switch|SwitchonFingerEnum _enumvalue
            (:NewEnumerator0
              (LocalVariables|SetYOffset (* -4 _item_width)))
            (:NewEnumerator10
              (LocalVariables|SetYOffset (* -3 _item_width)))
            (:NewEnumerator11
              (LocalVariables|SetYOffset (* -2 _item_width)))
            (:NewEnumerator12
              (LocalVariables|SetYOffset (* -1 _item_width)))
            (:NewEnumerator15
              (LocalVariables|SetYOffset (* 1 _item_width)))
            (:NewEnumerator16
              (LocalVariables|SetYOffset (* 2 _item_width)))
            (:NewEnumerator17
              (LocalVariables|SetYOffset (* 3 _item_width)))
            (:NewEnumerator18
              (LocalVariables|SetYOffset (* 4 _item_width)))))
        (:then_2
          (if (not (== (LocalVariables|GetYOffset) -5e+04))
            (Utilities|FlowControl|Sequence
              (:then_0
                (if (< (LocalVariables|GetYOffset) 0.0)
                  (LocalVariables|SetYOffset (- (LocalVariables|GetYOffset) (LocalVariables|GetOffset)))
                  (else
                    (LocalVariables|SetYOffset (+ (LocalVariables|GetYOffset) (LocalVariables|GetOffset))))))
              (:then_1
                (bind _returnvalue (AddComponent|AddStaticMeshComponent false (Math|Transform|MakeTransform (Math|Vector|MakeVector 0.0 (LocalVariables|GetYOffset) 0.0) "0, 0, 0" "0.100000,0.100000,0.100000")))
                (Utilities|Array|Add (Variables|Default|GetFinger%20Meshes) _returnvalue)
                (Utilities|Array|Add (Variables|Default|GetFinger%20Enums) _enumvalue)))))))))

(fn UpdateCurrentFinger
  (params (Finger :type FingerEnum%20Enum))
  (bind _finger_name (Variables|Default|GetFinger%20Name))
  (Utilities|FlowControl|Sequence
    (:then_0
      (for (_array_element _array_index) (Variables|Default|GetFinger%20Enums)
        (if (== _array_element Finger)
          (LocalVariables|SetMaterial (Variables|Default|GetSelected%20MID))
          (else
            (LocalVariables|SetMaterial (Variables|Default|GetMID))))
        (bind _asstatic_mesh_component (Utilities|Casting|CastToStaticMeshComponent (Utilities|Array|Get(acopy) (Variables|Default|GetFinger%20Meshes) _array_index)))
        (Rendering|Material|SetMaterial _asstatic_mesh_component 0 (LocalVariables|GetMaterial))))
    (:then_1
      (if (Utilities|Enum|Equal(Enum) Finger "NewEnumerator19")
        (Rendering|Components|TextRender|SetText _finger_name (Utilities|Text|MakeLiteralText ""))
        (else
          (Rendering|Components|TextRender|SetText _finger_name (Utilities|Text|ToText(String) (Utilities|String|EnumtoString Finger))))))
    (:then_2
      (Variables|Default|SetDisplayed%20Finger Finger))))

(fn RunFlashingAnimation
  (params (Flash%20Count :type Integer) (On%20State :type Boolean))
  (Utilities|FlowControl|Sequence
    (:then_0
      (if On%20State
        (LocalVariables|SetMaterial (Variables|Default|GetSelected%20MID))
        (else
          (LocalVariables|SetMaterial (Variables|Default|GetMID)))))
    (:then_1
      (for _array_element (Variables|Default|GetFinger%20Meshes)
        (bind _asstatic_mesh_component (Utilities|Casting|CastToStaticMeshComponent _array_element))
        (Rendering|Material|SetMaterial _asstatic_mesh_component 0 (LocalVariables|GetMaterial))))
    (:then_4
      (CallFunction|RefreshAfterDelay 0.4 (- Flash%20Count 1) (not On%20State)))))