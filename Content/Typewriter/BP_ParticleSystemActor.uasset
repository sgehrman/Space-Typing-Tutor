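; Preview actor that cycles one particle component through a hardcoded library of particle system effects.
; BeginPlay fills the array, applies the current index's template, and enables input when EnablePreviewHotkeys is set.
; Add and Subtract keys step the index via a NextIndex helper and swap the template, printing its name and index when hotkeys are enabled.
; Multiply rotates the component and Divide re-activates it from the start.
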(event `Key|Subtract`
  ;[1 1 1] Previous
  (:`Pressed`
    (bind _next_index (`/Game/ReusableAssets/Utilities/LIB_Utilities.NextIndex` (`self.Particle System Index`) (`KismetArrayLibrary.Array_Length` (`self.Particle Systems`)) -1))
    (set `self.Particle System Index` _next_index)
    (`self.Update Particle System`)))

(event `Update Particle System`
  (bind _particle_system_index (`self.Particle System Index`))
  (bind _item (`KismetArrayLibrary.Array_Get` (`self.Particle Systems`) _particle_system_index))
  (`ParticleSystemComponent.SetTemplate` (`self.Paticle System`) _item)
  (if (`self.Enable Preview Hotkeys`)
    (`KismetSystemLibrary.PrintString` (`VictoryBPFunctionLibrary.AppendMultiple` (`KismetSystemLibrary.GetDisplayName` _item) " - " (`KismetStringLibrary.Conv_IntToString` _particle_system_index)))))

(event `Key|Add`
  ;[1 1 1] Next
  (:`Pressed`
    (bind _next_index (`/Game/ReusableAssets/Utilities/LIB_Utilities.NextIndex` (`self.Particle System Index`) (`KismetArrayLibrary.Array_Length` (`self.Particle Systems`)) 1))
    (set `self.Particle System Index` _next_index)
    (`self.Update Particle System`)))

(event `self.ReceiveBeginPlay`
  (`|ExecutionSequence`
    (:`then_0`
      (`self.Create Particle Systems Array`))
    (:`then_1`
      (`self.Update Particle System`))
    (:`then_2`
      (if (`self.Enable Preview Hotkeys`)
        (`self.EnableInput` (`GameplayStatics.GetPlayerController` 0))))))

(event `Key|Multiply`
  ;[1 1 1] Rotate
  (:`Pressed`
    (`SceneComponent.K2_AddRelativeRotation` (`self.Paticle System`) (struct :`Yaw` 15.0) false)))

(event `Key|Divide`
  ;[1 1 1] Reset
  (:`Pressed`
    (`ActorComponent.Activate` (`self.Paticle System`) true)))

(fn `Create Particle Systems Array`
  (bind _particle_systems (`self.Particle Systems`))
  (`|ExecutionSequence`
    (:`then_0`
      (`KismetArrayLibrary.Array_Add` _particle_systems "/Game/Vectorfields/Particles/P_Atom.P_Atom")
      (`KismetArrayLibrary.Array_Add` _particle_systems "/Game/Vectorfields/Particles/P_Aura.P_Aura")
      (`KismetArrayLibrary.Array_Add` _particle_systems "/Game/Vectorfields/Particles/P_barrier2.P_barrier2")
      (`KismetArrayLibrary.Array_Add` _particle_systems "/Game/Vectorfields/Particles/P_Billowing.P_Billowing")
      (`KismetArrayLibrary.Array_Add` _particle_systems "/Game/Vectorfields/Particles/P_Blender.P_Blender")
      (`KismetArrayLibrary.Array_Add` _particle_systems "/Game/Vectorfields/Particles/P_CameraDistance.P_CameraDistance")
      (`KismetArrayLibrary.Array_Add` _particle_systems "/Game/Vectorfields/Particles/P_Conduit.P_Conduit")
      (`KismetArrayLibrary.Array_Add` _particle_systems "/Game/Vectorfields/Particles/P_DustDevil.P_DustDevil")
      (`KismetArrayLibrary.Array_Add` _particle_systems "/Game/Vectorfields/Particles/P_EddyCurrent.P_EddyCurrent")
      (`KismetArrayLibrary.Array_Add` _particle_systems "/Game/Vectorfields/Particles/P_EnergyWall.P_EnergyWall")
      (`KismetArrayLibrary.Array_Add` _particle_systems "/Game/Vectorfields/Particles/P_EnergyWall2.P_EnergyWall2")
      (`KismetArrayLibrary.Array_Add` _particle_systems "/Game/Vectorfields/Particles/P_EventHorizon.P_EventHorizon")
      (`KismetArrayLibrary.Array_Add` _particle_systems "/Game/Vectorfields/Particles/P_FireJet.P_FireJet")
      (`KismetArrayLibrary.Array_Add` _particle_systems "/Game/Vectorfields/Particles/P_Fishes.P_Fishes")
      (`KismetArrayLibrary.Array_Add` _particle_systems "/Game/Vectorfields/Particles/P_FlameShield.P_FlameShield")
      (`KismetArrayLibrary.Array_Add` _particle_systems "/Game/Vectorfields/Particles/P_ForceField.P_ForceField")
      (`KismetArrayLibrary.Array_Add` _particle_systems "/Game/Vectorfields/Particles/P_Froth2.P_Froth2")
      (`KismetArrayLibrary.Array_Add` _particle_systems "/Game/Vectorfields/Particles/P_Fumes.P_Fumes")
      (`KismetArrayLibrary.Array_Add` _particle_systems "/Game/Vectorfields/Particles/P_Gateway.P_Gateway")
      (`KismetArrayLibrary.Array_Add` _particle_systems "/Game/Vectorfields/Particles/P_GeoPole.P_GeoPole")
      (`KismetArrayLibrary.Array_Add` _particle_systems "/Game/Vectorfields/Particles/P_globalBombPop.P_globalBombPop")
      (`KismetArrayLibrary.Array_Add` _particle_systems "/Game/Vectorfields/Particles/P_globalSteamTight.P_globalSteamTight")
      (`KismetArrayLibrary.Array_Add` _particle_systems "/Game/Vectorfields/Particles/P_GroundFire.P_GroundFire")
      (`KismetArrayLibrary.Array_Add` _particle_systems "/Game/Vectorfields/Particles/P_Infinity.P_Infinity")
      (`KismetArrayLibrary.Array_Add` _particle_systems "/Game/Vectorfields/Particles/P_Interdimensional.P_Interdimensional")
      (`KismetArrayLibrary.Array_Add` _particle_systems "/Game/Vectorfields/Particles/P_Intersection.P_Intersection")
      (`KismetArrayLibrary.Array_Add` _particle_systems "/Game/Vectorfields/Particles/P_Magneto.P_Magneto")
      (`KismetArrayLibrary.Array_Add` _particle_systems "/Game/Vectorfields/Particles/P_Napalm.P_Napalm")
      (`KismetArrayLibrary.Array_Add` _particle_systems "/Game/Vectorfields/Particles/P_Nova.P_Nova")
      (`KismetArrayLibrary.Array_Add` _particle_systems "/Game/Vectorfields/Particles/P_Nucleus.P_Nucleus")
      (`KismetArrayLibrary.Array_Add` _particle_systems "/Game/Vectorfields/Particles/P_Nuke.P_Nuke")
      (`KismetArrayLibrary.Array_Add` _particle_systems "/Game/Vectorfields/Particles/P_PoisonVent.P_PoisonVent")
      (`KismetArrayLibrary.Array_Add` _particle_systems "/Game/Vectorfields/Particles/P_PortalShaft.P_PortalShaft")
      (`KismetArrayLibrary.Array_Add` _particle_systems "/Game/Vectorfields/Particles/P_Radiation.P_Radiation")
      (`KismetArrayLibrary.Array_Add` _particle_systems "/Game/Vectorfields/Particles/P_ramaTest.P_ramaTest")
      (`KismetArrayLibrary.Array_Add` _particle_systems "/Game/Vectorfields/Particles/P_Sprinkler.P_Sprinkler")
      (`KismetArrayLibrary.Array_Add` _particle_systems "/Game/Vectorfields/Particles/P_Subduction.P_Subduction")
      (`KismetArrayLibrary.Array_Add` _particle_systems "/Game/Vectorfields/Particles/P_Suction.P_Suction")
      (`KismetArrayLibrary.Array_Add` _particle_systems "/Game/Vectorfields/Particles/P_Swarm.P_Swarm")
      (`KismetArrayLibrary.Array_Add` _particle_systems "/Game/Vectorfields/Particles/P_Thaw.P_Thaw")
      (`KismetArrayLibrary.Array_Add` _particle_systems "/Game/Vectorfields/Particles/P_Tornado.P_Tornado")
      (`KismetArrayLibrary.Array_Add` _particle_systems "/Game/Vectorfields/Particles/P_vectorfield_global_Shield.P_vectorfield_global_Shield")
      (`KismetArrayLibrary.Array_Add` _particle_systems "/Game/Vectorfields/Particles/P_WaveSplash.P_WaveSplash")
      (`KismetArrayLibrary.Array_Add` _particle_systems "/Game/Vectorfields/Particles/P_WhiteDwarf.P_WhiteDwarf")
      (`KismetArrayLibrary.Array_Add` _particle_systems "/Game/Vectorfields/Particles/P_Wisps.P_Wisps")
      (`KismetArrayLibrary.Array_Add` _particle_systems "/Game/Vectorfields/Particles/P_Wormhole.P_Wormhole"))
    (:`then_1`
      (return))))

(fn `UserConstructionScript`)