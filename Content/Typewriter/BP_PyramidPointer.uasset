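; BP_PyramidPointer is a pyramid pointer for the typewriter feature that briefly flashes to signal an error or a correct result.
; The construction script creates three dynamic instances of MT_Opaque (non-emissive blue, glowing red, glowing green) and applies the blue one to the Pyramid.
; FlashError and FlashCorrect swap in the red or green instance, wait a fifth of a second, then restore the blue one.
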(event `FlashError`
  (`PrimitiveComponent.SetMaterial` (`self.Pyramid`) 0 (`self.Error MID`))
  (`KismetSystemLibrary.Delay` 0.2)
  (`PrimitiveComponent.SetMaterial` (`self.Pyramid`) 0 (`self.MID`)))

(event `FlashCorrect`
  (`PrimitiveComponent.SetMaterial` (`self.Pyramid`) 0 (`self.Correct MID`))
  (`KismetSystemLibrary.Delay` 0.2)
  (`PrimitiveComponent.SetMaterial` (`self.Pyramid`) 0 (`self.MID`)))

(event `self.ReceiveTick`
  (params (DeltaSeconds :type "Float (single-precision)")))

(fn `UserConstructionScript`
  (`|ExecutionSequence`
    (:`then_0`
      (bind _returnvalue (`KismetMaterialLibrary.CreateDynamicMaterialInstance` "/Game/ReusableAssets/Materials/MT_Opaque.MT_Opaque"))
      (bind _output_get (set `self.MID` _returnvalue))
      (`MaterialInstanceDynamic.SetScalarParameterValue` _output_get "Emission" 0.0)
      (`MaterialInstanceDynamic.SetVectorParameterValue` _output_get "Color" (struct :`G` 0.088432 :`B` 0.435 :`A` 1.0)))
    (:`then_1`
      (bind _returnvalue_2 (`KismetMaterialLibrary.CreateDynamicMaterialInstance` "/Game/ReusableAssets/Materials/MT_Opaque.MT_Opaque"))
      (bind _output_get_2 (set `self.Error MID` _returnvalue_2))
      (`MaterialInstanceDynamic.SetScalarParameterValue` _output_get_2 "Emission" 12.0)
      (`MaterialInstanceDynamic.SetVectorParameterValue` _output_get_2 "EmissiveColor" (struct :`R` 0.885 :`B` 0.008285 :`A` 1.0)))
    (:`then_2`
      (bind _returnvalue_3 (`KismetMaterialLibrary.CreateDynamicMaterialInstance` "/Game/ReusableAssets/Materials/MT_Opaque.MT_Opaque"))
      (bind _output_get_3 (set `self.Correct MID` _returnvalue_3))
      (`MaterialInstanceDynamic.SetScalarParameterValue` _output_get_3 "Emission" 12.0)
      (`MaterialInstanceDynamic.SetVectorParameterValue` _output_get_3 "EmissiveColor" (struct :`R` 0.079635 :`G` 0.395 :`B` 0.010245 :`A` 1.0)))
    (:`then_3`
      (`PrimitiveComponent.SetMaterial` (`self.Pyramid`) 0 (`self.MID`)))))