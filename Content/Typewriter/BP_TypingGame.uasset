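; Typing-lesson controller that spawns the typewriter keyboard, sentence spawner, finger indicator and WPM/mistake counters, then returns to KeyboardLessons on completion.
; Once PLM is ready, an optional tutorial chains messages through named key-sequence events before starting the first level.
; Key presses feed the spawner, whose result updates the counters; Enter can fire a missile.
; It also serves as the keyboard's delegate, supplying the next character and updating the finger indicator.
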(event Custom|Key%20Sequence%20Event
  (params (Event%20Name :type String))
  (switch string Event%20Name
    (:Any%20Key%20Event
      (Utilities|FlowControl|Delay 2.0)
      (CallFunction|ShowMessage (CallFunction|MessageforIndex 1))
      (CallFunction|ListenforKeySequence "FJ Event" (Utilities|Array|MakeArray (Utilities|Struct|MakeKeyboardKeySpec "f" "NewEnumerator0") (Utilities|Struct|MakeKeyboardKeySpec "j" "NewEnumerator0"))))
    (:FJ%20Event
      (Utilities|FlowControl|Delay 0.5)
      (CallFunction|ShowMessage (CallFunction|MessageforIndex 4))
      (CallFunction|ListenforKeySequence "Shift Keys Event" (Utilities|Array|MakeArray (Utilities|Struct|MakeKeyboardKeySpec "" "NewEnumerator4") (Utilities|Struct|MakeKeyboardKeySpec "" "NewEnumerator5"))))
    (:Enter%20Key%20Event
      (Utilities|FlowControl|Delay 0.5)
      (CallFunction|ShowMessage (CallFunction|MessageforIndex 3))
      (CallFunction|ListenforKeySequence "Start Level Event" (Utilities|Array|MakeArray (Utilities|Struct|MakeKeyboardKeySpec "" "NewEnumerator2")))
      (CallFunction|PreviewLevelforIntro))
    (:Start%20Level%20Event
      (Default|HideMessage (Variables|Default|GetMessage%20Manager))
      (CallFunction|BeginLevelGo))
    (:Shift%20Keys%20Event
      (Utilities|FlowControl|Delay 0.5)
      (CallFunction|ShowMessage (CallFunction|MessageforIndex 2))
      (CallFunction|ShowFingerIndicator)
      (CallFunction|ShowWPM)
      (Default|RunFlashingAnimation (Variables|Default|GetFinger%20Indicator) 8 true)
      (CallFunction|ListenforKeySequence "Enter Key Event" (Utilities|Array|MakeArray (Utilities|Struct|MakeKeyboardKeySpec "" "NewEnumerator2"))))))

(event Custom|Start%20Intro
  (CallFunction|PositionKeyboard)
  (Utilities|FlowControl|Delay 1.0)
  (CallFunction|MovePlayerIntoPosition false)
  (Utilities|FlowControl|Delay 1.0)
  (bind _show_intro (Default|ShouldShowIntro (Variables|Default|GetPLM)))
  (if _show_intro
    (CallFunction|ShowMessage (CallFunction|MessageforIndex))
    (CallFunction|ListenforKeySequence "Any Key Event" (Utilities|Array|MakeArray))
    (else
      (CallFunction|ShowFingerIndicator)
      (CallFunction|ShowWPM)
      (CallFunction|BeginLevelGo))))

(event Custom|Handle%20KeyPressed%20Event
  (params (Character :type String) (Key%20Type :type E_KeyType%20Enum))
  (CallFunction|HandleKeyboardEvent Character Key%20Type))

(event Custom|Handle%20Key%20Sequence
  (params (Event%20Name :type String))
  (CallFunction|KeySequenceEvent Event%20Name))

(event Custom|CustomEvent_0
  (params (Result :type BPI%20PMM%20Interface))
  (bind _output_get (Variables|Default|SetPLM Result))
  (Utilities|FlowControl|Sequence
    (:then_0
      (bind _listener (Default|GetKeyEventListener _output_get))
      (EventDispatchers|BindEventtoKeySequenceEvent _listener (delegate Custom|Handle%20Key%20Sequence)))
    (:then_1
      (bind _dialog_manager (Default|GetDialogManager (Variables|Default|GetPLM)))
      (Variables|Default|SetMessage%20Manager _dialog_manager))
    (:then_2
      (Default|PlayAmbientSound _output_get "/Game/Typewriter/LessonMap/SC_KeyboardMusicLoop.SC_KeyboardMusicLoop"))
    (:then_3
      (CallFunction|FadeOutScreen true))
    (:then_4
      (CallFunction|MovePlayerIntoPosition true))
    (:then_5
      (CallFunction|StartIntro))
    (:then_6
      (Default|EnableCrosshair _output_get true false))))

(event Custom|Lesson%20Finished
  (Default|LoadLevel (Variables|Default|GetPLM) "KeyboardLessons"))

(event Custom|Bind%20Keyboard%20Events
  (Utilities|FlowControl|Sequence
    (:then_0
      (Default|UpdateDelegate (Variables|Default|GetKeyboard) self))
    (:then_1
      (EventDispatchers|BindEventtoKeyPressedEvent (Variables|Default|GetKeyboard) (delegate Custom|Handle%20KeyPressed%20Event)))))

(event Custom|Spawner%20State%20changed
  (Default|RefreshfromDelegate (Variables|Default|GetKeyboard)))

(event Custom|Bind%20Sentence%20Spawner%20Events
  (Utilities|FlowControl|Sequence
    (:then_0
      (EventDispatchers|BindEventtoLessonFinished (Variables|Default|GetSentence%20Spawner) (delegate Custom|Lesson%20Finished)))
    (:then_1
      (EventDispatchers|BindEventtoStateChangeEvent (Variables|Default|GetSentence%20Spawner) (delegate Custom|Spawner%20State%20changed)))))

(event Custom|Begin%20Level%20Go
  (Default|LoadUpLevel (Variables|Default|GetSentence%20Spawner) 0 true))

(event Custom|Preview%20Level%20For%20Intro
  (Default|LoadUpLevel (Variables|Default|GetSentence%20Spawner) 0 false))

(event EventBeginPlay
  (Utilities|FlowControl|Sequence
    (:then_0
      (bind _returnvalue (AddComponent|AddChildActorComponent false (CallFunction|SentenceSpawnerTransform)))
      (bind _asbp_sentence_spawner (Utilities|Casting|CastToBP_SentenceSpawner (Variables|/Script/Engine.ChildActorComponent|GetChildActor _returnvalue)))
      (bind _output_get (Variables|Default|SetSentence%20Spawner _asbp_sentence_spawner))
      (Rendering|SetVisibility (Variables|/Game/Typewriter/BP_SentenceSpawner.BP_SentenceSpawner_C|GetRoot _output_get) false true)
      (CallFunction|BindSentenceSpawnerEvents))
    (:then_3
      (bind _outactors (Actor|GetAllActorsOfClass "/Game/ReusableAssets/MissleLauncher/BP_MissleLauncher.BP_MissleLauncher_C"))
      (Variables|Default|SetMissle%20Launcher (Utilities|Array|Get(acopy) _outactors)))
    (:then_6
      (bind _returnvalue_2 (AddComponent|AddBCPMMAccess))
      (EventDispatchers|BindEventtoPMMReady _returnvalue_2 (delegate Custom|CustomEvent_0))
      (Default|Setup _returnvalue_2))
    (:then_11
      (Game|LoadStreamLevel(byName) "FloorSubmap" true))))

(fn ConstructionScript)

(fn PositionKeyboard
  (Utilities|FlowControl|Sequence
    (:then_0
      (bind _returnvalue (AddComponent|AddChildActorComponent false (CallFunction|KeyboardTransform)))
      (bind _asbp_typewriter (Utilities|Casting|CastToBP_Typewriter (Variables|/Script/Engine.ChildActorComponent|GetChildActor _returnvalue)))
      (Variables|Default|SetKeyboard _asbp_typewriter)
      (CallFunction|BindKeyboardEvents))
    (:then_1
      (bind _output_get (LocalVariables|SetEnd%20Location (Transformation|GetActorLocation (Variables|Default|GetKeyboard))))
      (LocalVariables|SetStart%20Location (+ _output_get "0, 0,1200.000000"))
      (CallFunction|AnimatetoLocation (Variables|Default|GetKeyboard) (LocalVariables|GetStart%20Location) (LocalVariables|GetEnd%20Location) "/Game/UniversalSoundFX/Sound_Effects/DOORS_and_GATES/DOOR_Metal_Hollow_Deep_Close_mono.DOOR_Metal_Hollow_Deep_Close_mono" 0.8 true false false 1.0))))

(fn MovePlayerIntoPosition
  (params (Start%20Position :type Boolean))
  (bind _returnvalue (Game|Player|GetPlayerPawn 0))
  (if Start%20Position
    ;[1 1 1] Had to do this since persistent map stuff uses the previous playerstart
    (Transformation|SetActorLocation _returnvalue (Math|Vector|MakeVector -5e+02 0.0 0.0) false)
    (else
      (CallFunction|AnimateActor (Transformation|GetActorLocation _returnvalue) (Math|Vector|MakeVector 0.0 0.0 0.0) _returnvalue))))

(fn ShowMessage
  (params (Lines :type Array%20of%20Strings))
  (Default|ShowMessage (Variables|Default|GetMessage%20Manager) (CallFunction|MessageBoxLocation) Lines))

(fn MessageforIndex
  (params (Index :type Integer))
  (Utilities|FlowControl|Sequence
    (:then_0
      (switch int Index
        (:0
          (LocalVariables|SetResult (Utilities|Array|MakeArray "This is a virtual keyboard to help you locate the right key." "Press any key on your keyboard to see how it responds.")))
        (:1
          (LocalVariables|SetResult (Utilities|Array|MakeArray "Get your hands in the correct position.  Place your index fingers on F and J." "Press F and J to continue.")))
        (:2
          (LocalVariables|SetResult (Utilities|Array|MakeArray "This is the finger indicator." "Refer to it if you forget which finger to use for the next key.  Press Enter to continue.")))
        (:3
          (LocalVariables|SetResult (Utilities|Array|MakeArray "Behind me are the sentences you need to type to complete Level 1.  " "Press the Enter Key to begin.")))
        (:4
          (LocalVariables|SetResult (Utilities|Array|MakeArray "Use your pinky to press and hold one of the shift keys." "See how the keyboard changes?  If you can't remember where a key is, hold Shift.  Hit both Shift keys to continue.")))))
    (:then_1
      (return (LocalVariables|GetResult)))))

(fn ShowFingerIndicator
  (Utilities|FlowControl|Sequence
    (:then_0
      (bind _returnvalue (AddComponent|AddChildActorComponent false (CallFunction|FingerIndicatorTransform)))
      (bind _asbp_finger_indicator (Utilities|Casting|CastToBP_FingerIndicator (Variables|/Script/Engine.ChildActorComponent|GetChildActor _returnvalue)))
      (Variables|Default|SetFinger%20Indicator _asbp_finger_indicator))
    (:then_1
      (bind _output_get (LocalVariables|SetEnd%20Location (Transformation|GetActorLocation (Variables|Default|GetFinger%20Indicator))))
      (LocalVariables|SetStart%20Location (+ _output_get "0,0.000000,1200.000000"))
      (CallFunction|AnimateActor (LocalVariables|GetStart%20Location) (LocalVariables|GetEnd%20Location) (Variables|Default|GetFinger%20Indicator)))))

(fn StartMusic
  (params (Start :type Boolean))
  (if Start
    _))

(fn ProcessKeyDownforGameplay
  (params (Character :type String) (Key%20Type :type E_KeyType%20Enum))
  (Utilities|FlowControl|Sequence
    (:then_0
      (switch Utilities|FlowControl|Switch|SwitchonE_KeyType Key%20Type
        (:NewEnumerator0
          (bind _success (Default|ProcessTypedCharacter (Variables|Default|GetSentence%20Spawner) Character Key%20Type :!label _label))
          (LocalVariables|SetResult%20Success _success))
        (:NewEnumerator1
          (goto _label))
        (:NewEnumerator2
          (if (Variables|Default|GetEnable%20Missle%20Launcher)
            (Default|FireMissle (Variables|Default|GetMissle%20Launcher))))
        (:NewEnumerator3
          (goto _label))))
    (:then_3
      (return (LocalVariables|GetResult%20Success)))))

(fn UpdateWPM
  (params (Correct%20Key :type Boolean) (Key%20Type :type E_KeyType%20Enum))
  (Utilities|FlowControl|Sequence
    (:then_0
      (if (Variables|/Game/Typewriter/BP_SentenceSpawner.BP_SentenceSpawner_C|GetGame%20Playing (Variables|Default|GetSentence%20Spawner))
        (if (not (Utilities|Enum|Equal(Enum) Key%20Type "NewEnumerator1"))
          (if Correct%20Key
            (Default|KeyDownEvent (Variables|Default|GetWPM%20Indicator))
            (else
              (switch Utilities|FlowControl|Switch|SwitchonE_KeyType Key%20Type
                (:NewEnumerator0
                  (Default|IncrementEventCount (Variables|Default|GetMistake%20IIndicator)))))))))))

(fn ShowWPM
  (Utilities|FlowControl|Sequence
    (:then_0
      (bind _returnvalue (AddComponent|AddChildActorComponent false (CallFunction|WPMTransform)))
      (bind _asbp_words_per_minute (Utilities|Casting|CastToBP_WordsPerMinute (Variables|/Script/Engine.ChildActorComponent|GetChildActor _returnvalue)))
      (bind _output_get (Variables|Default|SetWPM%20Indicator _asbp_words_per_minute))
      (Default|Setup _output_get "WPM" true))
    (:then_1
      (bind _returnvalue_2 (AddComponent|AddChildActorComponent false (CallFunction|MistakesTransform)))
      (bind _asbp_words_per_minute_2 (Utilities|Casting|CastToBP_WordsPerMinute (Variables|/Script/Engine.ChildActorComponent|GetChildActor _returnvalue_2)))
      (bind _output_get_2 (Variables|Default|SetMistake%20IIndicator _asbp_words_per_minute_2))
      (Default|Setup _output_get_2 "Mistakes" false))
    (:then_2
      (CallFunction|AnimateActor (+ (Transformation|GetActorLocation (Variables|Default|GetMistake%20IIndicator)) "0,-1200.000000,0.000000") (Transformation|GetActorLocation (Variables|Default|GetMistake%20IIndicator)) (Variables|Default|GetMistake%20IIndicator)))
    (:then_3
      (CallFunction|AnimateActor (+ (Transformation|GetActorLocation (Variables|Default|GetWPM%20Indicator)) "0,1200.000000,0.000000") (Transformation|GetActorLocation (Variables|Default|GetWPM%20Indicator)) (Variables|Default|GetWPM%20Indicator)))))

(fn AnimateActor
  (params (Start%20Location :type Vector) (End%20Location :type Vector) (Actor :type Actor%20Object%20Reference))
  (CallFunction|AnimatetoLocation Actor Start%20Location End%20Location 0 1.0 false false false 1.0))

(fn ListenforKeySequence
  (params (Event%20Name :type String) (Key%20Specs :type Array%20of%20Keyboard%20Key%20Spec%20Structures))
  (bind _listener (Default|GetKeyEventListener (Variables|Default|GetPLM)))
  (Default|ListenforKeySequence _listener Event%20Name Key%20Specs)
  (Default|FlashKeysUntilPressed (Variables|Default|GetKeyboard) Key%20Specs))

(fn HandleKeyboardEvent
  (params (Character :type String) (Key%20Type :type E_KeyType%20Enum))
  (Utilities|FlowControl|Sequence
    (:then_0
      (bind _success (CallFunction|ProcessKeyDownforGameplay Character Key%20Type))
      (LocalVariables|SetResult%20Success _success))
    (:then_1
      (CallFunction|UpdateWPM (LocalVariables|GetResult%20Success) Key%20Type))))

(fn GetNextCharacter
  (bind (_valid _character) (Default|GetNextCharacter (Variables|Default|GetSentence%20Spawner)))
  (return _valid _character))

(fn NextMatchingKey
  (params (Key%20Data :type ST%20Key%20Data%20Structure))
  (Default|UpdateCurrentFinger (Variables|Default|GetFinger%20Indicator) (Utilities|Enum|ByteToEnumFingerEnum (Math|Conversions|ToByte(Integer) (.Finger (Utilities|Struct|BreakST_KeyData Key%20Data)))))
  (return true))