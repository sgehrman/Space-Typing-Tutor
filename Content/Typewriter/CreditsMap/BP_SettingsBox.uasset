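; Settings panel actor that lets the player toggle saved preferences for intro skipping, keyboard sounds, background music and developer mode.
; On BeginPlay it builds itself from two child actors: a BP_DisplayBox titled "Settings" and a BP_CheckboxBar filled by CheckboxData from the stored bool prefs.
; Checkbox clicks write straight back to those prefs, and the display box's Stop button fires SettingsClosed.
; The Developer Mode checkbox is added only when IsDebugging passes.
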(event Custom|Button%20Clicked%20Event
  (params (Button%20ID :type String) (On%20State :type Boolean))
  (switch string Button%20ID
    (:Default
      (CallFunction|Logg "Settings Map Actor error"))
    (:skip%20intro
      (Utilities|SetBoolPref "NewEnumerator0" On%20State))
    (:keyboard%20sounds
      (Utilities|SetBoolPref "NewEnumerator2" On%20State))
    (:background%20music
      (Utilities|SetBoolPref "NewEnumerator1" On%20State))
    (:Developer%20Mode
      (Utilities|SetBoolPref "NewEnumerator3" On%20State))))

(event Custom|Close%20Button%20Clicked
  (params (Button%20ID :type String))
  (switch string Button%20ID
    (:stop
      (Default|CallSettingsClosed))))

(event EventBeginPlay
  (Utilities|FlowControl|Sequence
    (:then_0
      (bind _returnvalue (AddComponent|AddChildActorComponent false (Math|Transform|MakeTransform "0, 0, 0")))
      (bind _asbp_display_box (Utilities|Casting|CastToBP_DisplayBox (Variables|/Script/Engine.ChildActorComponent|GetChildActor _returnvalue)))
      (EventDispatchers|BindEventtoCloseButtonClicked _asbp_display_box (delegate Custom|Close%20Button%20Clicked))
      (Default|Setup _asbp_display_box true "0, 0, 0" 0.0 0.0 0.0 0.0)
      (Default|SetTitle _asbp_display_box "Settings")
      (Default|UpdateButtonStates _asbp_display_box false true false))
    (:then_1
      (bind _returnvalue_2 (AddComponent|AddChildActorComponent false (Math|Transform|MakeTransform "-5.000000,-36.000000,0.000000")))
      (bind _asbp_checkbox_bar (Utilities|Casting|CastToBP_CheckboxBar (Variables|/Script/Engine.ChildActorComponent|GetChildActor _returnvalue_2)))
      (Default|ReplaceButtons _asbp_checkbox_bar (CallFunction|CheckboxData))
      (EventDispatchers|BindEventtoButtonClicked _asbp_checkbox_bar (delegate Custom|Button%20Clicked%20Event)))))

(fn ConstructionScript)

(fn CheckboxValues
  (Utilities|FlowControl|Sequence
    (:then_0
      (bind _bool (Utilities|BoolPref "NewEnumerator2")
        (:True
          _)
        (:False
          _))
      (LocalVariables|SetR%20Keyboard%20Sounds _bool))
    (:then_1
      (bind _bool_2 (Utilities|BoolPref "NewEnumerator1")
        (:True
          _)
        (:False
          _))
      (LocalVariables|SetR%20Background%20Music _bool_2))
    (:then_2
      (bind _bool_3 (Utilities|BoolPref "NewEnumerator0")
        (:True
          _)
        (:False
          _))
      (LocalVariables|SetR%20Skip%20Intro _bool_3))
    (:then_3
      (bind _bool_4 (Utilities|BoolPref "NewEnumerator3")
        (:True
          _)
        (:False
          _))
      (LocalVariables|SetR%20Developer%20Mode _bool_4))
    (:then_4
      (return (LocalVariables|GetR%20Skip%20Intro) (LocalVariables|GetR%20Keyboard%20Sounds) (LocalVariables|GetR%20Background%20Music) (LocalVariables|GetR%20Developer%20Mode)))))

(fn CheckboxData
  (bind (_skip_intro _key_sounds _background_music _developer_mode) (CallFunction|CheckboxValues))
  (Utilities|FlowControl|Sequence
    (:then_0
      (LocalVariables|SetResult (Utilities|Array|MakeArray (Utilities|Struct|MakeS_StringAndToken "Skip Intro" "skip intro" (Math|Conversions|ToInteger(Boolean) _skip_intro)) (Utilities|Struct|MakeS_StringAndToken "Disable Keyboard Sounds " "keyboard sounds" (Math|Conversions|ToInteger(Boolean) _key_sounds)) (Utilities|Struct|MakeS_StringAndToken "Disable Background Music" "background music" (Math|Conversions|ToInteger(Boolean) _background_music)))))
    (:then_2
      ;[1 1 1] Developer only preferences
      (Utilities|IsDebugging
        (:Yes
          (Utilities|Array|Add (LocalVariables|GetResult) (Utilities|Struct|MakeS_StringAndToken "Developer Mode" "developer mode" (Math|Conversions|ToInteger(Boolean) _developer_mode))))))
    (:then_3
      (return (LocalVariables|GetResult)))))