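; Settings map actor for the Typewriter game: builds the settings checkbox bar and a Credits button that loads the Credits level.
; On BeginPlay it spawns both as child actors, binds their clicks, moves the player into position and enables the crosshair once PMM is ready.
; Only the Dvorak layout option is read from and saved to Preferences; the keyboard sound and background music checkboxes are not wired to storage.
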(event Custom|CustomEvent_0
  (params (Result :type BPI%20PMM%20Interface))
  (bind _output_get (Variables|Default|SetPLM Result))
  (Default|EnableCrosshair _output_get true false))

(event Custom|Button%20Clicked%20Event
  (params (Button%20ID :type String) (On%20State :type Boolean))
  (bind _self self)
  (bind _preferences (CallFunction|GetPreferences _self))
  (switch string Button%20ID
    (:dvorak
      (if On%20State
        (Default|Set _preferences "keyboard layout" "NewEnumerator1" false 1 "" 0.0)
        (else
          (Default|Set _preferences "keyboard layout" "NewEnumerator1" false 0 "" 0.0))))))

(event Custom|Credits%20Button%20Clicked
  (params (Button%20ID :type String) (Hit%20Location :type Vector))
  (switch string Button%20ID
    (:credits
      (Default|LoadLevel (Variables|Default|GetPLM) "Credits"))))

(event EventBeginPlay
  (bind (_dvorak _key_sounds _background_music) (CallFunction|CheckboxValues))
  (Utilities|FlowControl|Sequence
    (:then_1
      (bind _returnvalue (AddComponent|AddBCPMMAccess))
      (EventDispatchers|BindEventtoPMMReady _returnvalue (delegate Custom|CustomEvent_0))
      (Default|Setup _returnvalue "Settings"))
    (:then_2
      (bind _returnvalue_2 (AddComponent|AddChildActorComponent false (Math|Transform|MakeTransform (CallFunction|StandardLocation "-12.000000,-111.000000,0.000000"))))
      (bind _asbp_checkbox_bar (Utilities|Casting|CastToBP_CheckboxBar (Variables|/Script/Engine.ChildActorComponent|GetChildActor _returnvalue_2)))
      (Default|ReplaceButtons _asbp_checkbox_bar (Utilities|Array|MakeArray (Utilities|Struct|MakeS_StringAndToken "Use Dvorak keyboard layout" "dvorak" (Math|Conversions|ToInteger(Boolean) _dvorak)) (Utilities|Struct|MakeS_StringAndToken "Keyboard Sounds Enabled" (Utilities|String|ToString(Boolean) _key_sounds)) (Utilities|Struct|MakeS_StringAndToken "Background Music Enabled" "background audio" (Math|Conversions|ToInteger(Boolean) _background_music))))
      (EventDispatchers|BindEventtoButtonClicked _asbp_checkbox_bar (delegate Custom|Button%20Clicked%20Event)))
    (:then_5
      (bind _returnvalue_3 (AddComponent|AddChildActorComponent false (Math|Transform|MakeTransform (CallFunction|StandardLocation "0,100.000000, 0"))))
      (bind _asbp_toggle_button (Utilities|Casting|CastToBP_ToggleButton (Variables|/Script/Engine.ChildActorComponent|GetChildActor _returnvalue_3)))
      (Default|SetTitleandSize _asbp_toggle_button (CallFunction|StandardButtonSize) false "Credits" "credits")
      (EventDispatchers|BindEventtoButtonClickedbyUser _asbp_toggle_button (delegate Custom|Credits%20Button%20Clicked)))
    (:then_7
      (Default|MovePlayerIntoPosition (Variables|Default|GetBC_LevelCommon) true)
      (Utilities|FlowControl|Delay 0.5)
      (Default|MovePlayerIntoPosition (Variables|Default|GetBC_LevelCommon) false))))

(fn ConstructionScript)

(fn CheckboxValues
  (Utilities|FlowControl|Sequence
    (:then_0
      (bind _integer (Default|Get (CallFunction|GetPreferences self) "keyboard layout" "NewEnumerator1"))
      (switch int _integer
        (:0
          (LocalVariables|SetR%20Dvorak false))
        (:1
          (LocalVariables|SetR%20Dvorak true))))
    (:then_2
      (bind _returnvalue (Class|SystemUtils|KeyboardLayout))
      (CallFunction|Logg _returnvalue))
    (:then_4
      (return (LocalVariables|GetR%20Dvorak) (LocalVariables|GetR%20Keyboard%20Sounds) (LocalVariables|GetR%20Background%20Music)))))