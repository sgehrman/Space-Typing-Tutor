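; BP_CreditsActor is the setup actor for the credits map, doing all of its work at BeginPlay.
; It registers a PMM access component under "credits", then caches the returned manager and enables the crosshair outside menu mode once it is ready.
; It also spawns an offset, tilted child actor with a face-camera rotator, and calls BCLevelCommon's MovePlayerIntoPosition with true, then false after a short delay.
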(event `CustomEvent_0`
  (params (Result :type "/Game/ReusableAssets/Utilities/BPI_PMM Interface"))
  (bind _output_get (set `self.PLM` Result))
  (`/Game/ReusableAssets/Utilities/BPI_PMM.Enable Crosshair` _output_get true false))

(event `self.ReceiveBeginPlay`
  (`|ExecutionSequence`
    (:`then_1`
      (bind _returnvalue (`AddComponent|BC_PMMAccess_C_0`))
      (add `/Game/ReusableAssets/Utilities/BC_PMMAccess.PMM Ready` _returnvalue (delegate `CustomEvent_0`))
      (`/Game/ReusableAssets/Utilities/BC_PMMAccess.Setup` _returnvalue "credits"))
    (:`then_2`
      (bind _returnvalue_2 (`AddComponent|ChildActorComponent_105` :`RelativeTransform` (`KismetMathLibrary.MakeTransform` (4444.0 0.0 4444.0) (struct :`Roll` 18.0) (1.0 1.0 1.0))))
      (`AddComponent|BP_FaceCameraRotator_C_0` :`ComponentTemplateContext` _returnvalue_2))
    (:`then_4`
      (`/Game/ReusableAssets/Utilities/BC_LevelCommon.Move Player into Position` (`self.BC_LevelCommon`) true)
      (`KismetSystemLibrary.Delay` 0.5)
      (`/Game/ReusableAssets/Utilities/BC_LevelCommon.Move Player into Position` (`self.BC_LevelCommon`) false))))

(fn `UserConstructionScript`)