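; Actor in the credits map that builds the four side faces of a box, without top or bottom, at BeginPlay.
; CreateTiledBox sizes and rotates each face from BoxSize and offsets it from the actor's location, with one material per face.
; Each face is a zero-thickness procedural mesh component filled by SetupBoxMesh.
; Its dynamic material instance gets TexCoordU set to the face's aspect ratio.
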(event `self.ReceiveBeginPlay`
  (`self.CreateTiledBox` (.location (`self.GetTransform`)) (`self.BoxSize`) (`self.TiledBoxMaterials`)))

(fn `CreateTiledBox`
  (params (Location :type "Vector Structure") (BoxSize :type "Vector Structure") (Materials :type "Array of MaterialInstance Object Reference"))
  (bind _x (.x BoxSize))
  (bind _y (.y BoxSize))
  (bind _z (.z BoxSize))
  (bind _returnvalue (`KismetMathLibrary.MakeVector2D` _x _z))
  (bind _returnvalue_2 (`KismetMathLibrary.MakeVector2D` _y _z))
  (`self.CreateTiledBoxFace` Location _returnvalue (* _y 0.5) (`KismetMathLibrary.MakeRotator` 0.0) (`KismetArrayLibrary.Array_Get` Materials))
  (`self.CreateTiledBoxFace` Location _returnvalue_2 (* _x 0.5) (`KismetMathLibrary.MakeRotator` 0.0 0.0 90.0) (`KismetArrayLibrary.Array_Get` Materials 1))
  (`self.CreateTiledBoxFace` Location _returnvalue (* _y -0.5) (`KismetMathLibrary.MakeRotator` 0.0) (`KismetArrayLibrary.Array_Get` Materials 2))
  (`self.CreateTiledBoxFace` Location _returnvalue_2 (* _x -0.5) (`KismetMathLibrary.MakeRotator` 0.0 0.0 90.0) (`KismetArrayLibrary.Array_Get` Materials 3))
  (return))

(fn `CreateTiledBoxFace`
  (params (Location :type "Vector Structure") (`Box Size` :type "Vector2D Structure") (BoxRadius :type "Float (double-precision)") (Rotation :type "Rotator Structure") (MaterialUV :type "MaterialInstance Object Reference"))
  (`self.CreateTiledRect` MaterialUV (`KismetMathLibrary.MakeTransform` (+ (`KismetMathLibrary.GreaterGreater_VectorRotator` (`KismetMathLibrary.MakeVector` BoxRadius) Rotation) Location) Rotation (1.0 1.0 1.0)) `Box Size`)
  (return))

(fn `CreateTiledRect`
  (params (MaterialInstance :type "MaterialInstance Object Reference") (RectTransform :type "Transform Structure") (`Box Size` :type "Vector2D Structure"))
  (bind (_x _y) (`KismetMathLibrary.BreakVector2D` `Box Size`))
  (bind _returnvalue (`AddComponent|ProceduralMeshComponent_3` :`RelativeTransform` RectTransform))
  (bind _returnvalue_2 (`KismetMaterialLibrary.CreateDynamicMaterialInstance` MaterialInstance))
  (`MaterialInstanceDynamic.SetScalarParameterValue` _returnvalue_2 "TexCoordU" (/ _x _y))
  (`/Game/ReusableAssets/Utilities/LIB_Utilities.Setup Box Mesh` _returnvalue (`KismetMathLibrary.MakeVector` 0.0 _x _y) _returnvalue_2)
  (return))

(fn `UserConstructionScript`)