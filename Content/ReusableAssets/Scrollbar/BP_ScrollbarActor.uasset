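; World-space scrollbar actor that acts as a titled, identifiable slider driven by crosshair mouse clicks and scroll wheel.
; Clicks off the thumb convert the hit to local Y and wheel steps nudge the value, which is clamped to 0–1 before firing ScrollbarChanged.
; The thumb moves along cached Box bounds inside a margin, and a text readout shows the value remapped to the Min/Max range.
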(event EventBeginPlay
  (CallFunction|UpdateCache)
  (CallFunction|UpdateScrollbar))

(fn ConstructionScript
  (bind _returnvalue (Rendering|Material|CreateDynamicMaterialInstance "/Game/ReusableAssets/Materials/MT_Opaque.MT_Opaque" :!class /Script/Engine.KismetMaterialLibrary))
  (bind _output_get (Variables|Default|SetThumb%20MID _returnvalue))
  (Rendering|Material|SetVectorParameterValue _output_get "Color" "(R=0.525000,G=0.000000,B=0.244571,A=1.000000)" :!class /Script/Engine.MaterialInstanceDynamic)
  (Rendering|Material|SetMaterial (Variables|Default|GetThumb) 0 (Variables|Default|GetThumb%20MID)))

(fn UpdateScrollbar
  (bind _thumb (Variables|Default|GetThumb))
  (bind _relativelocation (Variables|/Script/Engine.SceneComponent|GetRelativeLocation _thumb))
  (Utilities|FlowControl|Sequence
    (:then_0
      (Transformation|SetRelativeLocation (Variables|Default|GetThumb) (Math|Vector|MakeVector (.x _relativelocation) (+ (* (Variables|Default|GetScrollbar%20Width) (Variables|Default|GetValue)) (Variables|Default|GetMin%20Y%20Offset)) (.z _relativelocation)) false false))
    (:then_1
      (Rendering|Components|TextRender|SetText (Variables|Default|GetIndex%20Text) (Utilities|Text|ToText(String) (CallFunction|FloattoString (CallFunction|GetSliderValue false) 2))))))

(fn UpdateCache
  (bind _box (Variables|Default|GetBox))
  (bind (_min _max) (Components|StaticMesh|GetLocalBounds _box))
  (Variables|Default|SetScrollbar%20Width (- (.y (- _max _min)) (* (Variables|Default|GetMargin) 2.0)))
  (Variables|Default|SetMin%20Y%20Offset (+ (.Y (Math|Vector|BreakVector _min)) (Variables|Default|GetMargin))))

(fn UpdateValue
  (params (New%20Value :type Float%20%28single-precision%29 :default 0.0))
  (Variables|Default|SetValue (Math|Float|Clamp(Float) New%20Value))
  (CallFunction|UpdateScrollbar)
  (Default|CallScrollbarChanged))

(fn Setup
  (params (Title :type String) (Min :type Float%20%28single-precision%29 :default 0.0) (Max :type Float%20%28single-precision%29 :default 0.0) (Value :type Float%20%28single-precision%29 :default 0.0) (ID :type String))
  (Rendering|Components|TextRender|SetText (Variables|Default|GetTitle) (Utilities|Text|ToText(String) Title))
  (Variables|Default|SetMin%20Value Min)
  (Variables|Default|SetMax%20Value Max)
  (CallFunction|SetSliderValue false Value)
  (Variables|Default|SetIdentifier ID))

(fn GetSliderValue
  (params (Normalized :type Boolean :default false))
  (if Normalized
    (LocalVariables|SetResult (Variables|Default|GetValue))
    (else
      (LocalVariables|SetResult (Math|Float|MapRangeUnclamped (Variables|Default|GetValue) 0.0 1.0 (Variables|Default|GetMin%20Value) (Variables|Default|GetMax%20Value)))))
  (return (LocalVariables|GetResult)))

(fn SetSliderValue
  (params (Normalized :type Boolean :default false) (New%20Value :type Float%20%28single-precision%29 :default 0.0))
  (if Normalized
    (Variables|Default|SetValue New%20Value)
    (else
      (Variables|Default|SetValue (Math|Float|MapRangeUnclamped New%20Value (Variables|Default|GetMin%20Value) (Variables|Default|GetMax%20Value) 0.0 1.0))))
  (CallFunction|UpdateScrollbar))

(fn GetIdentifier
  (return (Variables|Default|GetIdentifier)))

(fn CrosshairHoverMoved
  (params (Hit%20Location :type Vector :default "0, 0, 0"))
  (return false))

(fn CrosshairHoverProgress
  (params (Progress :type Float%20%28single-precision%29) (Local%20Hit%20Location :type Vector :default "0, 0, 0") (Hit%20Component :type Primitive%20Component%20Object%20Reference))
  (return false))

(fn CrosshairHoverStart
  (params (Finished :type Boolean))
  (return false))

(fn CrosshairLeftRight
  (params (Left :type Boolean))
  (return false))

(fn CrosshairMouseClick
  (params (Mouse%20Down :type Boolean) (Event%20Type :type E_EventType%20Enum :default "NewEnumerator0") (Hit%20Location :type Vector :default "0, 0, 0") (Hit%20Component :type Primitive%20Component%20Object%20Reference))
  (Utilities|FlowControl|Sequence
    (:then_0
      (if Mouse%20Down
        (if (not (== Hit%20Component (Variables|Default|GetThumb)))
          (CallFunction|UpdateValue (/ (- (.y (Math|Transform|InverseTransformLocation (Transformation|GetActorTransform) Hit%20Location)) (Variables|Default|GetMin%20Y%20Offset)) (Variables|Default|GetScrollbar%20Width))))))
    (:then_1
      (return false))))

(fn CrosshairScrollWheel
  (params (Down :type Boolean) (Hit%20Location :type Vector :default "0, 0, 0") (Hit%20Component :type Primitive%20Component%20Object%20Reference))
  (if Down
    (LocalVariables|SetIncrement 0.05)
    (else
      (LocalVariables|SetIncrement -0.05)))
  (CallFunction|UpdateValue (+ (Variables|Default|GetValue) (LocalVariables|GetIncrement)))
  (return false))

(fn CrosshairUpDown
  (params (Up :type Boolean))
  (return false))