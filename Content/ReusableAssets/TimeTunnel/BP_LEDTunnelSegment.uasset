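; BP_LEDTunnelSegment is one ring of LEDs in a time tunnel that blinks in an alternating pattern or lights up entirely when selected.
; Setup adds zero-scale dim, bright and selected instances around a circle to three supplied instanced mesh components.
; A looping timer flips the modulo pattern choosing bright or dim LEDs, pausing visual updates while selected.
; States switch by rescaling instances, skipping those whose visibility is unchanged.
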(event Custom|BlinkLights
  (Utilities|FlowControl|Sequence
    (:then_0
      (if (not (Variables|Default|GetSelected))
        (CallFunction|UpdateMaterials)))
    (:then_1
      (Variables|Default|SetToggle (not (Variables|Default|GetToggle))))))

(event EventBeginPlay
  (Utilities|Time|SetTimerbyFunctionName 0 "BlinkLights" 0.5 true))

(fn ConstructionScript)

(fn Select
  (params (Select :type Boolean :default false))
  (bind _output_get (Variables|Default|SetSelected Select))
  (if _output_get
    (for _index (range 0 (Utilities|Array|LastIndex (Variables|Default|GetDim%20CLEDs)))
      (CallFunction|ShowInstance (Variables|Default|GetDim%20SIM) false (Utilities|Array|Get(acopy) (Variables|Default|GetDim%20CLEDs) _index))
      (CallFunction|ShowInstance (Variables|Default|GetBright%20SIM) false (Utilities|Array|Get(acopy) (Variables|Default|GetBright%20CLEDs) _index))
      (CallFunction|ShowInstance (Variables|Default|GetSelected%20SIM) true (Utilities|Array|Get(acopy) (Variables|Default|GetSelected%20CLEDs) _index)))
    (else
      (CallFunction|UpdateMaterials))))

(fn UpdateMaterials
  (Utilities|FlowControl|Sequence
    (:then_0
      (if (Variables|Default|GetToggle)
        (Default|UpdateParams (Variables|Default|GetC_LEDPatternFormula) 3)
        (else
          (Default|UpdateParams (Variables|Default|GetC_LEDPatternFormula) 3 1))))
    (:then_2
      (for _index (range 0 (Utilities|Array|LastIndex (Variables|Default|GetDim%20CLEDs)))
        (bind _result (Default|ShouldHighlightIndex (Variables|Default|GetC_LEDPatternFormula) _index))
        (if _result
          (CallFunction|ShowInstance (Variables|Default|GetDim%20SIM) false (Utilities|Array|Get(acopy) (Variables|Default|GetDim%20CLEDs) _index))
          (CallFunction|ShowInstance (Variables|Default|GetBright%20SIM) true (Utilities|Array|Get(acopy) (Variables|Default|GetBright%20CLEDs) _index))
          (CallFunction|ShowInstance (Variables|Default|GetSelected%20SIM) false (Utilities|Array|Get(acopy) (Variables|Default|GetSelected%20CLEDs) _index))
          (else
            (CallFunction|ShowInstance (Variables|Default|GetDim%20SIM) true (Utilities|Array|Get(acopy) (Variables|Default|GetDim%20CLEDs) _index))
            (CallFunction|ShowInstance (Variables|Default|GetBright%20SIM) false (Utilities|Array|Get(acopy) (Variables|Default|GetBright%20CLEDs) _index))
            (CallFunction|ShowInstance (Variables|Default|GetSelected%20SIM) false (Utilities|Array|Get(acopy) (Variables|Default|GetSelected%20CLEDs) _index))))))))

(fn Setup
  (params (Dim :type Instanced%20Static%20Mesh%20Component%20Object%20Reference) (Bright :type Instanced%20Static%20Mesh%20Component%20Object%20Reference) (Selected :type Instanced%20Static%20Mesh%20Component%20Object%20Reference) (XOffset :type Float%20%28single-precision%29))
  (Utilities|FlowControl|Sequence
    (:then_1
      (Variables|Default|SetBright%20SIM Bright)
      (Variables|Default|SetDim%20SIM Dim)
      (Variables|Default|SetSelected%20SIM Selected))
    (:then_2
      (for _index (range 0 (- (Variables|Default|GetNumber%20of%20Lights) 1))
        (Utilities|FlowControl|Sequence
          (:then_0
            (bind _returnvalue (Components|InstancedStaticMesh|AddInstance (Variables|Default|GetDim%20SIM) (Math|Transform|MakeTransform (Math|Vector|MakeVector XOffset (.y (.Location (CallFunction|LocationAroundCircle _index (Variables|Default|GetNumber%20of%20Lights) (Variables|Default|GetRadius) "1.000000,0.000000,0.000000" 0.0))) (.z (.Location (CallFunction|LocationAroundCircle _index (Variables|Default|GetNumber%20of%20Lights) (Variables|Default|GetRadius) "1.000000,0.000000,0.000000" 0.0)))) "0, 0, 0" "0.000000,0.000000,0.000000")))
            (bind _returnvalue_2 (AddComponent|AddBCLEDState))
            (Variables|/Game/ReusableAssets/TimeTunnel/BC_LEDState.BC_LEDState_C|SetInstance%20Index _returnvalue_2 _returnvalue)
            (Variables|/Game/ReusableAssets/TimeTunnel/BC_LEDState.BC_LEDState_C|SetLocation _returnvalue_2 (.Location (Math|Transform|BreakTransform (Math|Transform|MakeTransform (Math|Vector|MakeVector XOffset (.y (.Location (CallFunction|LocationAroundCircle _index (Variables|Default|GetNumber%20of%20Lights) (Variables|Default|GetRadius) "1.000000,0.000000,0.000000" 0.0))) (.z (.Location (CallFunction|LocationAroundCircle _index (Variables|Default|GetNumber%20of%20Lights) (Variables|Default|GetRadius) "1.000000,0.000000,0.000000" 0.0)))) "0, 0, 0" "0.000000,0.000000,0.000000"))))
            (Utilities|Array|Add (Variables|Default|GetDim%20CLEDs) _returnvalue_2))
          (:then_1
            (bind _returnvalue_3 (Components|InstancedStaticMesh|AddInstance (Variables|Default|GetBright%20SIM) (Math|Transform|MakeTransform (Math|Vector|MakeVector XOffset (.y (.Location (CallFunction|LocationAroundCircle _index (Variables|Default|GetNumber%20of%20Lights) (Variables|Default|GetRadius) "1.000000,0.000000,0.000000" 0.0))) (.z (.Location (CallFunction|LocationAroundCircle _index (Variables|Default|GetNumber%20of%20Lights) (Variables|Default|GetRadius) "1.000000,0.000000,0.000000" 0.0)))) "0, 0, 0" "0.000000,0.000000,0.000000")))
            (bind _returnvalue_4 (AddComponent|AddBCLEDState))
            (Variables|/Game/ReusableAssets/TimeTunnel/BC_LEDState.BC_LEDState_C|SetInstance%20Index _returnvalue_4 _returnvalue_3)
            (Variables|/Game/ReusableAssets/TimeTunnel/BC_LEDState.BC_LEDState_C|SetLocation _returnvalue_4 (.Location (Math|Transform|BreakTransform (Math|Transform|MakeTransform (Math|Vector|MakeVector XOffset (.y (.Location (CallFunction|LocationAroundCircle _index (Variables|Default|GetNumber%20of%20Lights) (Variables|Default|GetRadius) "1.000000,0.000000,0.000000" 0.0))) (.z (.Location (CallFunction|LocationAroundCircle _index (Variables|Default|GetNumber%20of%20Lights) (Variables|Default|GetRadius) "1.000000,0.000000,0.000000" 0.0)))) "0, 0, 0" "0.000000,0.000000,0.000000"))))
            (Utilities|Array|Add (Variables|Default|GetBright%20CLEDs) _returnvalue_4))
          (:then_2
            (bind _returnvalue_5 (Components|InstancedStaticMesh|AddInstance (Variables|Default|GetSelected%20SIM) (Math|Transform|MakeTransform (Math|Vector|MakeVector XOffset (.y (.Location (CallFunction|LocationAroundCircle _index (Variables|Default|GetNumber%20of%20Lights) (Variables|Default|GetRadius) "1.000000,0.000000,0.000000" 0.0))) (.z (.Location (CallFunction|LocationAroundCircle _index (Variables|Default|GetNumber%20of%20Lights) (Variables|Default|GetRadius) "1.000000,0.000000,0.000000" 0.0)))) "0, 0, 0" "0.000000,0.000000,0.000000")))
            (bind _returnvalue_6 (AddComponent|AddBCLEDState))
            (Variables|/Game/ReusableAssets/TimeTunnel/BC_LEDState.BC_LEDState_C|SetInstance%20Index _returnvalue_6 _returnvalue_5)
            (Variables|/Game/ReusableAssets/TimeTunnel/BC_LEDState.BC_LEDState_C|SetLocation _returnvalue_6 (.Location (Math|Transform|BreakTransform (Math|Transform|MakeTransform (Math|Vector|MakeVector XOffset (.y (.Location (CallFunction|LocationAroundCircle _index (Variables|Default|GetNumber%20of%20Lights) (Variables|Default|GetRadius) "1.000000,0.000000,0.000000" 0.0))) (.z (.Location (CallFunction|LocationAroundCircle _index (Variables|Default|GetNumber%20of%20Lights) (Variables|Default|GetRadius) "1.000000,0.000000,0.000000" 0.0)))) "0, 0, 0" "0.000000,0.000000,0.000000"))))
            (Utilities|Array|Add (Variables|Default|GetSelected%20CLEDs) _returnvalue_6)))))
    (:then_3
      (CallFunction|UpdateMaterials))))

(fn ShowInstance
  (params (Instances :type Instanced%20Static%20Mesh%20Component%20Object%20Reference) (Show :type Boolean) (CLED :type BC%20LED%20State%20Object%20Reference))
  (if (not (Math|Boolean|Equal(Boolean) (Variables|/Game/ReusableAssets/TimeTunnel/BC_LEDState.BC_LEDState_C|GetVisible CLED) Show))
    (Utilities|FlowControl|Sequence
      (:then_0
        (if Show
          (LocalVariables|SetScale "12.000000,12.000000,12.000000")))
      (:then_1
        (Components|InstancedStaticMesh|UpdateInstanceTransform Instances (Variables|/Game/ReusableAssets/TimeTunnel/BC_LEDState.BC_LEDState_C|GetInstance%20Index CLED) (Math|Transform|MakeTransform (Variables|/Game/ReusableAssets/TimeTunnel/BC_LEDState.BC_LEDState_C|GetLocation CLED) "0, 0, 0" (LocalVariables|GetScale)) false true)
        (Variables|/Game/ReusableAssets/TimeTunnel/BC_LEDState.BC_LEDState_C|SetVisible CLED Show)))))