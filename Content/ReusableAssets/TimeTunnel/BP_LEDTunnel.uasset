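; BP_LEDTunnel builds a time-tunnel LED corridor at BeginPlay and animates light pulses running along it.
; It spawns evenly spaced BP_LEDTunnelSegment child actors, all sharing three instanced static mesh components for dim, bright and selected materials.
; A fast looping timer steps two decrementing selection patterns and tells each segment whether it is selected.
; The particle system is moved to roughly 30% along the tunnel.
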(event `self.ReceiveBeginPlay`
  (`|ExecutionSequence`
    (:`then_0`
      (`self.Setup Tunnel`))
    (:`then_1`
      (`KismetSystemLibrary.K2_SetTimer` null "SelectSegment" 0.025 true)
      (`SceneComponent.K2_SetRelativeLocation` (`self.ParticleSystem`) (`self.Emitter Location`) false false))))

(event `SelectSegment`
  (`|ExecutionSequence`
    (:`then_0`
      (`/Game/ReusableAssets/TimeTunnel/C_LEDSelectionPattern.Next` (`self.SelectionPattern1`))
      (`/Game/ReusableAssets/TimeTunnel/C_LEDSelectionPattern.Next` (`self.SelectionPattern2`)))
    (:`then_1`
      (for (_array_element _array_index) (`self.Segments`)
        (bind _index (`/Game/ReusableAssets/TimeTunnel/C_LEDSelectionPattern.Current` (`self.SelectionPattern1`)))
        (bind _index_2 (`/Game/ReusableAssets/TimeTunnel/C_LEDSelectionPattern.Current` (`self.SelectionPattern2`)))
        (`/Game/ReusableAssets/TimeTunnel/BP_LEDTunnelSegment.Select` _array_element (or (== _index_2 _array_index) (== _index _array_index)))))))

(fn `Setup Tunnel`
  (bind _number_of_segments (`self.Number of Segments`))
  (`|ExecutionSequence`
    (:`then_0`
      (bind _returnvalue (`AddComponent|Instanced Static Mesh Component_0`))
      (bind _output_get (set `self.Dim Static Meshes` _returnvalue))
      (`PrimitiveComponent.SetMaterial` _output_get 0 "/Game/ReusableAssets/TimeTunnel/MT_LEDTunnel.MT_LEDTunnel"))
    (:`then_1`
      (bind _returnvalue_2 (`AddComponent|InstancedStaticMeshComponent_1`))
      (bind _output_get_2 (set `self.Selected Static Meshes` _returnvalue_2))
      (bind _returnvalue_3 (`KismetMaterialLibrary.CreateDynamicMaterialInstance` "/Game/ReusableAssets/TimeTunnel/MT_LEDTunnel.MT_LEDTunnel"))
      (`MaterialInstanceDynamic.SetScalarParameterValue` _returnvalue_3 "Emission" 22.0)
      (`PrimitiveComponent.SetMaterial` _output_get_2 0 _returnvalue_3))
    (:`then_2`
      (bind _returnvalue_4 (`AddComponent|InstancedStaticMeshComponent_2`))
      (bind _output_get_3 (set `self.Bright Static Meshes` _returnvalue_4))
      (bind _returnvalue_5 (`KismetMaterialLibrary.CreateDynamicMaterialInstance` "/Game/ReusableAssets/TimeTunnel/MT_LEDTunnel.MT_LEDTunnel"))
      (`MaterialInstanceDynamic.SetVectorParameterValue` _returnvalue_5 "Color" (struct :`R` 0.110026 :`G` 0.338758 :`B` 0.48 :`A` 1.0))
      (`MaterialInstanceDynamic.SetScalarParameterValue` _returnvalue_5 "Emission" 22.0)
      (`PrimitiveComponent.SetMaterial` _output_get_3 0 _returnvalue_5))
    (:`then_4`
      (for _index (range (`self.Number of Segments`))
        (bind _returnvalue_6 (`KismetMathLibrary.Conv_IntToDouble` (* _index 888)))
        (bind _returnvalue_7 (`KismetMathLibrary.MakeVector` _returnvalue_6))
        (bind _returnvalue_8 (`AddComponent|Child Actor Component_21` :`RelativeTransform` (`KismetMathLibrary.MakeTransform` _returnvalue_7)))
        (bind _asbp_ledtunnel_segment (cast `/Game/ReusableAssets/TimeTunnel/BP_LEDTunnelSegment` (`ChildActorComponent.ChildActor` _returnvalue_8)))
        (`KismetArrayLibrary.Array_Add` (`self.Segments`) _asbp_ledtunnel_segment)
        (`/Game/ReusableAssets/TimeTunnel/BP_LEDTunnelSegment.Setup` _asbp_ledtunnel_segment (`self.Dim Static Meshes`) (`self.Bright Static Meshes`) (`self.Selected Static Meshes`) _returnvalue_6)
        (if (== _index (`KismetMathLibrary.FFloor` (* (`self.Number of Segments`) 0.3)))
          (set `self.Emitter Location` _returnvalue_7))))
    (:`then_5`
      (`/Game/ReusableAssets/TimeTunnel/C_LEDSelectionPattern.Setup` (`self.SelectionPattern2`) 0 _number_of_segments -1)
      (`/Game/ReusableAssets/TimeTunnel/C_LEDSelectionPattern.Setup` (`self.SelectionPattern1`) 1 _number_of_segments -1))))

(fn `UserConstructionScript`)