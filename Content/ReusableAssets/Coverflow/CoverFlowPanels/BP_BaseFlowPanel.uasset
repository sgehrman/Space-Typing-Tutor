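; Base panel actor for the CoverFlow carousel, showing title, description and footer text with an index and identifier.
; Forwards crosshair click, scroll and directional input to the CoverFlow cached on BeginPlay, honoring its horizontal or vertical layout.
; Move and animate-out functions hand off to EventGraph events, where timelines lerp relative location.
; Selection highlights the panel with custom depth and a brighter light; animate-out lifts selected panels and slides others away.
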(event `self.ReceiveBeginPlay`
  ;[1 1 1] Cache Coverflow reference for crosshair events
  (bind _ascover_flow (cast `/Game/ReusableAssets/Coverflow/CoverFlow` (`.Actor` (`/Game/ReusableAssets/Utilities/LIB_Utilities.FindActorWithTag` "/Game/ReusableAssets/Coverflow/CoverFlow.CoverFlow_C" "None" self))))
  (set `self.Parent CoverFlow` _ascover_flow))

(event `Do Animate Out`
  (params (Selected :type Boolean))
  (bind _returnvalue_location (`KismetMathLibrary.BreakTransform` (`SceneComponent.GetRelativeTransform`)))
  (bind _tmp_actor_location (`self.TMP Actor Location`))
  (bind _tmp_actor_location_2 (`self.TMP Actor Location`))
  (set `self.TMP Actor Location` _returnvalue_location)
  (if Selected
    ;[1 1 1] Selected animation
    (`GameplayStatics.SpawnEmitterAtLocation` "/Game/ReusableAssets/Coverflow/SelectPuff.SelectPuff" _tmp_actor_location_2)
    (bind (_direction _alpha) (`Timeline|AnimateOutTimer` :!via `PlayFromStart`)
      (:`Update`
        (`self.K2_SetActorRelativeLocation` (`KismetMathLibrary.VLerp` _tmp_actor_location_2 (+ _tmp_actor_location_2 (0.0 0.0 2000.0)) _alpha))))
    (else
      (`GameplayStatics.PlaySoundAtLocation` "/Game/UserInterfaceSFX/Starts/start03_Cue.start03_Cue" _tmp_actor_location (struct) 0.1)
      (bind (_direction_2 _alpha_2) (`Timeline|AnimateOutTimerOther` :!via `PlayFromStart`)
        (:`Update`
          (`self.K2_SetActorRelativeLocation` (`KismetMathLibrary.VLerp` _tmp_actor_location (+ _tmp_actor_location (12000.0 0.0 0.0)) _alpha_2)))))))

(event `Do Move Panel To`
  (params (`New Location` :type "Vector Structure" :default (0.0 0.0 0.0)) (Animate :type Boolean) (Select :type Boolean :default false) (Hide :type Boolean))
  (bind _returnvalue_location (`KismetMathLibrary.BreakTransform` (`SceneComponent.GetRelativeTransform`)))
  (bind _pointlight1 (`self.PointLight1`))
  (bind _pointlight1_2 (`self.PointLight1`))
  (`self.SetActorHiddenInGame` Hide)
  (`PrimitiveComponent.SetRenderCustomDepth` (`self.Background Mesh`) false)
  (`LightComponent.SetIntensity` _pointlight1 3333.0)
  (`LightComponent.SetLightColor` _pointlight1 (struct :`R` 0.469 :`G` 0.67 :`B` 0.67 :`A` 1.0) true)
  (if (and Animate (not Hide))
    (set `self.TMP Actor Location` _returnvalue_location)
    (`TimelineComponent.SetPlayRate` (`self.Move Panel Play Rate`))
    (if Select
      (if (`/Game/ReusableAssets/Coverflow/CoverFlow.UI Sounds Enabled` (`self.Parent CoverFlow`))
        (`GameplayStatics.PlaySoundAtLocation` "/Game/UserInterfaceSFX/Select/select03_Cue.select03_Cue" (`self.TMP Actor Location`) (struct) 0.2 0.2)
        (bind (_direction _alpha) (`Timeline|Animation` :!via `PlayFromStart` :!label _label)
          (:`Update`
            (`self.K2_SetActorRelativeLocation` (`KismetMathLibrary.VLerp` (`self.TMP Actor Location`) `New Location` _alpha)))
          (:`Finished`
            (`PrimitiveComponent.SetRenderCustomDepth` Select :!label _label_2)
            (if Select
              (`LightComponent.SetIntensity` _pointlight1_2 22222.0)
              (`LightComponent.SetLightColor` _pointlight1_2 (struct :`R` 1.0 :`G` 1.0 :`B` 1.0 :`A` 1.0) true))))
        (else
          (goto _label :!via `PlayFromStart`)))
      (else
        (goto _label :!via `PlayFromStart`)))
    (else
      (`self.K2_SetActorRelativeLocation` `New Location`)
      (goto _label_2))))

(fn `Animate Out`
  (params (Selected :type Boolean))
  (returns (Success :type Boolean))
  (`self.Do Animate Out` Selected)
  (return false))

(fn `ClearPanelButtonClickedState`
  (returns (Success :type Boolean))
  (return false))

(fn `Crosshair Hover Moved`
  (params (`Hit Location` :type "Vector Structure"))
  (returns (Success :type Boolean))
  (return false))

(fn `Crosshair Hover Progress`
  (params (Progress :type "Float (double-precision)") (`Local Hit Location` :type "Vector Structure") (`Hit Component` :type "PrimitiveComponent Object Reference"))
  (returns (`Auto Click On Progress` :type Boolean))
  (return false))

(fn `Crosshair Hover Start`
  (params (Finished :type Boolean))
  (returns (Success :type Boolean))
  (bind _parent_coverflow (`self.Parent CoverFlow`))
  ;[1 1 1] Just needed for Gamepad A button, mouse is diff
  (if Finished
    (set `/Game/ReusableAssets/Coverflow/CoverFlow.Clicked on Panel Index` 0 _parent_coverflow)
    (else
      (set `/Game/ReusableAssets/Coverflow/CoverFlow.Clicked on Panel Index` (`self.PanelIndex`) _parent_coverflow)))
  (return true))

(fn `Crosshair LeftRight`
  (params (Left :type Boolean))
  (returns (Success :type Boolean))
  (bind _parent_coverflow (`self.Parent CoverFlow`))
  (`|ExecutionSequence`
    (:`then_0`
      ;[1 1 1] Ignore if vertical
      (if (`/Game/ReusableAssets/Coverflow/CoverFlow.Vertical Layout` (`self.Parent CoverFlow`))
        _
        (elif Left
          (`/Game/ReusableAssets/Coverflow/CoverFlow.Handle Move Right Input` _parent_coverflow -1.0 false 200)
          (else
            (`/Game/ReusableAssets/Coverflow/CoverFlow.Handle Move Right Input` _parent_coverflow 1.0 false 200)))))
    (:`then_1`
      (return false))))

(fn `Crosshair Mouse Click`
  (params (`Mouse Down` :type Boolean) (`Event Type` :type "/Game/ReusableAssets/Utilities/E_EventType Enum" :default "NewEnumerator0") (`Hit Location` :type "Vector Structure") (`Hit Component` :type "PrimitiveComponent Object Reference"))
  (returns (Success :type Boolean))
  (`/Game/ReusableAssets/Coverflow/CoverFlow.HandleCrosshairLeftMouse` (`self.Parent CoverFlow`) (`self.PanelIndex`) `Mouse Down`)
  (return false))

(fn `Crosshair Scroll Wheel`
  (params (Down :type Boolean) (`Hit Location` :type "Vector Structure") (`Hit Component` :type "PrimitiveComponent Object Reference"))
  (returns (Success :type Boolean))
  (bind _parent_coverflow (`self.Parent CoverFlow`))
  (`|ExecutionSequence`
    (:`then_0`
      (if Down
        (`/Game/ReusableAssets/Coverflow/CoverFlow.Handle Move Right Input` _parent_coverflow 1.0 false 200)
        (else
          (`/Game/ReusableAssets/Coverflow/CoverFlow.Handle Move Right Input` _parent_coverflow -1.0 false 200))))
    (:`then_1`
      (return false))))

(fn `Crosshair UpDown`
  (params (Up :type Boolean))
  (returns (Success :type Boolean))
  (bind _parent_coverflow (`self.Parent CoverFlow`))
  (`|ExecutionSequence`
    (:`then_0`
      ;[1 1 1] Ignore if not vertical
      (if (`/Game/ReusableAssets/Coverflow/CoverFlow.Vertical Layout` (`self.Parent CoverFlow`))
        (if Up
          (`/Game/ReusableAssets/Coverflow/CoverFlow.Handle Move Right Input` _parent_coverflow 1.0 false 200)
          (else
            (`/Game/ReusableAssets/Coverflow/CoverFlow.Handle Move Right Input` _parent_coverflow -1.0 false 200)))))
    (:`then_1`
      (return false))))

(fn `Get Identifier`
  (returns (Identifier :type String))
  (return (`self.Identifier`)))

(fn `Get Index`
  (returns (Index :type Integer))
  (return (`self.PanelIndex`)))

(fn `Get Size`
  (returns (Size :type "Vector Structure"))
  (return (* (`.BoxExtent` (`KismetSystemLibrary.GetComponentBounds` (`self.Background Mesh`))) 2.0)))

(fn `Move Panel To`
  (params (Location :type "Vector Structure") (Animate :type Boolean) (Select :type Boolean) (Hide :type Boolean))
  (returns (Success :type Boolean))
  (`self.Do Move Panel To` Location Animate Select Hide)
  (return false))

(fn `Set Info`
  (params (Index :type Integer) (Title :type String) (Description :type String) (`Description Two` :type String) (Info :type String) (Identifier :type String))
  (returns (Success :type Boolean))
  (`|ExecutionSequence`
    (:`then_0`
      (`TextRenderComponent.K2_SetText` (`self.FooterText`) (`KismetTextLibrary.Conv_StringToText` Info)))
    (:`then_1`
      (set `self.PanelIndex` Index))
    (:`then_2`
      (`TextRenderComponent.K2_SetText` (`self.DescriptionText`) (`KismetTextLibrary.Conv_StringToText` Description)))
    (:`then_3`
      (`TextRenderComponent.K2_SetText` (`self.DescriptionText2`) (`KismetTextLibrary.Conv_StringToText` `Description Two`)))
    (:`then_4`
      (`TextRenderComponent.K2_SetText` (`self.TitleText`) (`KismetTextLibrary.Conv_StringToText` Title)))
    (:`then_5`
      (set `self.Identifier` Identifier))
    (:`then_6`
      (return true))))

(fn `UserConstructionScript`)