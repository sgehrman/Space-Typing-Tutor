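; BP_ListFlow is a cover flow panel that carries an assign toggle button.
; Construction caches the BP_ToggleButton child actor as AssignButton and switches it off.
; User clicks on the button send its on state and the panel's index to the parent cover flow's click delegate.
; A clear function resets the button to off.
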(event `self.ReceiveBeginPlay`
  (`parent.ReceiveBeginPlay`)
  (add `/Game/ReusableAssets/Buttons/BP_ToggleButton.ButtonClickedByUser` (`self.Assign Button`) (delegate `AssignButtonClicked`)))

(event `AssignButtonClicked`
  (params (`Button ID` :type String) (`Hit Location` :type "Vector Structure"))
  (bind _index (`self.Get Index`))
  (`/Game/ReusableAssets/Coverflow/CoverFlow.SendPanelButtonClickToDelegate` (`self.Parent CoverFlow`) (`/Game/ReusableAssets/Buttons/BP_ToggleButton.On State` (`self.Assign Button`)) _index))

(fn `ClearPanelButtonClickedState`
  (returns (Success :type Boolean))
  (`/Game/ReusableAssets/Buttons/BP_ToggleButton.Set State` (`self.Assign Button`) false)
  (return false))

(fn `UserConstructionScript`
  (`parent.UserConstructionScript`)
  (bind _asbp_toggle_button (cast `/Game/ReusableAssets/Buttons/BP_ToggleButton` (`ChildActorComponent.ChildActor` (`self.Assign Mode Button Actor`))))
  (bind _output_get (set `self.Assign Button` _asbp_toggle_button))
  (`/Game/ReusableAssets/Buttons/BP_ToggleButton.Set State` _output_get false))