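; Scrollbar actor for a CoverFlow, showing the selected index with a sliding thumb and text label.
; On BeginPlay it finds the CoverFlow actor and binds to its change event, refreshing thumb and label on each change.
; Slot width comes from the box bounds divided by item count, recalculated only when that count changes.
; Crosshair hover progress maps local hit Y to a slot, updating the selection and triggering a relayout.
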(event `self.ReceiveBeginPlay`
  (`|ExecutionSequence`
    (:`then_0`
      (bind _ascover_flow (cast `/Game/ReusableAssets/Coverflow/CoverFlow` (`.Actor` (`/Game/ReusableAssets/Utilities/LIB_Utilities.FindActorWithTag` "/Game/ReusableAssets/Coverflow/CoverFlow.CoverFlow_C" "None" self))))
      (set `self.CachedCoverflow` _ascover_flow))
    (:`then_1`
      ;[1 1 1] Setup scrollbar to get updates
      (add `/Game/ReusableAssets/Coverflow/CoverFlow.CoverflowChangedEvent` (`self.CachedCoverflow`) (delegate `UpdateScrollBarForCoverflowChange`))
      (`self.UpdateCache` :!label _label)
      (`self.UpdateScrollbar`))))

(event `UpdateScrollBarForCoverflowChange`
  ;[1 1 1] Setup scrollbar to get updates
  (goto _label))

(fn `Crosshair Hover Moved`
  (params (`Hit Location` :type "Vector Structure"))
  (returns (Success :type Boolean))
  (return false))

(fn `Crosshair Hover Progress`
  (params (Progress :type "Float (double-precision)") (`Local Hit Location` :type "Vector Structure") (`Hit Component` :type "PrimitiveComponent Object Reference"))
  (returns (`Auto Click On Progress` :type Boolean))
  (bind _cachedcoverflow (`self.CachedCoverflow`))
  (bind (_cachedboxmin_x _cachedboxmin_y) (`KismetMathLibrary.BreakVector` (`self.CachedBoxMin`)))
  (bind _returnvalue (`KismetMathLibrary.FFloor` (/ (- `Local Hit Location_Y` _cachedboxmin_y) (`self.CachedSlotWidth`))))
  (`|ExecutionSequence`
    (:`then_0`
      (if (!= _returnvalue (`/Game/ReusableAssets/Coverflow/CoverFlow.Selected Index` (`self.CachedCoverflow`)))
        (set `/Game/ReusableAssets/Coverflow/CoverFlow.Selected Index` _returnvalue _cachedcoverflow)
        (`/Game/ReusableAssets/Coverflow/CoverFlow.Relayout Event` _cachedcoverflow true)))
    (:`then_1`
      (return false))))

(fn `Crosshair Hover Start`
  (params (Finished :type Boolean))
  (returns (Success :type Boolean))
  (return false))

(fn `Crosshair LeftRight`
  (params (Left :type Boolean))
  (returns (Success :type Boolean))
  (return false))

(fn `Crosshair Mouse Click`
  (params (`Mouse Down` :type Boolean) (`Event Type` :type "/Game/ReusableAssets/Utilities/E_EventType Enum" :default "NewEnumerator0") (`Hit Location` :type "Vector Structure") (`Hit Component` :type "PrimitiveComponent Object Reference"))
  (returns (Success :type Boolean))
  (return false))

(fn `Crosshair Scroll Wheel`
  (params (Down :type Boolean) (`Hit Location` :type "Vector Structure") (`Hit Component` :type "PrimitiveComponent Object Reference"))
  (returns (Success :type Boolean))
  (return false))

(fn `Crosshair UpDown`
  (params (Up :type Boolean))
  (returns (Success :type Boolean))
  (return false))

(fn `UpdateCache`
  (bind (_min _max) (`StaticMeshComponent.GetLocalBounds` (`self.Box`)))
  (bind _item_count (`/Game/ReusableAssets/Coverflow/CoverFlow.Item Count` (`self.CachedCoverflow`)))
  (if (not (== (`self.CachedItemCount`) _item_count))
    (set `self.CachedItemCount` _item_count)
    (set `self.CachedBoxMin` _min)
    (set `self.CachedBoxMax` _max)
    (set `self.CachedSlotWidth` (/ (.y (- (`self.CachedBoxMax`) (`self.CachedBoxMin`))) (`KismetMathLibrary.Conv_IntToDouble` (`/Game/ReusableAssets/Coverflow/CoverFlow.Item Count` (`self.CachedCoverflow`)))))))

(fn `UpdateScrollbar`
  (bind _cachedslotwidth (`self.CachedSlotWidth`))
  (bind (_cachedboxmin_x _cachedboxmin_y) (`KismetMathLibrary.BreakVector` (`self.CachedBoxMin`)))
  (bind (_relativelocation_x _relativelocation_y _relativelocation_z) (`KismetMathLibrary.BreakVector` (`SceneComponent.RelativeLocation` (`self.Thumb`))))
  (`|ExecutionSequence`
    (:`then_0`
      ;[1 1 1] Position Thumb
      (`SceneComponent.K2_SetRelativeLocation` (`self.Thumb`) (`KismetMathLibrary.MakeVector` _relativelocation_x (+ (+ (* (`/Game/ReusableAssets/Coverflow/CoverFlow.Selected Index` (`self.CachedCoverflow`)) _cachedslotwidth) (/ _cachedslotwidth 2.0)) _cachedboxmin_y) _relativelocation_z) false false))
    (:`then_1`
      (`TextRenderComponent.K2_SetText` (`self.Index Text`) (`KismetTextLibrary.Conv_IntToText` (`/Game/ReusableAssets/Coverflow/CoverFlow.Selected Index` (`self.CachedCoverflow`)))))))

(fn `UserConstructionScript`)