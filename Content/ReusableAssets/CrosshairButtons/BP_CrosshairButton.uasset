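; BP_CrosshairButton is an actor that responds to crosshair interaction, apparently as a reusable base for in-world buttons.
; On BeginPlay it finds and caches the CrosshairActor.
; Hover start resets that actor's progress to zero, and hover progress forwards the current value to it.
; Hover move, click, scroll and directional handlers are empty stubs, and every handler returns false.
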(event `self.ReceiveBeginPlay`
  (bind _ascrosshair_actor (cast `/Game/ReusableAssets/Crosshair/CrosshairActor` (`.Actor` (`/Game/ReusableAssets/Utilities/LIB_Utilities.FindActorWithTag` "/Game/ReusableAssets/Crosshair/CrosshairActor.CrosshairActor_C" "None" self))))
  (set `self.CrosshairActor` _ascrosshair_actor))

(event `self.ReceiveActorBeginOverlap`
  (params (OtherActor :type "Actor Object Reference")))

(event `self.ReceiveTick`
  (params (DeltaSeconds :type "Float (single-precision)")))

(fn `Crosshair Hover Moved`
  (params (`Hit Location` :type "Vector Structure"))
  (returns (Success :type Boolean))
  (return false))

(fn `Crosshair Hover Progress`
  (params (Progress :type "Float (double-precision)") (`Local Hit Location` :type "Vector Structure") (`Hit Component` :type "PrimitiveComponent Object Reference"))
  (returns (`Auto Click On Progress` :type Boolean))
  (`/Game/ReusableAssets/Crosshair/CrosshairActor.UpdateProgress` (`self.CrosshairActor`) Progress)
  (return false))

(fn `Crosshair Hover Start`
  (params (Finished :type Boolean))
  (returns (Success :type Boolean))
  (`/Game/ReusableAssets/Crosshair/CrosshairActor.UpdateProgress` (`self.CrosshairActor`) 0.0)
  (return false))

(fn `Crosshair LeftRight`
  (params (Left :type Boolean))
  (returns (Success :type Boolean))
  (return false))

(fn `Crosshair Mouse Click`
  (params (`Mouse Down` :type Boolean) (`Event Type` :type "/Game/ReusableAssets/Utilities/E_EventType Enum" :default "NewEnumerator10") (`Hit Location` :type "Vector Structure") (`Hit Component` :type "PrimitiveComponent Object Reference"))
  (returns (Success :type Boolean))
  (return false))

(fn `Crosshair Scroll Wheel`
  (params (Down :type Boolean) (`Hit Location` :type "Vector Structure") (`Hit Component` :type "PrimitiveComponent Object Reference"))
  (returns (Success :type Boolean))
  (return false))

(fn `Crosshair UpDown`
  (params (Up :type Boolean))
  (returns (Success :type Boolean))
  (return false))

(fn `UserConstructionScript`)