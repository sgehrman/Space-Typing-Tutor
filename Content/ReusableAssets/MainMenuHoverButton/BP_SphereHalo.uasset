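; BP_SphereHalo is an actor that displays an animated ring of spheres, apparently for main menu hover buttons.
; The construction script calls BuildHalo, which clears SphereContainer's children and adds mesh components spaced around a circle on the X axis, using configurable count, radius and scale.
; On BeginPlay, the ScaleAnimation timeline lerps the actor's current scale toward a uniform value mapped between one and AnimationScaleMax.
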(event `self.ReceiveBeginPlay`
  (bind (_direction _scale) (`Timeline|ScaleAnimation`)
    (:`Update`
      (bind _returnvalue (`KismetMathLibrary.MapRangeUnclamped` _scale 0.0 1.0 1.0 (`self.Animation Scale Max`)))
      (`self.SetActorScale3D` (`KismetMathLibrary.VLerp` (`self.GetActorScale3D`) (`KismetMathLibrary.MakeVector` _returnvalue _returnvalue _returnvalue) _scale)))))

(fn `BuildHalo`
  (bind _sphere_scale (`self.Sphere Scale`))
  (`|ExecutionSequence`
    (:`then_0`
      ;[1 1 1] Delete Existing
      (`/Game/ReusableAssets/Utilities/LIB_Utilities.DestroyChildComponents` (`self.SphereContainer`)))
    (:`then_1`
      _))
  ;[1 1 1] Create sphere mesh components
  (for _index (range (`self.Sphere Count`))
    (bind _returnvalue (`AddComponent|StaticMeshComponent_47` :`bManualAttachment` true :`RelativeTransform` (`KismetMathLibrary.MakeTransform` (`/Game/ReusableAssets/Utilities/LIB_Utilities.LocationAroundCircle` _index (`self.Sphere Count`) (`self.Radius`) (1.0 0.0 0.0)) (struct) (`KismetMathLibrary.MakeVector` _sphere_scale _sphere_scale _sphere_scale))))
    (`SceneComponent.K2_AttachTo` _returnvalue (`self.SphereContainer`) "None" "KeepRelativeOffset" true)
    (`StaticMeshComponent.SetStaticMesh` _returnvalue "/Game/ReusableAssets/MainMenuHoverButton/SM_MenuHover.SM_MenuHover")
    (`PrimitiveComponent.SetMaterial` _returnvalue 0 "/Game/ReusableAssets/MainMenuHoverButton/MT_MenuHover.MT_MenuHover")))

(fn `UserConstructionScript`
  (`self.BuildHalo`))