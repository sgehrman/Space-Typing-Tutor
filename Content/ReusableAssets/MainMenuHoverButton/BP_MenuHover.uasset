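; BP_MenuHover is a hover-activated menu button that spawns a BP_CircleMenu once crosshair hover progress completes.
; The construction script builds the center sphere with a dynamic material and passes public halo settings to a BP_SphereHalo child actor, working around unexposed subcomponent variables.
; A timeline animates the sphere's scale from BeginPlay.
; Hover progress drives the material's ColorBlend toward red, with guards against duplicate menu spawns.
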(event `self.ReceiveBeginPlay`
  ;[1 1 1] Scale Animation
  (bind (_direction _scale) (`Timeline|Scale Animation`)
    (:`Update`
      (bind _returnvalue (`KismetMathLibrary.MapRangeUnclamped` _scale 0.0 1.0 (`self.Center Sphere Scale`) (* (`self.Center Sphere Scale`) (`self.Center Animation Scale`))))
      (`SceneComponent.SetRelativeScale3D` (`self.Center Sphere`) (`KismetMathLibrary.VLerp` (`SceneComponent.RelativeScale3D` (`self.Center Sphere`)) (`KismetMathLibrary.MakeVector` _returnvalue _returnvalue _returnvalue) _scale)))))

(event `self.ReceiveTick`
  (params (DeltaSeconds :type "Float (single-precision)")))

(fn `Crosshair Hover Moved`
  (params (`Hit Location` :type "Vector Structure"))
  (returns (Success :type Boolean))
  (return false))

(fn `Crosshair Hover Progress`
  (params (Progress :type "Float (double-precision)") (`Local Hit Location` :type "Vector Structure") (`Hit Component` :type "PrimitiveComponent Object Reference"))
  (returns (`Auto Click On Progress` :type Boolean))
  (bind _returnvalue (`KismetMathLibrary.FClamp` Progress))
  (bind (_returnvalue_x _returnvalue_y _returnvalue_z) (`KismetMathLibrary.BreakVector` (`self.K2_GetActorLocation`)))
  (if (`self.Crosshair Hover Event Fired`)
    (return false)
    (elif (`KismetSystemLibrary.IsValid` (`self.Spawned Circle Menu`))
      (return false)
      (else
        (`|ExecutionSequence`
          (:`then_0`
            ;[1 1 1] Turns button red over time
            (`MaterialInstanceDynamic.SetScalarParameterValue` (`self.MID`) "ColorBlend" _returnvalue))
          (:`then_1`
            (if (== _returnvalue 1.0)
              (set `self.Crosshair Hover Event Fired` true)
              (bind _returnvalue_2 (`|SpawnActorFromClass` "/Game/StartMap/BP_CircleMenu.BP_CircleMenu_C" (`KismetMathLibrary.MakeTransform` (`KismetMathLibrary.MakeVector` _returnvalue_x _returnvalue_y _returnvalue_z)) "AdjustIfPossibleButDontSpawnIfColliding" "OverrideRootScale"))
              (set `self.Spawned Circle Menu` _returnvalue_2)
              (`/Game/StartMap/BP_CircleMenu.SetupFromSpawnedActor` _returnvalue_2)))
          (:`then_2`
            (return false)))))))

(fn `Crosshair Hover Start`
  (params (Finished :type Boolean))
  (returns (Success :type Boolean))
  (set `self.Crosshair Hover Event Fired` false)
  ;[1 1 1] If Finished, clear the hover material
  (if Finished
    (`MaterialInstanceDynamic.SetScalarParameterValue` (`self.MID`) "ColorBlend" 0.0))
  (return false))

(fn `Crosshair LeftRight`
  (params (Left :type Boolean))
  (returns (Success :type Boolean))
  (return false))

(fn `Crosshair Mouse Click`
  (params (`Mouse Down` :type Boolean) (`Event Type` :type "/Game/ReusableAssets/Utilities/E_EventType Enum" :default "NewEnumerator10") (`Hit Location` :type "Vector Structure") (`Hit Component` :type "PrimitiveComponent Object Reference"))
  (returns (Success :type Boolean))
  (return false))

(fn `Crosshair Scroll Wheel`
  (params (Down :type Boolean) (`Hit Location` :type "Vector Structure") (`Hit Component` :type "PrimitiveComponent Object Reference"))
  (returns (Success :type Boolean))
  (return false))

(fn `Crosshair UpDown`
  (params (Up :type Boolean))
  (returns (Success :type Boolean))
  (return false))

(fn `UserConstructionScript`
  (bind _center_sphere_scale (`self.Center Sphere Scale`))
  (`|ExecutionSequence`
    (:`then_0`
      (bind _returnvalue (`AddComponent|Static Mesh Component_27908` :`RelativeTransform` (`KismetMathLibrary.MakeTransform` (0.0 0.0 0.0) (struct) (`KismetMathLibrary.MakeVector` _center_sphere_scale _center_sphere_scale _center_sphere_scale))))
      (`StaticMeshComponent.SetStaticMesh` _returnvalue "/Game/ReusableAssets/MainMenuHoverButton/SM_MenuHover.SM_MenuHover")
      (set `self.Center Sphere` _returnvalue)
      (bind _returnvalue_2 (`KismetMaterialLibrary.CreateDynamicMaterialInstance` "/Game/ReusableAssets/MainMenuHoverButton/MT_MenuHoverCenter.MT_MenuHoverCenter"))
      (set `self.MID` _returnvalue_2)
      (`PrimitiveComponent.SetMaterial` _returnvalue 0 (`self.MID`)))
    (:`then_1`
      ;[1 1 1] Pass along our public variables.  I didn't figure out how to expose subcomponent public vars
      (bind _asbp_sphere_halo (cast `/Game/ReusableAssets/MainMenuHoverButton/BP_SphereHalo` (`ChildActorComponent.ChildActor` (`self.Halo`))))
      (set `/Game/ReusableAssets/MainMenuHoverButton/BP_SphereHalo.Radius` (`self.Radius`) _asbp_sphere_halo)
      (set `/Game/ReusableAssets/MainMenuHoverButton/BP_SphereHalo.Sphere Count` (`self.Shere Count`) _asbp_sphere_halo)
      (set `/Game/ReusableAssets/MainMenuHoverButton/BP_SphereHalo.Sphere Scale` (`self.Outer Sphere Scale`) _asbp_sphere_halo)
      (set `/Game/ReusableAssets/MainMenuHoverButton/BP_SphereHalo.Animation Scale Max` (`self.Outer Animation Scale`) _asbp_sphere_halo)
      (`/Game/ReusableAssets/MainMenuHoverButton/BP_SphereHalo.BuildHalo` _asbp_sphere_halo))))