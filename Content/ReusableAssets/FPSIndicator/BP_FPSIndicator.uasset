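; BP_FPSIndicator is an actor that displays average frame rate on a WBP_FPSIndicator widget hosted by its FPS component.
; Tick accumulates delta time and sample count, then writes the rounded-up average FPS since ticking began, not an instantaneous reading.
; On BeginPlay, the AnimateIn timeline moves the actor from world origin along X, and the actor destroys itself when the timeline finishes.
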(event `self.ReceiveTick`
  (params (DeltaSeconds :type "Float (single-precision)"))
  (set `self.Delta Seconds Total` (+ DeltaSeconds (`self.Delta Seconds Total`)))
  (set `self.Number of Samples` (+ (`self.Number of Samples`) 1))
  (bind _aswbp_fpsindicator (cast `/Game/ReusableAssets/FPSIndicator/WBP_FPSIndicator` (`WidgetComponent.GetUserWidgetObject` (`self.FPS`))))
  (set `/Game/ReusableAssets/FPSIndicator/WBP_FPSIndicator.FPS Text` (`KismetTextLibrary.Conv_IntToText` (`KismetMathLibrary.FCeil` (/ 1.0 (/ (`self.Delta Seconds Total`) (`KismetMathLibrary.Conv_IntToDouble` (`self.Number of Samples`))))) true 1 4) _aswbp_fpsindicator))

(event `self.ReceiveBeginPlay`
  (bind (_direction _alpha) (`Timeline|AnimateIn` :!via `PlayFromStart`)
    (:`Update`
      (`self.K2_SetActorLocation` (`KismetMathLibrary.VLerp` (`KismetMathLibrary.MakeVector` 0.0 0.0 0.0) (`KismetMathLibrary.MakeVector` 11111.0 0.0 0.0) _alpha)))
    (:`Finished`
      (`self.K2_DestroyActor`))))

(fn `UserConstructionScript`)