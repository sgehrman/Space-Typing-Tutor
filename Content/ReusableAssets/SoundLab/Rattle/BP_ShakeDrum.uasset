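; BP_ShakeDrum is a sound-lab drum pad of four colored, emissive procedural boxes in a grid, played by crosshair or mouse shaking.
; Clicks and scrolls on a box broadcast ShakeDrumInputEvent with its tagged drum index.
; With the child toggle button on, horizontal and vertical direction changes from BP_MouseLook each fire a drum and flash its box.
; A map of per-box countdowns, stepped on Tick, fades the flash emission.
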(event Custom|Horiz%20Change
  (params (Left :type Boolean))
  (if Left
    (CallFunction|DispatchDrumShake)
    (else
      (CallFunction|DispatchDrumShake 1))))

(event Custom|Vert%20Change
  (params (Up :type Boolean))
  (if Up
    (CallFunction|DispatchDrumShake 2)
    (else
      (CallFunction|DispatchDrumShake 3))))

(event EventTick
  (params (DeltaSeconds :type Float%20%28single-precision%29))
  (CallFunction|RestoreonTick))

(event EventBeginPlay
  (Utilities|FlowControl|Sequence
    (:then_0
      (bind _asbp_sound_player (Utilities|Casting|CastToBP_SoundPlayer (.Actor (CallFunction|FindActorwithTag "/Game/ReusableAssets/SoundLab/BP_SoundPlayer.BP_SoundPlayer_C" "MainSpeaker" self))))
      (Variables|Default|SetSound%20Player _asbp_sound_player))
    (:then_1
      (bind _asbp_mouse_look (Utilities|Casting|CastToBP_MouseLook (.Actor (CallFunction|FindActorwithTag "/Game/ReusableAssets/Utilities/BP_MouseLook.BP_MouseLook_C" "None" self))))
      (Variables|Default|SetMouse%20Look%20Ref _asbp_mouse_look))
    (:then_2
      (EventDispatchers|BindEventtoMouseDirectionChangedHorizontal (Variables|Default|GetMouse%20Look%20Ref) (delegate Custom|Horiz%20Change))
      (EventDispatchers|BindEventtoMouseDirectionChangedVertical (Variables|Default|GetMouse%20Look%20Ref) (delegate Custom|Vert%20Change)))
    (:then_3
      (Variables|Default|SetCube%20Fadeout%20Map (Class|KrishnaMap|Create)))))

(fn ConstructionScript
  (Utilities|FlowControl|Sequence
    (:then_0
      (bind _returnvalue (Rendering|Material|CreateDynamicMaterialInstance "/Game/ReusableAssets/Materials/MT_Opaque.MT_Opaque" :!class /Script/Engine.KismetMaterialLibrary))
      (Utilities|Array|Add (Variables|Default|GetCube%20MIDs) _returnvalue)
      (Rendering|Material|SetVectorParameterValue _returnvalue "EmissiveColor" "(R=0.235000,G=0.036874,B=0.110531,A=1.000000)" :!class /Script/Engine.MaterialInstanceDynamic)
      (Rendering|Material|SetScalarParameterValue _returnvalue "Emission" 12.0 :!class /Script/Engine.MaterialInstanceDynamic))
    (:then_1
      (bind _returnvalue_2 (Rendering|Material|CreateDynamicMaterialInstance "/Game/ReusableAssets/Materials/MT_Opaque.MT_Opaque" :!class /Script/Engine.KismetMaterialLibrary))
      (Utilities|Array|Add (Variables|Default|GetCube%20MIDs) _returnvalue_2)
      (Rendering|Material|SetVectorParameterValue _returnvalue_2 "EmissiveColor" "(R=0.034593,G=0.030942,B=0.235000,A=1.000000)" :!class /Script/Engine.MaterialInstanceDynamic)
      (Rendering|Material|SetScalarParameterValue _returnvalue_2 "Emission" 12.0 :!class /Script/Engine.MaterialInstanceDynamic))
    (:then_2
      (bind _returnvalue_3 (Rendering|Material|CreateDynamicMaterialInstance "/Game/ReusableAssets/Materials/MT_Opaque.MT_Opaque" :!class /Script/Engine.KismetMaterialLibrary))
      (Utilities|Array|Add (Variables|Default|GetCube%20MIDs) _returnvalue_3)
      (Rendering|Material|SetVectorParameterValue _returnvalue_3 "EmissiveColor" "(R=0.060890,G=0.235000,B=0.028989,A=1.000000)" :!class /Script/Engine.MaterialInstanceDynamic)
      (Rendering|Material|SetScalarParameterValue _returnvalue_3 "Emission" 12.0 :!class /Script/Engine.MaterialInstanceDynamic))
    (:then_3
      (bind _returnvalue_4 (Rendering|Material|CreateDynamicMaterialInstance "/Game/ReusableAssets/Materials/MT_Opaque.MT_Opaque" :!class /Script/Engine.KismetMaterialLibrary))
      (Utilities|Array|Add (Variables|Default|GetCube%20MIDs) _returnvalue_4)
      (Rendering|Material|SetVectorParameterValue _returnvalue_4 "EmissiveColor" "(R=0.235000,G=0.145967,B=0.019183,A=1.000000)" :!class /Script/Engine.MaterialInstanceDynamic)
      (Rendering|Material|SetScalarParameterValue _returnvalue_4 "Emission" 12.0 :!class /Script/Engine.MaterialInstanceDynamic))
    (:then_4
      (bind _asbp_toggle_button (Utilities|Casting|CastToBP_ToggleButton (Variables|/Script/Engine.ChildActorComponent|GetChildActor (Variables|Default|GetShake%20Toggle%20Component))))
      (bind _output_get (Variables|Default|SetShake%20Mode%20Button _asbp_toggle_button))
      (Default|SetState _output_get false)
      (Variables|/Game/ReusableAssets/Buttons/BP_ToggleButton.BP_ToggleButton_C|SetPush%20Button%20Mode _output_get false))
    (:then_5
      (CallFunction|CreateCubes))))

(fn CreateCubes
  (bind _cube_size (Variables|Default|GetCube%20Size))
  (bind _returnvalue (Math|Vector|MakeVector 12.0 _cube_size _cube_size))
  (Utilities|FlowControl|Sequence
    (:then_0
      (for _index (range 0 3)
        (Utilities|FlowControl|Sequence
          (:then_0
            (bind _returnvalue_2 (AddComponent|AddProceduralMeshComponent false (Math|Transform|MakeTransform (CallFunction|LocationinGrid (Math|Conversions|ToFloat(Integer) _index) 2.0 1.0 _returnvalue) "0, 0, 0" "1.000000,1.000000,1.000000")))
            (bind (_vertices _triangles _normals _uvs _tangents) (Class|KismetProceduralMeshLibrary|GenerateBoxMesh (/ _returnvalue 2.0)))
            (Class|ProceduralMeshComponent|CreateMeshSection _returnvalue_2 0 _vertices _triangles _normals _uvs 0 _tangents true)
            (Collision|SetCollisionEnabled _returnvalue_2 "QueryAndPhysics"))
          (:then_1
            (Variables|/Script/Engine.ActorComponent|SetComponentTags _returnvalue_2 (Utilities|Array|MakeArray (Utilities|String|StringToName (Utilities|String|ToString(Integer) _index)))))
          (:then_3
            (Rendering|Material|SetMaterial _returnvalue_2 0 (Utilities|Array|Get(acopy) (Variables|Default|GetCube%20MIDs) _index))))))
    (:then_3
      (return))))

(fn FlashCube
  (params (Index :type Integer))
  (Rendering|Material|SetScalarParameterValue (Utilities|Array|Get(acopy) (Variables|Default|GetCube%20MIDs) Index) "Emission" 88.0 :!class /Script/Engine.MaterialInstanceDynamic)
  (CallFunction|ScheduleCubeRestore Index))

(fn ScheduleCubeRestore
  (params (Index :type Integer))
  (Class|KrishnaMap|StringIntAddPair (Variables|Default|GetCube%20Fadeout%20Map) (Utilities|String|ToString(Integer) Index) 30))

(fn RestoreonTick
  (bind _returnvalue (Class|KrishnaMap|IsEmpty (Variables|Default|GetCube%20Fadeout%20Map)))
  (if (not _returnvalue)
    (for _array_element (Class|KrishnaMap|StringIntGetKeys (Variables|Default|GetCube%20Fadeout%20Map))
      (Utilities|FlowControl|Sequence
        (:then_0
          (if (.IsValid (Class|KrishnaMap|StringIntGet (Variables|Default|GetCube%20Fadeout%20Map) _array_element))
            (bind _output_get (LocalVariables|SetLocal%20Emission (+ (Variables|Default|GetBase%20Emission) (- (.ReturnValue (Class|KrishnaMap|StringIntGet (Variables|Default|GetCube%20Fadeout%20Map) _array_element)) 1))))
            (if (<= _output_get 0)
              (Utilities|Array|Add (LocalVariables|GetRemove%20Keys) _array_element)
              (LocalVariables|SetLocal%20Emission (Variables|Default|GetBase%20Emission))
              (else
                (Class|KrishnaMap|StringIntAddPair (Variables|Default|GetCube%20Fadeout%20Map) _array_element (- (.ReturnValue (Class|KrishnaMap|StringIntGet (Variables|Default|GetCube%20Fadeout%20Map) _array_element)) 1))))))
        (:then_2
          (Rendering|Material|SetScalarParameterValue (Utilities|Array|Get(acopy) (Variables|Default|GetCube%20MIDs) (Math|Conversions|ToInteger(Byte) _array_element)) "Emission" (Math|Conversions|ToFloat(Integer) (LocalVariables|GetLocal%20Emission)) :!class /Script/Engine.MaterialInstanceDynamic))
        (:then_4
          (for _array_element_2 (LocalVariables|GetRemove%20Keys)
            (Class|KrishnaMap|StringIntRemove (Variables|Default|GetCube%20Fadeout%20Map) _array_element_2))
          (return))))))

(fn DispatchInputEvent
  (params (Drum%20Tag :type String) (Event%20Type :type E_EventType%20Enum))
  (Default|CallShakeDrumInputEvent (Class|VictoryBPFunctionLibrary|AppendMultiple "Drum:" Drum%20Tag) Event%20Type))

(fn DispatchDrumShake
  (params (Index :type Integer))
  (Utilities|FlowControl|Sequence
    (:then_0
      (if (Variables|/Game/ReusableAssets/Buttons/BP_ToggleButton.BP_ToggleButton_C|GetOn%20State (Variables|Default|GetShake%20Mode%20Button))
        (CallFunction|DispatchInputEvent (Utilities|String|ToString(Integer) Index) "NewEnumerator10")
        (CallFunction|FlashCube Index)))
    (:then_1
      (return))))

(fn CrosshairHoverMoved
  (params (Hit%20Location :type Vector :default "0, 0, 0"))
  (return false))

(fn CrosshairHoverProgress
  (params (Progress :type Float%20%28single-precision%29) (Local%20Hit%20Location :type Vector :default "0, 0, 0") (Hit%20Component :type Primitive%20Component%20Object%20Reference))
  (return false))

(fn CrosshairHoverStart
  (params (Finished :type Boolean))
  (return false))

(fn CrosshairLeftRight
  (params (Left :type Boolean))
  (return false))

(fn CrosshairMouseClick
  (params (Mouse%20Down :type Boolean) (Event%20Type :type E_EventType%20Enum :default "NewEnumerator10") (Hit%20Location :type Vector :default "0, 0, 0") (Hit%20Component :type Primitive%20Component%20Object%20Reference))
  (Utilities|FlowControl|Sequence
    (:then_0
      (if Mouse%20Down
        (Default|CallShakeDrumInputEvent (Class|VictoryBPFunctionLibrary|AppendMultiple "Drum:" (Utilities|String|ToString(Name) (Utilities|Array|Get(acopy) (Variables|/Script/Engine.ActorComponent|GetComponentTags Hit%20Component)))) Event%20Type)))
    (:then_1
      (return false))))

(fn CrosshairScrollWheel
  (params (Down :type Boolean) (Hit%20Location :type Vector :default "0, 0, 0") (Hit%20Component :type Primitive%20Component%20Object%20Reference))
  (Utilities|FlowControl|Sequence
    (:then_0
      (if Down
        (LocalVariables|SetEvent%20Type "NewEnumerator2")
        (else
          (LocalVariables|SetEvent%20Type "NewEnumerator1"))))
    (:then_1
      (Default|CallShakeDrumInputEvent (Class|VictoryBPFunctionLibrary|AppendMultiple "Drum:" (Utilities|String|ToString(Name) (Utilities|Array|Get(acopy) (Variables|/Script/Engine.ActorComponent|GetComponentTags Hit%20Component)))) (LocalVariables|GetEvent%20Type)))
    (:then_3
      (return false))))

(fn CrosshairUpDown
  (params (Up :type Boolean))
  (return false))