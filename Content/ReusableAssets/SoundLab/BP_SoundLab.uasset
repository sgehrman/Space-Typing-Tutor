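; Sound lab controller actor for auditioning short OGG files from switchable hard-coded disk folders and assigning them to keys.
; On BeginPlay it finds and wires the coverflow browser, typewriter, key editor, sound player, buttons and shake drum.
; Coverflow actions play sounds at the button-set pitch and volume, rotating speakers.
; Input events save an armed panel's sound or play the mapped one, using a path-to-index cache that lazy-loads misses.
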(event Custom|VolumeButtonClicked
  (CallFunction|PlayLastSound))

(event Custom|PlaySelectedSound
  (CallFunction|PlaySoundbyID (Default|GetSelectedIdentifier (Variables|Default|GetCoverflow)) (CallFunction|CurrentPitch) (CallFunction|CurrentVolume)))

(event Custom|PanelAssignButtonClicked
  (params (Panel%20Index :type Integer :default 0) (On%20State :type Boolean :default false))
  (if On%20State
    (Variables|Default|SetAssign%20Key%20Mode%20Index Panel%20Index)
    (else
      (Variables|Default|SetAssign%20Key%20Mode%20Index -1))))

(event Custom|Setup%20Switch%20Dirs%20Button
  (bind _asbp_toggle_button (Utilities|Casting|CastToBP_ToggleButton (.Actor (CallFunction|FindActorwithTag "/Game/ReusableAssets/Buttons/BP_ToggleButton.BP_ToggleButton_C" "SwitchDirsButton" self))))
  (EventDispatchers|BindEventtoButtonClickedbyUser _asbp_toggle_button (delegate Custom|SwitchDirsButtonChanged))
  (Default|SetState _asbp_toggle_button false))

(event Custom|LoadSoundsFromCurrentDir
  (CallFunction|LoadSoundFiles)
  (CallFunction|ReloadCoverflow))

(event Custom|Play%20Last%20Sound
  (Default|PlayLastSound (Variables|Default|GetSound%20Player) (CallFunction|SoundforID (Default|GetSelectedIdentifier (Variables|Default|GetCoverflow))) (CallFunction|CurrentPitch) (CallFunction|CurrentVolume)))

(event Custom|SwitchDirsButtonChanged
  (params (Button%20ID :type String) (Hit%20Location :type Vector))
  (bind _next_index (CallFunction|NextIndex (Variables|Default|GetSound%20Directory%20Index) (Utilities|Array|Length (Variables|Default|GetSound%20Directories)) 1 true))
  (Variables|Default|SetSound%20Directory%20Index _next_index)
  (CallFunction|LoadSoundsfromCurrentDir)
  (CallFunction|Logg (Utilities|Array|Get(acopy) (Variables|Default|GetSound%20Directories) (Variables|Default|GetSound%20Directory%20Index))))

(event Custom|Coverflow%20Changed
  (CallFunction|PlaySelectedSound))

(event Custom|Setup%20Buttons
  (Utilities|FlowControl|Sequence
    (:then_0
      (bind _asbp_dual_push_button (Utilities|Casting|CastToBP_DualPushButton (.Actor (CallFunction|FindActorwithTag "/Game/ReusableAssets/Buttons/BP_DualPushButton.BP_DualPushButton_C" "PitchButton" self))))
      (bind _output_get (Variables|Default|SetPitch%20Button _asbp_dual_push_button))
      (EventDispatchers|BindEventtoDualButtonClicked _output_get (delegate Custom|VolumeButtonClicked)))
    (:then_1
      (bind _asbp_dual_push_button_2 (Utilities|Casting|CastToBP_DualPushButton (.Actor (CallFunction|FindActorwithTag "/Game/ReusableAssets/Buttons/BP_DualPushButton.BP_DualPushButton_C" "VolumeButton" self))))
      (bind _output_get_2 (Variables|Default|SetVolume%20Button _asbp_dual_push_button_2))
      (EventDispatchers|BindEventtoDualButtonClicked _output_get_2 (delegate Custom|PitchButtonClicked)))))

(event Custom|PitchButtonClicked
  (CallFunction|PlayLastSound))

(event Custom|Setup%20Shake%20Drum
  (bind _asbp_shake_drum (Utilities|Casting|CastToBP_ShakeDrum (.Actor (CallFunction|FindActorwithTag "/Game/ReusableAssets/SoundLab/Rattle/BP_ShakeDrum.BP_ShakeDrum_C" "" self)))
    (:then
      (bind _output_get (Variables|Default|SetShake%20Drum _asbp_shake_drum))
      (EventDispatchers|BindEventtoShakeDrumInputEvent _output_get (delegate Custom|ShakeDrumEvent)))
    (:CastFailed
      (CallFunction|Logg "No Shake drum?"))))

(event Custom|CoverflowClickEvent
  (params (Coverflow%20Data :type Cover%20Flow%20Panel%20Struct%20Structure))
  (CallFunction|PlaySoundbyID (.identifier Coverflow%20Data) (CallFunction|CurrentPitch) (CallFunction|CurrentVolume)))

(event Custom|ShakeDrumEvent
  (params (Character :type String) (Event%20Type :type E_EventType%20Enum))
  (CallFunction|ProcessInputEvent Character "NewEnumerator0" Event%20Type))

(event EventBeginPlay
  (bind _sound_directories (Variables|Default|GetSound%20Directories))
  (Utilities|FlowControl|Sequence
    (:then_0
      (Utilities|Array|Add _sound_directories "F:Sounds/Output")
      (Utilities|Array|Add _sound_directories "E:Sounds/Drummer")
      (Utilities|Array|Add _sound_directories "E:Sounds/Drummer2")
      (Utilities|Array|Add _sound_directories "E:Sounds/Output"))
    (:then_1
      (Variables|Default|SetSoundWaveMap (Class|KrishnaMap|Create)))
    (:then_2
      (Utilities|FlowControl|Sequence
        (:then_0
          (Input|EnableInput (Game|GetPlayerController 0)))
        (:then_1
          (bind _ascover_flow (Utilities|Casting|CastToCoverFlow (.Actor (CallFunction|FindActorwithTag "/Game/ReusableAssets/Coverflow/CoverFlow.CoverFlow_C" "None" self))))
          (bind _output_get (Variables|Default|SetCoverflow _ascover_flow))
          (EventDispatchers|BindEventtoCoverflowPanelClicked _output_get (delegate Custom|CoverflowClickEvent)))
        (:then_2
          (CallFunction|LoadSoundsfromCurrentDir))
        (:then_3
          (bind _asbp_typewriter (Utilities|Casting|CastToBP_Typewriter (.Actor (CallFunction|FindActorwithTag "/Game/ReusableAssets/Keyboard/BP_Typewriter.BP_Typewriter_C" "MainTypewriter" self))))
          (bind _output_get_2 (Variables|Default|SetTypewriter _asbp_typewriter))
          (Default|UpdateDelegate _output_get_2 self))
        (:then_4
          (bind _asbp_sound_key_editor (Utilities|Casting|CastToBP_SoundKeyEditor (.Actor (CallFunction|FindActorwithTag "/Game/ReusableAssets/SoundLab/BP_SoundKeyEditor.BP_SoundKeyEditor_C" "None" self))))
          (Variables|Default|SetSound%20Editor _asbp_sound_key_editor))
        (:then_5
          (EventDispatchers|BindEventtoCoverflowChangedEvent (Variables|Default|GetCoverflow) (delegate Custom|Coverflow%20Changed))
          (EventDispatchers|BindEventtoCoverflowPanelButtonClicked (Variables|Default|GetCoverflow) (delegate Custom|PanelAssignButtonClicked)))
        (:then_6
          (bind _asbp_sound_player (Utilities|Casting|CastToBP_SoundPlayer (.Actor (CallFunction|FindActorwithTag "/Game/ReusableAssets/SoundLab/BP_SoundPlayer.BP_SoundPlayer_C" "MainSpeaker" self))))
          (Variables|Default|SetSound%20Player _asbp_sound_player))
        (:then_7
          (CallFunction|SetupSwitchDirsButton)
          (CallFunction|SetupButtons)
          (CallFunction|SetupShakeDrum))))
    (:then_3
      (Class|GameplayStatics|ActivateReverbEffect "/Game/ReusableAssets/SoundLab/BP_SoundLabReverb.BP_SoundLabReverb" "KUNT"))))

(fn ConstructionScript)

(fn LoadSoundFiles
  (Utilities|FlowControl|Sequence
    (:then_0
      (Utilities|Array|Clear (Variables|Default|GetSound%20Structs)))
    (:then_1
      (for _array_element (.Files (Class|VictoryBPFunctionLibrary|JoyFileIOGetFilesinRootandAllSubFolders (Utilities|Array|Get(acopy) (Variables|Default|GetSound%20Directories) (Variables|Default|GetSound%20Directory%20Index)) "ogg"))
        (bind _returnvalue (Class|VictoryBPFunctionLibrary|GetSoundWavefromFile _array_element))
        ;[1 1 1] Just get short sounds
        (if (<= (Variables|/Script/Engine.SoundBase|GetDuration _returnvalue) (Variables|Default|GetMax%20Duration))
          (Utilities|Array|Add (Variables|Default|GetSound%20Structs) (Utilities|Struct|MakeS_SoundStruct _array_element _returnvalue))))
      (Utilities|FlowControl|Sequence
        (:then_0
          (for _array_element_2 (Variables|Default|GetSound%20Structs)
            (bind _returnvalue_2 (Utilities|Array|Add (Variables|Default|GetSoundWaveArray) (.sound _array_element_2)))
            (Class|KrishnaMap|StringIntAddPair (Variables|Default|GetSoundWaveMap) (.path _array_element_2) _returnvalue_2)))
        (:then_1
          (return))))))

(fn ReloadCoverflow
  (for _array_element (Variables|Default|GetSound%20Structs)
    (Utilities|Array|Add (LocalVariables|GetCoverFlowStructs) (Utilities|Struct|MakeCoverFlowPanelStruct "Untitled" (.Path (Utilities|Struct|BreakS_SoundStruct _array_element)) (.Path (Utilities|Struct|BreakS_SoundStruct _array_element)) (Class|VictoryBPFunctionLibrary|AppendMultiple "Duration: " (CallFunction|FloattoString (Variables|/Script/Engine.SoundBase|GetDuration (.Sound (Utilities|Struct|BreakS_SoundStruct _array_element))) 2) " sec"))))
  (Default|UpdateCoverflowData (Variables|Default|GetCoverflow) (LocalVariables|GetCoverFlowStructs)))

(fn CurrentPitch
  (bind _value (Default|GetValue (Variables|Default|GetPitch%20Button)))
  (return _value))

(fn PlaySoundbyID
  (params (ID :type String) (Pitch%20Multiplier :type Float%20%28single-precision%29 :default 0.0) (Volume%20Multiplier :type Float%20%28single-precision%29 :default 0.0))
  (Utilities|FlowControl|Sequence
    (:then_0
      (LocalVariables|SetLocal%20Sound (CallFunction|SoundforID ID)))
    (:then_1
      (bind _next_index (CallFunction|NextIndex (Variables|Default|GetSpeaker%20Index) 3 1 true))
      (bind _output_get (Variables|Default|SetSpeaker%20Index _next_index))
      (Default|PlaySound (Variables|Default|GetSound%20Player) (LocalVariables|GetLocal%20Sound) Pitch%20Multiplier Volume%20Multiplier _output_get))))

(fn CurrentVolume
  (bind _value (Default|GetValue (Variables|Default|GetVolume%20Button)))
  (return _value))

(fn SoundforID
  (params (Sound%20ID :type String))
  (bind _soundwavemap (Variables|Default|GetSoundWaveMap))
  (bind (_isvalid _returnvalue) (Class|KrishnaMap|StringIntGet _soundwavemap Sound%20ID))
  (Utilities|FlowControl|Sequence
    (:then_0
      ;[1 1 1] If blank string, play keyboard click sound
      (if (== (Utilities|String|Len Sound%20ID) 0)
        (LocalVariables|SetSound%20Result (Variables|/Game/ReusableAssets/Keyboard/BP_Typewriter.BP_Typewriter_C|GetKey%20Click%20Sound (Variables|Default|GetTypewriter)))
        (elif _isvalid
          (LocalVariables|SetSound%20Result (Utilities|Array|Get(acopy) (Variables|Default|GetSoundWaveArray) _returnvalue))
          (else
            (bind _returnvalue_2 (Class|VictoryBPFunctionLibrary|GetSoundWavefromFile Sound%20ID))
            (bind _returnvalue_3 (Utilities|Array|Add (Variables|Default|GetSoundWaveArray) _returnvalue_2))
            (Class|KrishnaMap|StringIntAddPair (Variables|Default|GetSoundWaveMap) Sound%20ID _returnvalue_3)
            (LocalVariables|SetSound%20Result _returnvalue_2)))))
    (:then_1
      (return (LocalVariables|GetSound%20Result)))))

(fn ProcessInputEvent
  (params (Character :type String) (Key%20Type :type E_KeyType%20Enum) (Event%20Type :type E_EventType%20Enum))
  (bind _volume (CallFunction|CurrentVolume))
  (bind _pitch (CallFunction|CurrentPitch))
  (bind _sound_editor (Variables|Default|GetSound%20Editor))
  (Utilities|FlowControl|Sequence
    (:then_0
      (if (>= (Variables|Default|GetAssign%20Key%20Mode%20Index) 0)
        (Default|SaveKeyboardEvent _sound_editor (.path (Utilities|Array|Get(acopy) (Variables|Default|GetSound%20Structs) (Variables|Default|GetAssign%20Key%20Mode%20Index))) Character Event%20Type _pitch _volume)
        (CallFunction|PlaySoundbyID (.path (Utilities|Array|Get(acopy) (Variables|Default|GetSound%20Structs) (Variables|Default|GetAssign%20Key%20Mode%20Index))) _pitch _volume)
        (Variables|Default|SetAssign%20Key%20Mode%20Index -1)
        (Default|ClearPanelButtonState (Variables|Default|GetCoverflow))
        (else
          (bind (_sound_path _pitch_multiplier _volume_multiplier) (Default|HandleKeyboardEvent _sound_editor Character Event%20Type))
          ;[1 1 1] If pitch or volume is 1 (default), then use current on screen values from buttons
          (Utilities|FlowControl|Sequence
            (:then_0
              (LocalVariables|SetFinal%20Pitch _pitch_multiplier)
              (LocalVariables|SetFinal%20Volume _volume_multiplier))
            (:then_1
              (if (== (LocalVariables|GetFinal%20Pitch) 1.0)
                (LocalVariables|SetFinal%20Pitch (CallFunction|CurrentPitch))))
            (:then_2
              (if (== (LocalVariables|GetFinal%20Volume) 1.0)
                (LocalVariables|SetFinal%20Volume (CallFunction|CurrentVolume))))
            (:then_3
              (CallFunction|PlaySoundbyID _sound_path (LocalVariables|GetFinal%20Pitch) (LocalVariables|GetFinal%20Volume)))))))))

(fn GetNextCharacter
  (return false ""))

(fn NextMatchingKey
  (params (Key%20Data :type ST%20Key%20Data%20Structure))
  (return false))