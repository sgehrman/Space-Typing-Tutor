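; Sound Lab actor that stores and looks up a sound path, pitch and volume for each keyboard character and event type.
; A two-level lookup map keyed "Character:EventType" loads from a JSON file on BeginPlay, normally under Content/AppData/Sounds.
; Each save also overwrites that character's entry for a fallback event type, which lookups use when the requested one is missing.
; Edits write back to JSON through a one-second delay that coalesces rapid saves.
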(event Custom|SaveAfterDelay
  (if (not (Variables|Default|GetSaving))
    (Variables|Default|SetSaving true)
    (Utilities|FlowControl|Delay 1.0)
    (Variables|Default|SetSaving false)
    (CallFunction|SavetoFile (Variables|Default|GetDirectory) (Variables|Default|GetFilename))))

(event EventBeginPlay
  (Utilities|FlowControl|Sequence
    (:then_0
      (Variables|Default|SetDirectory (Class|VictoryBPFunctionLibrary|AppendMultiple (Class|VictoryBPFunctionLibrary|VictoryPathsGameRootDirectory) "Content/" "AppData/" "Sounds/"))
      (if (Variables|Default|GetDebugging)
        (Variables|Default|SetDirectory "E:Sounds/Output")))
    (:then_1
      (Variables|Default|SetLookupMap (Class|KrishnaMapMap|Create))
      (CallFunction|LoadfromFile (Variables|Default|GetDirectory) (Variables|Default|GetFilename)))))

(event Collision|EventActorBeginOverlap
  (params (OtherActor :type Actor%20Object%20Reference)))

(event EventTick
  (params (DeltaSeconds :type Float%20%28single-precision%29)))

(fn ConstructionScript)

(fn SetStringValue
  (params (Character :type String) (Second%20Key :type String) (Value :type String) (Event%20Type :type E_EventType%20Enum :default "NewEnumerator0"))
  (Class|KrishnaMapMap|AddString (Variables|Default|GetLookupMap) (CallFunction|MakeMapKey Character Event%20Type) Second%20Key Value))

(fn GetStringValue
  (params (Character :type String) (Second%20Key :type String) (Event%20Type :type E_EventType%20Enum :default "NewEnumerator0"))
  (bind _map_key (CallFunction|MakeMapKey Character Event%20Type))
  (bind _lookupmap (Variables|Default|GetLookupMap))
  (bind (_isvalid _returnvalue) (Class|KrishnaMapMap|GetString _lookupmap _map_key Second%20Key))
  (return _isvalid _returnvalue))

(fn JsonString
  (LocalVariables|SetJSON%20Object%20Main (Class|KrishnaJSON|Create))
  (for _array_element (Class|KrishnaMapMap|GetStringKeys (Variables|Default|GetLookupMap))
    (LocalVariables|SetJSON%20Object (Class|KrishnaJSON|Create))
    (Class|KrishnaJSON|SetString (LocalVariables|GetJSON%20Object) "path" (.ReturnValue (Class|KrishnaMapMap|GetString (Variables|Default|GetLookupMap) _array_element "path")))
    (Class|KrishnaJSON|SetFloat (LocalVariables|GetJSON%20Object) "pitch" (.ReturnValue (Class|KrishnaMapMap|GetFloat (Variables|Default|GetLookupMap) _array_element "pitch")))
    (Class|KrishnaJSON|SetFloat (LocalVariables|GetJSON%20Object) "volume" (.ReturnValue (Class|KrishnaMapMap|GetFloat (Variables|Default|GetLookupMap) _array_element "volume")))
    (Class|KrishnaJSON|SetObject (LocalVariables|GetJSON%20Object%20Main) _array_element (LocalVariables|GetJSON%20Object)))
  (return (.OutStr (Class|KrishnaJSON|ToJsonString (LocalVariables|GetJSON%20Object%20Main)))))

(fn SavetoFile
  (params (Directory :type String) (Filename :type String))
  (bind _json (CallFunction|JsonString))
  (bind _returnvalue (Class|VictoryBPFunctionLibrary|FileIOSaveStringTexttoFile Directory Filename _json true))
  (if (not _returnvalue)
    (CallFunction|Logg "Save Failed")))

(fn LoadfromFile
  (params (Directory :type String) (Filename :type String))
  (bind _returnvalue (Class|VictoryBPFunctionLibrary|AppendMultiple Directory Filename))
  (bind (_outstring _returnvalue_2) (Class|FileSystemUtils|LoadFiletoString _returnvalue))
  (if _returnvalue_2
    (bind _returnvalue_3 (Class|KrishnaJSON|ParseJson (Class|KrishnaJSON|Create) _outstring))
    (for _array_element (Class|KrishnaJSON|GetKeys _returnvalue_3)
      (if (.IsValid (Class|KrishnaJSON|GetString (Class|KrishnaJSON|GetObject _returnvalue_3 _array_element) "path"))
        (Class|KrishnaMapMap|AddString (Variables|Default|GetLookupMap) _array_element "path" (.ReturnValue (Class|KrishnaJSON|GetString (Class|KrishnaJSON|GetObject _returnvalue_3 _array_element) "path"))))
      (if (.IsValid (Class|KrishnaJSON|GetFloat (Class|KrishnaJSON|GetObject _returnvalue_3 _array_element) "pitch"))
        (Class|KrishnaMapMap|AddFloat (Variables|Default|GetLookupMap) _array_element "pitch" (.ReturnValue (Class|KrishnaJSON|GetFloat (Class|KrishnaJSON|GetObject _returnvalue_3 _array_element) "pitch"))))
      (if (.IsValid (Class|KrishnaJSON|GetFloat (Class|KrishnaJSON|GetObject _returnvalue_3 _array_element) "volume"))
        (Class|KrishnaMapMap|AddFloat (Variables|Default|GetLookupMap) _array_element "volume" (.ReturnValue (Class|KrishnaJSON|GetFloat (Class|KrishnaJSON|GetObject _returnvalue_3 _array_element) "volume")))))
    (else
      (CallFunction|Logg "read error"))))

(fn HandleKeyboardEvent
  (params (Character :type String) (Event%20Type :type E_EventType%20Enum :default "NewEnumerator10"))
  (Utilities|FlowControl|Sequence
    (:then_0
      (bind (_sound_path _pitch_multiplier _volume_multiplier _valid) (CallFunction|DoHandleKeyboardEvent Character Event%20Type))
      (if _valid
        (LocalVariables|SetResult%20Sound _sound_path)
        (LocalVariables|SetResult%20Pitch _pitch_multiplier)
        (LocalVariables|SetResult%20Volume _volume_multiplier)
        (else
          (bind (_sound_path_2 _pitch_multiplier_2 _volume_multiplier_2 _valid_2) (CallFunction|DoHandleKeyboardEvent Character "NewEnumerator10"))
          (if _valid_2
            (LocalVariables|SetResult%20Sound _sound_path_2)
            (LocalVariables|SetResult%20Pitch _pitch_multiplier_2)
            (LocalVariables|SetResult%20Volume _volume_multiplier_2)))))
    (:then_1
      (return (LocalVariables|GetResult%20Sound) (LocalVariables|GetResult%20Pitch) (LocalVariables|GetResult%20Volume)))))

(fn SaveKeyboardEvent
  (params (Path :type String) (Character :type String) (Event%20Type :type E_EventType%20Enum :default "NewEnumerator10") (Pitch%20Multiplier :type Float%20%28single-precision%29 :default 0.0) (Volume%20Multiplier :type Float%20%28single-precision%29 :default 0.0))
  (CallFunction|DoSaveKeyboardEvent Path Character Event%20Type Pitch%20Multiplier Volume%20Multiplier)
  (CallFunction|DoSaveKeyboardEvent Path Character "NewEnumerator10" Pitch%20Multiplier Volume%20Multiplier)
  (CallFunction|SaveAfterDelay))

(fn MakeMapKey
  (params (Character :type String) (Event%20Type :type E_EventType%20Enum :default "NewEnumerator0"))
  (return (Class|VictoryBPFunctionLibrary|AppendMultiple Character ":" (Utilities|String|EnumtoString Event%20Type))))

(fn GetFloatValue
  (params (Character :type String) (Second%20Key :type String) (Event%20Type :type E_EventType%20Enum :default "NewEnumerator0"))
  (bind _map_key (CallFunction|MakeMapKey Character Event%20Type))
  (bind _lookupmap (Variables|Default|GetLookupMap))
  (bind (_isvalid _returnvalue) (Class|KrishnaMapMap|GetFloat _lookupmap _map_key Second%20Key))
  (return _isvalid _returnvalue))

(fn SetFloatValue
  (params (Character :type String) (Second%20Key :type String) (Value :type Float%20%28single-precision%29 :default 0.0) (Event%20Type :type E_EventType%20Enum :default "NewEnumerator0"))
  (Class|KrishnaMapMap|AddFloat (Variables|Default|GetLookupMap) (CallFunction|MakeMapKey Character Event%20Type) Second%20Key Value))

(fn DoSaveKeyboardEvent
  (params (Path :type String) (Character :type String) (Event%20Type :type E_EventType%20Enum :default "NewEnumerator0") (Pitch%20Multiplier :type Float%20%28single-precision%29 :default 0.0) (Volume%20Multiplier :type Float%20%28single-precision%29 :default 0.0))
  (CallFunction|SetStringValue Character "path" Path Event%20Type)
  (CallFunction|SetFloatValue Character "pitch" Pitch%20Multiplier Event%20Type)
  (CallFunction|SetFloatValue Character "volume" Volume%20Multiplier Event%20Type))

(fn DoHandleKeyboardEvent
  (params (Character :type String) (Event%20Type :type E_EventType%20Enum :default "NewEnumerator0"))
  (Utilities|FlowControl|Sequence
    (:then_0
      (bind (_valid _value) (CallFunction|GetStringValue Character "path" Event%20Type))
      (if _valid
        (LocalVariables|SetResult%20Sound _value)
        (LocalVariables|SetResult%20Valid true)))
    (:then_1
      (bind (_valid_2 _result) (CallFunction|GetFloatValue Character "pitch" Event%20Type))
      (if _valid_2
        (LocalVariables|SetResult%20Pitch _result)))
    (:then_2
      (bind (_valid_3 _result_2) (CallFunction|GetFloatValue Character "volume" Event%20Type))
      (if _valid_3
        (LocalVariables|SetResult%20Volume _result_2)))
    (:then_3
      (return (LocalVariables|GetResult%20Sound) (LocalVariables|GetResult%20Pitch) (LocalVariables|GetResult%20Volume) (LocalVariables|GetResult%20Valid)))))