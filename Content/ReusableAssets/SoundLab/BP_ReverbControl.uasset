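; Sound lab reverb control panel that edits a reverb effect through a column of sliders.
; Construction Script spawns one scrollbar child actor per parameter spec, seeded from BP_SoundLabReverb and the volume setting.
; BeginPlay finds the tagged audio volume, toggle button and speaker; the button switches the volume's reverb effect on or off.
; Any slider change rewrites all parameters through a helper object, forces reverb on and replays the last sound.
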(event Custom|SetupReverbButton
  (bind _asbp_toggle_button (Utilities|Casting|CastToBP_ToggleButton (.Actor (CallFunction|FindActorwithTag "/Game/ReusableAssets/Buttons/BP_ToggleButton.BP_ToggleButton_C" "ReverbButton" self))))
  (Variables|Default|SetReverbButton _asbp_toggle_button)
  (Default|SetState (Variables|Default|GetReverbButton) true)
  (CallFunction|UpdateReverb)
  (EventDispatchers|BindEventtoButtonClickedbyUser (Variables|Default|GetReverbButton) (delegate Custom|ReverbButtonClick)))

(event Custom|ReverbButtonClick
  (params (Button%20ID :type String) (Hit%20Location :type Vector))
  (CallFunction|UpdateReverb))

(event Custom|UpdateReverb
  (if (Variables|/Game/ReusableAssets/Buttons/BP_ToggleButton.BP_ToggleButton_C|GetOn%20State (Variables|Default|GetReverbButton))
    (Variables|/Script/Engine.AudioVolume|SetSettings (Variables|Default|GetReverb%20Box) (Utilities|Struct|MakeReverbSettings true (Variables|Default|GetReverb) (Variables|Default|GetSettings%20Volume) (Variables|Default|GetSettings%20Fade%20Time)))
    (else
      (Variables|/Script/Engine.AudioVolume|SetSettings (Variables|Default|GetReverb%20Box) (Utilities|Struct|MakeReverbSettings true 0 (Variables|Default|GetSettings%20Volume) (Variables|Default|GetSettings%20Fade%20Time))))))

(event Custom|Scrollbar%20Changed
  (for _array_element (Variables|Default|GetScrollbars)
    (bind _result (Default|GetIdentifier _array_element))
    (CallFunction|SetReverbParamwithID _result (Default|GetSliderValue _array_element false)))
  (Default|SetState (Variables|Default|GetReverbButton) true)
  (CallFunction|UpdateReverb)
  (Default|PlayLastSound (Variables|Default|GetSound%20Player) "/Game/UniversalSoundFX/Sound_Effects/8BIT/Beeps/8BIT_RETRO_Beep_Zap_Fast_mono.8BIT_RETRO_Beep_Zap_Fast_mono" 1.0 1.0))

(event EventBeginPlay
  (Utilities|FlowControl|Sequence
    (:then_0
      (bind _asaudio_volume (Utilities|Casting|CastToAudioVolume (.Actor (CallFunction|FindActorwithTag "/Script/Engine.AudioVolume" "ReverbAudioVolume" self))))
      (Variables|Default|SetReverb%20Box _asaudio_volume))
    (:then_1
      (for _array_element (Variables|Default|GetScrollbars)
        (EventDispatchers|BindEventtoScrollbarChanged _array_element (delegate Custom|Scrollbar%20Changed))))
    (:then_2
      (CallFunction|SetupReverbButton))
    (:then_3
      (bind _asbp_sound_player (Utilities|Casting|CastToBP_SoundPlayer (.Actor (CallFunction|FindActorwithTag "/Game/ReusableAssets/SoundLab/BP_SoundPlayer.BP_SoundPlayer_C" "MainSpeaker" self))))
      (Variables|Default|SetSound%20Player _asbp_sound_player))))

(fn ConstructionScript
  (bind _sliderspecs (Variables|Default|GetSliderSpecs))
  (Utilities|FlowControl|Sequence
    (:then_0
      (Variables|Default|SetReverb "/Game/ReusableAssets/SoundLab/BP_SoundLabReverb.BP_SoundLabReverb"))
    (:then_1
      (Utilities|Array|Add _sliderspecs (Utilities|Struct|MakeS_SliderSpec "Density" 0.0 1.0 "Density"))
      (Utilities|Array|Add _sliderspecs (Utilities|Struct|MakeS_SliderSpec "Diffusion" 0.0 1.0 "Diffusion"))
      (Utilities|Array|Add _sliderspecs (Utilities|Struct|MakeS_SliderSpec "Gain" 0.0 1.0 "Gain"))
      (Utilities|Array|Add _sliderspecs (Utilities|Struct|MakeS_SliderSpec "Gain HF" 0.0 1.0 "GainHF"))
      (Utilities|Array|Add _sliderspecs (Utilities|Struct|MakeS_SliderSpec "Decay Time" 0.1 2e+01 "DecayTime"))
      (Utilities|Array|Add _sliderspecs (Utilities|Struct|MakeS_SliderSpec "Decay HFRatio" 0.1 2.0 "DecayHFRatio"))
      (Utilities|Array|Add _sliderspecs (Utilities|Struct|MakeS_SliderSpec "Reflections Gain" 0.0 3.16 "ReflectionsGain"))
      (Utilities|Array|Add _sliderspecs (Utilities|Struct|MakeS_SliderSpec "Reflections Delay" 0.0 0.3 "ReflectionsDelay"))
      (Utilities|Array|Add _sliderspecs (Utilities|Struct|MakeS_SliderSpec "Late Gain" 0.0 1e+01 "LateGain"))
      (Utilities|Array|Add _sliderspecs (Utilities|Struct|MakeS_SliderSpec "Late Delay" 0.0 0.1 "LateDelay"))
      (Utilities|Array|Add _sliderspecs (Utilities|Struct|MakeS_SliderSpec "Air Absorption Gain HF" 0.892 1.0 "AirAbsorptionGainHF"))
      (Utilities|Array|Add _sliderspecs (Utilities|Struct|MakeS_SliderSpec "Room Rolloff Factor" 0.0 1e+01 "RoomRolloffFactor"))
      (Utilities|Array|Add _sliderspecs (Utilities|Struct|MakeS_SliderSpec "Volume" 0.0 2.0 "Volume")))
    (:then_2
      (for (_array_element _array_index) (Variables|Default|GetSliderSpecs)
        (bind _returnvalue (AddComponent|AddChildActorComponent false (Math|Transform|MakeTransform (Math|Vector|MakeVector 0.0 0.0 (* _array_index 88.0)))))
        (bind _asbp_scrollbar_actor (Utilities|Casting|CastToBP_ScrollbarActor (Variables|/Script/Engine.ChildActorComponent|GetChildActor _returnvalue)))
        (Utilities|Array|Add (Variables|Default|GetScrollbars) _asbp_scrollbar_actor)
        (Default|Setup _asbp_scrollbar_actor (.Title (Utilities|Struct|BreakS_SliderSpec _array_element)) (.MinValue (Utilities|Struct|BreakS_SliderSpec _array_element)) (.MaxValue (Utilities|Struct|BreakS_SliderSpec _array_element)) (CallFunction|GetReverbParamwithID (.Identifier (Utilities|Struct|BreakS_SliderSpec _array_element))) (.Identifier (Utilities|Struct|BreakS_SliderSpec _array_element)))))))

(fn GetReverbParamwithID
  (params (Identifier :type String))
  (Utilities|FlowControl|Sequence
    (:then_0
      (bind (_density _diffusion _gain _gainhf _decaytime _decayhfratio _reflectionsgain _reflectionsdelay _lategain _latedelay _airabsorptiongainhf _roomrollofffactor) (Class|SystemUtils|SplitReverbEffect (Variables|Default|GetReverb)))
      (switch string Identifier
        (:Default
          ;[1 1 1] Shouldn't happen.  Debug log
          (CallFunction|Logg (Class|VictoryBPFunctionLibrary|AppendMultiple "GetReverbParamWithID: " "ID: " Identifier)))
        (:Density
          (LocalVariables|SetResult _density))
        (:Diffusion
          (LocalVariables|SetResult _diffusion))
        (:Gain
          (LocalVariables|SetResult _gain))
        (:GainHF
          (LocalVariables|SetResult _gainhf))
        (:DecayTime
          (LocalVariables|SetResult _decaytime))
        (:DecayHFRatio
          (LocalVariables|SetResult _decayhfratio))
        (:ReflectionsGain
          (LocalVariables|SetResult _reflectionsgain))
        (:ReflectionsDelay
          (LocalVariables|SetResult _reflectionsdelay))
        (:LateGain
          (LocalVariables|SetResult _lategain))
        (:LateDelay
          (LocalVariables|SetResult _latedelay))
        (:AirAbsorptionGainHF
          (LocalVariables|SetResult _airabsorptiongainhf))
        (:RoomRolloffFactor
          (LocalVariables|SetResult _roomrollofffactor))
        (:Volume
          (LocalVariables|SetResult (Variables|Default|GetSettings%20Volume)))))
    (:then_1
      (return (LocalVariables|GetResult)))))

(fn SetReverbParamwithID
  (params (Identifier :type String) (New%20Value :type Float%20%28single-precision%29 :default 0.0))
  (Utilities|FlowControl|Sequence
    (:then_0
      (LocalVariables|SetLocal%20KrishnaReverb (Class|KrishnaReverbEffect|Create (Variables|Default|GetReverb))))
    (:then_1
      (switch string Identifier
        (:Default
          ;[1 1 1] Shouldn't happen.  Debug log
          (CallFunction|Logg (Class|VictoryBPFunctionLibrary|AppendMultiple "SetReverbParamWithID: " "ID: " Identifier)))
        (:Density
          (Variables|/Script/KrishnaPlugin.KrishnaReverbEffect|SetDensity (LocalVariables|GetLocal%20KrishnaReverb) New%20Value))
        (:Diffusion
          (Variables|/Script/KrishnaPlugin.KrishnaReverbEffect|SetDiffusion (LocalVariables|GetLocal%20KrishnaReverb) New%20Value))
        (:Gain
          (Variables|/Script/KrishnaPlugin.KrishnaReverbEffect|SetGain (LocalVariables|GetLocal%20KrishnaReverb) New%20Value))
        (:GainHF
          (Variables|/Script/KrishnaPlugin.KrishnaReverbEffect|SetGainHF (LocalVariables|GetLocal%20KrishnaReverb) New%20Value))
        (:DecayTime
          (Variables|/Script/KrishnaPlugin.KrishnaReverbEffect|SetDecayTime (LocalVariables|GetLocal%20KrishnaReverb) New%20Value))
        (:DecayHFRatio
          (Variables|/Script/KrishnaPlugin.KrishnaReverbEffect|SetDecayHFRatio (LocalVariables|GetLocal%20KrishnaReverb) New%20Value))
        (:ReflectionsGain
          (Variables|/Script/KrishnaPlugin.KrishnaReverbEffect|SetReflectionsGain (LocalVariables|GetLocal%20KrishnaReverb) New%20Value))
        (:ReflectionsDelay
          (Variables|/Script/KrishnaPlugin.KrishnaReverbEffect|SetReflectionsDelay (LocalVariables|GetLocal%20KrishnaReverb) New%20Value))
        (:LateGain
          (Variables|/Script/KrishnaPlugin.KrishnaReverbEffect|SetLateGain (LocalVariables|GetLocal%20KrishnaReverb) New%20Value))
        (:LateDelay
          (Variables|/Script/KrishnaPlugin.KrishnaReverbEffect|SetLateDelay (LocalVariables|GetLocal%20KrishnaReverb) New%20Value))
        (:AirAbsorptionGainHF
          (Variables|/Script/KrishnaPlugin.KrishnaReverbEffect|SetAirAbsorptionGainHF (LocalVariables|GetLocal%20KrishnaReverb) New%20Value))
        (:RoomRolloffFactor
          (Variables|/Script/KrishnaPlugin.KrishnaReverbEffect|SetRoomRolloffFactor (LocalVariables|GetLocal%20KrishnaReverb) New%20Value))
        (:Volume
          (Variables|Default|SetSettings%20Volume New%20Value))))
    (:then_2
      (Variables|Default|SetReverb (Class|KrishnaReverbEffect|GetReverbEffect (LocalVariables|GetLocal%20KrishnaReverb))))))