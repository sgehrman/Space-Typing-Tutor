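; BP_SoundPlayer is a sound player, filed under SoundLab, that plays one-shot requests from a centre or side speaker position.
; PlaySound maps SpeakerID to an offset on the Y axis, fades out the actor's existing audio components, attaches the new sound to the root and stores it as LastSound.
; PlayLastSound replays the stored sound through PlaySound, with a DefaultSound fallback.
; The event graph and construction script are empty.
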(event EventBeginPlay)

(event EventActorBeginOverlap
  (params (OtherActor :type Actor%20Object%20Reference)))

(event EventTick
  (params (DeltaSeconds :type Float%20%28single-precision%29)))

(fn ConstructionScript)

(fn PlaySound
  (params (Sound :type Sound%20Base%20Object%20Reference) (Pitch%20Multiplier :type Float%20%28single-precision%29) (Volume%20Multiplier :type Float%20%28single-precision%29) (Speaker%20ID :type Integer))
  (Utilities|FlowControl|Sequence
    (:then_0
      (switch int Speaker%20ID
        (:0
          (LocalVariables|SetSpeaker%20Position 0.0))
        (:1
          (LocalVariables|SetSpeaker%20Position 1.1e+04))
        (:2
          (LocalVariables|SetSpeaker%20Position -1.1e+04))))
    (:then_1
      (for _array_element (Actor|GetComponentsByClass "/Script/Engine.AudioComponent")
        (Audio|Components|Audio|FadeOut _array_element 0.5 0.0 :!class /Script/Engine.AudioComponent)))
    (:then_2
      (Class|GameplayStatics|PlaySoundAttached Sound (Variables|Default|GetRoot) "None" (Math|Vector|MakeVector 0.0 (LocalVariables|GetSpeaker%20Position) 0.0) "KeepRelativeOffset" false Volume%20Multiplier Pitch%20Multiplier))
    (:then_3
      (Variables|Default|SetLast%20Sound Sound))))

(fn PlayLastSound
  (params (Default%20Sound :type Sound%20Base%20Object%20Reference) (Pitch%20Multiplier :type Float%20%28single-precision%29) (Volume%20Multiplier :type Float%20%28single-precision%29) (Speaker%20ID :type Integer :default 0))
  (if (== (Variables|Default|GetLast%20Sound) 0)
    (CallFunction|PlaySound Default%20Sound Pitch%20Multiplier Volume%20Multiplier Speaker%20ID)
    (else
      (CallFunction|PlaySound (Variables|Default|GetLast%20Sound) Pitch%20Multiplier Volume%20Multiplier Speaker%20ID))))