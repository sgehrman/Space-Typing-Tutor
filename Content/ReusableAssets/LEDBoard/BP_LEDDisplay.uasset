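; LED board actor that shows text phrases as a grid of glowing instanced meshes, with an optional background panel.
; SetupDisplay maps grid tags to indices and builds a phrase component per sentence from letter coordinates supplied by a found or spawned BP_LEDAlphabet.
; RefreshLEDs draws only lit cells, reusing existing instances before adding or removing any.
; A looping timer scrolls the first phrase leftward, and optional crosshair wheel input shifts phrases vertically.
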(event Custom|Scroll%20In%20Text
  (bind _output_get (Variables|Default|SetCurrent%20LED%20Phrase (Utilities|Array|Get(acopy) (Variables|Default|GetLEDPhrases))))
  (Default|SetXYOffsets _output_get (Variables|Default|GetWidth))
  (CallFunction|RefreshLEDs _output_get)
  (Utilities|Time|SetTimerbyFunctionName 0 "ScrollTextEvent" 0.1 true))

(event Custom|Show%20Phrase
  (params (Index :type Integer))
  (bind _output_get (Variables|Default|SetCurrent%20LED%20Phrase (Utilities|Array|Get(acopy) (Variables|Default|GetLEDPhrases) Index)))
  (CallFunction|RefreshLEDs _output_get))

(event Custom|ScrollTextEvent
  (Default|IncrementXYOffsets (Variables|Default|GetCurrent%20LED%20Phrase) -1)
  (CallFunction|RefreshLEDs (Variables|Default|GetCurrent%20LED%20Phrase)))

(event EventBeginPlay
  (bind _self self)
  (bind (_is_valid _actor) (CallFunction|FindActorwithTag "/Game/ReusableAssets/LEDBoard/BP_LEDAlphabet.BP_LEDAlphabet_C" "" _self))
  (Utilities|FlowControl|Sequence
    (:then_0
      (if _is_valid
        (Utilities|Casting|CastToBP_LEDAlphabet _actor)
        (else
          (bind _returnvalue (Game|SpawnActorfromClass "/Game/ReusableAssets/LEDBoard/BP_LEDAlphabet.BP_LEDAlphabet_C" (Math|Transform|MakeTransform "0, 0, 0") "AlwaysSpawn" self 0))))
      (Variables|Default|SetLED%20Alphabet _returnvalue))
    (:then_1
      (Variables|Default|SetTagToIndexMap (Class|KrishnaMap|Create)))))

(fn ConstructionScript
  (bind _height (Variables|Default|GetHeight))
  (bind _led_extent (Variables|Default|GetLED%20Extent))
  (bind _returnvalue (* _height _led_extent))
  (Utilities|FlowControl|Sequence
    (:then_0
      (bind _returnvalue_2 (Rendering|Material|CreateDynamicMaterialInstance "/Game/ReusableAssets/Materials/MT_Opaque.MT_Opaque" :!class /Script/Engine.KismetMaterialLibrary))
      (bind _output_get (Variables|Default|SetOn%20MID _returnvalue_2))
      (Rendering|Material|SetScalarParameterValue _output_get "Emission" 33.0 :!class /Script/Engine.MaterialInstanceDynamic))
    (:then_1
      (bind _returnvalue_3 (AddComponent|AddInstancedStaticMeshComponent false))
      (bind _output_get_2 (Variables|Default|SetOn%20Instanced%20Static%20Mesh _returnvalue_3))
      (Rendering|Material|SetMaterial _output_get_2 0 (Variables|Default|GetOn%20MID))
      (Rendering|SetCastShadow _output_get_2 false))
    (:then_2
      (if (Variables|Default|GetDraw%20Background)
        (AddComponent|AddStaticMeshComponent false (Math|Transform|MakeTransform (Math|Vector|MakeVector (* _led_extent -0.1) 0.0 (/ _returnvalue 2.0)) "0, 0, 0" (Math|Vector|MakeVector 0.01 (/ (* (Variables|Default|GetWidth) _led_extent) 1e+02) (/ _returnvalue 1e+02))))))))

(fn TransformforIndex
  (params (Index :type Integer :default 0) (Number%20of%20Columns :type Integer :default 0))
  (bind _led_extent (Variables|Default|GetLED%20Extent))
  (bind _led_scale (Variables|Default|GetLED%20Scale))
  (return (Math|Transform|MakeTransform (CallFunction|LocationinGrid (Math|Conversions|ToFloat(Integer) Index) (Math|Conversions|ToFloat(Integer) Number%20of%20Columns) 0.0 (Math|Vector|MakeVector _led_extent _led_extent _led_extent)) "0, 0, 0" (Math|Vector|MakeVector _led_scale _led_scale _led_scale))))

(fn RefreshLEDs
  (params (Phrase :type BP%20LED%20Phrase%20Object%20Reference))
  (bind _on_instanced_static_mesh (Variables|Default|GetOn%20Instanced%20Static%20Mesh))
  (Utilities|FlowControl|Sequence
    (:then_0
      (LocalVariables|SetInstance%20Count (Components|InstancedStaticMesh|GetInstanceCount (Variables|Default|GetOn%20Instanced%20Static%20Mesh)))
      (LocalVariables|SetInstance%20Index 0))
    (:then_1
      (for _array_element (Default|GetXYStringArray Phrase)
        (if (.IsValid (Class|KrishnaMap|StringIntGet (Variables|Default|GetTagToIndexMap) _array_element))
          (bind _result (CallFunction|TransformforIndex (.ReturnValue (Class|KrishnaMap|StringIntGet (Variables|Default|GetTagToIndexMap) _array_element)) (Variables|Default|GetWidth)))
          (if (> (LocalVariables|GetInstance%20Count) 0)
            (Components|InstancedStaticMesh|UpdateInstanceTransform _on_instanced_static_mesh (LocalVariables|GetInstance%20Index) _result false true)
            (LocalVariables|SetInstance%20Count (- (LocalVariables|GetInstance%20Count) 1))
            (LocalVariables|SetInstance%20Index (+ (LocalVariables|GetInstance%20Index) 1))
            (else
              (Components|InstancedStaticMesh|AddInstance _on_instanced_static_mesh _result)))))
      (if (> (LocalVariables|GetInstance%20Count) 0)
        (for _index (range 0 (- (LocalVariables|GetInstance%20Count) 1))
          ;[1 1 1] Removing an item shifts the index down.  Looks weird, yes.
          (bind _returnvalue (Class|InstancedStaticMeshComponent|RemoveInstance (Variables|Default|GetOn%20Instanced%20Static%20Mesh) (LocalVariables|GetInstance%20Index)))
          (if (not _returnvalue)
            (CallFunction|Logg (Class|VictoryBPFunctionLibrary|AppendMultiple "ERR: Remove Index: " (Utilities|String|ToString(Integer) (LocalVariables|GetInstance%20Index))))))))))

(fn SetupDisplay
  (params (Sentences :type Array%20of%20Strings) (Height :type Integer) (Width :type Integer))
  (Utilities|FlowControl|Sequence
    (:then_0
      (Variables|Default|SetHeight Height)
      (Variables|Default|SetWidth Width))
    (:then_1
      (for _index (range 0 (- (* (Variables|Default|GetWidth) (Variables|Default|GetHeight)) 1))
        (Class|KrishnaMap|StringIntAddPair (Variables|Default|GetTagToIndexMap) (CallFunction|LEDTagforIndex _index (Variables|Default|GetWidth)) _index)
        (Utilities|Array|Add (Variables|Default|GetIndexToTagArray) (CallFunction|LEDTagforIndex _index (Variables|Default|GetWidth)))))
    (:then_4
      (for _array_element Sentences
        (bind _returnvalue (AddComponent|AddBPLEDPhrase))
        (Utilities|Array|Add (Variables|Default|GetLEDPhrases) _returnvalue)
        (Default|SetXYPositions _returnvalue (Default|GetLetterXYs (Variables|Default|GetLED%20Alphabet) _array_element)))
      (CallFunction|ShowPhrase))))

(fn CrosshairHoverMoved
  (params (Hit%20Location :type Vector :default "0, 0, 0"))
  (return false))

(fn CrosshairHoverProgress
  (params (Progress :type Float%20%28single-precision%29) (Local%20Hit%20Location :type Vector :default "0, 0, 0") (Hit%20Component :type Primitive%20Component%20Object%20Reference))
  (return false))

(fn CrosshairHoverStart
  (params (Finished :type Boolean))
  (return false))

(fn CrosshairLeftRight
  (params (Left :type Boolean))
  (return false))

(fn CrosshairMouseClick
  (params (Mouse%20Down :type Boolean) (Event%20Type :type E_EventType%20Enum :default "NewEnumerator10") (Hit%20Location :type Vector :default "0, 0, 0") (Hit%20Component :type Primitive%20Component%20Object%20Reference))
  (return false))

(fn CrosshairScrollWheel
  (params (Down :type Boolean) (Hit%20Location :type Vector :default "0, 0, 0") (Hit%20Component :type Primitive%20Component%20Object%20Reference))
  (Utilities|FlowControl|Sequence
    (:then_0
      (if (Variables|Default|GetEnable%20scroll%20wheel)
        (if Down
          (LocalVariables|SetYOffset 1)
          (else
            (LocalVariables|SetYOffset -1)))
        (for _array_element (Variables|Default|GetLEDPhrases)
          (Default|AddXYOffsets _array_element 0 (LocalVariables|GetYOffset))
          (CallFunction|RefreshLEDs))))
    (:then_1
      (return false))))

(fn CrosshairUpDown
  (params (Up :type Boolean))
  (return false))