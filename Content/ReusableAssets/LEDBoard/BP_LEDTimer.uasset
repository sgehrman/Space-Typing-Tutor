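; LED board stopwatch actor showing minutes, seconds and centiseconds as glowing dots, with start, pause and reset.
; A looping timer adds time since start to the total banked on pause, then redraws.
; Once a spawned BP_LEDAlphabet loads, digit and colon patterns are cached as grid tags mapped to cell indices.
; Each redraw reuses emissive instanced-mesh LEDs, adding any missing and shrinking extras instead of removing them.
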(event Custom|Update%20Seconds
  (Utilities|FlowControl|Sequence
    (:then_0
      (CallFunction|UpdateElapsedTime (Math|DateTime|Now)))
    (:then_2
      (CallFunction|UpdateDisplayedDigits))))

(event Custom|Start%20Stopwatch
  (if (Class|KismetSystemLibrary|IsTimerPaused 0 "Update Seconds")
    (Class|KismetSystemLibrary|UnPauseTimer 0 "Update Seconds")
    (Variables|Default|SetStart%20Time (Math|DateTime|Now))
    (else
      (CallFunction|ResetStopwatch)
      (Variables|Default|SetStart%20Time (Math|DateTime|Now))
      (Utilities|Time|SetTimerbyFunctionName 0 "Update Seconds" 0.093 true))))

(event Custom|Pause%20Stopwatch
  (Class|KismetSystemLibrary|PauseTimer 0 "Update Seconds")
  (Variables|Default|SetPrevious%20Timespan (+ (Variables|Default|GetPrevious%20Timespan) (Variables|Default|GetElapsed%20Timespan))))

(event Custom|Reset%20Stopwatch
  (bind _returnvalue (Class|KismetMathLibrary|TimespanZeroValue))
  (CallFunction|PauseStopwatch)
  (Utilities|FlowControl|Sequence
    (:then_0
      (Variables|Default|SetElapsed%20Timespan _returnvalue))
    (:then_1
      (Variables|Default|SetPrevious%20Timespan _returnvalue))
    (:then_2
      (CallFunction|UpdateDisplayedDigits))))

(event Custom|Update%20Displayed%20Digits
  (bind _elapsed_timespan (Variables|Default|GetElapsed%20Timespan))
  (bind _previous_timespan (Variables|Default|GetPrevious%20Timespan))
  (bind _returnvalue (+ _elapsed_timespan _previous_timespan))
  (bind _digits (CallFunction|TimerDigits (/ (Class|KismetMathLibrary|GetMilliseconds _returnvalue) 10) (Math|Timespan|GetSeconds _returnvalue) (Math|Timespan|GetMinutes _returnvalue)))
  (CallFunction|RefreshLEDs _digits))

(event Custom|Loaded
  (CallFunction|SetupDisplay 9 7))

(event EventBeginPlay
  (Utilities|FlowControl|Sequence
    (:then_0
      (bind _returnvalue (Game|SpawnActorfromClass "/Game/ReusableAssets/LEDBoard/BP_LEDAlphabet.BP_LEDAlphabet_C" (Math|Transform|MakeTransform "0, 0, 0") true self 0))
      (bind _output_get (Variables|Default|SetLED%20Alphabet _returnvalue))
      (EventDispatchers|BindEventtoLoadedandReady _output_get (delegate Custom|Loaded)))
    (:then_1
      (Variables|Default|SetTagToIndexMap (Class|KrishnaMap|Create)))
    (:then_2
      (Variables|Default|SetTag%20To%20Instance%20Index (Class|KrishnaMap|Create)))
    (:then_4
      (Default|Setup (Variables|Default|GetLED%20Alphabet)))))

(fn ConstructionScript
  (Utilities|FlowControl|Sequence
    (:then_0
      (bind _returnvalue (Rendering|Material|CreateDynamicMaterialInstance "/Game/ReusableAssets/Materials/MT_Opaque.MT_Opaque" :!class /Script/Engine.KismetMaterialLibrary))
      (bind _output_get (Variables|Default|SetOn%20MID _returnvalue))
      (Rendering|Material|SetScalarParameterValue _output_get "Emission" 33.0 :!class /Script/Engine.MaterialInstanceDynamic))
    (:then_1
      (bind _returnvalue_2 (AddComponent|AddInstancedStaticMeshComponent false))
      (bind _output_get_2 (Variables|Default|SetOn%20Instanced%20Static%20Mesh _returnvalue_2))
      (Rendering|Material|SetMaterial _output_get_2 0 (Variables|Default|GetOn%20MID))
      (Rendering|SetCastShadow _output_get_2 false)
      (Collision|SetCollisionEnabled _output_get_2 "NoCollision"))))

(fn TransformforIndex
  (params (Index :type Integer :default 0) (Number%20of%20Columns :type Integer :default 0) (Num%20LED%20Offset :type Integer))
  (bind _returnvalue (Math|Conversions|ToFloat(Integer) Index))
  (bind _returnvalue_2 (Math|Conversions|ToFloat(Integer) Number%20of%20Columns))
  (bind _led_scale (Variables|Default|GetLED%20Scale))
  (bind _led_extent (Variables|Default|GetLED%20Extent))
  (bind _returnvalue_3 (Math|Vector|MakeVector _led_extent _led_extent _led_extent))
  (bind _location (CallFunction|LocationinGrid _returnvalue _returnvalue_2 0.0 _returnvalue_3))
  (return (Math|Transform|MakeTransform (Math|Vector|MakeVector (.x _location) (+ (* Num%20LED%20Offset (Variables|Default|GetLED%20Extent)) (.y _location)) (.z _location)) "0, 0, 0" (Math|Vector|MakeVector _led_scale _led_scale _led_scale))))

(fn RefreshLEDs
  (params (XYStrings :type Array%20of%20S%20LED%20Digit%20Structures))
  (bind _on_instanced_static_mesh (Variables|Default|GetOn%20Instanced%20Static%20Mesh))
  (bind _on_instanced_static_mesh_2 (Variables|Default|GetOn%20Instanced%20Static%20Mesh))
  (Utilities|FlowControl|Sequence
    (:then_0
      (LocalVariables|SetInstance%20Count (Components|InstancedStaticMesh|GetInstanceCount (Variables|Default|GetOn%20Instanced%20Static%20Mesh)))
      (LocalVariables|SetInstance%20Index 0))
    (:then_1
      (for _array_element XYStrings
        (for _array_element_2 (.XYStrings (Utilities|Struct|BreakS_LED_Digit _array_element))
          (if (.IsValid (Class|KrishnaMap|StringIntGet (Variables|Default|GetTagToIndexMap) _array_element_2))
            (bind _result (CallFunction|TransformforIndex (.ReturnValue (Class|KrishnaMap|StringIntGet (Variables|Default|GetTagToIndexMap) _array_element_2)) (Variables|Default|GetWidth) (LocalVariables|GetNum%20LED%20Offset)))
            (if (> (LocalVariables|GetInstance%20Count) 0)
              (Components|InstancedStaticMesh|UpdateInstanceTransform _on_instanced_static_mesh (LocalVariables|GetInstance%20Index) _result false false)
              (Math|Integer|DecrementInt (LocalVariables|GetInstance%20Count)
                (:%20%20
                  (Math|Integer|IncrementInt (LocalVariables|GetInstance%20Index))))
              (else
                (Components|InstancedStaticMesh|AddInstance _on_instanced_static_mesh _result)))))
        (LocalVariables|SetNum%20LED%20Offset (+ (LocalVariables|GetNum%20LED%20Offset) (.LED_Width (Utilities|Struct|BreakS_LED_Digit _array_element)))))
      (if (> (LocalVariables|GetInstance%20Count) 0)
        ;[1 1 1] Comment
        (for _index (range (LocalVariables|GetInstance%20Index) (- (+ (LocalVariables|GetInstance%20Index) (LocalVariables|GetInstance%20Count)) 1))
          (bind _returnvalue (Components|InstancedStaticMesh|UpdateInstanceTransform (Variables|Default|GetOn%20Instanced%20Static%20Mesh) _index (Math|Transform|MakeTransform "0.000000,0.000000, 0" "0, 0, 0" "0.001000,0.001000,0.001000") false false))
          (if (not _returnvalue)
            (CallFunction|Logg (Class|VictoryBPFunctionLibrary|AppendMultiple "ERR: Transform Index: " (Utilities|String|ToString(Integer) _index)))))
        ;[1 1 1] Mark dirty at end.  seems weird, but hoping this is optimal
        (Components|InstancedStaticMesh|UpdateInstanceTransform _on_instanced_static_mesh_2 0 (.OutInstanceTransform (Components|InstancedStaticMesh|GetInstanceTransform _on_instanced_static_mesh_2 0 false)) false true)))))

(fn SetupDisplay
  (params (Height :type Integer) (Width :type Integer))
  (Utilities|FlowControl|Sequence
    (:then_0
      (Variables|Default|SetHeight Height)
      (Variables|Default|SetWidth Width))
    (:then_1
      (for _index (range 0 (- (* (Variables|Default|GetWidth) (Variables|Default|GetHeight)) 1))
        (Class|KrishnaMap|StringIntAddPair (Variables|Default|GetTagToIndexMap) (CallFunction|LEDTagforIndex _index (Variables|Default|GetWidth)) _index)
        (Utilities|Array|Add (Variables|Default|GetIndexToTagArray) (CallFunction|LEDTagforIndex _index (Variables|Default|GetWidth)))))
    (:then_2
      (for _index_2 (range 0 9)
        (bind _returnvalue (AddComponent|AddBPLEDPhrase))
        (Default|SetXYPositions _returnvalue (Default|GetLetterXYs (Variables|Default|GetLED%20Alphabet) (Utilities|String|ToString(Integer) _index_2)))
        (Utilities|Array|Add (Variables|Default|GetLED%20Digits) (Utilities|Struct|MakeS_LED_Digit (Default|GetXYStringArray _returnvalue) (Variables|Default|GetWidth)))))
    (:then_3
      (bind _returnvalue_2 (AddComponent|AddBPLEDPhrase))
      (Default|SetXYOffsets _returnvalue_2 -2)
      (Default|SetXYPositions _returnvalue_2 (Default|GetLetterXYs (Variables|Default|GetLED%20Alphabet) ":"))
      (Variables|Default|SetLED%20Colon (Utilities|Struct|MakeS_LED_Digit (Default|GetXYStringArray _returnvalue_2) 3))
      ;[1 1 1] For speed, no reason to create a new array every update
      (Variables|Default|SetLED%20Colon%20Array (Utilities|Array|MakeArray (Variables|Default|GetLED%20Colon))))))

(fn XYStringsforNumber
  (params (Number :type Integer))
  (Utilities|FlowControl|Sequence
    (:then_0
      (Utilities|Array|Add (LocalVariables|GetResult) (Utilities|Array|Get(acopy) (Variables|Default|GetLED%20Digits) (/ Number 10))))
    (:then_2
      (Utilities|Array|Add (LocalVariables|GetResult) (Utilities|Array|Get(acopy) (Variables|Default|GetLED%20Digits) (Math|Integer|%(Integer) Number 10))))
    (:then_3
      (return (LocalVariables|GetResult)))))

(fn TimerDigits
  (params (Centiseconds :type Integer) (Seconds :type Integer) (Minutes :type Integer))
  (Utilities|FlowControl|Sequence
    (:then_0
      (LocalVariables|SetResult%20Digits (CallFunction|XYStringsforNumber Minutes)))
    (:then_1
      (Utilities|Array|AppendArray (LocalVariables|GetResult%20Digits) (Variables|Default|GetLED%20Colon%20Array)))
    (:then_2
      (Utilities|Array|AppendArray (LocalVariables|GetResult%20Digits) (CallFunction|XYStringsforNumber Seconds)))
    (:then_3
      (Utilities|Array|AppendArray (LocalVariables|GetResult%20Digits) (Variables|Default|GetLED%20Colon%20Array)))
    (:then_4
      (Utilities|Array|AppendArray (LocalVariables|GetResult%20Digits) (CallFunction|XYStringsforNumber Centiseconds)))
    (:then_5
      (return (LocalVariables|GetResult%20Digits)))))

(fn UpdateElapsedTime
  (params (End%20Time :type Date%20Time%20Structure))
  (Variables|Default|SetElapsed%20Timespan (- End%20Time (Variables|Default|GetStart%20Time))))