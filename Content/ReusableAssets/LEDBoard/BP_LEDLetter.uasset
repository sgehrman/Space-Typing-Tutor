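; A single LED-matrix letter that builds a grid of mesh LEDs at BeginPlay and displays characters using patterns from BP_LEDAlphabet.
; It can listen to the main typewriter to show typed characters, or, after Enter in editor mode, save the current pattern under the next key.
; Crosshair clicks toggle LEDs by material swap, and lit LEDs serialize as comma-separated component tags.
; SetPhysics just plays a timeline gathering LEDs from a circle into the grid.
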(event Custom|DoIT
  (bind _result (CallFunction|BuildAnimationInfoArray))
  (Variables|Default|SetAnimationInfoArray _result)
  (Components|Timeline|SetPlayRate 2.0)
  (bind _alpha (Timeline|AnimateLEDs PlayFromStart)
    (:Update
      (for (_array_element _array_index) (Variables|Default|GetLEDs)
        (Transformation|SetRelativeLocation _array_element (Math|Vector|Lerp(Vector) (.start (Utilities|Array|Get(acopy) (Variables|Default|GetAnimationInfoArray) _array_index)) (.end (Utilities|Array|Get(acopy) (Variables|Default|GetAnimationInfoArray) _array_index)) _alpha) false)))))

(event Custom|KeyPressedEventHandler
  (params (Character :type String) (Key%20Type :type ESpecialKeyEnum%20Enum :default "Key_Other"))
  (switch Utilities|FlowControl|Switch|SwitchonESpecialKeyEnum Key%20Type
    (:Key_Other
      (if (Variables|Default|GetSaveMode)
        (Variables|Default|SetSaveMode false)
        (bind _result (CallFunction|LEDStatetoString))
        (Default|SaveLetter (Variables|Default|GetLED%20Alphabet) Character _result)
        (else
          (CallFunction|DisplayCharacter Character))))
    (:Key_Enter
      (if (Variables|Default|GetEnable%20Editor)
        (Variables|Default|SetSaveMode true)))))

(event EventBeginPlay
  (Utilities|FlowControl|Sequence
    (:then_0
      (bind _asbp_ledalphabet (Utilities|Casting|CastToBP_LEDAlphabet (.Actor (CallFunction|FindActorwithTag "/Game/ReusableAssets/LEDBoard/BP_LEDAlphabet.BP_LEDAlphabet_C" "" self)))
        (:then
          (Variables|Default|SetLED%20Alphabet _asbp_ledalphabet))
        (:CastFailed
          (CallFunction|Logg "Couldn't find BP_LEDAlphabet.  Drag that in to scene."))))
    (:then_1
      (CallFunction|CreateLEDs))
    (:then_2
      (if (Variables|Default|GetListen%20to%20Typewriter)
        (bind _asbp_typewriter (Utilities|Casting|CastToBP_Typewriter (.Actor (CallFunction|FindActorwithTag "/Game/ReusableAssets/Keyboard/BP_Typewriter.BP_Typewriter_C" "MainTypewriter" self))))
        (bind _output_get (Variables|Default|SetTypewriter _asbp_typewriter))
        (EventDispatchers|BindEventtoKeyPressedEvent _output_get (delegate Custom|KeyPressedEventHandler))))))

(fn ConstructionScript)

(fn LEDStatetoString
  (for _array_element (Variables|Default|GetLEDs)
    (if (== (Rendering|Material|GetMaterial _array_element 0) (Variables|/Game/ReusableAssets/LEDBoard/BP_LEDAlphabet.BP_LEDAlphabet_C|GetOn%20MID (Variables|Default|GetLED%20Alphabet)))
      (Utilities|Array|Add (LocalVariables|GetResult%20Array) (Utilities|String|ToString(Name) (Utilities|Array|Get(acopy) (Variables|/Script/Engine.ActorComponent|GetComponentTags _array_element))))))
  (for _array_element_2 (LocalVariables|GetResult%20Array)
    (Utilities|FlowControl|Sequence
      (:then_0
        (if (> (Utilities|String|Len (LocalVariables|GetResult%20String)) 0)
          (LocalVariables|SetResult%20String (Utilities|String|Append (LocalVariables|GetResult%20String) ","))))
      (:then_1
        (LocalVariables|SetResult%20String (Utilities|String|Append (LocalVariables|GetResult%20String) _array_element_2)))))
  (return (LocalVariables|GetResult%20String)))

(fn StringtoLEDState
  (params (LED%20State%20String :type String))
  ;[1 1 1] Set all to off state
  (for _array_element (Variables|Default|GetLEDs)
    (Rendering|Material|SetMaterial _array_element 0 (Variables|/Game/ReusableAssets/LEDBoard/BP_LEDAlphabet.BP_LEDAlphabet_C|GetOff%20MID (Variables|Default|GetLED%20Alphabet))))
  (for _array_element_2 (Class|VictoryBPFunctionLibrary|StringExplodeString LED%20State%20String "," 0 true)
    (if (.Valid (Default|IndexforTag (Variables|Default|GetLED%20Alphabet) _array_element_2))
      (Rendering|Material|SetMaterial (Utilities|Array|Get(acopy) (Variables|Default|GetLEDs) (.Index (Default|IndexforTag (Variables|Default|GetLED%20Alphabet) _array_element_2))) 0 (Variables|/Game/ReusableAssets/LEDBoard/BP_LEDAlphabet.BP_LEDAlphabet_C|GetOn%20MID (Variables|Default|GetLED%20Alphabet))))))

(fn CreateLEDs
  (bind _led_alphabet (Variables|Default|GetLED%20Alphabet))
  (bind _led_alphabet_2 (Variables|Default|GetLED%20Alphabet))
  (bind (_columns _rows _led_count) (Default|LEDSettings _led_alphabet_2))
  (for _index (range 0 (- _led_count 1))
    (bind _returnvalue (AddComponent|AddStaticMeshComponent false (CallFunction|TransformforIndex _index _columns)))
    (Utilities|Array|Add (Variables|Default|GetLEDs) _returnvalue)
    (Rendering|Material|SetMaterial _returnvalue 0 (Variables|/Game/ReusableAssets/LEDBoard/BP_LEDAlphabet.BP_LEDAlphabet_C|GetOff%20MID _led_alphabet))
    (Variables|/Script/Engine.ActorComponent|SetComponentTags _returnvalue (Utilities|Array|MakeArray (Utilities|String|StringToName (.Tag (Default|TagforIndex _led_alphabet _index)))))))

(fn DisplayCharacter
  (params (Character :type String))
  (bind _led_alphabet (Variables|Default|GetLED%20Alphabet))
  (bind (_valid _led_data) (Default|GetLetter _led_alphabet Character))
  (Utilities|FlowControl|Sequence
    (:then_0
      (if _valid
        (CallFunction|StringtoLEDState _led_data)))
    (:then_1
      (return))))

(fn SetPhysics
  (params (Simulate%20Physics :type Boolean :default false))
  (CallFunction|DoIT))

(fn TransformforIndex
  (params (Index :type Integer :default 0) (Num%20Columns :type Integer :default 0))
  (return (Math|Transform|MakeTransform (CallFunction|LocationinGrid (Math|Conversions|ToFloat(Integer) Index) (Math|Conversions|ToFloat(Integer) Num%20Columns) 0.5 "10.000000,10.000000,10.000000") "0, 0, 0" "0.100000,0.100000,0.100000")))

(fn BuildAnimationInfoArray
  (bind _leds (Variables|Default|GetLEDs))
  (Utilities|FlowControl|Sequence
    (:then_1
      (LocalVariables|SetColumns (.Columns (Default|LEDSettings (Variables|Default|GetLED%20Alphabet)))))
    (:then_2
      (for (_ _array_index) _leds
        (Utilities|Array|Add (LocalVariables|GetResult%20Array) (Utilities|Struct|MakeS_StartEndVectors (.Location (CallFunction|LocationAroundCircle _array_index (Utilities|Array|Length _leds) 1.11e+03 "1.000000,0.000000,0.000000" 0.0)) (.location (CallFunction|TransformforIndex _array_index (LocalVariables|GetColumns)))))))
    (:then_4
      (return (LocalVariables|GetResult%20Array)))))

(fn CrosshairHoverProgress
  (params (Progress :type Float%20%28single-precision%29) (Local%20Hit%20Location :type Vector :default "0, 0, 0") (Hit%20Component :type Primitive%20Component%20Object%20Reference))
  (return false))

(fn CrosshairHoverStart
  (params (Finished :type Boolean))
  (return false))

(fn CrosshairLeftRight
  (params (Left :type Boolean))
  (return false))

(fn CrosshairMouseClick
  (params (Mouse%20Down :type Boolean) (Event%20Type :type E_EventType%20Enum :default "NewEnumerator10") (Hit%20Location :type Vector :default "0, 0, 0") (Hit%20Component :type Primitive%20Component%20Object%20Reference))
  (bind _led_alphabet (Variables|Default|GetLED%20Alphabet))
  (bind _off_mid (Variables|/Game/ReusableAssets/LEDBoard/BP_LEDAlphabet.BP_LEDAlphabet_C|GetOff%20MID _led_alphabet))
  (Utilities|FlowControl|Sequence
    (:then_0
      (if Mouse%20Down
        (bind _asmesh_component (Utilities|Casting|CastToMeshComponent Hit%20Component))
        (if (== (Rendering|Material|GetMaterial _asmesh_component 0) _off_mid)
          (Rendering|Material|SetMaterial _asmesh_component 0 (Variables|/Game/ReusableAssets/LEDBoard/BP_LEDAlphabet.BP_LEDAlphabet_C|GetOn%20MID (Variables|Default|GetLED%20Alphabet)))
          (else
            (Rendering|Material|SetMaterial _asmesh_component 0 _off_mid)))))
    (:then_1
      (return false))))

(fn CrosshairScrollWheel
  (params (Down :type Boolean) (Hit%20Location :type Vector :default "0, 0, 0") (Hit%20Component :type Primitive%20Component%20Object%20Reference))
  (return false))

(fn CrosshairUpDown
  (params (Up :type Boolean))
  (return false))