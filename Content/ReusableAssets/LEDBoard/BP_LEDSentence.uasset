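; BP_LEDSentence is a Blueprint wrapper for an LED display that shows strings and numbers.
; On BeginPlay it adds a child actor component at runtime, stores its actor as a BP_LEDLayout and sets it up with a fixed height and width.
; Its Display String and Display Number functions forward directly to that layout, which handles the display itself.
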(event `self.ReceiveBeginPlay`
  (`self.SetupDisplay` 9 7))

(fn `Display Number`
  (params (Number :type Integer))
  (`/Game/ReusableAssets/LEDBoard/BP_LEDLayout.Display Number` (`self.LED Layout`) Number))

(fn `Display String`
  (params (String :type String))
  (`/Game/ReusableAssets/LEDBoard/BP_LEDLayout.Display String` (`self.LED Layout`) String))

(fn `SetupDisplay`
  (params (Height :type Integer) (Width :type Integer))
  (bind _returnvalue (`AddComponent|Child Actor Component_0`))
  (bind _asbp_ledlayout (cast `/Game/ReusableAssets/LEDBoard/BP_LEDLayout` (`ChildActorComponent.ChildActor` _returnvalue)))
  (bind _output_get (set `self.LED Layout` _asbp_ledlayout))
  (`/Game/ReusableAssets/LEDBoard/BP_LEDLayout.SetupDisplay` _output_get Height Width))

(fn `UserConstructionScript`)