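; Decorative LED pentagram that pulses its emissive color and cycles through looping light and fire animations.
; The construction script builds it from one instanced static mesh, placing LEDs around a circle and along the five star lines.
; A timeline tints the shared dynamic material, while a timer-driven state machine shrinks and restores LEDs one by one, spawns fire jets on alternate LEDs, then clears them, pausing between phases.
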(event Custom|FireAnimationStep
  (params (Forward :type Boolean :default false))
  (if Forward
    (bind _returnvalue (Effects|SpawnEmitterAttached "/Game/Vectorfields/Particles/P_FireJet.P_FireJet" (Variables|Default|GetRoot) "None" (.location (.OutInstanceTransform (Components|InstancedStaticMesh|GetInstanceTransform (Variables|Default|GetOn%20Instanced%20Static%20Mesh) (Variables|Default|GetFlickerIndex) false)))))
    (Utilities|Array|Add (Variables|Default|GetSpawned%20Emitters) _returnvalue)
    (bind _output_get (Variables|Default|SetFlickerIndex (- (Variables|Default|GetFlickerIndex) 2)))
    (if (< _output_get 0)
      (CallFunction|DoNextAnimation))
    (else
      (for _array_element (Variables|Default|GetSpawned%20Emitters)
        (Components|DestroyComponent _array_element))
      (Utilities|Array|Clear (Variables|Default|GetSpawned%20Emitters))
      (CallFunction|DoNextAnimation))))

(event Custom|StartNextAnimation
  (params (Animation :type E_PentagramAnimations%20Enum :default "NewEnumerator0"))
  (Variables|Default|SetCurrent%20Animation Animation)
  (Variables|Default|SetFlickerIndex (Components|InstancedStaticMesh|GetInstanceCount (Variables|Default|GetOn%20Instanced%20Static%20Mesh)))
  (Utilities|FlowControl|Delay 2.0)
  (Utilities|Time|SetTimerbyFunctionName 0 "AnimationTimerEvent" 0.01 true))

(event Custom|FlickerAnimationStep
  (params (Forward :type Boolean :default false))
  (bind _on_instanced_static_mesh (Variables|Default|GetOn%20Instanced%20Static%20Mesh))
  (if Forward
    (Variables|Default|SetFlickerScale (Math|Vector|MakeVector 0.1 0.1 0.1))
    (else
      (Variables|Default|SetFlickerScale (Math|Vector|MakeVector 1.0 1.0 1.0))))
  (Components|InstancedStaticMesh|UpdateInstanceTransform _on_instanced_static_mesh (Variables|Default|GetFlickerIndex) (Math|Transform|MakeTransform (.location (.OutInstanceTransform (Components|InstancedStaticMesh|GetInstanceTransform _on_instanced_static_mesh (Variables|Default|GetFlickerIndex) false))) (.rotation (.OutInstanceTransform (Components|InstancedStaticMesh|GetInstanceTransform _on_instanced_static_mesh (Variables|Default|GetFlickerIndex) false))) (Variables|Default|GetFlickerScale)) false true)
  (bind _output_get (Variables|Default|SetFlickerIndex (- (Variables|Default|GetFlickerIndex) 1)))
  (if (< _output_get 0)
    (CallFunction|DoNextAnimation)))

(event Custom|AnimationTimerEvent
  (switch Utilities|FlowControl|Switch|SwitchonE_PentagramAnimations (Variables|Default|GetCurrent%20Animation)
    (:NewEnumerator0
      (CallFunction|FlickerAnimationStep true))
    (:NewEnumerator1
      (CallFunction|FlickerAnimationStep false))
    (:NewEnumerator2
      (CallFunction|FireAnimationStep true))
    (:NewEnumerator3
      (CallFunction|FireAnimationStep false))))

(event Custom|DoNextAnimation
  (Utilities|Time|ClearTimerbyFunctionName 0 "AnimationTimerEvent")
  (switch Utilities|FlowControl|Switch|SwitchonE_PentagramAnimations (Variables|Default|GetCurrent%20Animation)
    (:NewEnumerator0
      (CallFunction|StartNextAnimation "NewEnumerator1"))
    (:NewEnumerator1
      (CallFunction|StartNextAnimation "NewEnumerator2"))
    (:NewEnumerator2
      (CallFunction|StartNextAnimation "NewEnumerator3"))
    (:NewEnumerator3
      (CallFunction|StartNextAnimation "NewEnumerator0"))))

(event EventBeginPlay
  (Utilities|FlowControl|Sequence
    (:then_0
      (bind _alpha (Timeline|Pulsate%20colors Play)
        (:Update
          (Rendering|Material|SetVectorParameterValue (Variables|Default|GetOn%20MID) "EmissiveColor" (Math|Color|Lerp(LinearColor) "(R=0.000000,G=0.001365,B=0.085000,A=1.000000)" "(R=0.035000,G=0.005704,B=0.003027,A=1.000000)" _alpha) :!class /Script/Engine.MaterialInstanceDynamic))))
    (:then_1
      (CallFunction|StartNextAnimation "NewEnumerator0"))))

(fn ConstructionScript
  (Utilities|FlowControl|Sequence
    (:then_0
      (bind _returnvalue (Rendering|Material|CreateDynamicMaterialInstance "/Game/ReusableAssets/Materials/MT_Opaque.MT_Opaque" :!class /Script/Engine.KismetMaterialLibrary))
      (bind _output_get (Variables|Default|SetOn%20MID _returnvalue))
      (Rendering|Material|SetScalarParameterValue _output_get "Emission" 333.0 :!class /Script/Engine.MaterialInstanceDynamic))
    (:then_1
      (bind _returnvalue_2 (AddComponent|AddInstancedStaticMeshComponent false))
      (bind _output_get_2 (Variables|Default|SetOn%20Instanced%20Static%20Mesh _returnvalue_2))
      (Rendering|Material|SetMaterial _output_get_2 0 (Variables|Default|GetOn%20MID))
      (Rendering|SetCastShadow _output_get_2 false))
    (:then_2
      (CallFunction|RefreshLEDs))))

(fn RefreshLEDs
  (bind _number_of_leds_on_circle (Variables|Default|GetNumber%20of%20LEDs%20on%20Circle))
  (Utilities|FlowControl|Sequence
    (:then_0
      (for _index (range 0 (- _number_of_leds_on_circle 1))
        (Components|InstancedStaticMesh|AddInstance (Variables|Default|GetOn%20Instanced%20Static%20Mesh) (Math|Transform|MakeTransform (.Location (CallFunction|LocationAroundCircle _index _number_of_leds_on_circle (Variables|Default|GetRadius) "1.000000, 0, 0" 0.0)) "0, 0, 0" "1.000000,1.000000,1.000000"))))
    (:then_1
      (for _index_2 (range 0 4)
        (bind _output_get (LocalVariables|SetStart%20Point (.Location (CallFunction|LocationAroundCircle _index_2 5 (Variables|Default|GetRadius) "1.000000, 0, 0" 0.0))))
        (bind _output_get_2 (LocalVariables|SetEnd%20Point (.Location (CallFunction|LocationAroundCircle (Math|Integer|%(Integer) (+ _index_2 2) 5) 5 (Variables|Default|GetRadius) "1.000000, 0, 0" 0.0))))
        (LocalVariables|SetLine%20Length (Math|Vector|VectorLength (- _output_get_2 _output_get)))
        (LocalVariables|SetRun%20Loop true)
        (LocalVariables|SetDirectional%20Offset 0.0)
        (while (LocalVariables|GetRun%20Loop)
          (Components|InstancedStaticMesh|AddInstance (Variables|Default|GetOn%20Instanced%20Static%20Mesh) (Math|Transform|MakeTransform (+ (LocalVariables|GetStart%20Point) (* (Math|Vector|Normalize (- (LocalVariables|GetEnd%20Point) (LocalVariables|GetStart%20Point))) (LocalVariables|GetDirectional%20Offset)))))
          (bind _output_get_3 (LocalVariables|SetDirectional%20Offset (+ (LocalVariables|GetDirectional%20Offset) (LocalVariables|GetWidth%20of%20Mesh))))
          (LocalVariables|SetRun%20Loop (< _output_get_3 (LocalVariables|GetLine%20Length))))))))