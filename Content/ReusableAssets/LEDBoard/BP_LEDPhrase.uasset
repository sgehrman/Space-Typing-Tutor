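; BP_LEDPhrase represents a phrase for an LED board as a set of XY positions plus a movable X/Y offset.
; GetXYStringArray lazily converts each offset position into an LED tag string through LEDTagForXY and caches the results.
; Setting positions or changing offsets clears that cache, so the tags are rebuilt on the next request.
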(event `self.ReceiveTick`
  (params (DeltaSeconds :type "Float (single-precision)")))

(event `self.ReceiveBeginPlay`)

(fn `AddXYOffsets`
  (params (`Add X` :type Integer :default 0) (`Add Y` :type Integer :default 0))
  (set `self.OffsetY` (+ (`self.OffsetY`) `Add Y`))
  (set `self.OffsetX` (+ (`self.OffsetX`) `Add X`))
  (`KismetArrayLibrary.Array_Clear` (`self.XY Strings`)))

(fn `GetXYStringArray`
  (returns (Result :type "Array of String"))
  (if (== (`KismetArrayLibrary.Array_Length` (`self.XY Strings`)) 0)
    (for _array_element (`self.XY Positions`)
      (bind (_x _y) (break `/Game/ReusableAssets/LEDBoard/S_LEDXY` _array_element))
      (`KismetArrayLibrary.Array_Add` (`self.XY Strings`) (`/Game/ReusableAssets/Utilities/LIB_Utilities.LEDTagForXY` (+ (`self.OffsetX`) _x) (+ (`self.OffsetY`) _y)))))
  (return (`self.XY Strings`)))

(fn `IncrementXYOffsets`
  (params (`X Increment` :type Integer :default 0) (`Y Increment` :type Integer :default 0))
  (`self.SetXYOffsets` (+ (`self.OffsetX`) `X Increment`) (+ (`self.OffsetY`) `Y Increment`)))

(fn `SetXYOffsets`
  (params (X :type Integer :default 0) (Y :type Integer :default 0))
  (set `self.OffsetX` X)
  (set `self.OffsetY` Y)
  (`KismetArrayLibrary.Array_Clear` (`self.XY Strings`)))

(fn `SetXYPositions`
  (params (Positions :type "Array of /Game/ReusableAssets/LEDBoard/S_LEDXY Structure"))
  (set `self.XY Positions` Positions)
  (`KismetArrayLibrary.Array_Clear` (`self.XY Strings`)))