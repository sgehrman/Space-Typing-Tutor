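; BP_LEDSign is an LED sign actor that embeds a BP_LEDTimer through a child actor component to provide stopwatch controls.
; The construction script casts the child actor and caches it as LEDTimer.
; Its start, pause and reset functions forward to that timer, with pause mapped to the timer's StopStopwatch.
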(event `self.ReceiveBeginPlay`)

(fn `Pause Stopwatch`
  (`/Game/ReusableAssets/LEDBoard/BP_LEDTimer.Stop Stopwatch` (`self.LED Timer`)))

(fn `Reset Stopwatch`
  (`/Game/ReusableAssets/LEDBoard/BP_LEDTimer.Reset Stopwatch` (`self.LED Timer`)))

(fn `Start Stopwatch`
  (`/Game/ReusableAssets/LEDBoard/BP_LEDTimer.Start Stopwatch` (`self.LED Timer`)))

(fn `UserConstructionScript`
  (bind _asbp_ledtimer (cast `/Game/ReusableAssets/LEDBoard/BP_LEDTimer` (`ChildActorComponent.ChildActor` (`self.LED Timer Component`))))
  (set `self.LED Timer` _asbp_ledtimer))