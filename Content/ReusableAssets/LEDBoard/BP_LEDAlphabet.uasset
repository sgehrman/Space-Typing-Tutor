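; BP_LEDAlphabet is the glyph store for an LED board, mapping characters to lit-LED data and converting strings into offset XY lists.
; Setup builds LED tag/index lookups and on/off dynamic materials, then loads letters from a JSON file and signals readiness.
; SaveLetter updates the map and triggers a one-second coalesced save back to JSON under Content/AppData/LED.
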(event Custom|SaveAfterDelay
  (if (not (Variables|Default|GetSaving))
    (Variables|Default|SetSaving true)
    (Utilities|FlowControl|Delay 1.0)
    (Variables|Default|SetSaving false)
    (CallFunction|SavetoFile)))

(fn ConstructionScript
  ;[1 1 1] This gets called early, so do it before eventbeingplay
  (Variables|Default|SetLED%20Count (* (Variables|Default|GetLED%20Columns) (Variables|Default|GetLED%20Rows))))

(fn GetLetter
  (params (Character :type String))
  (bind _lettersmap (Variables|Default|GetLettersMap))
  (bind (_isvalid _returnvalue) (Class|KrishnaMap|StringStringGet _lettersmap Character))
  (return _isvalid _returnvalue))

(fn SaveLetter
  (params (Character :type String) (LED%20Data :type String))
  (Class|KrishnaMap|StringStringAddPair (Variables|Default|GetLettersMap) Character LED%20Data)
  (CallFunction|SaveAfterDelay))

(fn SavetoFile
  (bind _returnvalue (Class|VictoryBPFunctionLibrary|FileIOSaveStringTexttoFile (Variables|Default|GetDirectory) (Variables|Default|GetFilename) (CallFunction|JSONString) true))
  (if (not _returnvalue)
    (CallFunction|Logg "Save Failed")))

(fn LoadfromFile
  (bind _directory (Variables|Default|GetDirectory))
  (bind _filename (Variables|Default|GetFilename))
  (bind _returnvalue (Class|VictoryBPFunctionLibrary|AppendMultiple _directory _filename))
  (bind (_outstring _returnvalue_2) (Class|FileSystemUtils|LoadFiletoString _returnvalue))
  (if _returnvalue_2
    (Variables|Default|SetLettersMap (Class|KrishnaMap|Create))
    (bind _returnvalue_3 (Class|KrishnaJSON|ParseJson (Class|KrishnaJSON|Create) _outstring))
    (for _array_element (Class|KrishnaJSON|GetKeys _returnvalue_3)
      (Class|KrishnaMap|StringStringAddPair (Variables|Default|GetLettersMap) _array_element (.ReturnValue (Class|KrishnaJSON|GetString _returnvalue_3 _array_element))))
    (Default|CallLoadedandReady)
    (else
      (CallFunction|Logg "read error"))))

(fn JSONString
  (Utilities|FlowControl|Sequence
    (:then_0
      (LocalVariables|SetJSON%20Object (Class|KrishnaJSON|Create)))
    (:then_1
      (for _array_element (Class|KrishnaMap|StringStringGetKeys (Variables|Default|GetLettersMap))
        (if (.IsValid (Class|KrishnaMap|StringStringGet (Variables|Default|GetLettersMap) _array_element))
          (Class|KrishnaJSON|SetString (LocalVariables|GetJSON%20Object) _array_element (.ReturnValue (Class|KrishnaMap|StringStringGet (Variables|Default|GetLettersMap) _array_element)))
          (else
            (CallFunction|Logg "failed to get key"))))
      (return (.OutStr (Class|KrishnaJSON|ToJsonString (LocalVariables|GetJSON%20Object)))))))

(fn TagforIndex
  (params (Index :type Integer :default 0))
  (bind _indextotagarray (Variables|Default|GetIndexToTagArray))
  (Utilities|FlowControl|Sequence
    (:then_0
      (if (< Index (Utilities|Array|Length _indextotagarray))
        (LocalVariables|SetResult%20Tag (Utilities|Array|Get(acopy) _indextotagarray Index))
        (LocalVariables|SetResult%20Valid true)))
    (:then_1
      (return (LocalVariables|GetResult%20Valid) (LocalVariables|GetResult%20Tag)))))

(fn IndexforTag
  (params (Tag :type String))
  (bind _tagtoindexmap (Variables|Default|GetTagToIndexMap))
  (bind (_isvalid _returnvalue) (Class|KrishnaMap|StringIntGet _tagtoindexmap Tag))
  (return _isvalid _returnvalue))

(fn SetupVariables
  (Utilities|FlowControl|Sequence
    (:then_1
      (Variables|Default|SetTagToIndexMap (Class|KrishnaMap|Create)))
    (:then_2
      (Variables|Default|SetDirectory (Class|VictoryBPFunctionLibrary|AppendMultiple (Class|VictoryBPFunctionLibrary|VictoryPathsGameRootDirectory) "Content/" "AppData/" "LED/")))
    (:then_4
      (for _index (range 0 (- (Variables|Default|GetLED%20Count) 1))
        (Class|KrishnaMap|StringIntAddPair (Variables|Default|GetTagToIndexMap) (CallFunction|LEDTagforIndex _index (Variables|Default|GetLED%20Columns)) _index)
        (Utilities|Array|Add (Variables|Default|GetIndexToTagArray) (CallFunction|LEDTagforIndex _index (Variables|Default|GetLED%20Columns)))))
    (:then_5
      (bind _returnvalue (Rendering|Material|CreateDynamicMaterialInstance "/Game/ReusableAssets/Materials/MT_Opaque.MT_Opaque" :!class /Script/Engine.KismetMaterialLibrary))
      (bind _output_get (Variables|Default|SetOff%20MID _returnvalue))
      (if true
        (Rendering|Material|SetVectorParameterValue _output_get "Color" "(R=0.035000,G=0.035000,B=0.035000,A=1.000000)" :!class /Script/Engine.MaterialInstanceDynamic)
        (Rendering|Material|SetScalarParameterValue _output_get "Roughness" 0.0 :!class /Script/Engine.MaterialInstanceDynamic)
        (else
          (Rendering|Material|SetVectorParameterValue _output_get "EmissiveColor" "(R=0.140000,G=0.132990,B=0.032055,A=1.000000)" :!class /Script/Engine.MaterialInstanceDynamic)
          (Rendering|Material|SetScalarParameterValue _output_get "Emission" 1.0 :!class /Script/Engine.MaterialInstanceDynamic))))
    (:then_6
      (bind _returnvalue_2 (Rendering|Material|CreateDynamicMaterialInstance "/Game/ReusableAssets/Materials/MT_Opaque.MT_Opaque" :!class /Script/Engine.KismetMaterialLibrary))
      (bind _output_get_2 (Variables|Default|SetOn%20MID _returnvalue_2))
      (Rendering|Material|SetVectorParameterValue _output_get_2 "EmissiveColor" "(R=0.140000,G=0.025281,B=0.003500,A=1.000000)" :!class /Script/Engine.MaterialInstanceDynamic)
      (Rendering|Material|SetScalarParameterValue _output_get_2 "Emission" 33.0 :!class /Script/Engine.MaterialInstanceDynamic)
      (Rendering|Material|SetScalarParameterValue _output_get_2 "Flicker Mode" 1.0 :!class /Script/Engine.MaterialInstanceDynamic))))

(fn LEDSettings
  (return (Variables|Default|GetLED%20Columns) (Variables|Default|GetLED%20Rows) (Variables|Default|GetLED%20Count)))

(fn GetLetterXYs
  (params (Characters :type String))
  (for _array_element (Utilities|String|GetCharacterArrayfromString Characters)
    (for _array_element_2 (Class|VictoryBPFunctionLibrary|StringExplodeString (.LED%20Data (CallFunction|GetLetter _array_element)) "," 0 false)
      (Utilities|Array|Add (LocalVariables|GetResult) (Utilities|Struct|MakeS_LEDXY (+ (LocalVariables|GetXOffset) (Math|Conversions|ToInteger(Byte) (.LeftS (Utilities|String|Split _array_element_2 ":")))) (Math|Conversions|ToInteger(Byte) (.RightS (Utilities|String|Split _array_element_2 ":"))))))
    (LocalVariables|SetXOffset (- (+ (LocalVariables|GetXOffset) (Variables|Default|GetLED%20Columns)) 1)))
  (return (LocalVariables|GetResult)))

(fn Setup
  (CallFunction|SetupVariables)
  (CallFunction|LoadfromFile))