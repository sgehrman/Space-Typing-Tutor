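; Reusable keyboard listener actor that rebroadcasts key and Shift presses and fires named events when registered key sequences are detected.
; It spawns a KrishnaKeyCatcherActor to intercept input, reclaiming widget focus while enabled and switching to game-only input when disabled.
; Character codes are classified into key types, separating Backspace, Enter and Tab from characters.
; Each registered sequence adds a detector component, which receives presses and is destroyed once matched.
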(event Custom|Private%20Detect%20Key%20Sequence
  (params (Character :type String) (Key%20Type :type E_KeyType%20Enum))
  (for _array_element (Actor|GetComponentsByClass "/Game/Typewriter/C_KeySequenceDetector.C_KeySequenceDetector_C")
    (bind _event_triggered (Default|HandleKeydown _array_element Character Key%20Type))
    (if _event_triggered
      (Default|CallKeySequenceEvent (Variables|/Game/Typewriter/C_KeySequenceDetector.C_KeySequenceDetector_C|GetEvent%20Name _array_element))
      (Components|DestroyComponent _array_element))))

(event Custom|KeyPressedEvent
  (params (CharacterCode :type Integer) (Character :type String))
  (bind (_key_type _clean_character) (CallFunction|KeyTypeforCharacterCode CharacterCode Character))
  (Default|CallKeyboardEvent _key_type _clean_character CharacterCode)
  (CallFunction|PrivateDetectKeySequence _clean_character _key_type))

(event Custom|ShiftPressedEvent
  (params (LeftShiftDown :type Boolean) (RightShiftDown :type Boolean))
  (Utilities|FlowControl|Sequence
    (:then_0
      (Default|CallKeyboardShiftKeyEvent LeftShiftDown RightShiftDown))
    (:then_1
      (if LeftShiftDown
        (CallFunction|PrivateDetectKeySequence "" "NewEnumerator4")))
    (:then_2
      (if RightShiftDown
        (CallFunction|PrivateDetectKeySequence "" "NewEnumerator5")))))

(event Custom|LostFocusEvent
  (if (Variables|Default|GetEnabled)
    (Class|KrishnaKeyCatcherActor|SetWidgetFocus (Variables|Default|GetKey%20Catcher%20Actor) true)))

(event EventBeginPlay
  (bind _returnvalue (Game|SpawnActorfromClass "/Script/KrishnaPlugin.KrishnaKeyCatcherActor" (Math|Transform|MakeTransform "0, 0, 0") false self 0))
  (bind _output_get (Variables|Default|SetKey%20Catcher%20Actor _returnvalue))
  (EventDispatchers|BindEventtoOnInterceptedKeyPress _output_get (delegate Custom|KeyPressedEvent))
  (EventDispatchers|BindEventtoOnInterceptedShiftPress (Variables|Default|GetKey%20Catcher%20Actor) (delegate Custom|ShiftPressedEvent))
  (EventDispatchers|BindEventtoOnLostWidgetFocus (Variables|Default|GetKey%20Catcher%20Actor) (delegate Custom|LostFocusEvent)))

(fn ConstructionScript)

(fn SetEnabled
  (params (Enabled :type Boolean))
  (bind _output_get (Variables|Default|SetEnabled Enabled))
  (if _output_get
    (Class|KrishnaKeyCatcherActor|SetWidgetFocus (Variables|Default|GetKey%20Catcher%20Actor) true)
    (else
      ;[1 1 1] Seems weird, but this is how to get focus back to view port
      (Input|SetInputModeGameOnly (Game|GetPlayerController 0)))))

(fn ListenforKeySequence
  (params (Event%20Name :type String) (Key%20Specs :type Array%20of%20Keyboard%20Key%20Spec%20Structures))
  (bind _returnvalue (AddComponent|AddCKeySequenceDetector))
  (Default|Setup _returnvalue Event%20Name Key%20Specs))

(fn KeyTypeforCharacterCode
  (params (Character%20Code :type Integer) (Character :type String))
  (Utilities|FlowControl|Sequence
    (:then_0
      (if (== Character%20Code 8)
        (LocalVariables|SetResult%20Key%20Type "NewEnumerator1")
        (elif (== Character%20Code 13)
          (LocalVariables|SetResult%20Key%20Type "NewEnumerator2")
          (elif (== Character%20Code 9)
            (LocalVariables|SetResult%20Key%20Type "NewEnumerator3")
            (else
              (LocalVariables|SetResult%20Clean%20Character Character))))))
    (:then_1
      (return (LocalVariables|GetResult%20Key%20Type) (LocalVariables|GetResult%20Clean%20Character)))))