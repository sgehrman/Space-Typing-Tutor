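; BP_DemoLetter is a single-character letter actor for the keyboard demo, pairing a static mesh with a text render.
; Construction gives the mesh a dynamic opaque material instance with zero roughness.
; It exposes functions to set the displayed character and report the mesh's width from its bounds.
; Its fall-away function enables physics and gravity, applies a random-direction force at world origin coordinates, then adds a delayed-destroy component.
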(fn `Fall Away and Destroy`
  (bind _staticmesh (`self.StaticMesh`))
  (`|ExecutionSequence`
    (:`then_0`
      (`PrimitiveComponent.SetSimulatePhysics` _staticmesh true)
      (`PrimitiveComponent.SetEnableGravity` _staticmesh true))
    (:`then_2`
      (`PrimitiveComponent.AddForceAtLocation` _staticmesh (* (`KismetMathLibrary.RandomUnitVector`) 55222.0) (0.0 0.0 0.0) "None"))
    (:`then_5`
      (`AddComponent|BC Delayed Destroy_0`))))

(fn `Get Width`
  (returns (Width :type "Float (double-precision)"))
  (return (* (.y (`.BoxExtent` (`KismetSystemLibrary.GetComponentBounds` (`self.StaticMesh`)))) 2.0)))

(fn `UpdateCharacter`
  (params (Character :type String))
  (`TextRenderComponent.K2_SetText` (`self.TextRender`) (`KismetTextLibrary.Conv_StringToText` Character)))

(fn `UserConstructionScript`
  (`|ExecutionSequence`
    (:`then_0`
      (bind _returnvalue (`KismetMaterialLibrary.CreateDynamicMaterialInstance` "/Game/ReusableAssets/Materials/MT_Opaque.MT_Opaque"))
      (bind _output_get (set `self.MID` _returnvalue))
      (`MaterialInstanceDynamic.SetScalarParameterValue` _output_get "Roughness" 0.0))
    (:`then_3`
      (`PrimitiveComponent.SetMaterial` (`self.StaticMesh`) 0 (`self.MID`)))))