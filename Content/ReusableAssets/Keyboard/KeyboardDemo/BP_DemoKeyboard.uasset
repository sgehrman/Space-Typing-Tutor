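; Keyboard demo actor that spawns a typewriter child actor, types a repeating "Press Enter to Continue" prompt on a timer, and reveals a sentence as keys are pressed.
; BeginPlay positions two tagged spotlights, starts a timeline rotating them, and builds hidden letter child actors in a centered row from cached width-based offsets.
; Each key press event, whatever the key, shows the next letter and flies it into place, wrapping after the last.
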(event Custom|Animate%20Lights
  (Components|Timeline|SetPlayRate (Variables|Default|GetLights%20Timeline) 0.3)
  (bind _alpha (Timeline|Lights%20Timeline PlayFromStart)
    (:Update
      (Transformation|SetRelativeRotation (Variables|/Script/Engine.SpotLight|GetSpotLightComponent (Variables|Default|GetLight%20One)) (Math|Rotator|Lerp(Rotator) "22.000000,-30.000000,0.000000" "0,30.000000, 0" _alpha) false)
      (Transformation|SetRelativeRotation (Variables|/Script/Engine.SpotLight|GetSpotLightComponent (Variables|Default|GetLight%20Two)) (Math|Rotator|Lerp(Rotator) "22.000000,30.000000,0.000000" "0,-30.000000, 0" _alpha) false))))

(event Custom|Message%20Loop
  (Default|TypeMessagetoUser (Variables|Default|GetKeyboard) "Press Enter to Continue"))

(event Custom|KeyPressed
  (params (Character :type String) (Key%20Type :type E_KeyType%20Enum))
  (CallFunction|HandleKeyPress))

(event EventBeginPlay
  (bind _self self)
  (Utilities|FlowControl|Sequence
    (:then_0
      (bind _returnvalue (AddComponent|AddChildActorComponent false (Math|Transform|MakeTransform "0, 0, 0")))
      (bind _asbp_typewriter (Utilities|Casting|CastToBP_Typewriter (Variables|/Script/Engine.ChildActorComponent|GetChildActor _returnvalue)))
      (Variables|Default|SetKeyboard _asbp_typewriter))
    (:then_1
      (Utilities|Time|SetTimerbyFunctionName 0 "Message Loop" 4.0 true))
    (:then_2
      (bind _asspot_light (Utilities|Casting|CastToSpotLight (.Actor (CallFunction|FindActorwithTag "/Script/Engine.SpotLight" "keylight" _self))))
      (bind _output_get (Variables|Default|SetLight%20One _asspot_light))
      (Transformation|SetActorTransform _output_get (Math|Transform|MakeTransform "-33.000000,-33.000000, 0")))
    (:then_3
      (bind _asspot_light_2 (Utilities|Casting|CastToSpotLight (.Actor (CallFunction|FindActorwithTag "/Script/Engine.SpotLight" "keylight2" _self))))
      (bind _output_get_2 (Variables|Default|SetLight%20Two _asspot_light_2))
      (Transformation|SetActorTransform _output_get_2 (Math|Transform|MakeTransform "-33.000000,33.000000, 0")))
    (:then_4
      (CallFunction|AnimateLights))
    (:then_5
      (CallFunction|BuildLetters)
      (CallFunction|LayoutLetters)
      (EventDispatchers|BindEventtoKeyPressedEvent (Variables|Default|GetKeyboard) (delegate Custom|KeyPressed)))))

(fn ConstructionScript)

(fn LetterPositions
  (Utilities|FlowControl|Sequence
    (:then_0
      (if (== (Utilities|Array|Length (Variables|Default|GetCached%20Positions)) 0)
        (for _array_element (Variables|Default|GetLetters)
          (Utilities|Array|Add (Variables|Default|GetCached%20Positions) (Math|Vector|MakeVector 0.0 (LocalVariables|GetYOffset) -9e+01))
          (bind _width (Default|GetWidth _array_element))
          (LocalVariables|SetYOffset (+ _width (LocalVariables|GetYOffset))))))
    (:then_2
      (return (Variables|Default|GetCached%20Positions)))))

(fn BuildLetters
  (if (== (Utilities|Array|Length (Variables|Default|GetLetters)) 0)
    (for _array_element (Utilities|String|GetCharacterArrayfromString (Variables|Default|GetSentence))
      (bind _returnvalue (AddComponent|AddChildActorComponent false))
      (bind _asbp_demo_letter (Utilities|Casting|CastToBP_DemoLetter (Variables|/Script/Engine.ChildActorComponent|GetChildActor _returnvalue)))
      (Utilities|Array|Add (Variables|Default|GetLetters) _asbp_demo_letter)
      (Default|UpdateCharacter _asbp_demo_letter _array_element)
      (Rendering|SetVisibility (Variables|/Game/ReusableAssets/Keyboard/KeyboardDemo/BP_DemoLetter.BP_DemoLetter_C|GetRoot _asbp_demo_letter) false true))))

(fn LayoutLetters
  (Utilities|FlowControl|Sequence
    (:then_0
      (bind (_min_position _max_position) (CallFunction|MinandMaxPositions (CallFunction|LetterPositions)))
      (LocalVariables|SetOffset (Class|TKMathFunctionLibrary|NegateFloat (/ (- (.Y (Math|Vector|BreakVector _max_position)) (.Y (Math|Vector|BreakVector _min_position))) 2.0))))
    (:then_1
      (for (_array_element _array_index) (Variables|Default|GetLetters)
        (Transformation|SetActorRelativeLocation _array_element (+ (Utilities|Array|Get(acopy) (CallFunction|LetterPositions) _array_index) (Math|Vector|MakeVector 0.0 (LocalVariables|GetOffset) 0.0)))))))

(fn HandleKeyPress
  (Rendering|SetVisibility (Variables|/Game/ReusableAssets/Keyboard/KeyboardDemo/BP_DemoLetter.BP_DemoLetter_C|GetRoot (Utilities|Array|Get(acopy) (Variables|Default|GetLetters) (Variables|Default|GetAnimation%20Counter))) true true)
  (CallFunction|AnimatetoLocation (Utilities|Array|Get(acopy) (Variables|Default|GetLetters) (Variables|Default|GetAnimation%20Counter)) (+ (Variables|/Script/Engine.SceneComponent|GetRelativeLocation (Variables|/Game/ReusableAssets/Keyboard/KeyboardDemo/BP_DemoLetter.BP_DemoLetter_C|GetRoot (Utilities|Array|Get(acopy) (Variables|Default|GetLetters) (Variables|Default|GetAnimation%20Counter)))) "2000.000000, 0, 0") (Variables|/Script/Engine.SceneComponent|GetRelativeLocation (Variables|/Game/ReusableAssets/Keyboard/KeyboardDemo/BP_DemoLetter.BP_DemoLetter_C|GetRoot (Utilities|Array|Get(acopy) (Variables|Default|GetLetters) (Variables|Default|GetAnimation%20Counter)))) 0 1.0 false false true 0.0)
  (bind _result (Math|Integer|IncrementInt (Variables|Default|GetAnimation%20Counter))
    (:%20%20
      (if (Utilities|Array|IsValidIndex (Variables|Default|GetLetters) _result)
        _
        (else
          (Variables|Default|SetAnimation%20Counter 0)))
      (return))))