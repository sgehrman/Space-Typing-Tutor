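; A single 3D key on a virtual keyboard, configured by its parent keyboard with a character, shift character and type.
; Key data sets the letter widget, icon and colour, with bumps on F and J.
; Dynamic material instances drive shift highlights, flashing and next-key indication, while a timeline animates press offset and glow alongside a puff emitter.
; Crosshair clicks and scrolls forward the key data to ParentKeyboard, which supplies sound settings.
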(event Custom|PlayKeyPressAnimation
  (Effects|SpawnEmitterAttached "/Game/ReusableAssets/Keyboard/KeyPuff.KeyPuff" (Variables|Default|GetKeyMesh) "None" "-30.000000, 0, 0")
  (bind _alpha (Timeline|FlashKeyTimeline PlayFromStart)
    (:Update
      (Transformation|SetActorRelativeScale3D (Math|Vector|Lerp(Vector) "1.000000,1.000000,1.000000" "1.000000,1.000000,1.000000" _alpha))
      (Transformation|SetActorRelativeLocation (Math|Vector|Lerp(Vector) "0, 0, 0" (Math|Vector|MakeVector (Variables|/Game/ReusableAssets/Keyboard/BP_Typewriter.BP_Typewriter_C|GetKey%20Click%20Offset (Variables|Default|GetParent%20Keyboard)) 0.0 0.0) _alpha))
      (bind _asmaterial_instance_dynamic (Utilities|Casting|CastToMaterialInstanceDynamic (Rendering|Material|GetMaterial (Variables|Default|GetKeyMesh) 0)))
      (Rendering|Material|SetScalarParameterValue _asmaterial_instance_dynamic "Emission" (Math|Float|Lerp 0.0 9e+01 _alpha) :!class /Script/Engine.MaterialInstanceDynamic))))

(fn ConstructionScript
  (CallFunction|CreateDynamicMaterials)
  (Rendering|Material|SetMaterial (Variables|Default|GetKeyMesh) 0 (Variables|Default|GetMID))
  (Rendering|Material|SetMaterial (Variables|Default|GetIndicator) 0 (Variables|Default|GetNext%20Key%20MID))
  (Rendering|Material|SetMaterial (Variables|Default|GetBump) 0 (Variables|Default|GetBump%20MID)))

(fn SetKeyDataStruct
  (params (Key%20Data :type ST%20Key%20Data%20Structure) (Parent%20Keyboard :type BP%20Typewriter%20Object%20Reference))
  (Variables|Default|SetParent%20Keyboard Parent%20Keyboard)
  (Utilities|FlowControl|Sequence
    (:then_0
      (Variables|Default|SetKey%20Data Key%20Data))
    (:then_1
      (Variables|Default|SetKey%20Character (.Key (Utilities|Struct|BreakST_KeyData (Variables|Default|GetKey%20Data))))
      (Variables|Default|SetShift%20Key%20Character (.Shift_Key (Utilities|Struct|BreakST_KeyData (Variables|Default|GetKey%20Data))))
      (Variables|Default|SetKey%20Type (.KeyType (Utilities|Struct|BreakST_KeyData (Variables|Default|GetKey%20Data)))))
    (:then_2
      (if (or (Utilities|Enum|Equal(Enum) (.Key (Utilities|Struct|BreakST_KeyData (Variables|Default|GetKey%20Data))) "f") (Utilities|Enum|Equal(Enum) (.Key (Utilities|Struct|BreakST_KeyData (Variables|Default|GetKey%20Data))) "j"))
        (Rendering|Material|SetMaterial (Variables|Default|GetKeyMesh) 0 (Variables|Default|GetFJ%20MID))
        (Development|SetHiddeninGame (Variables|Default|GetBump) false false)))
    (:then_3
      (switch Utilities|FlowControl|Switch|SwitchonE_KeyType (Variables|Default|GetKey%20Type)
        (:NewEnumerator0
          (if (Utilities|Enum|Equal(Enum) (Variables|Default|GetKey%20Character) " ")
            (Variables|Default|SetIcon "NewEnumerator3")))
        (:NewEnumerator1
          (Variables|Default|SetIcon "NewEnumerator9"))
        (:NewEnumerator2
          (Variables|Default|SetIcon "NewEnumerator2"))
        (:NewEnumerator3
          (Variables|Default|SetIcon "NewEnumerator4"))
        (:NewEnumerator4
          (Variables|Default|SetIcon "NewEnumerator1"))
        (:NewEnumerator5
          (Variables|Default|SetIcon "NewEnumerator1"))))
    (:then_5
      (if (!= (Variables|Default|GetKey%20Type) (Utilities|Enum|LiteralenumE_KeyType "NewEnumerator0"))
        (Rendering|Material|SetMaterial (Variables|Default|GetKeyMesh) 0 (Variables|Default|GetSpecial%20MID))))
    (:then_6
      (bind _aswbp_single_character (Utilities|Casting|CastToWBP_SingleCharacter (UserInterface|GetUserWidgetObject (Variables|Default|GetSingleLetter))))
      (Utilities|FlowControl|Sequence
        (:then_0
          (Variables|/Game/ReusableAssets/Keyboard/WBP_SingleCharacter.WBP_SingleCharacter_C|SetCharacter _aswbp_single_character (Variables|Default|GetKey%20Character))
          (Variables|/Game/ReusableAssets/Keyboard/WBP_SingleCharacter.WBP_SingleCharacter_C|SetShift%20Character _aswbp_single_character (Variables|Default|GetShift%20Key%20Character)))
        (:then_1
          (if (not (== (Variables|Default|GetIcon) (Utilities|Enum|LiteralenumE_KeyboardIcons "NewEnumerator0")))
            (Variables|/Game/ReusableAssets/Keyboard/WBP_SingleCharacter.WBP_SingleCharacter_C|SetIcon _aswbp_single_character (Variables|Default|GetIcon))))))
    (:then_7
      (CallFunction|UpdateShiftKeyDown false false))))

(fn UpdateShiftKeyDown
  (params (Left%20Shift%20Down :type Boolean :default false) (Right%20Shift%20Down :type Boolean :default false))
  (bind _returnvalue (or Left%20Shift%20Down Right%20Shift%20Down))
  (Utilities|FlowControl|Sequence
    (:then_0
      (bind _aswbp_single_character (Utilities|Casting|CastToWBP_SingleCharacter (UserInterface|GetUserWidgetObject (Variables|Default|GetSingleLetter))))
      (Default|UpdateforShiftDown _aswbp_single_character _returnvalue)
      (if _returnvalue
        (CallFunction|PlaySound (Variables|/Game/ReusableAssets/Keyboard/BP_Typewriter.BP_Typewriter_C|GetShift%20Key%20Click%20Sound (Variables|Default|GetParent%20Keyboard)))))
    (:then_1
      (if (Utilities|Enum|Equal(Enum) (Variables|Default|GetKey%20Type) "NewEnumerator4")
        (if Left%20Shift%20Down
          (Rendering|Material|SetMaterial (Variables|Default|GetKeyMesh) 0 (Variables|Default|GetSpecial%20MID%20Selected))
          (else
            (Rendering|Material|SetMaterial (Variables|Default|GetKeyMesh) 0 (Variables|Default|GetSpecial%20MID))))))
    (:then_2
      (if (Utilities|Enum|Equal(Enum) (Variables|Default|GetKey%20Type) "NewEnumerator5")
        (if Right%20Shift%20Down
          (Rendering|Material|SetMaterial (Variables|Default|GetKeyMesh) 0 (Variables|Default|GetSpecial%20MID%20Selected))
          (else
            (Rendering|Material|SetMaterial (Variables|Default|GetKeyMesh) 0 (Variables|Default|GetSpecial%20MID))))))))

(fn GetKeyExtent
  (LocalVariables|SetResult%20Extent (.y (.Max (Components|StaticMesh|GetLocalBounds (Variables|Default|GetKeyMesh)))))
  (return (LocalVariables|GetResult%20Extent)))

(fn GetKeyDataStruct
  (return (Variables|Default|GetKey%20Data)))

(fn CreateDynamicMaterials
  (Utilities|FlowControl|Sequence
    (:then_0
      (bind _returnvalue (Rendering|Material|CreateDynamicMaterialInstance "/Game/ReusableAssets/Materials/MT_Opaque.MT_Opaque" :!class /Script/Engine.KismetMaterialLibrary))
      (Variables|Default|SetMID _returnvalue))
    (:then_1
      (bind _returnvalue_2 (Rendering|Material|CreateDynamicMaterialInstance "/Game/ReusableAssets/Materials/MT_Opaque.MT_Opaque" :!class /Script/Engine.KismetMaterialLibrary))
      (bind _output_get (Variables|Default|SetFJ%20MID _returnvalue_2))
      (Rendering|Material|SetVectorParameterValue _output_get "Color" "(R=0.635000,G=0.302731,B=0.551932,A=1.000000)" :!class /Script/Engine.MaterialInstanceDynamic))
    (:then_2
      (bind _returnvalue_3 (Rendering|Material|CreateDynamicMaterialInstance "/Game/ReusableAssets/Materials/MT_Opaque.MT_Opaque" :!class /Script/Engine.KismetMaterialLibrary))
      (bind _output_get_2 (Variables|Default|SetSpecial%20MID _returnvalue_3))
      (Rendering|Material|SetVectorParameterValue _output_get_2 "Color" "(R=0.175455,G=0.364600,B=0.650000,A=1.000000)" :!class /Script/Engine.MaterialInstanceDynamic))
    (:then_3
      (bind _returnvalue_4 (Rendering|Material|CreateDynamicMaterialInstance "/Game/ReusableAssets/Materials/MT_Opaque.MT_Opaque" :!class /Script/Engine.KismetMaterialLibrary))
      (bind _output_get_3 (Variables|Default|SetSpecial%20MID%20Selected _returnvalue_4))
      (Rendering|Material|SetScalarParameterValue _output_get_3 "Emission" 35.0 :!class /Script/Engine.MaterialInstanceDynamic))
    (:then_4
      (bind _returnvalue_5 (Rendering|Material|CreateDynamicMaterialInstance "/Game/ReusableAssets/Materials/MT_Opaque.MT_Opaque" :!class /Script/Engine.KismetMaterialLibrary))
      (bind _output_get_4 (Variables|Default|SetNext%20Key%20MID _returnvalue_5))
      (Rendering|Material|SetVectorParameterValue _output_get_4 "EmissiveColor" "(R=0.000000,G=0.045000,B=0.005426,A=1.000000)" :!class /Script/Engine.MaterialInstanceDynamic)
      (Rendering|Material|SetScalarParameterValue _output_get_4 "Emission" 1.0 :!class /Script/Engine.MaterialInstanceDynamic)
      (Rendering|Material|SetScalarParameterValue _output_get_4 "Flicker Mode" 1.0 :!class /Script/Engine.MaterialInstanceDynamic)
      (Rendering|Material|SetScalarParameterValue _output_get_4 "Flicker Speed" 0.8 :!class /Script/Engine.MaterialInstanceDynamic)
      (Rendering|Material|SetScalarParameterValue _output_get_4 "Flicker Boost" 88.0 :!class /Script/Engine.MaterialInstanceDynamic))
    (:then_5
      (bind _returnvalue_6 (Rendering|Material|CreateDynamicMaterialInstance "/Game/ReusableAssets/Materials/MT_Opaque.MT_Opaque" :!class /Script/Engine.KismetMaterialLibrary))
      (bind _output_get_5 (Variables|Default|SetBump%20MID _returnvalue_6))
      (Rendering|Material|SetVectorParameterValue _output_get_5 "EmissiveColor" "(R=1.000000,G=1.000000,B=1.000000,A=1.000000)" :!class /Script/Engine.MaterialInstanceDynamic)
      (Rendering|Material|SetScalarParameterValue _output_get_5 "Emission" 33.0 :!class /Script/Engine.MaterialInstanceDynamic))
    (:then_6
      (bind _returnvalue_7 (Rendering|Material|CreateDynamicMaterialInstance "/Game/ReusableAssets/Materials/MT_Opaque.MT_Opaque" :!class /Script/Engine.KismetMaterialLibrary))
      (bind _output_get_6 (Variables|Default|SetMID%20Flashing _returnvalue_7))
      (Rendering|Material|SetScalarParameterValue _output_get_6 "Flicker Mode" 1.0 :!class /Script/Engine.MaterialInstanceDynamic)
      (Rendering|Material|SetVectorParameterValue _output_get_6 "EmissiveColor" "(R=0.006619,G=0.150000,B=0.035371,A=1.000000)" :!class /Script/Engine.MaterialInstanceDynamic)
      (Rendering|Material|SetScalarParameterValue _output_get_6 "Emission" 33.0 :!class /Script/Engine.MaterialInstanceDynamic)
      (Rendering|Material|SetScalarParameterValue _output_get_6 "Flicker Speed" 1.0 :!class /Script/Engine.MaterialInstanceDynamic)
      (Rendering|Material|SetScalarParameterValue _output_get_6 "Flicker Boost" 0.1 :!class /Script/Engine.MaterialInstanceDynamic))
    (:then_8
      (return))))

(fn FlashKeydown
  (CallFunction|FlashKeyUntilPressed false)
  (CallFunction|PlaySound (Variables|/Game/ReusableAssets/Keyboard/BP_Typewriter.BP_Typewriter_C|GetKey%20Click%20Sound (Variables|Default|GetParent%20Keyboard)))
  (CallFunction|PlayKeyPressAnimation))

(fn SetNextKeyMode
  (params (Set%20Mode :type Boolean :default false))
  (if (Math|Boolean|NotEqual(Boolean) Set%20Mode (Variables|Default|GetNext%20Key%20Mode))
    (bind _output_get (Variables|Default|SetNext%20Key%20Mode Set%20Mode))
    (Development|SetHiddeninGame (Variables|Default|GetIndicator) (not _output_get) false)))

(fn PlaySound
  (params (Sound :type Sound%20Base%20Object%20Reference))
  (if (Variables|/Game/ReusableAssets/Keyboard/BP_Typewriter.BP_Typewriter_C|GetPlay%20Keyclick%20sounds (Variables|Default|GetParent%20Keyboard))
    (Class|GameplayStatics|PlaySoundAttached Sound (Variables|Default|GetKeyMesh) "None" "0, 0, 0" "KeepRelativeOffset" false 0.5)))

(fn FlashKeyUntilPressed
  (params (Flash :type Boolean))
  (bind _keymesh (Variables|Default|GetKeyMesh))
  (if Flash
    (Variables|Default|SetSaved%20MID%20when%20Flashing (Rendering|Material|GetMaterial _keymesh 0))
    (Rendering|Material|SetMaterial _keymesh 0 (Variables|Default|GetMID%20Flashing))
    (elif (!= (Variables|Default|GetSaved%20MID%20when%20Flashing) 0)
      (Rendering|Material|SetMaterial (Variables|Default|GetKeyMesh) 0 (Variables|Default|GetSaved%20MID%20when%20Flashing))
      (Variables|Default|SetSaved%20MID%20when%20Flashing 0))))

(fn CrosshairHoverProgress
  (params (Progress :type Float%20%28single-precision%29) (Local%20Hit%20Location :type Vector :default "0, 0, 0") (Hit%20Component :type Primitive%20Component%20Object%20Reference))
  (return false))

(fn CrosshairHoverStart
  (params (Finished :type Boolean))
  (return true))

(fn CrosshairLeftRight
  (params (Left :type Boolean))
  (return false))

(fn CrosshairMouseClick
  (params (Mouse%20Down :type Boolean) (Event%20Type :type E_EventType%20Enum :default "NewEnumerator0") (Hit%20Location :type Vector :default "0, 0, 0") (Hit%20Component :type Primitive%20Component%20Object%20Reference))
  (Utilities|FlowControl|Sequence
    (:then_0
      (if Mouse%20Down
        (Default|HandleCrosshairClick (Variables|Default|GetParent%20Keyboard) (Variables|Default|GetKey%20Data) Event%20Type)))
    (:then_1
      (return true))))

(fn CrosshairScrollWheel
  (params (Down :type Boolean) (Hit%20Location :type Vector :default "0, 0, 0") (Hit%20Component :type Primitive%20Component%20Object%20Reference))
  (if Down
    (LocalVariables|SetEvent%20Type "NewEnumerator2")
    (else
      (LocalVariables|SetEvent%20Type "NewEnumerator1")))
  (Default|HandleCrosshairClick (Variables|Default|GetParent%20Keyboard) (Variables|Default|GetKey%20Data) (LocalVariables|GetEvent%20Type))
  (return false))

(fn CrosshairUpDown
  (params (Up :type Boolean))
  (return false))