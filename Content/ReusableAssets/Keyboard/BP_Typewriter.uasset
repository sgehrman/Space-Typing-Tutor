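; BP_Typewriter is an on-screen typewriter keyboard actor that mirrors physical key presses and crosshair clicks as key flashes and key-pressed events.
; BuildKeys reads a JSON keymap and spawns centred rows of BP_TypewriterKey child actors.
; A string-to-index map keyed by character and key type speeds lookup, covering shifted characters.
; It also highlights the delegate's next character, flashes keys until pressed, and auto-types messages through a delayed loop.
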(event Custom|HandleCrosshairClick
  (params (Key%20Data :type ST%20Key%20Data%20Structure) (Event%20Type :type E_EventType%20Enum :default "NewEnumerator0"))
  (bind (_key _shift_key _finger _keytype) (Utilities|Struct|BreakST_KeyData Key%20Data))
  (CallFunction|ProcessKeyDown (Utilities|String|SelectString _shift_key _key (Variables|Default|GetShiftKeyDown)) Event%20Type _keytype))

(event Custom|KeyboardShiftEvent
  (params (Left%20Shift%20Down :type Boolean) (Right%20Shift%20Down :type Boolean))
  (bind _returnvalue (or Left%20Shift%20Down Right%20Shift%20Down))
  (Utilities|FlowControl|Sequence
    (:then_0
      (if Left%20Shift%20Down
        (Default|CallKeyPressedEvent "" "NewEnumerator4")))
    (:then_1
      (if Right%20Shift%20Down
        (Default|CallKeyPressedEvent "" "NewEnumerator5")))
    (:then_2
      (if (Math|Boolean|NotEqual(Boolean) _returnvalue (Variables|Default|GetShiftKeyDown))
        (Variables|Default|SetShiftKeyDown _returnvalue)
        (for _array_element (Variables|Default|GetTypewriter%20Keys)
          (Default|UpdateShiftKeyDown _array_element Left%20Shift%20Down Right%20Shift%20Down))))))

(event Custom|CustomEvent_0
  (params (Result :type BPI%20PMM%20Interface))
  (bind _output_get (Variables|Default|SetPLM Result))
  (bind _listener (Default|GetKeyEventListener _output_get))
  (EventDispatchers|BindEventtoKeyboardShiftKeyEvent _listener (delegate Custom|KeyboardShiftEvent))
  (EventDispatchers|BindEventtoKeyboardEvent _listener (delegate Custom|Keyboard%20Event))
  (Default|SetEnabled _listener true))

(event Custom|Keyboard%20Event
  (params (Key%20Type :type E_KeyType%20Enum) (Character :type String) (Character%20Code :type Integer))
  (CallFunction|ProcessKeyDown Character "NewEnumerator0" Key%20Type))

(event Custom|ProcessKeyDown
  (params (Character :type String) (Event%20Type :type E_EventType%20Enum :default "NewEnumerator0") (Key%20Type :type E_KeyType%20Enum))
  (Utilities|FlowControl|Sequence
    (:then_0
      (CallFunction|FlashKey Character Key%20Type))
    (:then_1
      (Default|CallKeyPressedEvent Character Key%20Type))))

(event Custom|Type%20Message%20to%20user
  (params (Message :type String))
  (bind _returnvalue (Utilities|String|GetCharacterArrayfromString Message))
  ;[1 1 1] Don't run two at once, just bail
  (if (== (Variables|Default|GetLocal_LoopIndex) 0)
    (if (< (Variables|Default|GetLocal_LoopIndex) (Utilities|Array|Length _returnvalue)) :!label _label
      (CallFunction|ProcessKeyDown (Utilities|Array|Get(acopy) _returnvalue (Variables|Default|GetLocal_LoopIndex)) "NewEnumerator0" "NewEnumerator0")
      (Math|Integer|IncrementInt (Variables|Default|GetLocal_LoopIndex)
        (:%20%20
          (Utilities|FlowControl|Delay 0.4)
          (goto _label)))
      (else
        (Variables|Default|SetLocal_LoopIndex 0)))
    (else
      (CallFunction|Logg "Type message to User failed to run"))))

(event EventBeginPlay
  (Utilities|FlowControl|Sequence
    (:then_0
      (CallFunction|BuildKeys))
    (:then_1
      (Input|EnableInput (Game|GetPlayerController 0)))
    (:then_2
      (bind _returnvalue (AddComponent|AddBCPMMAccess))
      (EventDispatchers|BindEventtoPMMReady _returnvalue (delegate Custom|CustomEvent_0))
      (Default|Setup _returnvalue))))

(fn ConstructionScript
  (Utilities|FlowControl|Sequence
    (:then_0
      (bind _returnvalue (AddComponent|AddVictoryTMapComp))
      (Variables|Default|SetKey%20Index%20Map _returnvalue))
    (:then_1
      (CallFunction|BuildKeys)
      (Variables|/Game/ReusableAssets/Components/BP_FaceCameraRotator.BP_FaceCameraRotator_C|SetRotation%20Offset (Variables|Default|GetBP_FaceCameraRotator) (Class|KismetMathLibrary|MakeRot (Variables|Default|GetKeyboard%20Pitch) 0.0 0.0)))))

(fn BuildKeys
  (Utilities|FlowControl|Sequence
    (:then_0
      (CallFunction|DeleteKeys))
    (:then_1
      (bind _key_data (CallFunction|ReadKeyMapfromFile "KeyMap_US.json"))
      (LocalVariables|SetLocal%20Key%20Data _key_data))
    (:then_2
      (for _array_element (LocalVariables|GetLocal%20Key%20Data)
        ;[1 1 1] End of Row?
        (if (Utilities|Enum|Equal(Enum) (.Key (Utilities|Struct|BreakST_KeyData _array_element)) "----")
          ;[1 1 1] Center the keys
          (Transformation|AddLocalOffset (LocalVariables|GetCurrentContainer) (Math|Vector|MakeVector 0.0 (* (/ (LocalVariables|GetRowOffset) 2.0) -1.0) 0.0) false)
          (LocalVariables|SetCurrentContainer 0)
          (LocalVariables|Setcol (+ (LocalVariables|Getcol) 1))
          (LocalVariables|SetRowOffset 0.0)
          (LocalVariables|SetLastKeyExtent 0.0)
          (else
            (Utilities|FlowControl|Sequence
              (:then_0
                (if (== (LocalVariables|GetCurrentContainer) 0)
                  ;[1 1 1] Create a row container
                  (bind _returnvalue (AddComponent|AddSceneComponent true (Math|Transform|MakeTransform (Math|Vector|MakeVector 0.0 0.0 (* (* (LocalVariables|Getcol) (LocalVariables|GetKey%20Size)) -1.0)))))
                  (Class|SceneComponent|Attachto _returnvalue (Variables|Default|GetRow%20Container) "None" "KeepRelativeOffset" true)
                  (bind _output_get (LocalVariables|SetCurrentContainer _returnvalue))
                  (Utilities|Array|Add (LocalVariables|GetRow%20Containers) _output_get)))
              (:then_1
                (bind _returnvalue_2 (AddComponent|AddChildActorComponent true (Math|Transform|MakeTransform "0, 0, 0" "0.000000, 0, 0")))
                (Class|SceneComponent|Attachto _returnvalue_2 (LocalVariables|GetCurrentContainer) "None" "KeepRelativeOffset" true)
                (bind _asbp_typewriter_key (Utilities|Casting|CastToBP_TypewriterKey (Variables|/Script/Engine.ChildActorComponent|GetChildActor _returnvalue_2)))
                (bind _returnvalue_3 (Utilities|Array|Add (Variables|Default|GetTypewriter%20Keys) _asbp_typewriter_key))
                (Utilities|FlowControl|Sequence
                  (:then_0
                    (Class|VictoryTMapComp|StringIntAddPair (Variables|Default|GetKey%20Index%20Map) (CallFunction|CreateKeyIndexMapKey (.Key (Utilities|Struct|BreakST_KeyData _array_element)) (.KeyType (Utilities|Struct|BreakST_KeyData _array_element))) _returnvalue_3))
                  (:then_1
                    ;[1 1 1] Add shift key if different
                    (if (not (Utilities|Enum|Equal(Enum) (.Key (Utilities|Struct|BreakST_KeyData _array_element)) (.Shift_Key (Utilities|Struct|BreakST_KeyData _array_element))))
                      (if (> (Utilities|String|Len (.Shift_Key (Utilities|Struct|BreakST_KeyData _array_element))) 0)
                        (Class|VictoryTMapComp|StringIntAddPair (Variables|Default|GetKey%20Index%20Map) (CallFunction|CreateKeyIndexMapKey (.Shift_Key (Utilities|Struct|BreakST_KeyData _array_element)) (.KeyType (Utilities|Struct|BreakST_KeyData _array_element))) _returnvalue_3))))
                  (:then_2
                    (Default|SetKeyDataStruct _asbp_typewriter_key _array_element self))))
              (:then_2
                (bind _extent (Default|GetKeyExtent _asbp_typewriter_key))
                (if (!= (LocalVariables|GetLastKeyExtent) 0.0)
                  (LocalVariables|SetRowOffset (+ _extent (Variables|Default|GetMargin) (LocalVariables|GetLastKeyExtent) (LocalVariables|GetRowOffset)))
                  (Transformation|SetRelativeLocation _returnvalue_2 (Math|Vector|MakeVector 0.0 (LocalVariables|GetRowOffset) 0.0) false))
                (LocalVariables|SetLastKeyExtent _extent)))))))))

(fn FlashKey
  (params (Character :type String) (Key%20Type :type E_KeyType%20Enum))
  (bind (_valid _keyboard_key) (CallFunction|GetKey Character Key%20Type))
  (if _valid
    (Default|FlashKeydown _keyboard_key)))

(fn DeleteKeys
  (Utilities|FlowControl|Sequence
    (:then_0
      (Utilities|Array|Clear (Variables|Default|GetTypewriter%20Keys))
      (CallFunction|DestroyChildComponents (Variables|Default|GetRow%20Container))
      (Class|VictoryTMapComp|StringIntClear (Variables|Default|GetKey%20Index%20Map)))
    (:then_1
      (return))))

(fn UpdateMatOfNextKey
  (bind (_valid _character) (Default|GetNextCharacter (Variables|Default|GetDelegate)))
  (if _valid
    (for _array_element (Variables|Default|GetTypewriter%20Keys)
      (Default|SetNextKeyMode _array_element false))
    (if (.Valid (CallFunction|GetKey _character "NewEnumerator0"))
      (Default|SetNextKeyMode (.Keyboard%20Key (CallFunction|GetKey _character "NewEnumerator0")) true)
      (bind _character_2 (Default|GetKeyDataStruct (.Keyboard%20Key (CallFunction|GetKey _character "NewEnumerator0"))))
      (Default|NextMatchingKey (Variables|Default|GetDelegate) _character_2))))

(fn ReadKeyMapfromFile
  (params (Filename :type String))
  (LocalVariables|SetFile%20Contents (.OutString (Class|FileSystemUtils|LoadFiletoString (Class|VictoryBPFunctionLibrary|AppendMultiple (Class|VictoryBPFunctionLibrary|VictoryPathsGameRootDirectory) "Content/" "AppData/" Filename))))
  (bind _returnvalue (Class|KrishnaJSON|ParseJson (Class|KrishnaJSON|Create) (LocalVariables|GetFile%20Contents)))
  (for _array_element (Class|KrishnaJSON|GetObjectArray _returnvalue "keys")
    (Utilities|FlowControl|Sequence
      (:then_0
        (bind _output_get (LocalVariables|SetLocal%20Key (.ReturnValue (Class|KrishnaJSON|GetString _array_element "key"))))
        (LocalVariables|SetKey%20Type "NewEnumerator0")
        (switch string _output_get
          (:backspace
            (LocalVariables|SetKey%20Type "NewEnumerator1")
            ;[1 1 1] Clear the junk in the file (enter, lshift, etc.)
            (LocalVariables|SetLocal%20Key "" :!label _label))
          (:tab
            (LocalVariables|SetKey%20Type "NewEnumerator3")
            (goto _label))
          (:lshift
            (LocalVariables|SetKey%20Type "NewEnumerator4")
            (goto _label))
          (:rshift
            (LocalVariables|SetKey%20Type "NewEnumerator5")
            (goto _label))
          (:enter
            (LocalVariables|SetKey%20Type "NewEnumerator2")
            (goto _label))
          (:space
            (LocalVariables|SetLocal%20Key " "))))
      (:then_1
        (Utilities|Array|Add (LocalVariables|GetKey%20Data%20Array) (Utilities|Struct|MakeST_KeyData (LocalVariables|GetLocal%20Key) (.ReturnValue (Class|KrishnaJSON|GetString _array_element "shift")) (.ReturnValue (Class|KrishnaJSON|GetInteger _array_element "finger")) (LocalVariables|GetKey%20Type))))))
  (return (LocalVariables|GetKey%20Data%20Array)))

(fn CreateKeyIndexMapKey
  (params (Key :type String) (Key%20Type :type E_KeyType%20Enum))
  (return (Class|VictoryBPFunctionLibrary|AppendMultiple Key ":" (Utilities|String|EnumtoString Key%20Type))))

(fn FlashKeysUntilPressed
  (params (Key%20Specs :type Array%20of%20Keyboard%20Key%20Spec%20Structures))
  (for _array_element Key%20Specs
    (if (.Valid (CallFunction|GetKey (.Character (Utilities|Struct|BreakKeyboardKeySpec _array_element)) (.KeyType (Utilities|Struct|BreakKeyboardKeySpec _array_element))))
      (Default|FlashKeyUntilPressed (.Keyboard%20Key (CallFunction|GetKey (.Character (Utilities|Struct|BreakKeyboardKeySpec _array_element)) (.KeyType (Utilities|Struct|BreakKeyboardKeySpec _array_element)))) true))))

(fn GetKey
  (params (Character :type String) (Key%20Type :type E_KeyType%20Enum))
  (bind _map_key (CallFunction|CreateKeyIndexMapKey Character Key%20Type))
  (bind _key_index_map (Variables|Default|GetKey%20Index%20Map))
  (bind (_isvalid _returnvalue) (Class|VictoryTMapComp|StringIntGet _key_index_map _map_key))
  (Utilities|FlowControl|Sequence
    (:then_0
      (if _isvalid
        (LocalVariables|SetResult%20Key (Utilities|Array|Get(acopy) (Variables|Default|GetTypewriter%20Keys) _returnvalue))
        (else
          ;[1 1 1] Debug only
          (if (LocalVariables|GetDebug)
            (CallFunction|Logg (Class|VictoryBPFunctionLibrary|AppendMultiple Character " : " (Utilities|String|EnumtoString Key%20Type) "Not found"))))))
    (:then_1
      (return (!= (LocalVariables|GetResult%20Key) 0) (LocalVariables|GetResult%20Key)))))

(fn UpdateDelegate
  (params (Delegate :type BP%20Typewriter%20Delegate%20Interface%20Interface))
  (Variables|Default|SetDelegate Delegate))

(fn RefreshfromDelegate
  (CallFunction|UpdateMatOfNextKey))