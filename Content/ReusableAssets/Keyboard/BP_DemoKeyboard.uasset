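; Demo actor that shows off a BP_Typewriter keyboard under animated key lighting.
; On BeginPlay it adds the typewriter as a child actor and starts a looping timer meant to repeatedly type a "Press Enter to Continue" prompt.
; It also finds two tagged spotlights, places them on either side of the world origin, and rotates them in mirrored sweeps with a slowed timeline.
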(event `Message Loop`
  (`/Game/ReusableAssets/Keyboard/BP_Typewriter.Type Message to user` (`self.Keyboard`) "Press Enter to Continue"))

(event `self.ReceiveBeginPlay`
  (`|ExecutionSequence`
    (:`then_0`
      (bind _returnvalue (`AddComponent|Child Actor Component_1069` :`RelativeTransform` (`KismetMathLibrary.MakeTransform` (0.0 0.0 0.0))))
      (bind _asbp_typewriter (cast `/Game/ReusableAssets/Keyboard/BP_Typewriter` (`ChildActorComponent.ChildActor` _returnvalue)))
      (set `self.Keyboard` _asbp_typewriter))
    (:`then_1`
      (`KismetSystemLibrary.K2_SetTimer` null "Message Loop" 4.0 true))
    (:`then_2`
      (bind _asspot_light (cast `SpotLight` (`.Actor` (`/Game/ReusableAssets/Utilities/LIB_Utilities.FindActorWithTag` "/Script/Engine.SpotLight" "keylight" self))))
      (bind _output_get (set `self.Light One` _asspot_light))
      (`self.K2_SetActorTransform` _output_get (`KismetMathLibrary.MakeTransform` (-33.0 -33.0 0.0)) false))
    (:`then_3`
      (bind _asspot_light_2 (cast `SpotLight` (`.Actor` (`/Game/ReusableAssets/Utilities/LIB_Utilities.FindActorWithTag` "/Script/Engine.SpotLight" "keylight2" self))))
      (bind _output_get_2 (set `self.Light Two` _asspot_light_2))
      (`self.K2_SetActorTransform` _output_get_2 (`KismetMathLibrary.MakeTransform` (-33.0 33.0 0.0)) false))
    (:`then_4`
      (`self.Animate Lights`))))

(event `Animate Lights`
  (`TimelineComponent.SetPlayRate` (`self.Lights Timeline`) 0.3)
  (bind (_direction _alpha) (`Timeline|Lights Timeline` :`NewTime` 0.0 :!via `PlayFromStart`)
    (:`Update`
      (`SceneComponent.K2_SetRelativeRotation` (`SpotLight.SpotLightComponent` (`self.Light One`)) (`KismetMathLibrary.RLerp` (struct :`Pitch` 22.0 :`Yaw` -30.0) (struct :`Yaw` 30.0) _alpha) false)
      (`SceneComponent.K2_SetRelativeRotation` (`SpotLight.SpotLightComponent` (`self.Light Two`)) (`KismetMathLibrary.RLerp` (struct :`Pitch` 22.0 :`Yaw` 30.0) (struct :`Yaw` -30.0) _alpha) false))))

(fn `UserConstructionScript`)