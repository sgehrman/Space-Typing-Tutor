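; BP_LightController is a reusable Blueprint that smoothly rotates the level's main directional light to a target rotation.
; RotateMainLight sets a timeline's play rate and passes the current rotation, target and light to a private event that lerps the rotation along a curve.
; GetMainLight lazily finds and caches the first DirectionalLight in the world.
; Helper functions read and set the relative rotation on the light's root component.
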(event `Private Rotate Light`
  (params (Start :type "Rotator Structure") (End :type "Rotator Structure") (Light :type "DirectionalLight Object Reference"))
  (bind (_direction _c_genericcurve) (`Timeline|Animation Timeline` :!via `PlayFromStart`)
    (:`Update`
      (`self.Set Light Rotation` Light (`KismetMathLibrary.RLerp` Start End _c_genericcurve)))))

(fn `Get Main Light`
  (returns (Light :type "DirectionalLight Object Reference"))
  (`|ExecutionSequence`
    (:`then_0`
      (`/Engine/EditorBlueprintResources/StandardMacros.IsValid` (`self.Cached Light`)
        (:`Is Not Valid`
          (bind _outactors (`GameplayStatics.GetAllActorsOfClass` "/Script/Engine.DirectionalLight"))
          (set `self.Cached Light` (`KismetArrayLibrary.Array_Get` _outactors)))))
    (:`then_1`
      (return (`self.Cached Light`)))))

(fn `Get Main Light Rotation`
  (returns (Rotation :type "Rotator Structure"))
  (return (`SceneComponent.RelativeRotation` (`self.K2_GetRootComponent` (`self.Get Main Light`)))))

(fn `Rotate Main Light`
  (params (Rotation :type "Rotator Structure") (Rate :type "Float (double-precision)"))
  (`TimelineComponent.SetPlayRate` (`self.Animation Timeline`) Rate)
  (`self.Private Rotate Light` (`self.Get Main Light Rotation`) Rotation (`self.Get Main Light`)))

(fn `Set Light Rotation`
  (params (Light :type "DirectionalLight Object Reference") (Rotation :type "Rotator Structure"))
  (`SceneComponent.K2_SetRelativeRotation` (`self.K2_GetRootComponent` Light) Rotation false false))

(fn `UserConstructionScript`)