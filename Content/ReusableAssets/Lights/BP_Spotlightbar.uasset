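; BP_Spotlightbar is a reusable light fixture that builds an evenly spaced row of spotlights in its construction script.
; LayoutLights destroys the previous lights and markers, then adds spotlight components stepped along a fixed offset from a start point.
; When DrawMarkers is set, it also places small static meshes at the same spots, sharing one emissive dynamic material instance.
; The event graph has no active logic.
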(event `self.ReceiveBeginPlay`)

(event `self.ReceiveActorBeginOverlap`
  (params (OtherActor :type "Actor Object Reference")))

(event `self.ReceiveTick`
  (params (DeltaSeconds :type "Float (single-precision)")))

(fn `Layout Lights`
  (params (`Start Offset` :type "Vector Structure") (Offset :type "Vector Structure") (`Number Of Lights` :type Integer))
  (`|ExecutionSequence`
    (:`then_0`
      (for _array_element (`self.Lights`)
        (`ActorComponent.K2_DestroyComponent` _array_element))
      (`KismetArrayLibrary.Array_Clear` (`self.Lights`)))
    (:`then_1`
      (for _array_element_2 (`self.Markers`)
        (`ActorComponent.K2_DestroyComponent` _array_element_2))
      (`KismetArrayLibrary.Array_Clear` (`self.Markers`)))
    (:`then_4`
      (for _index (range `Number Of Lights`)
        (bind _returnvalue (`AddComponent|Spot Light Component_0` :`RelativeTransform` (`KismetMathLibrary.MakeTransform` (+ `Start Offset` (* Offset (`KismetMathLibrary.Conv_IntToDouble` _index))) (struct) (0.1 0.1 0.1))))
        (`KismetArrayLibrary.Array_Add` (`self.Lights`) _returnvalue)))
    (:`then_5`
      (if (`self.Draw Markers`)
        (for _index_2 (range `Number Of Lights`)
          (bind _returnvalue_2 (`AddComponent|Static Mesh Component_15` :`RelativeTransform` (`KismetMathLibrary.MakeTransform` (+ `Start Offset` (* Offset (`KismetMathLibrary.Conv_IntToDouble` _index_2))) (struct) (0.02 0.02 0.02))))
          (`KismetArrayLibrary.Array_Add` (`self.Markers`) _returnvalue_2)
          (`PrimitiveComponent.SetMaterial` _returnvalue_2 0 (`self.MID`)))))))

(fn `UserConstructionScript`
  (`|ExecutionSequence`
    (:`then_0`
      (bind _returnvalue (`KismetMaterialLibrary.CreateDynamicMaterialInstance` "/Game/ReusableAssets/Materials/MT_Opaque.MT_Opaque"))
      (bind _output_get (set `self.MID` _returnvalue))
      (`MaterialInstanceDynamic.SetScalarParameterValue` _output_get "Emission" 222.0))
    (:`then_1`
      (`self.Layout Lights` (0.0 0.0 0.0) (0.0 222.0 0.0) 10))))