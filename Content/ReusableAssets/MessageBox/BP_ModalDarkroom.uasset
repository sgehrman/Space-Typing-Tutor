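; Modal darkroom backdrop that fades to near-black around its interior and displays a centred title and subtitle.
; On BeginPlay, Setup builds a procedural box with reversed triangles to render inside out, adds a transparent dynamic material and creates both text renders.
; FadeIn sets the text and plays an opacity timeline, revealing the text on completion.
; FadeOut hides the text first, then reverses the timeline.
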(event `self.ReceiveBeginPlay`
  (`self.Setup`))

(event `FadeOutAnimation`
  (params (`Fade In` :type Boolean))
  (`|ExecutionSequence`
    (:`then_0`
      ;[1 1 1] Hide Title before the fadeout
      (if (not `Fade In`)
        (`SceneComponent.SetVisibility` (`self.Title Text Render`) false true)
        (`SceneComponent.SetVisibility` (`self.Subtitle Text Render`) false true)))
    (:`then_1`
      (`TimelineComponent.SetPlayRate` (`self.Timeline_0`) 3.0)
      (if `Fade In`
        (bind (_direction _c_genericcurve) (`Timeline|Timeline_0` :!via `PlayFromStart` :!label _label)
          (:`Update`
            (`MaterialInstanceDynamic.SetScalarParameterValue` (`self.MID Background`) "Opacity" (`KismetMathLibrary.MapRange` _c_genericcurve 0.0 1.0 0.0 0.95)))
          (:`Finished`
            ;[1 1 1] Show Title after fade in
            (if `Fade In`
              (`SceneComponent.SetVisibility` (`self.Title Text Render`) true true)
              (`SceneComponent.SetVisibility` (`self.Subtitle Text Render`) true true))))
        (else
          (goto _label :!via `ReverseFromEnd`))))))

(fn `Content X Offset`
  (returns (XOffset :type "Float (double-precision)"))
  (return (/ (`self.Background Size`) 3.0)))

(fn `Create Text Render`
  (params (Text :type Text) (`Text Size` :type "Float (double-precision)"))
  (returns (`Text Render` :type "TextRenderComponent Object Reference"))
  (`|ExecutionSequence`
    (:`then_0`
      (bind _returnvalue (`AddComponent|TextRenderComponent_0` :`RelativeTransform` (`KismetMathLibrary.MakeTransform` (0.0 0.0 0.0))))
      (`TextRenderComponent.K2_SetText` _returnvalue Text)
      (`SceneComponent.SetVisibility` _returnvalue false false)
      (`TextRenderComponent.SetWorldSize` _returnvalue `Text Size`)
      (`TextRenderComponent.SetHorizontalAlignment` _returnvalue "EHTA_Center")
      (`SceneComponent.K2_SetRelativeRotation` _returnvalue (struct :`Yaw` 180.0) false))
    (:`then_1`
      (return _returnvalue))))

(fn `Fade In`
  (params (Title :type Text) (Subtitle :type Text))
  (`self.FadeOutAnimation` true)
  (`TextRenderComponent.K2_SetText` (`self.Title Text Render`) Title)
  (`TextRenderComponent.K2_SetText` (`self.Subtitle Text Render`) Subtitle))

(fn `Fade Out`
  (`self.FadeOutAnimation` false))

(fn `Setup`
  (bind _background_size (`self.Background Size`))
  (`|ExecutionSequence`
    (:`then_0`
      (bind _returnvalue (`KismetMaterialLibrary.CreateDynamicMaterialInstance` "/Game/ReusableAssets/Materials/MT_Transparent.MT_Transparent"))
      (bind _output_get (set `self.MID Background` _returnvalue))
      (`MaterialInstanceDynamic.SetScalarParameterValue` _output_get "Opacity" 0.0)
      (`MaterialInstanceDynamic.SetVectorParameterValue` _output_get "Color" (struct :`A` 1.0)))
    (:`then_1`
      (bind _returnvalue_2 (`AddComponent|ProceduralMeshComponent_0` :`RelativeTransform` (`KismetMathLibrary.MakeTransform` (0.0 0.0 0.0) (struct) (1.0 1.0 1.0))))
      (set `self.BackgroundMesh` _returnvalue_2)
      ;[1 1 1] Readonline to reverse the vector order to get it inside out.  maybe a hack?
      (bind (_vertices _triangles _normals _uvs _tangents) (`KismetProceduralMeshLibrary.GenerateBoxMesh` (/ (`KismetMathLibrary.MakeVector` _background_size _background_size _background_size) 2.0)))
      (`ProceduralMeshComponent.CreateMeshSection` :`self` (`self.BackgroundMesh`) :`Vertices` _vertices :`Triangles` (`/Game/ReusableAssets/Utilities/LIB_Utilities.Reversed Array` _triangles) :`Normals` _normals :`UV0` _uvs :`Tangents` _tangents)
      (`PrimitiveComponent.SetMaterial` (`self.BackgroundMesh`) 0 (`self.MID Background`)))
    (:`then_2`
      (bind _text_render (`self.Create Text Render` "Title Goes Here" 7.0))
      (bind _output_get_2 (set `self.Title Text Render` _text_render))
      (`SceneComponent.SetVisibility` _output_get_2 true true)
      (`SceneComponent.K2_SetRelativeLocation` (`self.Title Text Render`) (`KismetMathLibrary.MakeVector` (`self.Content X Offset`) 0.0 46.0) false))
    (:`then_3`
      (bind _text_render_2 (`self.Create Text Render` "Subtitle Goes Here" 5.0))
      (bind _output_get_3 (set `self.Subtitle Text Render` _text_render_2))
      (`SceneComponent.SetVisibility` _output_get_3 true true)
      (`SceneComponent.K2_SetRelativeLocation` (`self.Subtitle Text Render`) (`KismetMathLibrary.MakeVector` (`self.Content X Offset`) 0.0 40.0) false))))

(fn `UserConstructionScript`)