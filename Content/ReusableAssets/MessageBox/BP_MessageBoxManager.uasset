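; Manager Blueprint that shows and dismisses a single animated BP_MessageBox at a given world location.
; ShowMessage hides any current box, spawns a new one above the target, fills in its lines, then animates it down with a bounce and whoosh sound.
; HideMessage animates the box far off along X with destroy-on-finish and clears the reference immediately, so a replacement can animate in meanwhile.
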(fn ConstructionScript)

(fn ShowMessage
  (params (Location :type Vector) (Lines :type Array%20of%20Strings))
  (Utilities|FlowControl|Sequence
    (:then_0
      (CallFunction|HideMessage))
    (:then_2
      (bind _output_get (LocalVariables|SetEnd%20Location Location))
      (LocalVariables|SetStart%20Location (+ _output_get "0, 0,1200.000000")))
    (:then_3
      (bind _returnvalue (Game|SpawnActorfromClass "/Game/ReusableAssets/MessageBox/BP_MessageBox.BP_MessageBox_C" (Math|Transform|MakeTransform (LocalVariables|GetStart%20Location)) "AdjustIfPossibleButDontSpawnIfColliding" self 0))
      (Variables|Default|SetMessage%20Box _returnvalue))
    (:then_5
      (Default|UpdateLines (Variables|Default|GetMessage%20Box) Lines)
      (CallFunction|AnimatetoLocation (Variables|Default|GetMessage%20Box) (LocalVariables|GetStart%20Location) (LocalVariables|GetEnd%20Location) "/Game/UniversalSoundFX/Sound_Effects/WHOOSHES/WHOOSH_Miss_mono.WHOOSH_Miss_mono" 1.0 true false false 1.0))))

(fn HideMessage
  (if (not (== (Variables|Default|GetMessage%20Box) 0))
    (Utilities|FlowControl|Sequence
      (:then_0
        (bind _output_get (LocalVariables|SetStart%20Location (Transformation|GetActorLocation (Variables|Default|GetMessage%20Box))))
        (LocalVariables|SetEnd%20Location (+ _output_get "22222.000000, 0,0.000000")))
      (:then_4
        (CallFunction|AnimatetoLocation (Variables|Default|GetMessage%20Box) (LocalVariables|GetStart%20Location) (LocalVariables|GetEnd%20Location) 0 1.0 false true false 1.0))
      (:then_5
        (Variables|Default|SetMessage%20Box 0)))))