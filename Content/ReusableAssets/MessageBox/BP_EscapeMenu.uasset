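; In-world escape menu actor that offers Quit, Continue and return to the KeyboardLessons level.
; On BeginPlay it spawns a BP_ModalDarkroom child actor and, once PMM access is ready, pushes a menu-mode crosshair.
; Show fades in the darkroom with title and subtitle, then spawns three stacked BP_ToggleButton child actors as push buttons bound to one click handler.
; Continue and Menu hide the buttons, pop the crosshair, fade out and self-destroy after a delay.
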(event Custom|Destroy%20After%20Delay
  (params (Delay :type Float%20%28single-precision%29))
  (Utilities|FlowControl|Delay Delay)
  (Actor|DestroyActor))

(event Custom|CustomEvent_0
  (params (Result :type BPI%20PMM%20Interface))
  (bind _output_get (Variables|Default|SetPLM Result))
  (Default|PushCrosshair _output_get)
  (Default|EnableCrosshair _output_get true true))

(event Custom|Setup%20Button%20Events
  (for _array_element (Variables|Default|GetButtons)
    (EventDispatchers|BindEventtoButtonClickedbyUser _array_element (delegate Custom|Button%20Clicked))))

(event Custom|Button%20Clicked
  (params (Button%20ID :type String) (Hit%20Location :type Vector))
  (switch string Button%20ID
    (:Default
      (CallFunction|Logg Button%20ID))
    (:quit
      (Game|QuitGame 0 "Quit"))
    (:continue
      (CallFunction|HideandDestroy :!label _label))
    (:menu
      (Default|LoadLevel (Variables|Default|GetPLM) "KeyboardLessons")
      (goto _label))))

(event EventBeginPlay
  (Utilities|FlowControl|Sequence
    (:then_0
      (bind _returnvalue (AddComponent|AddBCPMMAccess))
      (EventDispatchers|BindEventtoPMMReady _returnvalue (delegate Custom|CustomEvent_0))
      (Default|Setup _returnvalue))
    (:then_1
      (bind _returnvalue_2 (AddComponent|AddChildActorComponent false (Math|Transform|MakeTransform "0, 0, 0")))
      (bind _asbp_modal_darkroom (Utilities|Casting|CastToBP_ModalDarkroom (Variables|/Script/Engine.ChildActorComponent|GetChildActor _returnvalue_2)))
      (Variables|Default|SetDarkroom _asbp_modal_darkroom))))

(fn ConstructionScript)

(fn CreateTextRender
  (params (Text :type Text) (Text%20Size :type Float%20%28single-precision%29))
  (Utilities|FlowControl|Sequence
    (:then_0
      (bind _returnvalue (AddComponent|AddTextRenderComponent false (Math|Transform|MakeTransform "0, 0,0.000000")))
      (Rendering|Components|TextRender|SetText _returnvalue Text)
      (Rendering|SetVisibility _returnvalue false false)
      (Rendering|Components|TextRender|SetWorldSize _returnvalue Text%20Size)
      (Rendering|Components|TextRender|SetHorizontalAlignment _returnvalue "EHTA_Center")
      (Transformation|SetRelativeRotation _returnvalue "0.000000,180.000000,0.000000" false)
      (Class|SystemUtils|SetTextRendersVerticalAlign _returnvalue))
    (:then_1
      (return _returnvalue))))

(fn Show
  (params (Title :type Text) (Subtitle :type Text))
  (Default|Fadein (Variables|Default|GetDarkroom) Title Subtitle)
  (CallFunction|CreateButtons))

(fn HideandDestroy
  (Utilities|FlowControl|Sequence
    (:then_0
      (for _array_element (Variables|Default|GetButtons)
        (Rendering|SetVisibility (Variables|/Game/ReusableAssets/Buttons/BP_ToggleButton.BP_ToggleButton_C|GetRoot _array_element) false true)))
    (:then_1
      (Default|PopCrosshair (Variables|Default|GetPLM)))
    (:then_3
      (Default|FadeOut (Variables|Default|GetDarkroom))
      (CallFunction|DestroyAfterDelay 1.0))))

(fn CreateButtons
  (bind _button_scale (LocalVariables|GetButton%20Scale))
  (bind _darkroom (Variables|Default|GetDarkroom))
  (bind _xoffset (Default|ContentXOffset _darkroom))
  (bind _returnvalue (Math|Conversions|ToVector(Float) _button_scale))
  (Utilities|FlowControl|Sequence
    (:then_1
      (bind _returnvalue_2 (AddComponent|AddChildActorComponent false (Math|Transform|MakeTransform (Math|Vector|MakeVector _xoffset 0.0 22.0) "0, 0, 0" _returnvalue)))
      (bind _asbp_toggle_button (Utilities|Casting|CastToBP_ToggleButton (Variables|/Script/Engine.ChildActorComponent|GetChildActor _returnvalue_2)))
      (Default|SetState _asbp_toggle_button false)
      (Utilities|Array|Add (Variables|Default|GetButtons) _asbp_toggle_button))
    (:then_2
      (bind _returnvalue_3 (AddComponent|AddChildActorComponent false (Math|Transform|MakeTransform (Math|Vector|MakeVector _xoffset 0.0 0.0) "0, 0, 0" _returnvalue)))
      (bind _asbp_toggle_button_2 (Utilities|Casting|CastToBP_ToggleButton (Variables|/Script/Engine.ChildActorComponent|GetChildActor _returnvalue_3)))
      (Default|SetState _asbp_toggle_button_2 false)
      (Utilities|Array|Add (Variables|Default|GetButtons) _asbp_toggle_button_2))
    (:then_3
      (bind _returnvalue_4 (AddComponent|AddChildActorComponent false (Math|Transform|MakeTransform (Math|Vector|MakeVector _xoffset 0.0 -22.0) "0, 0, 0" _returnvalue)))
      (bind _asbp_toggle_button_3 (Utilities|Casting|CastToBP_ToggleButton (Variables|/Script/Engine.ChildActorComponent|GetChildActor _returnvalue_4)))
      (Default|SetState _asbp_toggle_button_3 false)
      (Utilities|Array|Add (Variables|Default|GetButtons) _asbp_toggle_button_3))
    (:then_4
      (for _array_element (Variables|Default|GetButtons)
        (Variables|/Game/ReusableAssets/Buttons/BP_ToggleButton.BP_ToggleButton_C|SetPush%20Button%20Mode _array_element true)))
    (:then_5
      (CallFunction|SetupButtonEvents))))