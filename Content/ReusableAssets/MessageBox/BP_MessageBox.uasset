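; BP_MessageBox is a reusable in-world message box actor that displays lines of text inside a bordered background.
; The construction script sets a fixed content size, then scales the 5x5 background mesh and four border meshes to fit it plus margins.
; UpdateLines stores the text and forwards it to the BP_MessageBoxContents child actor.
; BeginPlay makes the first call, as UMG bindings don't work during construction.
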(event EventBeginPlay
  (CallFunction|UpdateLines (Variables|Default|GetLines)))

(fn ConstructionScript
  (Utilities|FlowControl|Sequence
    (:then_1
      (LocalVariables|SetContent%20Size "(X=200.000000,Y=125.000000)"))
    (:then_4
      (Transformation|SetRelativeScale3D (Variables|Default|GetBackground) (Math|Vector|MakeVector 1.0 (+ (Variables|Default|GetHorizontal%20Margin) (.x (/ (LocalVariables|GetContent%20Size) 5.0))) (+ (.y (/ (LocalVariables|GetContent%20Size) 5.0)) (Variables|Default|GetVertical%20Margin))))
      (Transformation|SetRelativeScale3D (Variables|Default|GetBottom%20Border) (Math|Vector|MakeVector 1.0 (+ (Variables|Default|GetHorizontal%20Margin) (.x (/ (LocalVariables|GetContent%20Size) 5.0))) 1.0))
      (Transformation|SetRelativeScale3D (Variables|Default|GetLeft%20Border) (Math|Vector|MakeVector 1.0 (+ (.y (/ (LocalVariables|GetContent%20Size) 5.0)) (Variables|Default|GetVertical%20Margin)) 1.0)))))

(fn UpdateLines
  (params (Lines :type Array%20of%20Strings))
  (Variables|Default|SetLines Lines)
  ;[1 1 1] UMG Bindings don't work in Construction script
  (bind _asbp_message_box_contents (Utilities|Casting|CastToBP_MessageBoxContents (Variables|/Script/Engine.ChildActorComponent|GetChildActor (Variables|Default|GetContents))))
  (Default|UpdateText _asbp_message_box_contents (Variables|Default|GetLines)))