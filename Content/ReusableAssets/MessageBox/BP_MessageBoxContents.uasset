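; Actor that displays message box text through a widget component hosting WBP_MessageBoxContents.
; UpdateText concatenates an array of lines into one string, converts it to text and passes it to the widget's own UpdateText.
; The event graph and construction script hold no logic, so content changes only when UpdateText is called.
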(event EventBeginPlay)

(event Collision|EventActorBeginOverlap
  (params (OtherActor :type Actor%20Object%20Reference)))

(event EventTick
  (params (DeltaSeconds :type Float%20%28single-precision%29)))

(fn ConstructionScript)

(fn UpdateText
  (params (Lines :type Array%20of%20Strings))
  (for _array_element Lines
    (if (== (Utilities|String|Len (LocalVariables|GetText%20String)) 0)
      (LocalVariables|SetText%20String _array_element)
      (else
        (LocalVariables|SetText%20String (Class|VictoryBPFunctionLibrary|AppendMultiple (LocalVariables|GetText%20String) " 
 
" _array_element)))))
  (bind _aswbp_message_box_contents (Utilities|Casting|CastToWBP_MessageBoxContents (UserInterface|GetUserWidgetObject (Variables|Default|GetWidget))))
  (Default|UpdateText _aswbp_message_box_contents (Utilities|Text|ToText(String) (LocalVariables|GetText%20String))))