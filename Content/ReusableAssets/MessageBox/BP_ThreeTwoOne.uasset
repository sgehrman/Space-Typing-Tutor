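; BP_ThreeTwoOne is a self-destroying "3, 2, 1, Go!" countdown actor with a modal darkroom backdrop.
; Start fades in the BP_ModalDarkroom child actor with a title and subtitle, then builds hidden text renders.
; AnimateAndDestroy triggers a recursive loop that reveals each text, moving it along a timeline curve, with a sound before "Go!".
; On reaching "Go!", it fades out the darkroom and fires AnimationDone early for the buzzer.
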(event `self.ReceiveBeginPlay`
  (bind _returnvalue (`AddComponent|Child Actor Component_0` :`RelativeTransform` (`KismetMathLibrary.MakeTransform` (0.0 0.0 0.0))))
  (bind _asbp_modal_darkroom (cast `/Game/ReusableAssets/MessageBox/BP_ModalDarkroom` (`ChildActorComponent.ChildActor` _returnvalue)))
  (set `self.Darkroom` _asbp_modal_darkroom))

(event `Animate And Destroy`
  ;[1 1 1] Create one, and call this.  Destroys self when done
  (`KismetSystemLibrary.Delay` 1.0)
  (`self.Animate Text Render`))

(event `Start Count Down`
  (`|ExecutionSequence`
    (:`then_0`
      (for _array_element (`|MakeArray` "3" "2" "1" "Go!")
        (bind _text_render (`self.Create Text Render` _array_element 44.0))
        (`KismetArrayLibrary.Array_Add` (`self.Text Renders`) _text_render)))
    (:`then_1`
      (`TimelineComponent.SetPlayRate` (`self.Animate Render`) 3.0))))

(event `Animate Text Render`
  (bind _returnvalue (`GameplayStatics.GetPlayerPawn` 0))
  (bind _item (`KismetArrayLibrary.Array_Get` (`self.Text Renders`) (`self.Index`)))
  (bind (_returnvalue_location _returnvalue_rotation) (`KismetMathLibrary.BreakTransform` (`SceneComponent.GetRelativeTransform` _item)))
  (bind _returnvalue_2 (`KismetMathLibrary.InverseTransformLocation` (`self.GetTransform` _returnvalue) (`self.K2_GetActorLocation` _returnvalue)))
  (`SceneComponent.SetVisibility` _item true true)
  (if (< (`self.Index`) (- (`KismetArrayLibrary.Array_Length` (`self.Text Renders`)) 1))
    (`GameplayStatics.PlaySoundAtLocation` "/Game/UserInterfaceSFX/Cancel/cancel_error06_Cue.cancel_error06_Cue")
    (bind (_direction _c_genericcurve) (`Timeline|Animate Render` :!via `PlayFromStart` :!label _label)
      (:`Update`
        (`SceneComponent.K2_SetRelativeTransform` _item (`KismetMathLibrary.TLerp` (`KismetMathLibrary.MakeTransform` _returnvalue_2 _returnvalue_rotation (1.0 1.0 1.0)) (`KismetMathLibrary.MakeTransform` (`KismetMathLibrary.MakeVector` (+ (.x _returnvalue_2) 100.0) (.y _returnvalue_2) (.z _returnvalue_2)) _returnvalue_rotation (1.0 1.0 1.0)) _c_genericcurve) false))
      (:`Finished`
        (`KismetSystemLibrary.Delay` 0.3)
        (`SceneComponent.SetVisibility` _item false true)
        (`/Engine/EditorBlueprintResources/StandardMacros.IncrementInt` (`self.Index`)
          (:`  `
            (if (< (`self.Index`) (`KismetArrayLibrary.Array_Length` (`self.Text Renders`)))
              (`KismetSystemLibrary.Delay` 0.5)
              (`self.Animate Text Render`)
              ;[1 1 1] Call Animation Done on the last item so the buzzer will sound a bit earlier
              (if (== (`self.Index`) (- (`KismetArrayLibrary.Array_Length` (`self.Text Renders`)) 1))
                (`/Game/ReusableAssets/MessageBox/BP_ModalDarkroom.Fade Out` (`self.Darkroom`))
                (`self.AnimationDone`))
              (else
                (`KismetSystemLibrary.Delay` 1.0)
                (`self.K2_DestroyActor`)))))))
    (else
      (goto _label :!via `PlayFromStart`))))

(fn `Create Text Render`
  (params (Text :type Text) (`Text Size` :type "Float (double-precision)"))
  (returns (`Text Render` :type "TextRenderComponent Object Reference"))
  (`|ExecutionSequence`
    (:`then_0`
      (bind _returnvalue (`AddComponent|TextRenderComponent_0` :`RelativeTransform` (`KismetMathLibrary.MakeTransform` (0.0 0.0 0.0))))
      (`TextRenderComponent.K2_SetText` _returnvalue Text)
      (`SceneComponent.SetVisibility` _returnvalue false false)
      (`TextRenderComponent.SetWorldSize` _returnvalue `Text Size`)
      (`TextRenderComponent.SetHorizontalAlignment` _returnvalue "EHTA_Center")
      (`SceneComponent.K2_SetRelativeRotation` _returnvalue (struct :`Yaw` 180.0) false))
    (:`then_1`
      (return _returnvalue))))

(fn `Start`
  (params (Title :type Text) (Subtitle :type Text))
  (`/Game/ReusableAssets/MessageBox/BP_ModalDarkroom.Fade In` (`self.Darkroom`) Title Subtitle)
  (`self.Start Count Down`))

(fn `UserConstructionScript`)