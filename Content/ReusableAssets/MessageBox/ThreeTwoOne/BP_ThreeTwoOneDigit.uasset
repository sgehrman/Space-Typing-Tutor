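; BP_ThreeTwoOneDigit displays one animated text item of a three-two-one countdown and signals when its animation finishes.
; Start creates a centred TextRender component, then plays a beep that differs for the last item.
; Two timelines lerp it from above the origin to the middle, pause, then drop it below and hide it before calling AnimationDone.
; A Debugging flag speeds up the intro and removes the pause.
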(event Custom|Animate%20Text%20Render
  (Rendering|SetVisibility (Variables|Default|GetText%20Render) true true)
  (if (Variables|Default|GetLast%20Item)
    (Audio|PlaySoundatLocation "/Game/ReusableAssets/MessageBox/ThreeTwoOne/StartBeep.StartBeep" "0, 0, 0")
    (bind _c_genericcurve (Timeline|AnimateIn PlayFromStart)
      (:Update
        (Transformation|SetRelativeTransform (Variables|Default|GetText%20Render) (Math|Transform|Lerp(Transform) (CallFunction|AnimationTransform "Start") (CallFunction|AnimationTransform "Middle") _c_genericcurve) false false))
      (:Finished
        (Utilities|FlowControl|Delay (Math|Float|SelectFloat 0.0 0.3 (Variables|Default|GetDebugging)))
        (bind _c_genericcurve_2 (Timeline|AnimateOut PlayFromStart)
          (:Update
            (Transformation|SetRelativeTransform (Variables|Default|GetText%20Render) (Math|Transform|Lerp(Transform) (CallFunction|AnimationTransform "Middle") (CallFunction|AnimationTransform "End") _c_genericcurve_2) false false))
          (:Finished
            (Rendering|SetVisibility (Variables|Default|GetText%20Render) false true)
            (Default|CallAnimationDone)))))
    (else
      (Audio|PlaySoundatLocation "/Game/UserInterfaceSFX/Cancel/cancel_error06_Cue.cancel_error06_Cue" "0, 0, 0")
      (Timeline|AnimateIn PlayFromStart))))

(event Custom|Start
  (params (Text :type Text) (Last%20Item :type Boolean))
  (Utilities|FlowControl|Sequence
    (:then_0
      (bind _text_render (CallFunction|CreateTextRender Text 44.0))
      (Variables|Default|SetText%20Render _text_render))
    (:then_1
      (Components|Timeline|SetPlayRate (Variables|Default|GetAnimateIn) (Math|Float|SelectFloat 1e+02 3.0 (Variables|Default|GetDebugging))))
    (:then_2
      (Variables|Default|SetLast%20Item Last%20Item))
    (:then_3
      (CallFunction|AnimateTextRender))))

(fn ConstructionScript)

(fn CreateTextRender
  (params (Text :type Text) (Text%20Size :type Float%20%28single-precision%29))
  (Utilities|FlowControl|Sequence
    (:then_0
      (bind _returnvalue (AddComponent|AddTextRenderComponent false (Math|Transform|MakeTransform "0, 0,0.000000")))
      (Rendering|Components|TextRender|SetText _returnvalue Text)
      (Rendering|SetVisibility _returnvalue false false)
      (Rendering|Components|TextRender|SetWorldSize _returnvalue Text%20Size)
      (Rendering|Components|TextRender|SetHorizontalAlignment _returnvalue "EHTA_Center")
      (Transformation|SetRelativeRotation _returnvalue "0.000000,180.000000,0.000000" false false)
      (Class|SystemUtils|SetTextRendersVerticalAlign _returnvalue))
    (:then_1
      (return _returnvalue))))

(fn AnimationTransform
  (params (Identifier :type Name))
  (bind _returnvalue (Game|Player|GetPlayerPawn 0))
  (Utilities|FlowControl|Sequence
    (:then_0
      (LocalVariables|SetPlayer%20Local%20Location (Math|Transform|InverseTransformLocation (Transformation|GetActorTransform _returnvalue) (Transformation|GetActorLocation _returnvalue))))
    (:then_1
      (switch name Identifier
        (:Default
          (LocalVariables|SetResult%20Location (LocalVariables|GetPlayer%20Local%20Location) :!label _label))
        (:Start
          (LocalVariables|SetResult%20Location (Math|Vector|MakeVector (.X (Math|Vector|BreakVector (LocalVariables|GetPlayer%20Local%20Location))) (.Y (Math|Vector|BreakVector (LocalVariables|GetPlayer%20Local%20Location))) (+ (.Z (Math|Vector|BreakVector (LocalVariables|GetPlayer%20Local%20Location))) 1e+02))))
        (:Middle
          (goto _label))
        (:End
          (LocalVariables|SetResult%20Location (Math|Vector|MakeVector (.X (Math|Vector|BreakVector (LocalVariables|GetPlayer%20Local%20Location))) (.Y (Math|Vector|BreakVector (LocalVariables|GetPlayer%20Local%20Location))) (+ (.Z (Math|Vector|BreakVector (LocalVariables|GetPlayer%20Local%20Location))) -1e+02))))))
    (:then_2
      (return (Math|Transform|MakeTransform (LocalVariables|GetResult%20Location) (.rotation (Transformation|GetRelativeTransform (Variables|Default|GetText%20Render))) "1.000000,1.000000,1.000000")))))