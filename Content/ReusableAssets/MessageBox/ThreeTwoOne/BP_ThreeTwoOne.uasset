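; BP_ThreeTwoOne is a "3, 2, 1, Go!" countdown actor with a titled backdrop.
; It adds a BP_ModalDarkroom child actor at the player pawn's location, which Start fades in with title and subtitle.
; After a short delay, BP_ThreeTwoOneDigit child actors animate each string in turn, chained through their completion event.
; After the last, it fades out the darkroom, broadcasts AnimationDone and destroys itself.
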(event `self.ReceiveBeginPlay`
  (bind _returnvalue (`AddComponent|Child Actor Component_0` :`RelativeTransform` (`KismetMathLibrary.MakeTransform` (`self.K2_GetActorLocation` (`GameplayStatics.GetPlayerPawn` 0)))))
  (bind _asbp_modal_darkroom (cast `/Game/ReusableAssets/MessageBox/ThreeTwoOne/BP_ModalDarkroom` (`ChildActorComponent.ChildActor` _returnvalue)))
  (set `self.Darkroom` _asbp_modal_darkroom))

(event `Start Count Down`
  (`|ExecutionSequence`
    (:`then_0`
      (set `self.Text Strings` (`|MakeArray` "3" "2" "1" "Go!")))
    (:`then_1`
      (`KismetSystemLibrary.Delay` 1.0)
      (`self.Animate Text Render`))))

(event `Animate Text Render`
  (bind _returnvalue (`AddComponent|Child Actor Component_2483` :`RelativeTransform` (`KismetMathLibrary.MakeTransform` (0.0 0.0 0.0))))
  (bind _asbp_three_two_one_digit (cast `/Game/ReusableAssets/MessageBox/ThreeTwoOne/BP_ThreeTwoOneDigit` (`ChildActorComponent.ChildActor` _returnvalue)))
  (add `/Game/ReusableAssets/MessageBox/ThreeTwoOne/BP_ThreeTwoOneDigit.AnimationDone` _asbp_three_two_one_digit (delegate `Animation Done`))
  (`/Game/ReusableAssets/MessageBox/ThreeTwoOne/BP_ThreeTwoOneDigit.Start` _asbp_three_two_one_digit (`KismetArrayLibrary.Array_Get` (`self.Text Strings`) (`self.Index`)) (== (`KismetArrayLibrary.Array_LastIndex` (`self.Text Strings`)) (`self.Index`)) (`self.Debugging`)))

(event `Animation Done`
  (`/Engine/EditorBlueprintResources/StandardMacros.IncrementInt` (`self.Index`)
    (:`  `
      (if (< (`self.Index`) (`KismetArrayLibrary.Array_Length` (`self.Text Strings`)))
        (`self.Animate Text Render`)
        (else
          (`/Game/ReusableAssets/MessageBox/ThreeTwoOne/BP_ModalDarkroom.Fade Out` (`self.Darkroom`))
          (`self.AnimationDone`)
          (`KismetSystemLibrary.Delay` 1.0)
          (`self.K2_DestroyActor`))))))

(fn `Start`
  (params (Title :type Text) (Subtitle :type Text) (Debugging :type Boolean))
  (`|ExecutionSequence`
    (:`then_0`
      (set `self.Debugging` Debugging))
    (:`then_1`
      (`/Game/ReusableAssets/MessageBox/ThreeTwoOne/BP_ModalDarkroom.Fade In` (`self.Darkroom`) Title Subtitle)
      (`self.Start Count Down`))))

(fn `UserConstructionScript`)