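; BP_TextActor is an actor that shows one intro text message through a WBP_TextMessage widget component, then destroys itself.
; DisplayMessage sets the text at zero opacity, then a timeline fades it in while slightly scaling up the widget.
; After a short hold, a second timeline fades it out, calls the FinishedMessage dispatcher and destroys the actor.
; Interrupt hides the message and suppresses that dispatcher call.
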(event `Fade In Message`
  ;[1 1 1] Fade In
  (`|ExecutionSequence`
    (:`then_0`
      (bind _aswbp_text_message (cast `/Game/ReusableAssets/TextFadeIntro/WBP_TextMessage` (`WidgetComponent.GetUserWidgetObject` (`self.Text Widget`)))))
    (:`then_1`
      (bind (_direction _alpha) (`Timeline|Timeline_1` :!via `PlayFromStart`)
        (:`Update`
          (`UserWidget.SetColorAndOpacity` _aswbp_text_message (make `LinearColor` 1.0 1.0 1.0 _alpha))
          (`SceneComponent.SetRelativeScale3D` (`self.Text Widget`) (`KismetMathLibrary.Conv_DoubleToVector` (`KismetMathLibrary.MapRange` _alpha 0.0 1.0 1.0 1.1))))
        (:`Finished`
          (`KismetSystemLibrary.Delay` 2.0)
          (`self.Fade Out Current Message`))))))

(event `Fade Out Current Message`
  (`|ExecutionSequence`
    (:`then_1`
      (bind (_direction _alpha) (`Timeline|Timeline_0` :!via `PlayFromStart`)
        (:`Update`
          (`UserWidget.SetColorAndOpacity` (`self.Text Message`) (make `LinearColor` 1.0 1.0 1.0 _alpha)))
        (:`Finished`
          (if (not (`self.Interrupted`))
            (`self.Finished Message`))
          (`self.K2_DestroyActor`))))))

(fn `Display Message`
  (params (Message :type Text))
  (`|ExecutionSequence`
    (:`then_0`
      (`UserWidget.SetColorAndOpacity` (`self.Text Message`) (make `LinearColor` 1.0 1.0 1.0 0.0)))
    (:`then_1`
      (`/Game/ReusableAssets/TextFadeIntro/WBP_TextMessage.UpdateMessageText` (`self.Text Message`) Message))
    (:`then_2`
      (`self.Fade In Message`))))

(fn `Interrupt`
  (set `self.Interrupted` true)
  (`SceneComponent.SetVisibility` false true))

(fn `UserConstructionScript`
  (bind _aswbp_text_message (cast `/Game/ReusableAssets/TextFadeIntro/WBP_TextMessage` (`WidgetComponent.GetUserWidgetObject` (`self.Text Widget`))))
  (set `self.Text Message` _aswbp_text_message))