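; BP_TextDisplay runs a text intro that shows a sequence of messages, then loads a target map.
; On BeginPlay it reads lines and map name from a JSON file, sets up BP_ProgressBoxes, and waits for PLM to start ambient music.
; Each message gets a new BP_TextActor child component, whose finished event triggers the next.
; Click, Enter or gamepad bottom button interrupts the current message and advances, while Tab jumps straight to level loading.
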(event Custom|CustomEvent_0
  (params (Result :type BPI%20PMM%20Interface))
  ;[1 1 1] Event begin play - setup
  (bind _output_get (Variables|Default|SetPLM Result))
  (Default|PlayAmbientSound _output_get "/Game/ReusableAssets/TextFadeIntro/SC_TextIntroMapMusic.SC_TextIntroMapMusic")
  (Utilities|FlowControl|Delay 1.0)
  (CallFunction|ShowNextMessage))

(event Custom|Finished%20Event
  ;[1 1 1] Show Next Message
  (Variables|Default|SetCurrent%20Text%20Actor 0)
  (CallFunction|MessageFinished))

(event Custom|MessageFinished
  ;[1 1 1] Message Finished
  (if (Utilities|Array|IsValidIndex (Variables|Default|GetMessageArray) (Variables|Default|GetCurrent%20Index))
    (CallFunction|ShowNextMessage)
    (else
      (Default|LoadLevel (Variables|Default|GetPLM) (Variables|Default|GetMapNameToLoad)))))

(event Custom|Show%20Next%20Message
  ;[1 1 1] Show Next Message
  (if (Utilities|Array|IsValidIndex (Variables|Default|GetMessageArray) (Variables|Default|GetCurrent%20Index))
    (Utilities|FlowControl|Sequence
      (:then_1
        (bind _returnvalue (AddComponent|AddChildActorComponent false))
        (bind _asbp_text_actor (Utilities|Casting|CastToBP_TextActor (Variables|/Script/Engine.ChildActorComponent|GetChildActor _returnvalue)))
        (bind _output_get (Variables|Default|SetCurrent%20Text%20Actor _asbp_text_actor))
        (EventDispatchers|BindEventtoFinishedMessage _output_get (delegate Custom|Finished%20Event))
        (Default|DisplayMessage _output_get (Utilities|Array|Get(acopy) (Variables|Default|GetMessageArray) (Variables|Default|GetCurrent%20Index))))
      (:then_2
        (Default|UpdateSelection (Variables|Default|GetProgress%20Boxes) (Variables|Default|GetCurrent%20Index))
        (Variables|Default|SetCurrent%20Index (+ (Variables|Default|GetCurrent%20Index) 1))))))

(event EventBeginPlay
  ;[1 1 1] Event begin play - setup
  (Utilities|FlowControl|Sequence
    (:then_0
      (Input|EnableInput (Game|GetPlayerController 0)))
    (:then_1
      (bind _result (CallFunction|LoadMessagesfromFile (Variables|Default|GetFilename)))
      (Variables|Default|SetMessageArray _result))
    (:then_2
      (bind _asbp_progress_boxes (Utilities|Casting|CastToBP_ProgressBoxes (Variables|/Script/Engine.ChildActorComponent|GetChildActor (Variables|Default|GetProgress%20Box%20Component))))
      (Variables|Default|SetProgress%20Boxes _asbp_progress_boxes))
    (:then_3
      (Default|UpdateCount (Variables|Default|GetProgress%20Boxes) (Utilities|Array|Length (Variables|Default|GetMessageArray)))
      (Default|UpdateSelection (Variables|Default|GetProgress%20Boxes)))
    (:then_5
      (bind _returnvalue (AddComponent|AddBCPMMAccess))
      (EventDispatchers|BindEventtoPMMReady _returnvalue (delegate Custom|CustomEvent_0))
      (Default|Setup _returnvalue "None"))))

(event Input|GamepadEvents|GamepadFaceButtonBottom
  (params (Key :type Key%20Structure))
  ;[1 1 1] User hit button To skip ahead
  (:Pressed
    (Utilities|FlowControl|Sequence
      (:then_0
        (if (!= (Variables|Default|GetCurrent%20Text%20Actor) 0)
          (Default|Interrupt (Variables|Default|GetCurrent%20Text%20Actor))
          (Variables|Default|SetCurrent%20Text%20Actor 0)))
      (:then_1
        (CallFunction|MessageFinished)))))

(event Input|MouseEvents|LeftMouseButton
  (params (Key :type Key%20Structure))
  ;[1 1 1] User hit button To skip ahead
  (:Pressed
    (Utilities|FlowControl|Sequence
      (:then_0
        (if (!= (Variables|Default|GetCurrent%20Text%20Actor) 0)
          (Default|Interrupt (Variables|Default|GetCurrent%20Text%20Actor))
          (Variables|Default|SetCurrent%20Text%20Actor 0)))
      (:then_1
        (CallFunction|MessageFinished)))))

(event Input|KeyboardEvents|Enter
  (params (Key :type Key%20Structure))
  ;[1 1 1] User hit button To skip ahead
  (:Pressed
    (Utilities|FlowControl|Sequence
      (:then_0
        (if (!= (Variables|Default|GetCurrent%20Text%20Actor) 0)
          (Default|Interrupt (Variables|Default|GetCurrent%20Text%20Actor))
          (Variables|Default|SetCurrent%20Text%20Actor 0)))
      (:then_1
        (CallFunction|MessageFinished)))))

(event Input|KeyboardEvents|Tab
  (params (Key :type Key%20Structure))
  ;[1 1 1] Message Finished
  (:Pressed
    (Default|LoadLevel (Variables|Default|GetPLM) (Variables|Default|GetMapNameToLoad))))

(fn ConstructionScript)

(fn LoadMessagesfromFile
  (params (Filename :type String))
  (bind _returnvalue (Class|KrishnaJSON|ParseJson (Class|KrishnaJSON|Create) (.OutString (Class|FileSystemUtils|LoadFiletoString (Class|VictoryBPFunctionLibrary|AppendMultiple (Class|VictoryBPFunctionLibrary|VictoryPathsGameRootDirectory) "\\Content" "\\AppData" "\\" Filename)))))
  (Variables|Default|SetMapNameToLoad (Utilities|String|StringToName (.ReturnValue (Class|KrishnaJSON|GetString _returnvalue "maptoload"))))
  (for _array_element (Class|KrishnaJSON|GetStringArray _returnvalue "lines")
    (Utilities|Array|Add (LocalVariables|GetResultTexts) (Utilities|Text|ToText(String) _array_element)))
  (return (LocalVariables|GetResultTexts)))