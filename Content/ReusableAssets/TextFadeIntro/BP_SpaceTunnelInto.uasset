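; Intro actor for a space tunnel scene that waits for a confirm press, then loads TextIntroMap.
; BeginPlay spawns a demo keyboard child actor, positions the player and binds to PMM readiness, which caches the level loader, starts music and calls a screen fade.
; Gamepad, mouse or Enter input animates the keyboard out, then after a brief delay the LED tunnel, UE4 logo and title, and requests the level load.
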(event `Key|Gamepad_FaceButton_Bottom`
  (:`Pressed`
    (`|ExecutionSequence` :!label _label
      (:`then_0`
        (`self.Hide Keyboard`))
      (:`then_1`
        (`KismetSystemLibrary.Delay` 0.25)
        (`self.Hide Time Tunnel`)
        (`self.Hide UE4 Logo`)
        (`self.Hide Title Text`)
        (`/Game/ReusableAssets/Utilities/BPI_PMM.Load Level` (`self.PLM`) "TextIntroMap" "")))))

(event `Key|LeftMouseButton`
  (:`Pressed`
    (goto _label)))

(event `Key|Enter`
  (:`Pressed`
    (goto _label)))

(event `self.ReceiveBeginPlay`
  (`|ExecutionSequence`
    (:`then_0`
      (`self.EnableInput` (`GameplayStatics.GetPlayerController` 0)))
    (:`then_1`
      (bind _returnvalue (`AddComponent|Child Actor Component_84` :`RelativeTransform` (`KismetMathLibrary.MakeTransform` (250.0 0.0 111.0))))
      (bind _asbp_demo_keyboard (cast `/Game/ReusableAssets/Keyboard/KeyboardDemo/BP_DemoKeyboard` (`ChildActorComponent.ChildActor` _returnvalue)))
      (set `self.Demo Keyboard` _asbp_demo_keyboard))
    (:`then_2`
      (`/Game/ReusableAssets/Utilities/BC_LevelCommon.Move Player into Position` (`self.BC_LevelCommon`) true)
      (`KismetSystemLibrary.Delay` 0.5)
      (`/Game/ReusableAssets/Utilities/BC_LevelCommon.Move Player into Position` (`self.BC_LevelCommon`) false))
    (:`then_5`
      (bind _returnvalue_2 (`AddComponent|BC_PMMAccess_C_2`))
      (add `/Game/ReusableAssets/Utilities/BC_PMMAccess.PMM Ready` _returnvalue_2 (delegate `CustomEvent_0`))
      (`/Game/ReusableAssets/Utilities/BC_PMMAccess.Setup` _returnvalue_2))))

(event `Hide UE4 Logo`
  (bind _outactors (`GameplayStatics.GetAllActorsOfClass` "/Game/ReusableAssets/TextFadeIntro/BP_UE4Logo.BP_UE4Logo_C"))
  (`/Game/ReusableAssets/Utilities/LIB_Utilities.AnimateOutAndDestroy` (`KismetArrayLibrary.Array_Get` _outactors) (0.0 0.0 2000.0)))

(event `Hide Title Text`
  (`/Game/ReusableAssets/Utilities/LIB_Utilities.AnimateOutAndDestroy` (`.Actor` (`/Game/ReusableAssets/Utilities/LIB_Utilities.FindActorWithTag` "/Game/ReusableAssets/TextFadeIntro/BP_MainTitle.BP_MainTitle_C" "None" self)) (0.0 0.0 2000.0)))

(event `CustomEvent_0`
  (params (Result :type "/Game/ReusableAssets/Utilities/BPI_PMM Interface"))
  (bind _output_get (set `self.PLM` Result))
  (`/Game/ReusableAssets/Utilities/BPI_PMM.Play Ambient Sound` _output_get "/Game/ReusableAssets/TextFadeIntro/SC_TextIntroMapMusic.SC_TextIntroMapMusic")
  (`/Game/ReusableAssets/Utilities/LIB_Utilities.FadeOutScreen` true))

(event `Hide Keyboard`
  (bind _outactors (`GameplayStatics.GetAllActorsOfClass` "/Game/ReusableAssets/Keyboard/KeyboardDemo/BP_DemoKeyboard.BP_DemoKeyboard_C"))
  (`/Game/ReusableAssets/Utilities/LIB_Utilities.AnimateOutAndDestroy` (`KismetArrayLibrary.Array_Get` _outactors) (0.0 0.0 2000.0)))

(event `Hide Time Tunnel`
  (bind _outactors (`GameplayStatics.GetAllActorsOfClass` "/Game/ReusableAssets/TimeTunnel/BP_LEDTunnel.BP_LEDTunnel_C"))
  (bind _item (`KismetArrayLibrary.Array_Get` _outactors))
  (`/Game/ReusableAssets/Utilities/LIB_Utilities.AnimateOutAndDestroy` _item (`KismetMathLibrary.MakeVector` (* (.x (`.BoxExtent` (`self.GetActorBounds` _item false))) -10.0))))

(fn `UserConstructionScript`)