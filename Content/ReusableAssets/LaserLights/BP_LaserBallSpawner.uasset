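; BP_LaserBallSpawner spawns laser balls (UFOs) around itself in two modes: bouncing or fly-by.
; Above-actor mode spawns a bouncing ball at a random nearby offset after a short delay, repeating when LaserBallDestroyed is called.
; Fly-by mode uses a looping timer to add randomly delayed child-actor balls at varied heights, each running a fly-over animation with a random argument.
; Both play a spawn sound.
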(event `Start Spawn FlyBy`
  (`KismetSystemLibrary.K2_SetTimer` null "Spawn UFO FlyOver" 4.0 true))

(event `Start Spawn Above Actor`
  (`KismetSystemLibrary.Delay` 0.2 :!label _label)
  (`self.Spawn UFO`))

(event `Laser Ball Destroyed`
  (goto _label))

(event `Spawn UFO`
  (bind (_returnvalue_x _returnvalue_y _returnvalue_z) (`KismetMathLibrary.BreakVector` (`self.K2_GetActorLocation`)))
  (bind _returnvalue (`KismetMathLibrary.MakeVector` (+ (`KismetMathLibrary.RandomFloatInRange` -4000.0 4000.0) _returnvalue_x) (+ _returnvalue_y (`KismetMathLibrary.RandomFloatInRange` -4000.0 4000.0)) (+ _returnvalue_z (`KismetMathLibrary.RandomFloatInRange` -500.0 0.0))))
  (bind _returnvalue_2 (`|SpawnActorFromClass` "/Game/ReusableAssets/LaserLights/BP_LaserBall.BP_LaserBall_C" (`KismetMathLibrary.MakeTransform` _returnvalue) "AdjustIfPossibleButDontSpawnIfColliding" "OverrideRootScale" self))
  (`/Game/ReusableAssets/LaserLights/BP_LaserBall.Run Bounce Animation` _returnvalue_2)
  (`GameplayStatics.PlaySoundAtLocation` "/Game/ReusableAssets/LaserLights/LaserBall_Spawn_Sound.LaserBall_Spawn_Sound" _returnvalue (struct) 0.4 1.0 0.0 "/Game/Attenuation/Normal.Normal"))

(event `Spawn UFO FlyOver`
  (`KismetSystemLibrary.Delay` (`KismetMathLibrary.RandomFloatInRange` 0.0 2.0))
  (bind _returnvalue (`AddComponent|Child Actor Component_308` :`RelativeTransform` (`KismetMathLibrary.MakeTransform` (`KismetMathLibrary.MakeVector` 0.0 0.0 (+ 0.0 (`KismetMathLibrary.RandomFloatInRange` -500.0 0.0))))))
  (bind _asbp_laser_ball (cast `/Game/ReusableAssets/LaserLights/BP_LaserBall` (`ChildActorComponent.ChildActor` _returnvalue)))
  (`/Game/ReusableAssets/LaserLights/BP_LaserBall.Run FlyOver Animation` _asbp_laser_ball (`KismetMathLibrary.RandomFloatInRange` 12000.0 20000.0))
  (`GameplayStatics.SpawnSoundAttached` "/Game/ReusableAssets/LaserLights/LaserBall_Spawn_Sound.LaserBall_Spawn_Sound" _returnvalue "None" (0.0 0.0 0.0) (struct) "KeepRelativeOffset" false 0.4 1.0 0.0 "/Game/Attenuation/Normal.Normal"))

(fn `UserConstructionScript`)