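; Death Star laser weapon actor that charges on right mouse or X, then fires an electric beam at a BP_LaserBall and destroys it.
; The construction script builds a ring of instanced laser beams aimed at a focal point, with dynamic materials for glow and color.
; Firing chains timelines that extend the beams and brighten the power ball, then spawns the beam emitter with sound and camera shake before resetting.
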(event `Key|RightMouseButton`
  (params (Key :type "Key Structure"))
  (:`Pressed`
    (`self.ShowLasers` :!label _label)))

(event `Key|X`
  (params (Key :type "Key Structure"))
  (:`Pressed`
    (goto _label)))

(event `ShowLasers`
  (bind _small_beam_instanced_sm (`self.Small Beam Instanced SM`))
  (if (not (`self.IsFiring?`))
    (set `self.IsFiring?` true)
    (`GameplayStatics.PlaySoundAtLocation` "/Game/UniversalSoundFX/Sound_Effects/SPACE_WARPS/SPACE_WARP_Type_03A_Charge_Up_2_stereo.SPACE_WARP_Type_03A_Charge_Up_2_stereo" (`self.K2_GetActorLocation`))
    (`TimelineComponent.SetPlayRate` 3.0)
    (set `RotatingMovementComponent.RotationRate` (struct :`Yaw` 100.0) (`self.RotatingMovement`))
    (bind (_direction _alpha) (`Timeline|ChargeLaser` :!via `PlayFromStart`)
      (:`Update`
        (for _index (range (`InstancedStaticMeshComponent.GetInstanceCount` (`self.Small Beam Instanced SM`)))
          (bind _outinstancetransform (`InstancedStaticMeshComponent.GetInstanceTransform` _small_beam_instanced_sm _index false))
          (`InstancedStaticMeshComponent.UpdateInstanceTransform` _small_beam_instanced_sm _index (`KismetMathLibrary.MakeTransform` (.location _outinstancetransform) (.rotation _outinstancetransform) (`KismetMathLibrary.MakeVector` (`KismetMathLibrary.Lerp` 0.1 (`self.Laser Length`) _alpha) (.y (.scale _outinstancetransform)) (.z (.scale _outinstancetransform)))) false true)))
      (:`Finished`
        (`self.ShowPowerBall`)))))

(event `self.ReceiveBeginPlay`
  (`self.EnableInput` (`GameplayStatics.GetPlayerController` 0)))

(event `ShowPowerBall`
  (`SceneComponent.K2_SetRelativeLocation` (`self.Power Ball`) (`KismetMathLibrary.MakeVector` 0.0 0.0 (`self.Focal Point Height`)) false false)
  (bind (_direction _alpha) (`Timeline|PowerBall` :!via `PlayFromStart`)
    (:`Update`
      (`MaterialInstanceDynamic.SetScalarParameterValue` (`self.Power Ball MID`) "Emission" (`KismetMathLibrary.Lerp` 12.0 3333.0 _alpha)))
    (:`Finished`
      (`self.FireWeapon`))))

(event `FireWeapon`
  (bind _returnvalue (`self.K2_GetActorLocation`))
  (bind _returnvalue_2 (`SceneComponent.K2_GetComponentLocation` (`self.Power Ball`)))
  (bind _returnvalue_3 (`GameplayStatics.SpawnEmitterAtLocation` "/Game/ExampleContent/Effects/ParticleSystems/P_electricity_arc.P_electricity_arc" _returnvalue_2))
  (`ParticleSystemComponent.SetBeamSourcePoint` _returnvalue_3 0 _returnvalue_2 0)
  (bind _asbp_laser_ball (cast `/Game/ReusableAssets/LaserLights/BP_LaserBall` (`.Actor` (`/Game/ReusableAssets/Utilities/LIB_Utilities.FindActorWithTag` "/Game/ReusableAssets/LaserLights/BP_LaserBall.BP_LaserBall_C" "None" self))))
  (`ParticleSystemComponent.SetBeamTargetPoint` _returnvalue_3 0 (`self.K2_GetActorLocation` _asbp_laser_ball) 0)
  (`GameplayStatics.PlaySoundAtLocation` "/Game/UniversalSoundFX/Sound_Effects/SPACE_WARPS/SPACE_WARP_Complex_02_stereo.SPACE_WARP_Complex_02_stereo" _returnvalue)
  (`GameplayStatics.PlayWorldCameraShake` "/Game/ReusableAssets/LaserLights/BP_CameraShake.BP_CameraShake_C" _returnvalue 0.0 1500.0)
  (`/Game/ReusableAssets/LaserLights/BP_LaserBall.DestroyLaserBall` _asbp_laser_ball)
  (`KismetSystemLibrary.Delay` 1.0)
  (`ActorComponent.Deactivate` _returnvalue_3)
  (`KismetSystemLibrary.Delay` 1.0)
  (`GameplayStatics.PlaySoundAtLocation` "/Game/UniversalSoundFX/Sound_Effects/WHOOSHES/WHOOSH_Wide_Deep_Slow_stereo.WHOOSH_Wide_Deep_Slow_stereo" (`self.K2_GetActorLocation`))
  (`self.FinishFireWeapon`))

(event `FinishFireWeapon`
  (bind _small_beam_instanced_sm (`self.Small Beam Instanced SM`))
  (set `RotatingMovementComponent.RotationRate` (struct) (`self.RotatingMovement`))
  (for _index (range (`InstancedStaticMeshComponent.GetInstanceCount` (`self.Small Beam Instanced SM`)))
    (bind _outinstancetransform (`InstancedStaticMeshComponent.GetInstanceTransform` _small_beam_instanced_sm _index false))
    (`InstancedStaticMeshComponent.UpdateInstanceTransform` _small_beam_instanced_sm _index (`KismetMathLibrary.MakeTransform` (.location _outinstancetransform) (.rotation _outinstancetransform) (`KismetMathLibrary.MakeVector` 0.1 (.y (.scale _outinstancetransform)) (.z (.scale _outinstancetransform)))) false true))
  (set `self.IsFiring?` false)
  (`SceneComponent.K2_SetRelativeLocation` (`self.Power Ball`) (`KismetMathLibrary.MakeVector` 0.0) false false))

(fn `UserConstructionScript`
  (bind _laser_width (`self.Laser Width`))
  (bind _returnvalue (`KismetMathLibrary.MakeVector` 0.0 0.0 (`self.Focal Point Height`)))
  (`|ExecutionSequence`
    (:`then_1`
      (bind _returnvalue_2 (`KismetMaterialLibrary.CreateDynamicMaterialInstance` "/Game/ReusableAssets/LaserLights/MT_Laser.MT_Laser"))
      (bind _output_get (set `self.Small Beam MID` _returnvalue_2))
      (`MaterialInstanceDynamic.SetScalarParameterValue` _output_get "Emission" (`self.Emission`))
      (`MaterialInstanceDynamic.SetVectorParameterValue` _output_get "Color" (`self.Laser Color`)))
    (:`then_2`
      (bind _returnvalue_3 (`AddComponent|InstancedStaticMeshComponent_1`))
      (`PrimitiveComponent.SetMaterial` _returnvalue_3 0 (`self.Small Beam MID`))
      (set `self.Small Beam Instanced SM` _returnvalue_3))
    (:`then_3`
      (for _index (range (`self.Num Lasers`))
        (bind _returnvalue_4 (+ (`/Game/ReusableAssets/Utilities/LIB_Utilities.LocationAroundCircle` _index (`self.Num Lasers`) 155.0 (0.0 0.0 1.0)) (0.0 0.0 66.0)))
        (set `self.Laser Length` (`KismetMathLibrary.VSize` (- _returnvalue_4 _returnvalue)))
        (`InstancedStaticMeshComponent.AddInstance` (`self.Small Beam Instanced SM`) (`KismetMathLibrary.MakeTransform` _returnvalue_4 (`KismetMathLibrary.FindLookAtRotation` _returnvalue_4 _returnvalue) (`KismetMathLibrary.MakeVector` 0.1 _laser_width _laser_width)))))
    (:`then_4`
      (bind _returnvalue_5 (`KismetMaterialLibrary.CreateDynamicMaterialInstance` (`PrimitiveComponent.GetMaterial` (`self.Power Ball`) 0)))
      (bind _output_get_2 (set `self.Power Ball MID` _returnvalue_5))
      (`PrimitiveComponent.SetMaterial` (`self.Power Ball`) 0 _output_get_2))))