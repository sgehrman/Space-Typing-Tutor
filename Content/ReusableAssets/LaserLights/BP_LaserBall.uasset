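; BP_LaserBall is a flying, destructible ball that randomly fires short-lived laser beams at ground points around it.
; Construction adds child LaserWheels with randomized looks, caches its spawner and creates the emissive beam material.
; Bounce or fly-over animations start a looping timer that occasionally spawns stretched-mesh beams with impact explosion and sound, removed by a delayed destroyer.
; A sphere hit triggers a one-time explosion, notifies the spawner and destroys the actor.
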(event OnComponentHit(Sphere)
  (params (OtherActor :type Actor%20Object%20Reference) (OtherComp :type Primitive%20Component%20Object%20Reference) (NormalImpulse :type Vector :default "0, 0, 0") (Hit :type Hit%20Result%20Structure%20%28by%20ref%29))
  (bind _returnvalue (Transformation|GetActorLocation))
  (Utilities|FlowControl|DoOnce false
    (:Completed
      (Audio|PlaySoundatLocation "/Game/StarterContent/Audio/Explosion_Cue.Explosion_Cue" _returnvalue "0, 0, 0" 5.0 1.0 0.0 "/Game/UserInterfaceSFX/Attenuation/Interface_att.Interface_att")
      (Effects|SpawnEmitteratLocation "/Game/StarterContent/Particles/P_Explosion.P_Explosion" _returnvalue)
      (Rendering|ToggleVisibility true)
      (Utilities|FlowControl|Delay 2.0)
      (Default|LaserBallDestroyed (Variables|Default|GetSpawner))
      (Actor|DestroyActor))))

(event Custom|Start%20Laser%20Cannon%20Timer
  (params (Time :type Float%20%28single-precision%29))
  (Utilities|Time|SetTimerbyFunctionName 0 "FireLaserCannon" Time true))

(event Custom|DestroyLaserBall
  (bind _returnvalue (Transformation|GetActorLocation))
  (Utilities|FlowControl|DoOnce false
    (:Completed
      (Audio|PlaySoundatLocation "/Game/StarterContent/Audio/Explosion_Cue.Explosion_Cue" _returnvalue "0, 0, 0" 5.0 1.0 0.0 "/Game/UserInterfaceSFX/Attenuation/Interface_att.Interface_att")
      (Effects|SpawnEmitteratLocation "/Game/StarterContent/Particles/P_Explosion.P_Explosion" _returnvalue)
      (Rendering|ToggleVisibility true)
      (Utilities|FlowControl|Delay 2.0)
      (Default|LaserBallDestroyed (Variables|Default|GetSpawner))
      (Actor|DestroyActor))))

(event Custom|Destory%20component
  (params (Component :type Actor%20Component%20Object%20Reference))
  (Components|DestroyComponent Component))

(event Custom|FireLaserCannon
  (if (Rendering|IsVisible)
    ;[1 1 1] Fire Randomly
    (if (> (Math|Random|RandomFloat) 0.8)
      (bind _mesh_component (CallFunction|CreateLaserBeam))
      (bind _returnvalue (AddComponent|AddBCComponentDelayedDestroyer))
      (EventDispatchers|BindEventtoDestroyComponent _returnvalue (delegate Custom|Destory%20component))
      (Default|DestroyAfterDelay _returnvalue _mesh_component 0.2))))

(event Custom|Run%20Bounce%20Animation
  (Utilities|FlowControl|Sequence
    (:then_0
      (Variables|Default|SetStart%20Location (Transformation|GetActorLocation)))
    (:then_1
      (CallFunction|StartLaserCannonTimer 5.0))
    (:then_2
      (Components|Timeline|SetPlayRate 0.1)
      (bind _alpha (Timeline|Bouncer Play)
        (:Update
          (Transformation|SetActorLocation (Math|Vector|Lerp(Vector) (Variables|Default|GetStart%20Location) (+ (Variables|Default|GetStart%20Location) "1222.000000,1222.000000,333.000000") _alpha) false false))))))

(fn ConstructionScript
  (Utilities|FlowControl|Sequence
    (:then_0
      (for _index (range 0 6)
        (AddComponent|AddChildActorComponent false (Math|Transform|MakeTransform "0, 0, 0"))))
    (:then_1
      (for _array_element (Actor|GetComponentsByClass "/Script/Engine.ChildActorComponent")
        (bind _aslaser_wheel (Utilities|Casting|CastToLaserWheel (Variables|/Script/Engine.ChildActorComponent|GetChildActor _array_element)))
        (Utilities|Array|Add (Variables|Default|GetLaser%20Wheels) _aslaser_wheel)))
    (:then_2
      (for _array_element_2 (Variables|Default|GetLaser%20Wheels)
        (Variables|/Game/ReusableAssets/LaserLights/LaserWheel.LaserWheel_C|SetColor_0 _array_element_2 (Class|KismetMathLibrary|HSVtoRGB (Math|Random|RandomFloatinRange 0.0 359.0) (Math|Random|RandomFloatinRange 1.0 1.0) (Math|Random|RandomFloatinRange 0.1 0.2) 1.0))
        (Variables|/Game/ReusableAssets/LaserLights/LaserWheel.LaserWheel_C|SetNum%20Lasers _array_element_2 (Math|Random|RandomIntegerinRange 33 55))
        (Variables|/Game/ReusableAssets/LaserLights/LaserWheel.LaserWheel_C|SetLaser%20Length _array_element_2 (Math|Random|RandomFloatinRange 34.0 122.0))
        (Variables|/Game/ReusableAssets/LaserLights/LaserWheel.LaserWheel_C|SetEmission _array_element_2 55.0)
        (Default|UpdateLasers _array_element_2)))
    (:then_3
      (bind _asbp_laser_ball_spawner (Utilities|Casting|CastToBP_LaserBallSpawner (.Actor (CallFunction|FindActorwithTag "/Game/ReusableAssets/LaserLights/BP_LaserBallSpawner.BP_LaserBallSpawner_C" "None" self))))
      (Variables|Default|SetSpawner _asbp_laser_ball_spawner))
    (:then_4
      (bind _returnvalue (Rendering|Material|CreateDynamicMaterialInstance "/Game/ReusableAssets/LaserLights/MT_Laser.MT_Laser" :!class /Script/Engine.KismetMaterialLibrary))
      (bind _output_get (Variables|Default|SetLaser%20Cannon%20MID _returnvalue))
      (Rendering|Material|SetScalarParameterValue _output_get "Emission" 1222.0 :!class /Script/Engine.MaterialInstanceDynamic))))

(fn RunFlyOverAnimation
  (params (Distance :type Float%20%28single-precision%29))
  (bind _returnvalue (/ Distance 2.0))
  (Utilities|FlowControl|Sequence
    (:then_0
      (LocalVariables|SetStart (Math|Vector|MakeVector 0.0 (Class|TKMathFunctionLibrary|NegateFloat _returnvalue) 0.0))
      (LocalVariables|SetEnd (Math|Vector|MakeVector 0.0 _returnvalue 0.0)))
    (:then_1
      (CallFunction|StartLaserCannonTimer 0.2))
    (:then_3
      (CallFunction|AnimatewithParams (Utilities|Array|MakeArray (Utilities|Struct|MakeS_AnimationParams self true (LocalVariables|GetStart) (LocalVariables|GetEnd) true false "0, 0, 0" "0, 0, 0" 1.0 false 0 0.1 0.0 true)) true))))

(fn LaserTargetPosition
  (params (Target%20Pawn :type Boolean))
  (bind _returnvalue (Transformation|GetActorLocation))
  (bind _spread (LocalVariables|GetSpread))
  (bind _spread_2 (LocalVariables|GetSpread))
  (bind (_x _y) (Math|Vector|BreakVector _returnvalue))
  (bind _returnvalue_2 (Class|TKMathFunctionLibrary|NegateFloat _spread))
  (bind _returnvalue_3 (Math|Random|RandomFloatinRange _returnvalue_2 _spread_2))
  (Utilities|FlowControl|Sequence
    (:then_0
      (if Target%20Pawn
        (LocalVariables|SetResult (Transformation|GetActorLocation (Game|Player|GetPlayerPawn 0)))
        (else
          (LocalVariables|SetResult (Math|Vector|MakeVector (+ _x _returnvalue_3) (+ _y _returnvalue_3) -2e+02)))))
    (:then_2
      (return (LocalVariables|GetResult)))))

(fn CreateLaserBeam
  (bind _returnvalue (Transformation|GetActorLocation))
  (bind _position (CallFunction|LaserTargetPosition false))
  (Utilities|FlowControl|Sequence
    (:then_0
      (bind _returnvalue_2 (AddComponent|AddStaticMeshComponent false (Math|Transform|MakeTransform (Math|Vector|MakeVector 0.0 0.0 0.0) (Math|Rotator|FindLookatRotation _returnvalue _position) (Math|Vector|MakeVector (+ (Math|Vector|VectorLength (- _returnvalue _position)) 5e+02) 8.0 8.0))))
      (bind _output_get (LocalVariables|SetResult _returnvalue_2))
      (Components|StaticMesh|SetStaticMesh _output_get "/Game/ReusableAssets/LaserLights/SM_RopeX.SM_RopeX")
      (Rendering|SetCastShadow _output_get false)
      (Rendering|Material|SetMaterial _output_get 0 (Variables|Default|GetLaser%20Cannon%20MID))
      (Audio|PlaySoundatLocation "/Game/UserInterfaceSFX/Select/Wavs/select13.select13" _position "0, 0, 0" 1.0 1.0 0.0 "/Game/Attenuation/Normal.Normal")
      (Effects|SpawnEmitteratLocation "/Game/StarterContent/Particles/P_Explosion.P_Explosion" _position))
    (:then_1
      (return (LocalVariables|GetResult)))))