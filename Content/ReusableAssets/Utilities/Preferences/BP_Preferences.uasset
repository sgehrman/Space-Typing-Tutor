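; Preferences actor that keeps typed key/value settings (Float, Integer, String, Bool) in a BP_SaveGame slot.
; On BeginPlay it loads the main slot, or creates a new save object if none exists.
; Set stores each value as a string and immediately saves to disk.
; Get converts the string back to the requested type, but its IsValid output is fed by the Bool result, not the lookup's validity.
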(event EventBeginPlay
  (CallFunction|LoadPrefs (Variables|Default|GetMain%20Slot%20Name)))

(event EventActorBeginOverlap
  (params (OtherActor :type Actor%20Object%20Reference)))

(event EventTick
  (params (DeltaSeconds :type Float%20%28single-precision%29)))

(fn ConstructionScript)

(fn Get
  (params (Key :type String) (Data%20Type :type E_DataType%20Enum))
  (bind _save_game_prefs (Variables|Default|GetSave%20Game%20Prefs))
  (bind (_is_valid _value) (Default|Get _save_game_prefs Key))
  (Utilities|FlowControl|Sequence
    (:then_0
      (bind _output_get (LocalVariables|SetR_IsValid _is_valid))
      (if _output_get
        (LocalVariables|SetValue _value)
        (switch Utilities|FlowControl|Switch|SwitchonE_DataType Data%20Type
          (:NewEnumerator0
            (LocalVariables|SetR_Float (Math|Conversions|ToFloat(Integer) (LocalVariables|GetValue))))
          (:NewEnumerator1
            (LocalVariables|SetR_Integer (Math|Conversions|ToInteger(Byte) (LocalVariables|GetValue))))
          (:NewEnumerator2
            (LocalVariables|SetR_String (LocalVariables|GetValue)))
          (:NewEnumerator3
            (switch string (LocalVariables|GetValue)
              (:True
                (LocalVariables|SetR_Bool true))
              (:False
                (LocalVariables|SetR_Bool false)))))))
    (:then_2
      (return (LocalVariables|GetR_Bool) (LocalVariables|GetR_Bool) (LocalVariables|GetR_Float) (LocalVariables|GetR_String) (LocalVariables|GetR_Integer)))))

(fn Set
  (params (Key :type String) (Data%20Type :type E_DataType%20Enum) (Bool :type Boolean) (Integer :type Integer) (String :type String) (Float :type Float%20%28single-precision%29))
  (Utilities|FlowControl|Sequence
    (:then_0
      (switch Utilities|FlowControl|Switch|SwitchonE_DataType Data%20Type
        (:NewEnumerator0
          (LocalVariables|SetString%20Value (Utilities|String|ToString(Float) Float)))
        (:NewEnumerator1
          (LocalVariables|SetString%20Value (Utilities|String|ToString(Integer) Integer)))
        (:NewEnumerator2
          (LocalVariables|SetString%20Value String))
        (:NewEnumerator3
          (LocalVariables|SetString%20Value (Utilities|String|ToString(Boolean) Bool)))))
    (:then_1
      (Default|Set (Variables|Default|GetSave%20Game%20Prefs) Key (LocalVariables|GetString%20Value))
      (CallFunction|SavePrefs (Variables|Default|GetMain%20Slot%20Name)))))

(fn LoadPrefs
  (params (Slot%20Name :type String))
  (bind _returnvalue (SaveGame|DoesSaveGameExist Slot%20Name))
  (if _returnvalue
    (bind _returnvalue_2 (SaveGame|LoadGamefromSlot Slot%20Name))
    (bind _asbp_save_game (Utilities|Casting|CastToBP_SaveGame _returnvalue_2))
    (Variables|Default|SetSave%20Game%20Prefs _asbp_save_game)
    (else
      (bind _returnvalue_3 (SaveGame|CreateSaveGameObject "/Game/ReusableAssets/Utilities/BP_SaveGame.BP_SaveGame_C"))
      (bind _asbp_save_game_2 (Utilities|Casting|CastToBP_SaveGame _returnvalue_3))
      (Variables|Default|SetSave%20Game%20Prefs _asbp_save_game_2))))

(fn SavePrefs
  (params (Slot%20Name :type String))
  (SaveGame|SaveGametoSlot (Variables|Default|GetSave%20Game%20Prefs) Slot%20Name))