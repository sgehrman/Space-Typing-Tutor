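; BP_SaveGame is a key-value store for the Preferences utility, kept in two parallel arrays.
; Set finds the key's index in KeyIndexArray, appending the key if absent, and writes the value at the same index in ValueArray, resizing as needed.
; Get looks up that index and returns the value with an IsValid flag that is set only when both key and index exist.
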(fn Get
  (params (Key :type String))
  (bind _key_index_array (Variables|Default|GetKey%20Index%20Array))
  (bind _returnvalue (Utilities|Array|FindItem _key_index_array Key))
  (Utilities|FlowControl|Sequence
    (:then_0
      (if (!= _returnvalue -1)
        (if (Utilities|Array|IsValidIndex (Variables|Default|GetValue%20Array) _returnvalue)
          (LocalVariables|SetR_Result (Utilities|Array|Get(acopy) (Variables|Default|GetValue%20Array) _returnvalue))
          (LocalVariables|SetR_IsValid true))))
    (:then_3
      (return (LocalVariables|GetR_IsValid) (LocalVariables|GetR_Result)))))

(fn Set
  (params (Key :type String) (Value :type String))
  (bind _key_index_array (Variables|Default|GetKey%20Index%20Array))
  (bind _returnvalue (Utilities|Array|FindItem _key_index_array Key))
  (Utilities|FlowControl|Sequence
    (:then_0
      (if (!= _returnvalue -1)
        (LocalVariables|SetValue%20Index _returnvalue)
        (else
          (bind _returnvalue_2 (Utilities|Array|Add (Variables|Default|GetKey%20Index%20Array) Key))
          (LocalVariables|SetValue%20Index _returnvalue_2))))
    (:then_1
      (Utilities|Array|SetArrayElem (Variables|Default|GetValue%20Array) (LocalVariables|GetValue%20Index) Value true))))