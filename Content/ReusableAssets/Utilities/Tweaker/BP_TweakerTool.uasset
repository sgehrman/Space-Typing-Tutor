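; In-world debug tool for tweaking the level's directional light with the scroll wheel.
; After a short delay, BeginPlay spawns a 3x3 grid of BP_ToggleButton child actors in push mode and grabs the first DirectionalLight.
; Scroll events, routed by button ID, step that light's intensity or actor rotation and log the result; clicks only log.
; The last three buttons rotate a Light component, whose creation code is never executed.
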(event Custom|Listen%20to%20Button%20Events
  (for _array_element (Variables|Default|GetButtons)
    (EventDispatchers|BindEventtoButtonClickedbyUser _array_element (delegate Custom|Button%20Clicked))
    (EventDispatchers|BindEventtoScrollWheelMoved _array_element (delegate Custom|Scrolled))))

(event Custom|Button%20Clicked
  (params (Button%20ID :type String) (Hit%20Location :type Vector))
  (CallFunction|Logg Button%20ID))

(event Custom|Scrolled
  (params (Scrolled%20Down :type Boolean) (Button%20ID :type String))
  (bind _light_source_actor (Variables|Default|GetLight%20Source%20Actor))
  (bind _light (Variables|Default|GetLight))
  (switch string Button%20ID
    (:2
      (CallFunction|AdjustLight Scrolled%20Down))
    (:3
      (CallFunction|RotateActor "0, 0,1.000000" Scrolled%20Down _light_source_actor))
    (:4
      (CallFunction|RotateActor "1.000000, 0, 0" Scrolled%20Down _light_source_actor))
    (:5
      (CallFunction|RotateActor "0,1.000000, 0" Scrolled%20Down _light_source_actor))
    (:6
      (CallFunction|RotateComponent "0, 0,1.000000" Scrolled%20Down _light))
    (:7
      (CallFunction|RotateComponent "1.000000, 0,0.000000" Scrolled%20Down _light))
    (:8
      (CallFunction|RotateComponent "0,1.000000,0.000000" Scrolled%20Down _light))))

(event EventBeginPlay
  ;[1 1 1] Let map get built first
  (Utilities|FlowControl|Delay 0.2)
  (Utilities|FlowControl|Sequence
    (:then_0
      (bind _locations (CallFunction|ButtonTransforms))
      (for (_array_element _array_index) _locations
        (bind _returnvalue (AddComponent|AddChildActorComponent false _array_element))
        (bind _asbp_toggle_button (Utilities|Casting|CastToBP_ToggleButton (Variables|/Script/Engine.ChildActorComponent|GetChildActor _returnvalue)))
        (Default|SetTitleandSize _asbp_toggle_button (Variables|Default|GetButton%20Size) false (CallFunction|TitleforIndex _array_index) (Utilities|String|ToString(Integer) _array_index))
        (Utilities|Array|Add (Variables|Default|GetButtons) _asbp_toggle_button)
        (Variables|/Game/ReusableAssets/Buttons/BP_ToggleButton.BP_ToggleButton_C|SetPush%20Button%20Mode _asbp_toggle_button true)))
    (:then_1
      (CallFunction|ListentoButtonEvents))
    (:then_4
      (bind _outactors (Actor|GetAllActorsOfClass "/Script/Engine.DirectionalLight"))
      (if (Utilities|Array|IsValidIndex _outactors)
        (Variables|Default|SetLight%20Source%20Actor (Utilities|Array|Get(acopy) _outactors))
        (CallFunction|Logg "niggaaa")
        (else
          (CallFunction|Logg "you got shit"))))))

(fn ConstructionScript)

(fn ButtonTransforms
  (Utilities|FlowControl|Sequence
    (:then_0
      (for _array_element (CallFunction|PositionsinGrid 9 3 1.0 (Variables|Default|GetButton%20Size) true)
        (Utilities|Array|Add (LocalVariables|GetResult) (Math|Transform|MakeTransform _array_element))))
    (:then_2
      (return (LocalVariables|GetResult)))))

(fn TitleforIndex
  (params (Index :type Integer))
  (Utilities|FlowControl|Sequence
    (:then_0
      (switch int Index
        (:0
          (LocalVariables|SetResult "M"))
        (:1
          (LocalVariables|SetResult "^"))
        (:2
          (LocalVariables|SetResult "!"))
        (:3
          (LocalVariables|SetResult "X"))
        (:4
          (LocalVariables|SetResult "Y"))
        (:5
          (LocalVariables|SetResult "Z"))
        (:6
          (LocalVariables|SetResult "R"))
        (:7
          (LocalVariables|SetResult "P"))
        (:8
          (LocalVariables|SetResult "Y"))))
    (:then_1
      (return (LocalVariables|GetResult)))))

(fn AdjustLight
  (params (Down :type Boolean))
  (Utilities|FlowControl|Sequence
    (:then_0
      (if Down
        (LocalVariables|SetIntensity (+ (Variables|/Script/Engine.LightComponentBase|GetIntensity (Variables|/Script/Engine.Light|GetLightComponent (Variables|Default|GetLight%20Source%20Actor))) -0.3))
        (else
          (LocalVariables|SetIntensity (+ (Variables|/Script/Engine.LightComponentBase|GetIntensity (Variables|/Script/Engine.Light|GetLightComponent (Variables|Default|GetLight%20Source%20Actor))) 0.3)))))
    (:then_1
      (Rendering|Components|Light|SetIntensity (Variables|/Script/Engine.Light|GetLightComponent (Variables|Default|GetLight%20Source%20Actor)) (LocalVariables|GetIntensity))
      (CallFunction|Logg (Class|VictoryBPFunctionLibrary|AppendMultiple "Intensity: " (Utilities|String|ToString(Float) (LocalVariables|GetIntensity)))))))

(fn RotateComponent
  (params (Rotator :type Rotator) (Down :type Boolean) (Component :type Scene%20Component%20Object%20Reference))
  (bind _result (CallFunction|AdjustedRotation Rotator (Variables|/Script/Engine.SceneComponent|GetRelativeRotation Component) Down))
  (Transformation|SetRelativeRotation Component _result false)
  (CallFunction|Logg (Class|VictoryBPFunctionLibrary|AppendMultiple "Rot: " (Utilities|String|ToString(Rotator) _result))))

(fn AdjustedRotation
  (params (Rotation%20Flags :type Rotator) (Current%20Rotation :type Rotator) (Down :type Boolean))
  (bind (_pitch _yaw _roll) (Class|KismetMathLibrary|BreakRot Current%20Rotation))
  (bind (_pitch_2 _yaw_2 _roll_2) (Class|KismetMathLibrary|BreakRot Rotation%20Flags))
  (Utilities|FlowControl|Sequence
    (:then_0
      (if Down
        (LocalVariables|SetOffset -3.0)
        (else
          (LocalVariables|SetOffset 3.0))))
    (:then_2
      (return (Class|KismetMathLibrary|MakeRot (+ _pitch (* _pitch_2 (LocalVariables|GetOffset))) (+ _yaw (* _yaw_2 (LocalVariables|GetOffset))) (+ _roll (* _roll_2 (LocalVariables|GetOffset))))))))

(fn RotateActor
  (params (Rotator :type Rotator) (Down :type Boolean) (Actor :type Actor%20Object%20Reference))
  (bind _result (CallFunction|AdjustedRotation Rotator (Transformation|GetActorRotation Actor) Down))
  (Transformation|SetActorRotation Actor _result)
  (CallFunction|Logg (Class|VictoryBPFunctionLibrary|AppendMultiple "ARot: " (Utilities|String|ToString(Rotator) _result))))