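; BP_DebugLogger is a debug utility that shows a running message log in its LogText component.
; Logg appends each message after a <br> line break, substituting "(blank)" for empty input.
; The displayed text itself serves as the log buffer, and is discarded before appending once it grows past a length cap.
; ClearLogg empties the log, and the construction script starts it blank.
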(event `Logg`
  (params (Message :type String))
  (if (== (`KismetStringLibrary.Len` Message) 0)
    (set `self.In Message` "(blank)")
    (else
      (set `self.In Message` Message)))
  (if (> (`KismetStringLibrary.Len` (`KismetTextLibrary.Conv_TextToString` (`TextRenderComponent.Text` (`self.Log Text`)))) 5000)
    (set `self.Previous Text` "")
    (else
      (set `self.Previous Text` (`KismetTextLibrary.Conv_TextToString` (`TextRenderComponent.Text` (`self.Log Text`))))))
  (`TextRenderComponent.K2_SetText` (`self.Log Text`) (`KismetTextLibrary.Conv_StringToText` (`VictoryBPFunctionLibrary.AppendMultiple` (`self.Previous Text`) "<br>" (`self.In Message`)))))

(event `Clear Logg`
  (bind _output_get (set `self.Previous Text` ""))
  (`TextRenderComponent.K2_SetText` (`self.Log Text`) (`KismetTextLibrary.Conv_StringToText` _output_get)))

(fn `UserConstructionScript`
  (`TextRenderComponent.K2_SetText` (`self.Log Text`) ""))