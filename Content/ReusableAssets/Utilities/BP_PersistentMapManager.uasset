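; BP_PersistentMapManager is the persistent-level manager for what appears to be a typing lesson game.
; On BeginPlay it spawns shared helper actors (crosshair, fader, key listener, debug tools), signals initialization, then loads the start level.
; Level changes set the lesson index, fade out, disable key listening and swap streamed sublevels.
; It also exposes lesson data, switches ambient sound and opens an F9/Escape menu, where a second press quits.
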(event Custom|Load%20Level%20Event
  (params (Name :type Name) (Lesson%20Index :type Integer))
  (Utilities|FlowControl|Sequence
    (:then_0
      (Default|SetCurrentLessonIndex (Variables|Default|GetBC_KeyboardLessonData) Lesson%20Index))
    (:then_1
      (CallFunction|FadeOutScreen false))
    (:then_2
      (Utilities|FlowControl|Delay 0.5)
      (Utilities|FlowControl|Sequence
        (:then_0
          (if (Utilities|Name|NotEqual(Name) (Variables|Default|GetLoaded%20Level%20Name) "None")
            ;[1 1 1] Disable this if last map enabled it
            (Default|SetEnabled (Variables|Default|GetKey%20Event%20Listener) false)
            (Game|UnloadStreamLevel(byName) (Variables|Default|GetLoaded%20Level%20Name))))
        (:then_1
          (Game|LoadStreamLevel(byName) Name true true)
          (Variables|Default|SetLoaded%20Level%20Name Name))))))

(event Custom|Play%20Ambient%20Sound%20Event
  (params (Sound :type Sound%20Base%20Object%20Reference))
  (Utilities|FlowControl|Sequence
    (:then_0
      (if (!= (Variables|Default|GetAmbient%20Sound) 0)
        (bind _sound_playing (Default|IsPlayingThisSound (Variables|Default|GetAmbient%20Sound) Sound))
        (if (not _sound_playing)
          (Default|FadeOutandDestroy (Variables|Default|GetAmbient%20Sound))
          (Variables|Default|SetAmbient%20Sound 0))))
    (:then_1
      ;[1 1 1] Only start sound if different than the last sound
      (if (== (Variables|Default|GetAmbient%20Sound) 0)
        (bind _returnvalue (AddComponent|AddBCAmbientSound))
        (bind _output_get (Variables|Default|SetAmbient%20Sound _returnvalue))
        (Default|Play _output_get Sound)))))

(event EventBeginPlay
  (bind _returnvalue (Math|Transform|MakeTransform "0, 0, 0"))
  (bind _self self)
  (Utilities|FlowControl|Sequence
    (:then_0
      (Input|EnableInput (Game|GetPlayerController 0)))
    (:then_2
      (bind _returnvalue_2 (Game|SpawnActorfromClass "/Game/ReusableAssets/Crosshair/CrosshairActor.CrosshairActor_C" _returnvalue false _self 0))
      (Variables|/Game/ReusableAssets/Crosshair/CrosshairActor.CrosshairActor_C|SetDefault%20Distance _returnvalue_2 4e+02)
      (Variables|/Game/ReusableAssets/Crosshair/CrosshairActor.CrosshairActor_C|SetShow%20Particle%20System _returnvalue_2 false))
    (:then_3
      (Game|SpawnActorfromClass "/Game/ReusableAssets/Utilities/StandardSetup.StandardSetup_C" _returnvalue false _self 0))
    (:then_5
      (Game|SpawnActorfromClass "/Game/ReusableAssets/Utilities/BP_DebugLogger.BP_DebugLogger_C" (Math|Transform|MakeTransform "111.000000,44.000000, 0") false _self 0))
    (:then_6
      (Game|SpawnActorfromClass "/Game/ReusableAssets/Utilities/ScreenFader.ScreenFader_C" _returnvalue false _self 0))
    (:then_7
      (if (Variables|Default|GetMemory%20Debugger%20Enabled)
        (bind _returnvalue_3 (Game|SpawnActorfromClass "/Game/ReusableAssets/Utilities/BP_GarbageCollectorDebugger.BP_GarbageCollectorDebugger_C" _returnvalue false _self 0))
        (Default|Start _returnvalue_3 2.0)))
    (:then_8
      (bind _returnvalue_4 (Game|SpawnActorfromClass "/Game/ReusableAssets/Keyboard/BP_KeyEventListener.BP_KeyEventListener_C" _returnvalue false _self 0))
      (Variables|Default|SetKey%20Event%20Listener _returnvalue_4))
    (:then_10
      (Utilities|FlowControl|Delay 0.2)
      (Utilities|FlowControl|Sequence
        (:then_0
          (Variables|Default|SetInitialized true))
        (:then_1
          (Default|CallPMMInitialized))
        (:then_2
          (if (not (Utilities|Name|Equal(Name) (Variables|Default|GetStart%20Level%20Name) "None"))
            (CallFunction|LoadLevelEvent (Variables|Default|GetStart%20Level%20Name))))))))

(event Input|KeyboardEvents|Escape
  (:Pressed
    (if (!= (Variables|Default|GetEscape%20Menu) 0)
      (Default|HideandDestroy (Variables|Default|GetEscape%20Menu))
      (Variables|Default|SetEscape%20Menu 0)
      (Utilities|FlowControl|Delay 2.0)
      (Game|QuitGame 0 "Quit")
      (else
        (bind _returnvalue (Game|SpawnActorfromClass "/Game/ReusableAssets/MessageBox/BP_EscapeMenu.BP_EscapeMenu_C" (Math|Transform|MakeTransform "0.000000,0.000000,0.000000" "0, 0,0.000000") false self 0))
        (bind _output_get (Variables|Default|SetEscape%20Menu _returnvalue))
        (Default|Show _output_get "Fuck off" "Honkey lips")))))

(event Input|KeyboardEvents|F9
  (:Pressed
    (if (!= (Variables|Default|GetEscape%20Menu) 0)
      (Default|HideandDestroy (Variables|Default|GetEscape%20Menu))
      (Variables|Default|SetEscape%20Menu 0)
      (Utilities|FlowControl|Delay 2.0)
      (Game|QuitGame 0 "Quit")
      (else
        (bind _returnvalue (Game|SpawnActorfromClass "/Game/ReusableAssets/MessageBox/BP_EscapeMenu.BP_EscapeMenu_C" (Math|Transform|MakeTransform "0.000000,0.000000,0.000000" "0, 0,0.000000") false self 0))
        (bind _output_get (Variables|Default|SetEscape%20Menu _returnvalue))
        (Default|Show _output_get "Fuck off" "Honkey lips")))))

(fn ConstructionScript)

(fn IsInitialized
  (return (Variables|Default|GetInitialized)))

(fn CurrentLesson
  (return (Default|GetCurrentLesson (Variables|Default|GetBC_KeyboardLessonData))))

(fn GetKeyEventListener
  (return (Variables|Default|GetKey%20Event%20Listener)))

(fn LessonatIndex
  (params (Index :type Integer))
  (return (Default|LessonatIndex (Variables|Default|GetBC_KeyboardLessonData) Index)))

(fn LoadLevel
  (params (Level%20Name :type Name) (Lesson%20Index :type Integer))
  (CallFunction|LoadLevelEvent Level%20Name Lesson%20Index)
  (return false))

(fn NumberOfLessons
  (return (Default|NumberOfLessons (Variables|Default|GetBC_KeyboardLessonData))))

(fn PlayAmbientSound
  (params (Sound :type Sound%20Base%20Object%20Reference))
  (CallFunction|PlayAmbientSoundEvent Sound)
  (return true))

(fn ShouldShowIntro
  (Utilities|FlowControl|Sequence
    (:then_0
      ;[1 1 1] Only show once, turn off after first call
      (if (Variables|Default|GetShould%20Show%20Typing%20Intro)
        (Variables|Default|SetShould%20Show%20Typing%20Intro false)
        (LocalVariables|SetResult true)))
    (:then_1
      (if (Variables|Default|GetIn%20Development%20Mode)
        ;[1 1 1] Skip when debugging
        (LocalVariables|SetResult false)))
    (:then_2
      (return (LocalVariables|GetResult)))))