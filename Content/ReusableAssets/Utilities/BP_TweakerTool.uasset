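; BP_TweakerTool is an in-world 3x3 pad of push buttons labeled like a directional control, with arrows, a center plus and dashes in the corners.
; On BeginPlay it spawns BP_ToggleButton child actors at grid-computed transforms, setting each title, size and index-based ID.
; It then binds every button's click and scroll-wheel events to handlers that currently only log the input.
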(event Custom|Listen%20to%20Button%20Events
  (for _array_element (Variables|Default|GetButtons)
    (EventDispatchers|BindEventtoButtonClickedbyUser _array_element (delegate Custom|Button%20Clicked))
    (EventDispatchers|BindEventtoScrollWheelMoved _array_element (delegate Custom|Scrolled))))

(event Custom|Button%20Clicked
  (params (Button%20ID :type String) (Hit%20Location :type Vector))
  (CallFunction|Logg Button%20ID))

(event Custom|Scrolled
  (params (Scrolled%20Down :type Boolean))
  (CallFunction|Logg (Utilities|String|ToString(Boolean) Scrolled%20Down)))

(event EventBeginPlay
  (Utilities|FlowControl|Sequence
    (:then_0
      (bind _locations (CallFunction|ButtonTransforms))
      (for (_array_element _array_index) _locations
        (bind _returnvalue (AddComponent|AddChildActorComponent false _array_element))
        (bind _asbp_toggle_button (Utilities|Casting|CastToBP_ToggleButton (Variables|/Script/Engine.ChildActorComponent|GetChildActor _returnvalue)))
        (Default|SetTitleandSize _asbp_toggle_button (Variables|Default|GetButton%20Size) false (CallFunction|TitleforIndex _array_index) (Utilities|String|ToString(Integer) _array_index))
        (Utilities|Array|Add (Variables|Default|GetButtons) _asbp_toggle_button)
        (Variables|/Game/ReusableAssets/Buttons/BP_ToggleButton.BP_ToggleButton_C|SetPush%20Button%20Mode _asbp_toggle_button true)))
    (:then_1
      (CallFunction|ListentoButtonEvents))))

(fn ConstructionScript)

(fn ButtonTransforms
  (Utilities|FlowControl|Sequence
    (:then_0
      (for _array_element (CallFunction|PositionsinGrid 9 3 1.0 (Variables|Default|GetButton%20Size) true)
        (Utilities|Array|Add (LocalVariables|GetResult) (Math|Transform|MakeTransform _array_element))))
    (:then_2
      (return (LocalVariables|GetResult)))))

(fn TitleforIndex
  (params (Index :type Integer))
  (Utilities|FlowControl|Sequence
    (:then_0
      (switch int Index
        (:0
          (LocalVariables|SetResult "-"))
        (:1
          (LocalVariables|SetResult "^"))
        (:2
          (LocalVariables|SetResult "-"))
        (:3
          (LocalVariables|SetResult "<"))
        (:4
          (LocalVariables|SetResult "+"))
        (:5
          (LocalVariables|SetResult ">"))
        (:6
          (LocalVariables|SetResult "-"))
        (:7
          (LocalVariables|SetResult "v"))
        (:8
          (LocalVariables|SetResult "-"))))
    (:then_1
      (return (LocalVariables|GetResult)))))