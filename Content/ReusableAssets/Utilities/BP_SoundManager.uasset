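; BP_SoundManager is a reusable utility that plays keyboard click sounds by sound ID.
; PlaySound selects a sound and volume for the ID, then spawns it attached to a given component with attenuation.
; ShouldPlaySound gates playback, setting its result to false for both click types when a boolean preference is on.
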(fn ConstructionScript)

(fn PlaySound
  (params (Sound%20ID :type E_SoundIDs%20Enum) (Component :type Scene%20Component%20Object%20Reference))
  (if (CallFunction|ShouldPlaySound Sound%20ID)
    (Utilities|FlowControl|Sequence
      (:then_0
        (switch Utilities|FlowControl|Switch|SwitchonE_SoundIDs Sound%20ID
          (:NewEnumerator0
            (LocalVariables|SetSound "/Game/UniversalSoundFX/Sound_Effects/USER_INTERFACES/Clicks_and_Taps/UI_Click_Aftertap_mono.UI_Click_Aftertap_mono")
            (LocalVariables|SetVolume 0.5))
          (:NewEnumerator1
            (LocalVariables|SetSound "/Game/UniversalSoundFX/Sound_Effects/USER_INTERFACES/Clicks_and_Taps/UI_Click_Distinct_mono.UI_Click_Distinct_mono")
            (LocalVariables|SetVolume 0.2))))
      (:then_2
        (Audio|SpawnSoundAttached (LocalVariables|GetSound) Component "None" "0, 0, 0" "0, 0, 0" "KeepRelativeOffset" false (LocalVariables|GetVolume) (LocalVariables|GetPitch) 0.0 "/Game/Attenuation/Normal.Normal")))))

(fn ShouldPlaySound
  (params (Sound%20ID :type E_SoundIDs%20Enum))
  (Utilities|FlowControl|Sequence
    (:then_0
      (switch Utilities|FlowControl|Switch|SwitchonE_SoundIDs Sound%20ID
        (:NewEnumerator0
          _)
        (:NewEnumerator1
          _))
      (Utilities|BoolPref "NewEnumerator2"
        (:True
          (LocalVariables|SetB%20Result false))))
    (:then_1
      (return (LocalVariables|GetB%20Result)))))