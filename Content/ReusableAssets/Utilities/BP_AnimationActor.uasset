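; Short-lived helper actor that tweens a target actor's location, rotation and scale after an optional delay.
; Animate unpacks a params struct and drives a shared step function from either a bounce or generic curve timeline at a set play rate, playing an attached sound once near the end.
; On finish it optionally destroys the target, notifies its parent runner and destroys itself.
; A separate event bounces an actor out by an offset, then destroys both.
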(event `Animate`
  (params (Params :type "/Game/ReusableAssets/Utilities/S_AnimationParams Structure") (`Parent Runner` :type "/Game/ReusableAssets/Utilities/BP_AnimationRunner Object Reference"))
  (bind (_actor _move _startlocation _endlocation _relativelocations _rotate _startrotation _endrotation _startscale _bounce _sound _animationrate _startdelay _destroyactor) (break `/Game/ReusableAssets/Utilities/S_AnimationParams` Params))
  (set `self.Parent Runner` `Parent Runner`)
  (`KismetSystemLibrary.Delay` _startdelay)
  (`self.Animate To Location` _actor _startlocation _endlocation _sound _animationrate _bounce _destroyactor _relativelocations _startscale _startrotation _endrotation _rotate _move))

(event `Animate Out and Destroy`
  (params (Actor :type "Actor Object Reference") (Offset :type "Vector Structure" :default (0.0 0.0 0.0)))
  (`|ExecutionSequence`
    (:`then_0`
      (bind _output_get (set `self.Start Location` (`self.K2_GetActorLocation` Actor)))
      (set `self.End Location` (+ _output_get Offset)))
    (:`then_1`
      (bind (_direction _alpha) (`Timeline|BounceOut` :!via `PlayFromStart`)
        (:`Update`
          (`self.K2_SetActorLocation` Actor (`KismetMathLibrary.VLerp` (`self.Start Location`) (`self.End Location`) _alpha) false))
        (:`Finished`
          (`self.K2_DestroyActor` Actor)
          (`self.K2_DestroyActor`))))))

(event `Animate To Location`
  (params (Actor :type "Actor Object Reference") (`Start Location` :type "Vector Structure") (`End Location` :type "Vector Structure") (Sound :type "SoundBase Object Reference") (`Animation Rate` :type "Float (double-precision)") (Bounce :type Boolean) (`Destroy Actor` :type Boolean) (`Relative Locations` :type Boolean) (`Start Scale` :type "Float (double-precision)") (`Start Rotation` :type "Rotator Structure") (`End Rotation` :type "Rotator Structure") (Rotate :type Boolean) (Move :type Boolean))
  (if Bounce
    (`TimelineComponent.SetPlayRate` (`self.Bounce Timeline`) `Animation Rate`)
    (bind (_direction _c_bounceanimationcurve) (`Timeline|Bounce Timeline` :!via `PlayFromStart`)
      (:`Update`
        (`self.Private Animation Step` Actor _c_bounceanimationcurve Move `Start Location` `End Location` `Relative Locations` Sound `Start Scale` Rotate `Start Rotation` `End Rotation`))
      (:`Finished`
        (`|ExecutionSequence` :!label _label
          (:`then_0`
            (if `Destroy Actor`
              (`self.K2_DestroyActor` Actor)))
          (:`then_1`
            (`/Game/ReusableAssets/Utilities/BP_AnimationRunner.Animation Actor Finished` (`self.Parent Runner`)))
          (:`then_2`
            (`self.K2_DestroyActor`)))))
    (else
      (`TimelineComponent.SetPlayRate` (`self.Animation Timeline`) `Animation Rate`)
      (bind (_direction_2 _c_genericcurve) (`Timeline|Animation Timeline` :!via `PlayFromStart`)
        (:`Update`
          (`self.Private Animation Step` Actor _c_genericcurve Move `Start Location` `End Location` `Relative Locations` Sound `Start Scale` Rotate `Start Rotation` `End Rotation`))
        (:`Finished`
          (goto _label))))))

(event `Private Animation Step`
  (params (Actor :type "Actor Object Reference") (alpha :type "Float (double-precision)") (Move :type Boolean) (`Start Location` :type "Vector Structure") (`End Location` :type "Vector Structure") (`Relative Locations` :type Boolean) (Sound :type "SoundBase Object Reference") (`Start Scale` :type "Float (double-precision)") (Rotate :type Boolean) (`Start Rotation` :type "Rotator Structure") (`End Rotation` :type "Rotator Structure"))
  (bind _returnvalue (`KismetMathLibrary.VLerp` `Start Location` `End Location` alpha))
  ;[1 1 1] Destroyed already?
  (if (!= Actor null)
    (`|ExecutionSequence`
      (:`then_0`
        (if Move
          (if `Relative Locations`
            (`self.K2_SetActorRelativeLocation` Actor _returnvalue false)
            (else
              (`self.K2_SetActorLocation` Actor _returnvalue false)))))
      (:`then_1`
        (if (!= `Start Scale` 1.0)
          (`self.SetActorRelativeScale3D` Actor (`KismetMathLibrary.Conv_DoubleToVector` (`KismetMathLibrary.Lerp` `Start Scale` 1.0 alpha)))))
      (:`then_2`
        (if Rotate
          (`self.K2_SetActorRelativeRotation` Actor (`KismetMathLibrary.RLerp` `Start Rotation` `End Rotation` alpha) false)))
      (:`then_3`
        ;[1 1 1] Play Sound near end
        (if (!= Sound null)
          (if (> alpha 0.9)
            (`/Engine/EditorBlueprintResources/StandardMacros.DoOnce` false
              (:`Completed`
                (`GameplayStatics.PlaySoundAttached` Sound (`self.K2_GetRootComponent` Actor))))))))
    (else
      (`self.K2_DestroyActor`))))

(fn `UserConstructionScript`)