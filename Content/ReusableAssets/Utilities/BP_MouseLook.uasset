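; Reusable mouse look actor that either passes Turn and LookUp input straight to the player or runs a toggleable lagged aim mode.
; With lag on, input moves a separate MouseRotation, and Tick eases control rotation toward it once it leaves a degree dead zone.
; GetMouseLookRotation returns that aim, or the camera rotation when lag is off.
; In both modes, threshold-based detection signals horizontal and vertical mouse direction changes.
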(event Custom|RotateOnTick
  (params (Delta%20Seconds :type Float%20%28single-precision%29))
  (bind _returnvalue (Game|GetPlayerController 0))
  (bind _returnvalue_2 (Pawn|GetControlRotation _returnvalue :!class /Script/Engine.Controller))
  (if (Variables|Default|GetRotate%20On%20Tick)
    (if (Math|Rotator|Equal(Rotator) (Variables|Default|GetTarget%20Rotation) _returnvalue_2 0.0001)
      (Variables|Default|SetRotate%20On%20Tick false)
      (else
        (Pawn|SetControlRotation (Game|GetPlayerController 0) (Math|Interpolation|RInterpTo _returnvalue_2 (Variables|Default|GetTarget%20Rotation) Delta%20Seconds 2.0))))))

(event EventBeginPlay
  (Utilities|FlowControl|Sequence
    (:then_0
      (Variables|Default|SetMouse%20Rotation (Pawn|GetControlRotation (Game|GetPlayerController 0) :!class /Script/Engine.Controller)))
    (:then_1
      (Input|EnableInput (Game|GetPlayerController 0)))))

(event EventTick
  (params (DeltaSeconds :type Float%20%28single-precision%29))
  (if (Variables|Default|GetMouse%20Lag%20Flag)
    (Utilities|FlowControl|Sequence
      (:then_0
        (if (CallFunction|ShouldRotatetoCrosshair)
          (Variables|Default|SetTarget%20Rotation (Variables|Default|GetMouse%20Rotation))
          (Variables|Default|SetRotate%20On%20Tick true)))
      (:then_1
        (CallFunction|RotateonTick DeltaSeconds)))
    (else
      (CallFunction|Logg "Tick should be disabled"))))

(event Input|AxisEvents|InputAxisTurn
  (params (AxisValue :type Float%20%28single-precision%29))
  (CallFunction|DetectDirectionChange false AxisValue)
  (if (!= AxisValue 0.0)
    (if (Variables|Default|GetMouse%20Lag%20Flag)
      (Variables|Default|SetMouse%20Rotation (Math|Rotator|MakeRotator 0.0 (.pitch (Math|Rotator|CombineRotators (Math|Rotator|MakeRotator 0.0 0.0 (* AxisValue 3.0)) (Variables|Default|GetMouse%20Rotation))) (.yaw (Math|Rotator|CombineRotators (Math|Rotator|MakeRotator 0.0 0.0 (* AxisValue 3.0)) (Variables|Default|GetMouse%20Rotation)))))
      (elif (!= AxisValue 0.0)
        (Pawn|Input|AddControllerYawInput (Game|Player|GetPlayerPawn 0) AxisValue)))))

(event Input|AxisEvents|InputAxisLookUp
  (params (AxisValue :type Float%20%28single-precision%29))
  (CallFunction|DetectDirectionChange true AxisValue)
  (if (!= AxisValue 0.0)
    (if (Variables|Default|GetMouse%20Lag%20Flag)
      (Variables|Default|SetMouse%20Rotation (Math|Rotator|MakeRotator 0.0 (.pitch (Math|Rotator|CombineRotators (Math|Rotator|MakeRotator 0.0 (* AxisValue -3.0) 0.0) (Variables|Default|GetMouse%20Rotation))) (.yaw (Math|Rotator|CombineRotators (Math|Rotator|MakeRotator 0.0 (* AxisValue -3.0) 0.0) (Variables|Default|GetMouse%20Rotation)))))
      (elif (!= AxisValue 0.0)
        (Pawn|Input|AddControllerPitchInput (Game|Player|GetPlayerPawn 0) AxisValue)))))

(fn ConstructionScript)

(fn GetMouseLookRotation
  (Utilities|FlowControl|Sequence
    (:then_0
      (if (Variables|Default|GetMouse%20Lag%20Flag)
        (LocalVariables|SetResult (Variables|Default|GetMouse%20Rotation))
        (else
          (LocalVariables|SetResult (Camera|GetCameraRotation (Game|GetPlayerCameraManager 0))))))
    (:then_1
      (return (LocalVariables|GetResult)))))

(fn ShouldRotatetoCrosshair
  (bind _degrees_til_scroll (Variables|Default|GetDegrees%20Til%20Scroll))
  (Utilities|FlowControl|Sequence
    (:then_0
      (if (Variables|Default|GetRotate%20On%20Tick)
        (LocalVariables|SetLocal%20Rotation (Variables|Default|GetTarget%20Rotation))
        (else
          (LocalVariables|SetLocal%20Rotation (Pawn|GetControlRotation (Game|GetPlayerController 0) :!class /Script/Engine.Controller)))))
    (:then_1
      (if (or (> (Math|Float|Absolute(Float) (.pitch (Math|Rotator|Delta(Rotator) (Variables|Default|GetMouse%20Rotation) (LocalVariables|GetLocal%20Rotation)))) _degrees_til_scroll) (> (Math|Float|Absolute(Float) (.yaw (Math|Rotator|Delta(Rotator) (Variables|Default|GetMouse%20Rotation) (LocalVariables|GetLocal%20Rotation)))) _degrees_til_scroll))
        (LocalVariables|SetResult true)))
    (:then_2
      (return (LocalVariables|GetResult)))))

(fn DetectDirectionChange
  (params (Vertical :type Boolean) (Axis%20Value :type Float%20%28single-precision%29))
  (if Vertical
    (if (>= (Math|Float|Absolute(Float) Axis%20Value) (Variables|Default|GetTrigger%20Threshold))
      (if (< Axis%20Value 0.0)
        (LocalVariables|SetNew%20Value -1.0)
        (else
          (LocalVariables|SetNew%20Value 1.0)))
      (if (!= (Variables|Default|GetPrevious%20Vertical%20Value) (LocalVariables|GetNew%20Value))
        (Default|CallMouseDirectionChangedVertical (> (LocalVariables|GetNew%20Value) 0.0))
        (Variables|Default|SetPrevious%20Vertical%20Value (LocalVariables|GetNew%20Value)))
      (else
        (Variables|Default|SetPrevious%20Vertical%20Value 0.0)))
    (elif (>= (Math|Float|Absolute(Float) Axis%20Value) (Variables|Default|GetTrigger%20Threshold))
      (if (< Axis%20Value 0.0)
        (LocalVariables|SetNew%20Value -1.0)
        (else
          (LocalVariables|SetNew%20Value 1.0)))
      (if (!= (Variables|Default|GetPrevious%20Horizontal%20Value) (LocalVariables|GetNew%20Value))
        (Default|CallMouseDirectionChangedHorizontal (< (LocalVariables|GetNew%20Value) 0.0))
        (Variables|Default|SetPrevious%20Horizontal%20Value (LocalVariables|GetNew%20Value)))
      (else
        (Variables|Default|SetPrevious%20Horizontal%20Value 0.0)))))

(fn EnableMouseLag
  (params (Enable :type Boolean))
  (bind _output_get (Variables|Default|SetMouse%20Lag%20Flag Enable))
  (Actor|Tick|SetActorTickEnabled _output_get))