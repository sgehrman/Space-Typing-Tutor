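; Disposable utility actor that animates a queue of actors between locations one after another, then destroys itself.
; Each step waits its delay, then plays a generic or bounce timeline to lerp world or relative location, optionally destroying the animated actor afterward.
; Non-unit start scales lerp to one, with an attached sound played once per runner near completion.
; A separate event bounces an actor out by an offset, destroying both.
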(event `Animate`
  (params (Params :type "Array of /Game/ReusableAssets/Utilities/S_AnimationParams Structure"))
  (bind _output_get (set `self.Param Array` Params))
  (`self.Private Animate Next` (`KismetArrayLibrary.Array_Get` _output_get)))

(event `Private Animate Next`
  (params (Params :type "/Game/ReusableAssets/Utilities/S_AnimationParams Structure"))
  (bind (_actor _startlocation _endlocation _relativelocations _startscale _bounce _sound _animationrate _startdelay _destroyactor) (break `/Game/ReusableAssets/Utilities/S_AnimationParams` Params))
  (`KismetSystemLibrary.Delay` _startdelay)
  (`self.Animate To Location` _actor _startlocation _endlocation _sound _animationrate _bounce _destroyactor _relativelocations _startscale))

(event `Animate Out and Destroy`
  (params (Actor :type "Actor Object Reference") (Offset :type "Vector Structure" :default (0.0 0.0 0.0)))
  (`|ExecutionSequence`
    (:`then_0`
      (bind _output_get (set `self.Start Location` (`self.K2_GetActorLocation` Actor)))
      (set `self.End Location` (+ _output_get Offset)))
    (:`then_1`
      (bind (_direction _alpha) (`Timeline|BounceOut` :!via `PlayFromStart`)
        (:`Update`
          (`self.K2_SetActorLocation` Actor (`KismetMathLibrary.VLerp` (`self.Start Location`) (`self.End Location`) _alpha) false))
        (:`Finished`
          (`self.K2_DestroyActor` Actor)
          (`self.K2_DestroyActor`))))))

(event `Animate To Location`
  (params (Actor :type "Actor Object Reference") (`Start Location` :type "Vector Structure") (`End Location` :type "Vector Structure") (Sound :type "SoundBase Object Reference") (`Animation Rate` :type "Float (double-precision)") (Bounce :type Boolean) (`Destroy Actor` :type Boolean) (`Relative Locations` :type Boolean) (`Start Scale` :type "Float (double-precision)"))
  (if Bounce
    (`TimelineComponent.SetPlayRate` (`self.Bounce Timeline`) `Animation Rate`)
    (bind (_direction _c_bounceanimationcurve) (`Timeline|Bounce Timeline` :!via `PlayFromStart`)
      (:`Update`
        (`self.Private Animation Step` Actor _c_bounceanimationcurve `Start Location` `End Location` Sound `Relative Locations` `Start Scale`))
      (:`Finished`
        (`|ExecutionSequence` :!label _label
          (:`then_0`
            (if `Destroy Actor`
              (`self.K2_DestroyActor` Actor)))
          (:`then_1`
            (if (!= (`KismetArrayLibrary.Array_Length` (`self.Param Array`)) 0)
              (`KismetArrayLibrary.Array_Remove` (`self.Param Array`))))
          (:`then_2`
            (if (!= (`KismetArrayLibrary.Array_Length` (`self.Param Array`)) 0)
              (`self.Private Animate Next` (`KismetArrayLibrary.Array_Get` (`self.Param Array`)))
              (else
                (`self.K2_DestroyActor`)))))))
    (else
      (`TimelineComponent.SetPlayRate` (`self.Animation Timeline`) `Animation Rate`)
      (bind (_direction_2 _c_genericcurve) (`Timeline|Animation Timeline` :!via `PlayFromStart`)
        (:`Update`
          (`self.Private Animation Step` Actor _c_genericcurve `Start Location` `End Location` Sound `Relative Locations` `Start Scale`))
        (:`Finished`
          (goto _label))))))

(event `Private Animation Step`
  (params (Actor :type "Actor Object Reference") (alpha :type "Float (double-precision)") (`Start Location` :type "Vector Structure") (`End Location` :type "Vector Structure") (Sound :type "SoundBase Object Reference") (`Relative Locations` :type Boolean) (`Start Scale` :type "Float (double-precision)"))
  (bind _returnvalue (`KismetMathLibrary.VLerp` `Start Location` `End Location` alpha))
  (if `Relative Locations`
    (`self.K2_SetActorRelativeLocation` Actor _returnvalue false)
    (else
      (`self.K2_SetActorLocation` Actor _returnvalue false)))
  (if (!= `Start Scale` 1.0)
    (`self.SetActorRelativeScale3D` Actor (`KismetMathLibrary.Conv_DoubleToVector` (`KismetMathLibrary.Lerp` `Start Scale` 1.0 alpha)))
    (if (> alpha 0.9)
      (`/Engine/EditorBlueprintResources/StandardMacros.DoOnce` false
        (:`Completed`
          (`GameplayStatics.PlaySoundAttached` Sound (`self.K2_GetRootComponent` Actor)))))))

(fn `UserConstructionScript`)