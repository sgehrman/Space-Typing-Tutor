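; Actor component that turns its owning actor to track player 0's camera, like a smoothed billboard.
; Each tick it finds the look-at rotation from the camera manager's location to the owner, so forward points away from the camera before RotationOffset is combined in.
; RInterpTo eases the owner's whole rotation toward that target at a fixed speed, with no axis locked.
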(event `self.ReceiveTick`
  (params (DeltaSeconds :type "Float (single-precision)"))
  (bind _returnvalue (`self.GetOwner`))
  (`Actor.SetActorRotation` _returnvalue (`KismetMathLibrary.RInterpTo` (`Actor.K2_GetActorRotation` (`self.GetOwner`)) (`KismetMathLibrary.ComposeRotators` (`KismetMathLibrary.FindLookAtRotation` (`Actor.K2_GetActorLocation` (`GameplayStatics.GetPlayerCameraManager` 0)) (`Actor.K2_GetActorLocation` _returnvalue)) (`self.Rotation Offset`)) DeltaSeconds 5.0)))