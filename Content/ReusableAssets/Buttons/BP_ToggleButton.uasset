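; BP_ToggleButton is a reusable crosshair-operated world button that toggles on and off, or acts momentarily in push-button mode.
; BuildButton creates a procedural box with collision, optionally matching its width to the title text.
; Crosshair hover and click handlers update state and swap between on, off and hover materials, which UpdateMaterials can override.
; State changes and user clicks are broadcast through dispatchers, and downward scrolling simulates a click event without toggling.
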(event `self.ReceiveBeginPlay`)

(event `self.ReceiveActorBeginOverlap`
  (params (OtherActor :type "Actor Object Reference")))

(event `self.ReceiveTick`
  (params (DeltaSeconds :type "Float (single-precision)")))

(fn `Build Button`
  (bind (_button_size_x _button_size_y _button_size_z) (`KismetMathLibrary.BreakVector` (`self.Button Size`)))
  (`|ExecutionSequence`
    (:`then_0`
      (`ActorComponent.K2_DestroyComponent` (`self.Body Mesh`)))
    (:`then_1`
      (`self.Set Font Size` (`self.Font Size`)))
    (:`then_3`
      (if (`self.Match Width to Text`)
        (set `self.Button Size` (`KismetMathLibrary.MakeVector` _button_size_x (.y (`TextRenderComponent.GetTextWorldSize` (`self.Title Component`))) _button_size_z))))
    (:`then_4`
      (bind _returnvalue (`AddComponent|ProceduralMeshComponent_0` :`RelativeTransform` (`/Game/ReusableAssets/Utilities/LIB_Utilities.Trans`)))
      (bind _output_get (set `self.Body Mesh` _returnvalue))
      (`/Game/ReusableAssets/Utilities/LIB_Utilities.Setup Box Mesh` _output_get (`self.Button Size`) null true))
    (:`then_5`
      (`self.Set State` (`self.On State`)))))

(fn `Crosshair Hover Progress`
  (params (Progress :type "Float (double-precision)") (`Local Hit Location` :type "Vector Structure") (`Hit Component` :type "PrimitiveComponent Object Reference"))
  (returns (Success :type Boolean))
  (return false))

(fn `Crosshair Hover Start`
  (params (Finished :type Boolean))
  (returns (Success :type Boolean))
  (`|ExecutionSequence`
    (:`then_1`
      (if Finished
        (set `self.Hover Over` false)
        (else
          (set `self.Hover Over` true))))
    (:`then_2`
      (`self.Update Material`))
    (:`then_4`
      (return true))))

(fn `Crosshair LeftRight`
  (params (Left :type Boolean))
  (returns (Success :type Boolean))
  (return false))

(fn `Crosshair Mouse Click`
  (params (`Mouse Down` :type Boolean) (`Event Type` :type "/Game/ReusableAssets/Utilities/E_EventType Enum" :default "NewEnumerator0") (`Hit Location` :type "Vector Structure") (`Hit Component` :type "PrimitiveComponent Object Reference"))
  (returns (Success :type Boolean))
  (`|ExecutionSequence`
    (:`then_0`
      (if `Mouse Down`
        (`self.Set State` (not (`self.On State`)))
        (elif (`self.Push Button Mode`)
          (`self.Set State` (not (`self.On State`))))))
    (:`then_1`
      (if `Mouse Down`
        (`self.ButtonClickedByUser` (`self.Button ID`) `Hit Location`)))
    (:`then_2`
      (return true))))

(fn `Crosshair Scroll Wheel`
  (params (Down :type Boolean) (`Hit Location` :type "Vector Structure") (`Hit Component` :type "PrimitiveComponent Object Reference"))
  (returns (Success :type Boolean))
  (`|ExecutionSequence`
    (:`then_0`
      (if Down
        (`self.Simulate Click Event`)))
    (:`then_1`
      (return false))))

(fn `Crosshair UpDown`
  (params (Up :type Boolean))
  (returns (Success :type Boolean))
  (return false))

(fn `Get State`
  (returns (State :type Boolean))
  (return (`self.On State`)))

(fn `Get Width`
  (returns (Width :type "Float (double-precision)"))
  (bind (_button_size_x _button_size_y) (`KismetMathLibrary.BreakVector` (`self.Button Size`)))
  (return _button_size_y))

(fn `Set Font Size`
  (params (`Font Size` :type "Float (double-precision)"))
  (set `self.Font Size` `Font Size`)
  (`TextRenderComponent.SetWorldSize` (`self.Title Component`) (`self.Font Size`)))

(fn `Set State`
  (params (`On State` :type Boolean))
  (`|ExecutionSequence`
    (:`then_0`
      (if (!= `On State` (`self.On State`))
        (bind _output_get (set `self.On State` `On State`))
        (`self.State Changed` _output_get)))
    (:`then_1`
      (`self.Update Material`))))

(fn `Set Title and Size`
  (params (`Button Size` :type "Vector Structure") (`Width To Text` :type Boolean) (Title :type String) (`Button ID` :type String))
  (bind _button_size_x (`KismetMathLibrary.BreakVector` (`self.Button Size`)))
  (`|ExecutionSequence`
    (:`then_0`
      (set `self.Button Size` `Button Size`)
      (set `self.Match Width to Text` `Width To Text`)
      (bind _output_get (set `self.Title` Title))
      (`TextRenderComponent.K2_SetText` (`self.Title Component`) (`KismetTextLibrary.Conv_StringToText` _output_get)))
    (:`then_1`
      (set `self.Button ID` `Button ID`))
    (:`then_2`
      (`self.Build Button`))
    (:`then_3`
      (`SceneComponent.K2_SetRelativeLocation` (`self.Title Component`) (`KismetMathLibrary.MakeVector` (- (+ (/ _button_size_x 2.0) 1.0))) false))))

(fn `Simulate Click Event`
  ;[1 1 1] Called from dual buttons scroll wheel event
  (`self.ButtonClickedByUser` (`self.Button ID`)))

(fn `Update Material`
  (bind _body_mesh (`self.Body Mesh`))
  (if (`self.Hover Over`)
    (`PrimitiveComponent.SetMaterial` _body_mesh 0 (`self.MID Hover`))
    (elif (`self.On State`)
      (`PrimitiveComponent.SetMaterial` _body_mesh 0 (`self.MID On`))
      (else
        (`PrimitiveComponent.SetMaterial` _body_mesh 0 (`self.MID Off`))))))

(fn `Update Materials`
  (params (`On Material` :type "MaterialInterface Object Reference") (`Off Material` :type "MaterialInterface Object Reference") (`Hover Material` :type "MaterialInterface Object Reference"))
  (`|ExecutionSequence`
    (:`then_0`
      (if (!= `On Material` null)
        (set `self.MID On` `On Material`)))
    (:`then_1`
      (if (!= `Off Material` null)
        (set `self.MID Off` `Off Material`)))
    (:`then_2`
      (if (!= `Hover Material` null)
        (set `self.MID Hover` `Hover Material`)))
    (:`then_3`
      (`self.Update Material`))))

(fn `UserConstructionScript`
  (`|ExecutionSequence`
    (:`then_0`
      (bind _returnvalue (`KismetMaterialLibrary.CreateDynamicMaterialInstance` "/Game/ReusableAssets/Materials/MT_Opaque.MT_Opaque"))
      (set `self.MID On` _returnvalue)
      (`MaterialInstanceDynamic.SetScalarParameterValue` _returnvalue "Emission" 22.0))
    (:`then_1`
      (bind _returnvalue_2 (`KismetMaterialLibrary.CreateDynamicMaterialInstance` "/Game/ReusableAssets/Materials/MT_Opaque.MT_Opaque"))
      (set `self.MID Off` _returnvalue_2)
      (`MaterialInstanceDynamic.SetVectorParameterValue` _returnvalue_2 "Color" (struct :`R` 0.053081 :`G` 0.366474 :`B` 0.64 :`A` 1.0)))
    (:`then_2`
      (bind _returnvalue_3 (`KismetMaterialLibrary.CreateDynamicMaterialInstance` "/Game/ReusableAssets/Materials/MT_Opaque.MT_Opaque"))
      (set `self.MID Hover` _returnvalue_3)
      (`MaterialInstanceDynamic.SetScalarParameterValue` _returnvalue_3 "Emission" 5.0))
    (:`then_4`
      (`self.Build Button`))))