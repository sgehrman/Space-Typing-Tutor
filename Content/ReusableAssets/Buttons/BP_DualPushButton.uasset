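; BP_DualPushButton is a numeric stepper control with title and value text, built from two child BP_ToggleButton actors.
; Right raises and left lowers the clamped value by Increment, despite handlers named Minus and Plus respectively, then updates the text and fires DualButtonClicked.
; Crosshair scroll-wheel input simulates clicks on those buttons.
; The construction script initializes buttons and labels and generates a procedural box mesh with collision.
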(event `self.ReceiveBeginPlay`
  (`|ExecutionSequence`
    (:`then_0`
      (bind _asbp_toggle_button (cast `/Game/ReusableAssets/Buttons/BP_ToggleButton` (`ChildActorComponent.ChildActor` (`self.Right Button`))))
      (add `/Game/ReusableAssets/Buttons/BP_ToggleButton.ButtonClickedByUser` _asbp_toggle_button (delegate `MinusButtonClicked`)))
    (:`then_1`
      (bind _asbp_toggle_button_2 (cast `/Game/ReusableAssets/Buttons/BP_ToggleButton` (`ChildActorComponent.ChildActor` (`self.Left Button`))))
      (add `/Game/ReusableAssets/Buttons/BP_ToggleButton.ButtonClickedByUser` _asbp_toggle_button_2 (delegate `PlusButtonClicked`)))))

(event `MinusButtonClicked`
  (params (`Button ID` :type String) (`Hit Location` :type "Vector Structure"))
  (set `self.Value` (`KismetMathLibrary.FClamp` (+ (`self.Value`) (`self.Increment`)) (`self.Min Value`) (`self.Max Value`)))
  (`self.Update Value Text` :!label _label)
  (`self.DualButtonClicked`))

(event `PlusButtonClicked`
  (params (`Button ID` :type String) (`Hit Location` :type "Vector Structure"))
  (set `self.Value` (`KismetMathLibrary.FClamp` (- (`self.Value`) (`self.Increment`)) (`self.Min Value`) (`self.Max Value`)))
  (goto _label))

(fn `Crosshair Hover Moved`
  (params (`Hit Location` :type "Vector Structure"))
  (returns (Success :type Boolean))
  (return false))

(fn `Crosshair Hover Progress`
  (params (Progress :type "Float (double-precision)") (`Local Hit Location` :type "Vector Structure") (`Hit Component` :type "PrimitiveComponent Object Reference"))
  (returns (`Auto Click On Progress` :type Boolean))
  (return false))

(fn `Crosshair Hover Start`
  (params (Finished :type Boolean))
  (returns (Success :type Boolean))
  (return false))

(fn `Crosshair LeftRight`
  (params (Left :type Boolean))
  (returns (Success :type Boolean))
  (return false))

(fn `Crosshair Mouse Click`
  (params (`Mouse Down` :type Boolean) (`Event Type` :type "/Game/ReusableAssets/Utilities/E_EventType Enum" :default "NewEnumerator0") (`Hit Location` :type "Vector Structure") (`Hit Component` :type "PrimitiveComponent Object Reference"))
  (returns (Success :type Boolean))
  (return false))

(fn `Crosshair Scroll Wheel`
  (params (Down :type Boolean) (`Hit Location` :type "Vector Structure") (`Hit Component` :type "PrimitiveComponent Object Reference"))
  (returns (Success :type Boolean))
  (`|ExecutionSequence`
    (:`then_0`
      (if Down
        (bind _asbp_toggle_button (cast `/Game/ReusableAssets/Buttons/BP_ToggleButton` (`ChildActorComponent.ChildActor` (`self.Left Button`))))
        (`/Game/ReusableAssets/Buttons/BP_ToggleButton.Simulate Click Event` _asbp_toggle_button)
        (else
          (bind _asbp_toggle_button_2 (cast `/Game/ReusableAssets/Buttons/BP_ToggleButton` (`ChildActorComponent.ChildActor` (`self.Right Button`))))
          (`/Game/ReusableAssets/Buttons/BP_ToggleButton.Simulate Click Event` _asbp_toggle_button_2))))
    (:`then_1`
      (return true))))

(fn `Crosshair UpDown`
  (params (Up :type Boolean))
  (returns (Success :type Boolean))
  (return false))

(fn `Get Value`
  (returns (Value :type "Float (double-precision)"))
  (return (`self.Value`)))

(fn `Update Value Text`
  (`|ExecutionSequence`
    (:`then_0`
      (`TextRenderComponent.K2_SetText` (`self.ValueText`) (`KismetTextLibrary.Conv_DoubleToText` (`self.Value`) "HalfToEven")))
    (:`then_1`
      (return))))

(fn `UserConstructionScript`
  (bind _font_size (`self.Font Size`))
  (`|ExecutionSequence`
    (:`then_0`
      (bind _asbp_toggle_button (cast `/Game/ReusableAssets/Buttons/BP_ToggleButton` (`ChildActorComponent.ChildActor` (`self.Right Button`))))
      (`/Game/ReusableAssets/Buttons/BP_ToggleButton.Set State` _asbp_toggle_button false))
    (:`then_1`
      (bind _asbp_toggle_button_2 (cast `/Game/ReusableAssets/Buttons/BP_ToggleButton` (`ChildActorComponent.ChildActor` (`self.Left Button`))))
      (`/Game/ReusableAssets/Buttons/BP_ToggleButton.Set State` _asbp_toggle_button_2 false))
    (:`then_2`
      (`TextRenderComponent.K2_SetText` (`self.TitleText`) (`KismetTextLibrary.Conv_StringToText` (`self.Title`))))
    (:`then_3`
      (`self.Update Value Text`))
    (:`then_4`
      (bind _asbp_toggle_button_3 (cast `/Game/ReusableAssets/Buttons/BP_ToggleButton` (`ChildActorComponent.ChildActor` (`self.Left Button`))))
      (`/Game/ReusableAssets/Buttons/BP_ToggleButton.Set Font Size` _asbp_toggle_button_3 _font_size))
    (:`then_5`
      (bind _asbp_toggle_button_4 (cast `/Game/ReusableAssets/Buttons/BP_ToggleButton` (`ChildActorComponent.ChildActor` (`self.Right Button`))))
      (`/Game/ReusableAssets/Buttons/BP_ToggleButton.Set Font Size` _asbp_toggle_button_4 _font_size))
    (:`then_6`
      (bind _returnvalue (`AddComponent|ProceduralMeshComponent_6` :`RelativeTransform` (`KismetMathLibrary.MakeTransform` (0.0 0.0 0.0) (struct) (1.0 1.0 1.0))))
      (bind (_vertices _triangles _normals _uvs _tangents) (`KismetProceduralMeshLibrary.GenerateBoxMesh` (/ (`KismetMathLibrary.MakeVector` 33.0 100.0 100.0) 2.0)))
      (`ProceduralMeshComponent.CreateMeshSection` :`self` _returnvalue :`Vertices` _vertices :`Triangles` _triangles :`Normals` _normals :`UV0` _uvs :`Tangents` _tangents :`bCreateCollision` true)
      (`PrimitiveComponent.SetCollisionEnabled` _returnvalue "QueryAndPhysics")
      (`PrimitiveComponent.SetMaterial` _returnvalue 0 "/Game/ReusableAssets/Materials/MT_Opaque.MT_Opaque"))))