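; Reusable in-world checkbox with a title, toggled and hovered through crosshair interaction events.
; Construction builds inner and outer procedural box meshes; BeginPlay creates dynamic materials and a translucent background sized from the title bounds.
; Mouse down flips OnState, which swaps the inner box material, while hover changes the background opacity by swapping materials.
; Setup sets title and state, then rebuilds the background.
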(event EventBeginPlay
  (CallFunction|BuildMaterials)
  (CallFunction|BuildBackground)
  (CallFunction|SynctoState))

(fn ConstructionScript
  (CallFunction|BuildButton))

(fn BuildBackground
  (bind _title (Variables|Default|GetTitle))
  (bind _boxextent (Collision|GetComponentBounds _title))
  (bind _returnvalue (* _boxextent 2.0))
  (bind (_x _y _z) (Math|Vector|BreakVector _returnvalue))
  (Utilities|FlowControl|Sequence
    (:then_0
      (if (!= (Variables|Default|GetButton%20Backgound) 0)
        (Components|DestroyComponent (Variables|Default|GetButton%20Backgound))))
    (:then_1
      (LocalVariables|SetBackground%20Size (Math|Vector|MakeVector _x (+ (+ _y (.Y (Math|Vector|BreakVector (Variables|Default|GetButton%20Size)))) 22.0) _z)))
    (:then_2
      (bind _returnvalue_2 (AddComponent|AddProceduralMeshComponent false (Math|Transform|MakeTransform (Math|Vector|MakeVector 2.0 (+ (.Y (Math|Vector|BreakVector (/ (LocalVariables|GetBackground%20Size) 2.0))) -14.0) 0.0))))
      (bind _output_get (Variables|Default|SetButton%20Backgound _returnvalue_2))
      (CallFunction|SetupBoxMesh _output_get (LocalVariables|GetBackground%20Size) (Variables|Default|GetMID%20Background%20Normal) true))))

(fn SetState
  (params (On%20State :type Boolean))
  (Variables|Default|SetOn%20State On%20State)
  (CallFunction|SynctoState))

(fn SynctoState
  (if (Variables|Default|GetOn%20State)
    (Rendering|Material|SetMaterial (Variables|Default|GetInnerMesh) 0 (Variables|Default|GetMID%20On))
    (else
      (Rendering|Material|SetMaterial (Variables|Default|GetInnerMesh) 0 (Variables|Default|GetMID%20Off)))))

(fn GetState
  (return (Variables|Default|GetOn%20State)))

(fn BuildMaterials
  (Utilities|FlowControl|Sequence
    (:then_0
      (bind _returnvalue (Rendering|Material|CreateDynamicMaterialInstance "/Game/ReusableAssets/Materials/MT_Opaque.MT_Opaque" :!class /Script/Engine.KismetMaterialLibrary))
      (bind _output_get (Variables|Default|SetMID%20On _returnvalue))
      (Rendering|Material|SetVectorParameterValue _output_get "Color" "(R=0.007179,G=0.121279,B=0.350000,A=1.000000)" :!class /Script/Engine.MaterialInstanceDynamic))
    (:then_1
      (bind _returnvalue_2 (Rendering|Material|CreateDynamicMaterialInstance "/Game/ReusableAssets/Materials/MT_Opaque.MT_Opaque" :!class /Script/Engine.KismetMaterialLibrary))
      (bind _output_get_2 (Variables|Default|SetMID%20Off _returnvalue_2))
      (Rendering|Material|SetVectorParameterValue _output_get_2 "Color" "(R=0.615000,G=0.615000,B=0.615000,A=1.000000)" :!class /Script/Engine.MaterialInstanceDynamic))
    (:then_2
      (bind _returnvalue_3 (Rendering|Material|CreateDynamicMaterialInstance "/Game/ReusableAssets/Materials/MT_Opaque.MT_Opaque" :!class /Script/Engine.KismetMaterialLibrary))
      (bind _output_get_3 (Variables|Default|SetMID%20Outer _returnvalue_3))
      (Rendering|Material|SetVectorParameterValue _output_get_3 "Color" "(R=1.000000,G=1.000000,B=1.000000,A=1.000000)" :!class /Script/Engine.MaterialInstanceDynamic))
    (:then_3
      (bind _returnvalue_4 (Rendering|Material|CreateDynamicMaterialInstance "/Game/ReusableAssets/Materials/MT_Transparent.MT_Transparent" :!class /Script/Engine.KismetMaterialLibrary))
      (bind _output_get_4 (Variables|Default|SetMID%20Background%20Hover _returnvalue_4))
      (Rendering|Material|SetVectorParameterValue _output_get_4 "Color" (Variables|Default|GetBackground%20Color) :!class /Script/Engine.MaterialInstanceDynamic)
      (Rendering|Material|SetScalarParameterValue _output_get_4 "Opacity" 0.4 :!class /Script/Engine.MaterialInstanceDynamic))
    (:then_4
      (bind _returnvalue_5 (Rendering|Material|CreateDynamicMaterialInstance "/Game/ReusableAssets/Materials/MT_Transparent.MT_Transparent" :!class /Script/Engine.KismetMaterialLibrary))
      (bind _output_get_5 (Variables|Default|SetMID%20Background%20Normal _returnvalue_5))
      (Rendering|Material|SetVectorParameterValue _output_get_5 "Color" (Variables|Default|GetBackground%20Color) :!class /Script/Engine.MaterialInstanceDynamic)
      (Rendering|Material|SetScalarParameterValue _output_get_5 "Opacity" 0.1 :!class /Script/Engine.MaterialInstanceDynamic))))

(fn Setup
  (params (Title :type Text) (On%20State :type Boolean))
  (Utilities|FlowControl|Sequence
    (:then_0
      (Rendering|Components|TextRender|SetText (Variables|Default|GetTitle) Title))
    (:then_1
      (CallFunction|SetState On%20State))
    (:then_2
      (CallFunction|BuildBackground)
      (CallFunction|SynctoState))))

(fn BuildButton
  (Utilities|FlowControl|Sequence
    (:then_1
      (bind _returnvalue (AddComponent|AddProceduralMeshComponent false (Math|Transform|MakeTransform (Math|Vector|MakeVector -2.0 0.0 0.0))))
      (bind _output_get (Variables|Default|SetInnerMesh _returnvalue))
      (CallFunction|SetupBoxMesh _output_get (Variables|Default|GetInner%20Button%20Size) (Variables|Default|GetMID%20Off) true))
    (:then_2
      (bind _returnvalue_2 (AddComponent|AddProceduralMeshComponent false))
      (bind _output_get_2 (Variables|Default|SetOuterMesh _returnvalue_2))
      (CallFunction|SetupBoxMesh _output_get_2 (Variables|Default|GetButton%20Size) (Variables|Default|GetMID%20Outer) true))))

(fn CrosshairHoverMoved
  (params (Hit%20Location :type Vector :default "0, 0, 0"))
  (return false))

(fn CrosshairHoverProgress
  (params (Progress :type Float%20%28single-precision%29) (Local%20Hit%20Location :type Vector :default "0, 0, 0") (Hit%20Component :type Primitive%20Component%20Object%20Reference))
  (return false))

(fn CrosshairHoverStart
  (params (Finished :type Boolean))
  (Utilities|FlowControl|Sequence
    (:then_0
      (if Finished
        (Rendering|Material|SetMaterial (Variables|Default|GetButton%20Backgound) 0 (Variables|Default|GetMID%20Background%20Normal))
        (else
          (Rendering|Material|SetMaterial (Variables|Default|GetButton%20Backgound) 0 (Variables|Default|GetMID%20Background%20Hover)))))
    (:then_2
      (return false))))

(fn CrosshairLeftRight
  (params (Left :type Boolean))
  (return false))

(fn CrosshairMouseClick
  (params (Mouse%20Down :type Boolean) (Event%20Type :type E_EventType%20Enum :default "NewEnumerator10") (Hit%20Location :type Vector :default "0, 0, 0") (Hit%20Component :type Primitive%20Component%20Object%20Reference))
  (Utilities|FlowControl|Sequence
    (:then_0
      (if Mouse%20Down
        (CallFunction|SetState (not (Variables|Default|GetOn%20State)))))
    (:then_3
      (return false))))

(fn CrosshairScrollWheel
  (params (Down :type Boolean) (Hit%20Location :type Vector :default "0, 0, 0") (Hit%20Component :type Primitive%20Component%20Object%20Reference))
  (return false))

(fn CrosshairUpDown
  (params (Up :type Boolean))
  (return false))