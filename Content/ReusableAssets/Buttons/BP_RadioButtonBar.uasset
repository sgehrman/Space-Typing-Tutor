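; BP_RadioButtonBar is a reusable radio button bar actor that keeps one option selected at a time.
; CreateButtons spawns BP_ToggleButton child actors in a one-column grid, built from test data at construction or from new data through ReplaceButtons.
; A click runs UpdateMode, which stores the ID, switches on only the matching button, then fires a radio state change notification.
; BeginPlay sets a default selection, binds clicks and adds a face-camera rotator.
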(event Custom|Bind%20Button%20Events
  (for _array_element (Variables|Default|GetButtons)
    (EventDispatchers|BindEventtoButtonClickedbyUser _array_element (delegate Custom|click))))

(event Custom|click
  (params (Button%20ID :type String) (Hit%20Location :type Vector))
  (CallFunction|UpdateMode Button%20ID)
  (Default|CallRadioStateChanged))

(event EventBeginPlay
  (Utilities|FlowControl|Sequence
    (:then_0
      (CallFunction|UpdateMode "2"))
    (:then_1
      (CallFunction|BindButtonEvents))
    (:then_4
      (AddComponent|AddBPFaceCameraRotator))))

(fn ConstructionScript
  (for _index (range 0 3)
    (Utilities|Array|Add (LocalVariables|GetTest%20Data) (Utilities|Struct|MakeS_StringAndToken "Test Button" (Utilities|String|ToString(Integer) _index))))
  (Variables|Default|SetButton%20Structs (LocalVariables|GetTest%20Data))
  (CallFunction|CreateButtons))

(fn CreateButtons
  (Utilities|FlowControl|Sequence
    (:then_0
      (for _array_element (Variables|Default|GetButtons)
        (Actor|DestroyActor _array_element))
      (Utilities|Array|Clear (Variables|Default|GetButtons)))
    (:then_1
      (LocalVariables|SetButton%20Positions (CallFunction|PositionsinGrid (Utilities|Array|Length (Variables|Default|GetButton%20Structs)) 1 6.0 (CallFunction|StandardButtonSize) true)))
    (:then_2
      (for (_array_element_2 _array_index) (Variables|Default|GetButton%20Structs)
        (bind _returnvalue (AddComponent|AddChildActorComponent false (Math|Transform|MakeTransform (Utilities|Array|Get(acopy) (LocalVariables|GetButton%20Positions) _array_index))))
        (bind _asbp_toggle_button (Utilities|Casting|CastToBP_ToggleButton (Variables|/Script/Engine.ChildActorComponent|GetChildActor _returnvalue)))
        (Default|SetTitleandSize _asbp_toggle_button (CallFunction|StandardButtonSize) false (.String (Utilities|Struct|BreakS_StringAndToken _array_element_2)) (.DataToken (Utilities|Struct|BreakS_StringAndToken _array_element_2)))
        (Variables|/Game/ReusableAssets/Buttons/BP_ToggleButton.BP_ToggleButton_C|SetPush%20Button%20Mode _asbp_toggle_button false)
        (Utilities|Array|Add (Variables|Default|GetButtons) _asbp_toggle_button)))))

(fn UpdateMode
  (params (Button%20ID :type String))
  (Utilities|FlowControl|Sequence
    (:then_0
      (Variables|Default|SetMode Button%20ID))
    (:then_1
      (for _array_element (Variables|Default|GetButtons)
        (if (Utilities|Enum|Equal(Enum) (Variables|/Game/ReusableAssets/Buttons/BP_ToggleButton.BP_ToggleButton_C|GetButton%20ID _array_element) Button%20ID)
          (Default|SetState _array_element true)
          (else
            (Default|SetState _array_element false)))))))

(fn ReplaceButtons
  (params (Button%20Structs :type Array%20of%20S%20String%20and%20Token%20Structures) (Default%20Selection :type String))
  (Variables|Default|SetButton%20Structs Button%20Structs)
  (CallFunction|CreateButtons)
  (CallFunction|BindButtonEvents)
  (CallFunction|UpdateMode Default%20Selection))

(fn SetSelection
  (params (Button%20ID :type String))
  (CallFunction|UpdateMode Button%20ID))

(fn GetSelection
  (return (Variables|Default|GetMode)))