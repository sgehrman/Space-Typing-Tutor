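; BP_ButtonBar is a reusable actor that shows a grid of push buttons and reports which one is clicked by ID.
; CreateButtons spawns BP_ToggleButton child actors in push-button mode at computed grid positions, titling each from a string-and-token struct.
; Construction fills the bar with test buttons, and ReplaceButtons rebuilds and rebinds it with new data and columns.
; BeginPlay binds clicks, relayed through ButtonClicked, and adds a face-camera rotator.
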(event Custom|Bind%20Button%20Events
  (for _array_element (Variables|Default|GetButtons)
    (EventDispatchers|BindEventtoButtonClickedbyUser _array_element (delegate Custom|click))))

(event Custom|click
  (params (Button%20ID :type String) (Hit%20Location :type Vector))
  (Default|CallButtonClicked Button%20ID))

(event EventBeginPlay
  (Utilities|FlowControl|Sequence
    (:then_1
      (CallFunction|BindButtonEvents))
    (:then_4
      (AddComponent|AddBPFaceCameraRotator))))

(fn ConstructionScript
  (for _index (range 0 3)
    (Utilities|Array|Add (LocalVariables|GetTest%20Data) (Utilities|Struct|MakeS_StringAndToken "Test Button" (Utilities|String|ToString(Integer) _index))))
  (Variables|Default|SetButton%20Structs (LocalVariables|GetTest%20Data))
  (CallFunction|CreateButtons))

(fn CreateButtons
  (Utilities|FlowControl|Sequence
    (:then_0
      (for _array_element (Variables|Default|GetButtons)
        (Actor|DestroyActor _array_element))
      (Utilities|Array|Clear (Variables|Default|GetButtons)))
    (:then_1
      (LocalVariables|SetButton%20Positions (CallFunction|PositionsinGrid (Utilities|Array|Length (Variables|Default|GetButton%20Structs)) (Variables|Default|GetColumns) (Variables|Default|GetMargin) (CallFunction|StandardButtonSize) true)))
    (:then_2
      (for (_array_element_2 _array_index) (Variables|Default|GetButton%20Structs)
        (bind _returnvalue (AddComponent|AddChildActorComponent false (Math|Transform|MakeTransform (Utilities|Array|Get(acopy) (LocalVariables|GetButton%20Positions) _array_index))))
        (bind _asbp_toggle_button (Utilities|Casting|CastToBP_ToggleButton (Variables|/Script/Engine.ChildActorComponent|GetChildActor _returnvalue)))
        (Default|SetTitleandSize _asbp_toggle_button (CallFunction|StandardButtonSize) false (.String (Utilities|Struct|BreakS_StringAndToken _array_element_2)) (.DataToken (Utilities|Struct|BreakS_StringAndToken _array_element_2)))
        (Variables|/Game/ReusableAssets/Buttons/BP_ToggleButton.BP_ToggleButton_C|SetPush%20Button%20Mode _asbp_toggle_button true)
        (Utilities|Array|Add (Variables|Default|GetButtons) _asbp_toggle_button)))))

(fn ReplaceButtons
  (params (Button%20Structs :type Array%20of%20S%20String%20and%20Token%20Structures) (Columns :type Integer))
  (Utilities|FlowControl|Sequence
    (:then_0
      (Variables|Default|SetColumns Columns))
    (:then_1
      (if (<= (Variables|Default|GetColumns) 0)
        (Variables|Default|SetColumns 1)))
    (:then_2
      (Variables|Default|SetButton%20Structs Button%20Structs)
      (CallFunction|CreateButtons)
      (CallFunction|BindButtonEvents))))