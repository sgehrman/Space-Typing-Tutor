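; BP_CheckboxBar is a reusable bar that stacks BP_Checkbox child actors in a single-column grid.
; Each checkbox takes its title, initial state and ID from an array of structs, which the construction script fills with test entries.
; ReplaceButtons swaps in new data, destroys and rebuilds the checkboxes, then rebinds their events.
; Checkbox state changes are relayed through one ButtonClicked call carrying the ID and state.
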(event Custom|CustomEvent_0
  (params (Button%20ID :type String) (On%20State :type Boolean))
  (Default|CallButtonClicked Button%20ID On%20State))

(event Custom|Bind%20Button%20Events
  (for _array_element (Variables|Default|GetButtons)
    (EventDispatchers|BindEventtoStateChanged _array_element (delegate Custom|CustomEvent_0))))

(event EventBeginPlay
  (Utilities|FlowControl|Sequence
    (:then_1
      (CallFunction|BindButtonEvents))))

(fn ConstructionScript
  (for _index (range 0 3)
    (Utilities|Array|Add (LocalVariables|GetTest%20Data) (Utilities|Struct|MakeS_StringAndToken "Test Button" (Utilities|String|ToString(Integer) _index))))
  (Variables|Default|SetButton%20Structs (LocalVariables|GetTest%20Data))
  (CallFunction|CreateButtons))

(fn CreateButtons
  (Utilities|FlowControl|Sequence
    (:then_0
      (for _array_element (Variables|Default|GetButtons)
        (Actor|DestroyActor _array_element))
      (Utilities|Array|Clear (Variables|Default|GetButtons)))
    (:then_1
      (LocalVariables|SetButton%20Positions (CallFunction|PositionsinGrid (Utilities|Array|Length (Variables|Default|GetButton%20Structs)) 1 (Variables|Default|GetMargin) "2.000000,80.000000,8.000000" true)))
    (:then_2
      (for (_array_element_2 _array_index) (Variables|Default|GetButton%20Structs)
        (bind _returnvalue (AddComponent|AddChildActorComponent false (Math|Transform|MakeTransform (Utilities|Array|Get(acopy) (LocalVariables|GetButton%20Positions) _array_index))))
        (bind _asbp_checkbox (Utilities|Casting|CastToBP_Checkbox (Variables|/Script/Engine.ChildActorComponent|GetChildActor _returnvalue)))
        (Default|Setup _asbp_checkbox (Utilities|Text|ToText(String) (.String (Utilities|Struct|BreakS_StringAndToken _array_element_2))) (!= (.Integer (Utilities|Struct|BreakS_StringAndToken _array_element_2)) 0) (.DataToken (Utilities|Struct|BreakS_StringAndToken _array_element_2)))
        (Utilities|Array|Add (Variables|Default|GetButtons) _asbp_checkbox)))))

(fn ReplaceButtons
  (params (Button%20Structs :type Array%20of%20S%20String%20and%20Token%20Structures))
  (Variables|Default|SetButton%20Structs Button%20Structs)
  (CallFunction|CreateButtons)
  (CallFunction|BindButtonEvents))