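; BP_ProgressBoxes is a reusable actor that shows progress as a row of procedural box meshes with one box highlighted.
; The construction script creates normal and selected dynamic instances of MT_ProgressBox, builds the boxes, then applies the selection.
; RebuildBoxes destroys and recreates Count procedural mesh components in a single grid row.
; UpdateCount changes the count and rebuilds, while UpdateSelection swaps materials to highlight the box at the given index.
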(event `self.ReceiveBeginPlay`)

(event `self.ReceiveActorBeginOverlap`
  (params (OtherActor :type "Actor Object Reference")))

(event `self.ReceiveTick`
  (params (DeltaSeconds :type "Float (single-precision)")))

(fn `RebuildBoxes`
  (bind _meshcomponentarray (`self.MeshComponentArray`))
  (bind _count (`self.Count`))
  (`|ExecutionSequence`
    (:`then_0`
      (`/Game/ReusableAssets/Utilities/LIB_Utilities.Destroy Components` _meshcomponentarray)
      (`KismetArrayLibrary.Array_Clear` _meshcomponentarray))
    (:`then_1`
      (for _index (range _count)
        (bind _returnvalue (`AddComponent|ProceduralMeshComponent_0` :`RelativeTransform` (`KismetMathLibrary.MakeTransform` (`/Game/ReusableAssets/Utilities/LIB_Utilities.Location In Grid` (`KismetMathLibrary.Conv_IntToDouble` _index) (`KismetMathLibrary.Conv_IntToDouble` _count) 6.0 (`KismetMathLibrary.Conv_DoubleToVector` (`self.Cube Size`))) (struct) (1.0 1.0 1.0))))
        (`KismetArrayLibrary.Array_Add` (`self.MeshComponentArray`) _returnvalue)
        (`/Game/ReusableAssets/Utilities/LIB_Utilities.Setup Box Mesh` _returnvalue (`KismetMathLibrary.Conv_DoubleToVector` (`self.Cube Size`)) (`self.MID`))))))

(fn `UpdateCount`
  (params (Count :type Integer :default 0))
  (set `self.Count` Count)
  (`self.RebuildBoxes`))

(fn `UpdateSelection`
  (params (Index :type Integer :default 0))
  (for (_array_element _array_index) (`self.MeshComponentArray`)
    (if (== Index _array_index)
      (`PrimitiveComponent.SetMaterial` _array_element 0 (`self.Selected MID`))
      (else
        (`PrimitiveComponent.SetMaterial` _array_element 0 (`self.MID`))))))

(fn `UserConstructionScript`
  (`|ExecutionSequence`
    (:`then_0`
      (bind _returnvalue (`KismetMaterialLibrary.CreateDynamicMaterialInstance` "/Game/ReusableAssets/ProgressBoxes/MT_ProgressBox.MT_ProgressBox"))
      (`MaterialInstanceDynamic.SetScalarParameterValue` _returnvalue "Selected" 1.0)
      (set `self.Selected MID` _returnvalue)
      (bind _returnvalue_2 (`KismetMaterialLibrary.CreateDynamicMaterialInstance` "/Game/ReusableAssets/ProgressBoxes/MT_ProgressBox.MT_ProgressBox"))
      (set `self.MID` _returnvalue_2))
    (:`then_1`
      (`self.RebuildBoxes`))
    (:`then_2`
      (`self.UpdateSelection` (`self.Index`)))))